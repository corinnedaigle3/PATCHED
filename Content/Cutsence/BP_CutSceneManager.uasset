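; BP_CutSceneManager plays the level's intro cutscene and tracks its state in the game instance.
; On BeginPlay it finds the level's LevelSequenceActor and branches on the game instance's cutscene setting.
; At level start it plays the sequence with a skip widget whose event jumps to the end; finishing or skipping sets the state to InLevel.
; On restart it skips playback, and separate PlayCutscene and Skip events offer manual control.
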(event Custom|PlayCutscene
  (bind _cutscene (Variables|Default|GetCutscene))
  (bind _sequenceplayer (Variables|/Script/LevelSequence.LevelSequenceActor|GetSequencePlayer _cutscene))
  (if (Utilities|Enum|Equal(Enum) (Variables|/Game/Blueprints_Code/SaveData/UISetting.UISetting_C|GetCutscene (Variables|/Game/Blueprints_Code/SaveData/BP_GameInstance.BP_GameInstance_C|GetUISetting (Variables|Default|GetBP%20Game%20Instance))) "NewEnumerator0")
    (Sequencer|Player|Play _sequenceplayer :!class /Script/MovieScene.MovieSceneSequencePlayer)
    (EventDispatchers|BindEventtoOnFinished _sequenceplayer (delegate Custom|FinishCutscene))))

(event Custom|FinishCutscene
  (Default|CutsceneEnable (Variables|Default|GetBP%20Game%20Instance) "NewEnumerator2")
  (Development|PrintString "inLevel"))

(event Custom|Skip
  (Class|MovieSceneSequencePlayer|GotoEndandStop (Variables|/Script/LevelSequence.LevelSequenceActor|GetSequencePlayer (Variables|Default|GetCutscene)))
  (Default|CutsceneEnable (Variables|Default|GetBP%20Game%20Instance) "NewEnumerator2")
  (Development|PrintString "SkippedCutscene" true true "(R=1.000000,G=0.068513,B=0.000000,A=1.000000)" 1e+01))

(event Custom|FinishSkip
  (Class|MovieSceneSequencePlayer|GotoEndandStop (Variables|/Script/LevelSequence.LevelSequenceActor|GetSequencePlayer (Variables|Default|GetCutscene)))
  (Default|CutsceneEnable (Variables|Default|GetBP%20Game%20Instance) "NewEnumerator2"))

(event EventBeginPlay
  (Utilities|FlowControl|Sequence
    (:then_0
      (bind _asbp_game_instance (Utilities|Casting|CastToBP_GameInstance (Game|GetGameInstance)))
      (Variables|Default|SetBP%20Game%20Instance _asbp_game_instance)
      (bind _asbp_third_person_character (Utilities|Casting|CastToBP_ThirdPersonCharacter (Game|GetPlayerCharacter 0)))
      (Variables|Default|SetBP%20Third%20Person%20Character _asbp_third_person_character))
    (:then_1
      (bind _returnvalue (Actor|GetActorOfClass "/Script/LevelSequence.LevelSequenceActor"))
      (bind _output_get (Variables|Default|SetCutscene _returnvalue))
      (Utilities|IsValid _output_get
        (:Is%20Valid
          (switch Utilities|FlowControl|Switch|SwitchonCutsceneState (Variables|/Game/Blueprints_Code/SaveData/UISetting.UISetting_C|GetCutscene (Variables|/Game/Blueprints_Code/SaveData/BP_GameInstance.BP_GameInstance_C|GetUISetting (Variables|Default|GetBP%20Game%20Instance)))
            (:NewEnumerator0
              (Sequencer|Player|Play (Variables|/Script/LevelSequence.LevelSequenceActor|GetSequencePlayer (Variables|Default|GetCutscene)) :!class /Script/MovieScene.MovieSceneSequencePlayer)
              (bind _returnvalue_2 (UserInterface|CreateWidget "/Game/Blueprints_UI/WBP_SkipCutscene.WBP_SkipCutscene_C"))
              (bind _output_get_2 (Variables|Default|SetWBP_Skipcutscene _returnvalue_2))
              (UserInterface|Viewport|AddtoViewport _output_get_2 0)
              (EventDispatchers|BindEventtoStartSkip _output_get_2 (delegate Custom|FinishSkip))
              (EventDispatchers|BindEventtoOnFinished (Variables|/Script/LevelSequence.LevelSequenceActor|GetSequencePlayer (Variables|Default|GetCutscene)) (delegate Custom|FinishCutscene)))
            (:NewEnumerator1
              (Default|CutsceneEnable (Variables|Default|GetBP%20Game%20Instance) "NewEnumerator1")
              (Development|PrintString "restartLevel"))))))))

(event Collision|EventActorBeginOverlap
  (params (OtherActor :type Actor%20Object%20Reference)))

(event EventTick
  (params (DeltaSeconds :type Float%20%28single-precision%29)))

(fn ConstructionScript)