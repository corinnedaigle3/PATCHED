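; BP_Broke is a cutscene actor that shows a character's missing limbs by swapping the patch material on its mesh.
; Every Tick calls BodyStatus, which maps PlayerStatus to a material for full body, no arm, no leg or neither.
; The BodyState event directly applies the no-arm material.
; The limb, shield and VB attach/drop logic and the hold-to-interact widget nodes are disconnected and never run.
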(event Custom|BodyState
  (Rendering|Material|SetMaterial (Variables|Character|GetMesh) 0 "/Game/Art/Patch/Materials/m_Patch_noARM.m_Patch_noARM"))

(event EventTick
  (params (DeltaSeconds :type Float%20%28single-precision%29))
  (CallFunction|BodyStatus))

(fn ConstructionScript)

(fn BodyStatus
  (bind _mesh (Variables|Character|GetMesh))
  (switch Utilities|FlowControl|Switch|SwitchonEnum_PlayerBodyStae (Variables|Default|GetPlayerStatus)
    (:NewEnumerator2
      (Rendering|Material|SetMaterial _mesh 0 "/Game/Art/Patch/Materials/m_Patch_AllLimbs.m_Patch_AllLimbs"))
    (:NewEnumerator0
      (Rendering|Material|SetMaterial _mesh 0 "/Game/Art/Patch/Materials/m_Patch_noARM.m_Patch_noARM"))
    (:NewEnumerator3
      (Rendering|Material|SetMaterial _mesh 0 "/Game/Art/Patch/Materials/m_Patch_noLEG.m_Patch_noLEG"))
    (:NewEnumerator1
      (Rendering|Material|SetMaterial _mesh 0 "/Game/Art/Patch/Materials/m_Patch_noARMLEG.m_Patch_noARMLEG"))))