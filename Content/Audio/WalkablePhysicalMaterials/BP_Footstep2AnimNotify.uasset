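; BP_Footstep2AnimNotify is an animation notify that plays surface-specific doll footstep sounds.
; It acts only when the player pawn is a BP_ThirdPersonCharacter with HasLeg set.
; A short downward Visibility trace from the mesh owner reads the physical surface type.
; That surface selects a metal, carpet, wood or cardboard sound, with concrete as the default, played at the owner's location.
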(fn ReceivedNotify
  (params (MeshComp :type Skeletal%20Mesh%20Component%20Object%20Reference) (Animation :type Anim%20Sequence%20Base%20Object%20Reference) (EventReference :type Anim%20Notify%20Event%20Reference%20Structure%20%28by%20ref%29))
  (bind _returnvalue (Components|GetOwner MeshComp))
  (bind _returnvalue_2 (Transformation|GetActorLocation _returnvalue))
  (bind _returnvalue_3 (Transformation|GetActorLocation _returnvalue))
  ;[0.15 0.15 0.15 0.5] Play move SFX
  (bind _asbp_third_person_character (Utilities|Casting|CastToBP_ThirdPersonCharacter (Game|Player|GetPlayerPawn 0)))
  (if (Variables|/Game/BP_ThirdPersonCharacter.BP_ThirdPersonCharacter_C|GetHasLeg _asbp_third_person_character)
    (bind _outhit (Collision|LineTraceByChannel _returnvalue_3 (+ _returnvalue_3 (* (Transformation|GetActorUpVector _returnvalue) -5e+01)) "TraceTypeQuery1" false 0 "None"))
    (switch Utilities|FlowControl|Switch|SwitchonEPhysicalSurface (Collision|GetSurfaceType _outhit)
      (:SurfaceType_Default
        (Audio|PlaySoundatLocation "/Game/Audio/SFX/Character/SFX_ConcreteDollFS2.SFX_ConcreteDollFS2" _returnvalue_2 "0, 0, 0" 1.0 1.0 0.0 0 0 0 0))
      (:SurfaceType1
        (Audio|PlaySoundatLocation "/Game/Audio/SFX/Character/SFX_MetalDollFS2.SFX_MetalDollFS2" _returnvalue_2 "0, 0, 0" 1.0 1.0 0.0 0 0 0 0))
      (:SurfaceType2
        (Audio|PlaySoundatLocation "/Game/Audio/SFX/Character/SFX_ConcreteDollFS2NC.SFX_ConcreteDollFS2NC" _returnvalue_2 "0, 0, 0" 1.0 1.0 0.0 0 0 0 0))
      (:SurfaceType3
        (Audio|PlaySoundatLocation "/Game/Audio/SFX/Character/SFX_WoodDollFS2.SFX_WoodDollFS2" _returnvalue_2 "0, 0, 0" 1.0 1.0 0.0 0 0 0 0))
      (:SurfaceType4
        (Audio|PlaySoundatLocation "/Game/Audio/SFX/Character/SFX_CardboardDollFS2.SFX_CardboardDollFS2" _returnvalue_2 "0, 0, 0" 1.0 1.0 0.0 0 0 0 0)))
    (return false)))