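; Level-tracking actor that records which of the game's five levels the player has reached, for saving.
; On BeginPlay it matches the current level name to set one of five level flags.
; After a one-second delay it passes that name to BP_GameInstance's SaveCurrentLevel and prints it on screen.
; Its SaveData event copies the current level's flag into the supplied save game object.
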(event EventBeginPlay
  (bind _asbp_game_instance (Utilities|Casting|CastToBP_GameInstance (Game|GetGameInstance)))
  (Variables|Default|SetAs%20BP%20Game%20Instance _asbp_game_instance)
  (bind _returnvalue (Game|GetCurrentLevelName true))
  (switch string _returnvalue
    (:Default
      _)
    (:IntroLevel
      (Variables|Default|SetLevel1 true))
    (:PackagingZach
      (Variables|Default|SetLevel2 true))
    (:Manufactoring
      (Variables|Default|SetLevel3 true))
    (:BoilerRoom
      (Variables|Default|SetLevel4 true))
    (:FinalOfficeBoss
      (Variables|Default|SetLevel5 true)))
  (Utilities|FlowControl|Delay 1.0)
  (Default|SaveCurrentLevel (Variables|Default|GetAs%20BP%20Game%20Instance) _returnvalue)
  (Development|PrintString _returnvalue true true "(R=1.000000,G=0.752141,B=0.004957,A=1.000000)"))

(event Collision|EventActorBeginOverlap
  (params (OtherActor :type Actor%20Object%20Reference)))

(event EventTick
  (params (DeltaSeconds :type Float%20%28single-precision%29)))

(event EventSaveData
  (params (SaveGameRef :type BP%20Save%20Game%20Object%20Reference))
  (bind _returnvalue (Game|GetCurrentLevelName true))
  (switch string _returnvalue
    (:IntroLevel
      (Variables|/Game/Blueprints_Code/SaveData/BP_SaveGame.BP_SaveGame_C|SetLevel1 SaveGameRef (Variables|Default|GetLevel1)))
    (:PackagingZach
      (Variables|/Game/Blueprints_Code/SaveData/BP_SaveGame.BP_SaveGame_C|SetLevel2 SaveGameRef (Variables|Default|GetLevel2)))
    (:Manufactoring
      (Variables|/Game/Blueprints_Code/SaveData/BP_SaveGame.BP_SaveGame_C|SetLevel3 SaveGameRef (Variables|Default|GetLevel3)))
    (:BoilerRoom
      (Variables|/Game/Blueprints_Code/SaveData/BP_SaveGame.BP_SaveGame_C|SetLevel4 SaveGameRef (Variables|Default|GetLevel4)))
    (:FinalOfficeBoss
      (Variables|/Game/Blueprints_Code/SaveData/BP_SaveGame.BP_SaveGame_C|SetLevel5 SaveGameRef (Variables|Default|GetLevel5)))))

(fn ConstructionScript)