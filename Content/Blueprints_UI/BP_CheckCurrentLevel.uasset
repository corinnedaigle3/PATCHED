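; BP_CheckCurrentLevel is an actor that flags which level is being played, for storage in a save game.
; On BeginPlay it matches the current level name against the intro and packaging levels, sets the Level1 or Level2 boolean, and prints it for debugging.
; Its SaveData event copies both flags onto the passed save game reference; nothing here loads them back.
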(event EventBeginPlay
  (bind _returnvalue (Game|GetCurrentLevelName true))
  (switch string _returnvalue
    (:IntroLevel
      (bind _output_get (Variables|Default|SetLevel1 true))
      (Development|PrintString (Utilities|String|Append "CurrentLevel: " (Utilities|String|ToString(Boolean) _output_get))))
    (:PackagingZach
      (bind _output_get_2 (Variables|Default|SetLevel2 true))
      (Development|PrintString (Utilities|String|Append "CurrentLevel: " (Utilities|String|ToString(Boolean) _output_get_2))))))

(event Collision|EventActorBeginOverlap
  (params (OtherActor :type Actor%20Object%20Reference)))

(event EventTick
  (params (DeltaSeconds :type Float%20%28single-precision%29)))

(event EventSaveData
  (params (SaveGameRef :type BP%20Save%20Game%20Object%20Reference))
  (Variables|/Game/Blueprints_Code/SaveData/BP_SaveGame.BP_SaveGame_C|SetLevel1 SaveGameRef (Variables|Default|GetLevel1))
  (Variables|/Game/Blueprints_Code/SaveData/BP_SaveGame.BP_SaveGame_C|SetLevel2 SaveGameRef (Variables|Default|GetLevel2)))

(fn ConstructionScript)