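; Interactable voice box pickup that unlocks the voice box, and also the grapple flag, on the third-person character.
; BeginPlay caches the character and adds the pickup audio component.
; Interact triggers PickUpVB, which plays the sound, disables the meshes' visibility, physics and collision, and sets both flags.
; After a short delay it destroys itself, then creates an objective widget showing the voice box control hint.
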(event Custom|PickUpVB
  (bind _charref (Variables|Default|GetCharRef))
  ;[0.15 0.15 0.15 0.5] Pick up voicebox
  (Audio|Components|Audio|Play (Variables|Default|GetPickUp) 0.0)
  (Rendering|SetVisibility (Variables|Default|GetCube) false false)
  (Physics|SetSimulatePhysics (Variables|Default|GetCube) false)
  (Collision|SetCollisionEnabled (Variables|Default|GetSphere1) "NoCollision")
  (bind _output_get (Variables|/Game/BP_ThirdPersonCharacter.BP_ThirdPersonCharacter_C|SethasVoiceBox _charref true))
  (Variables|/Game/BP_ThirdPersonCharacter.BP_ThirdPersonCharacter_C|SetHasGrapple _charref _output_get)
  (Utilities|FlowControl|Delay 0.4)
  (Actor|DestroyActor)
  ;;[0.15 0.15 0.15 0.5] Control Hint
  (bind _returnvalue (UserInterface|CreateWidget "/Game/Blueprints_UI/WBP_Ojective.WBP_Ojective_C" 0 "Press Y to use Voice Box"))
  (Default|ObjectiveActive _returnvalue))

(event EventBeginPlay
  (bind _returnvalue (Actor|GetActorOfClass "/Game/BP_ThirdPersonCharacter.BP_ThirdPersonCharacter_C"))
  (Variables|Default|SetCharRef _returnvalue)
  (bind _returnvalue_2 (AddComponent|AddAudioComponent false))
  (Variables|Default|SetPickUp _returnvalue_2))

(fn ConstructionScript)

(fn Interact
  (params (Character :type BP%20Third%20Person%20Character%20Object%20Reference))
  (CallFunction|PickUpVB)
  (return false))