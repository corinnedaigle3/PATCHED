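; Grapple helper for the Patch character that shows an aim marker on grappable surfaces and also opens the pause menu.
; GrappleIndicator sphere-traces from the camera, or from Patch's 2D start location in spline-cam mode, looking for a BP_Grappable3D that allows grappling.
; A hit creates or moves a sphere HookDisplay according to move state; a missed trace or the Grappling state removes it.
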(event Custom|Pause
  (bind _returnvalue (Game|GetPlayerController 0))
  (bind _returnvalue_2 (UserInterface|CreateWidget "/Game/Blueprints_UI/WBP_PauseMenu.WBP_PauseMenu_C"))
  (UserInterface|Animation|PlayAnimation _returnvalue_2 (Variables|/Game/Blueprints_UI/WBP_PauseMenu.WBP_PauseMenu_C|GetPauseMenu _returnvalue_2) 0.0 1 "Forward" 1.0 false)
  (UserInterface|Viewport|AddtoViewport _returnvalue_2 0)
  (Input|SetInputModeUIOnly _returnvalue _returnvalue_2 "DoNotLock" false)
  (Variables|/Script/Engine.PlayerController|SetbShowMouseCursor _returnvalue true))

(event Custom|GrappleIndicator
  (bind (_start _end) (CallFunction|DetermineAimGrapple))
  (bind (_hit_result _return_value) (CallFunction|TracingforGrapple _start _end "TraceTypeQuery3" "None" 1.0))
  (if _return_value
    (bind _asbp_grappable_3d (Utilities|Casting|CastToBP_Grappable3D (.HitActor (Collision|BreakHitResult _hit_result))))
    (if (Variables|/Game/Blueprints_Code/BP_Grappable3D.BP_Grappable3D_C|GetCanGrappleHere _asbp_grappable_3d)
      (Variables|/Game/BP_ThirdPersonCharacter.BP_ThirdPersonCharacter_C|GetHook%20Display (Variables|Default|GetPatch)
        (:then
          (switch Utilities|FlowControl|Switch|SwitchonEnum_PlayerMovementState (Variables|/Game/BP_ThirdPersonCharacter.BP_ThirdPersonCharacter_C|GetPlayerMoveState (Variables|Default|GetPatch))
            (:NewEnumerator1
              (Transformation|SetWorldLocation (Variables|/Game/BP_ThirdPersonCharacter.BP_ThirdPersonCharacter_C|GetHook%20Display (Variables|Default|GetPatch)) (.ImpactPoint (Collision|BreakHitResult _hit_result)) false false :!label _label)
              (switch Utilities|FlowControl|Switch|SwitchonEnum_PlayerMovementState (Variables|/Game/BP_ThirdPersonCharacter.BP_ThirdPersonCharacter_C|GetPlayerMoveState (Variables|Default|GetPatch))
                (:NewEnumerator2
                  _)))
            (:NewEnumerator6
              (goto _label))
            (:NewEnumerator5
              (goto _label))
            (:NewEnumerator7
              (goto _label))
            (:NewEnumerator2
              _))
          (Variables|/Game/BP_ThirdPersonCharacter.BP_ThirdPersonCharacter_C|GetHook%20Display (Variables|Default|GetPatch) :!label _label_2
            (:then
              (Default|DestroyHook (Variables|Default|GetPatch))
              (Development|PrintString "destroyed")
              (Utilities|FlowControl|Delay 3.0)
              (Variables|/Game/BP_ThirdPersonCharacter.BP_ThirdPersonCharacter_C|SetisGrappling (Variables|Default|GetPatch) false))
            (:else)))
        (:else
          (switch Utilities|FlowControl|Switch|SwitchonEnum_PlayerMovementState (Variables|/Game/BP_ThirdPersonCharacter.BP_ThirdPersonCharacter_C|GetPlayerMoveState (Variables|Default|GetPatch))
            (:NewEnumerator1
              _)
            (:NewEnumerator6
              _)
            (:NewEnumerator5
              _)
            (:NewEnumerator7
              _)
            (:NewEnumerator2
              (goto _label_2)))
          (bind _returnvalue (Game|AddComponentbyClass (Variables|Default|GetPatch) "/Script/Engine.StaticMeshComponent" false))
          (bind _output_get (Variables|/Game/BP_ThirdPersonCharacter.BP_ThirdPersonCharacter_C|SetHook%20Display (Variables|Default|GetPatch) _returnvalue))
          (Components|StaticMesh|SetStaticMesh _output_get "/Engine/InteractiveToolsFramework/Meshes/GizmoSphereHandle.GizmoSphereHandle")
          (Rendering|Material|SetMaterial (Variables|/Game/BP_ThirdPersonCharacter.BP_ThirdPersonCharacter_C|GetHook%20Display (Variables|Default|GetPatch)) 0 "/Engine/EditorMaterials/Cloth/CameraLitVertexColor.CameraLitVertexColor")
          (Transformation|SetRelativeScale3D (Variables|/Game/BP_ThirdPersonCharacter.BP_ThirdPersonCharacter_C|GetHook%20Display (Variables|Default|GetPatch)) "1.500000,1.500000,1.500000")
          (Rendering|SetVisibility (Variables|/Game/BP_ThirdPersonCharacter.BP_ThirdPersonCharacter_C|GetHook%20Display (Variables|Default|GetPatch)) false false)
          (Utilities|FlowControl|Delay 0.2)
          (bind _hook_display (Variables|/Game/BP_ThirdPersonCharacter.BP_ThirdPersonCharacter_C|GetHook%20Display (Variables|Default|GetPatch))
            (:then
              (Rendering|SetVisibility _hook_display true false)
              (Development|PrintString "Created"))
            (:else)))))
    (else
      (Variables|/Game/BP_ThirdPersonCharacter.BP_ThirdPersonCharacter_C|GetHook%20Display (Variables|Default|GetPatch)
        (:then
          (Default|DestroyHook (Variables|Default|GetPatch)))
        (:else)))))

(fn ConstructionScript)

(fn DetermineAimGrapple
  (bind _returnvalue (Game|GetPlayerCameraManager 0))
  (bind _patch (Variables|Default|GetPatch))
  (bind _2dstartinglocation (Variables|/Game/BP_ThirdPersonCharacter.BP_ThirdPersonCharacter_C|Get2DStartingLocation _patch))
  (if (Variables|/Game/BP_ThirdPersonCharacter.BP_ThirdPersonCharacter_C|GetisSplineCam (Variables|Default|GetPatch))
    (return _2dstartinglocation _2dstartinglocation)
    (else
      (return (Camera|GetCameraLocation _returnvalue) (Math|Vector|GetForwardVector (Camera|GetCameraRotation _returnvalue))))))

(fn TracingforGrapple
  (params (Start :type Vector) (End :type Vector) (Trace%20Channel :type ETraceTypeQuery%20Enum :default "TraceTypeQuery1") (DrawDebugType :type EDrawDebugTrace%20Enum :default "None") (DrawTime :type Float%20%28double-precision%29))
  (bind (_outhit _returnvalue) (Collision|SphereTraceByChannel Start (+ Start (* End (Variables|Default|GetGrappleRange))) (Variables|Default|GetGrappleRadius) Trace%20Channel true 0 DrawDebugType true "(R=1.000000,G=0.000000,B=0.000000,A=1.000000)" "(R=0.000000,G=1.000000,B=0.000000,A=1.000000)" DrawTime))
  (return _outhit _returnvalue))