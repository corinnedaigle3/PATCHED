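; Flying grapple target that shuttles between two points until caught, then is reeled in by the player to spawn a hat.
; A self-recalling timeline drives the patrol until StopMoving halts it.
; GotCaught locks move input and links a HUD mini-game widget; Struggle eases the mesh toward the player by progress, and MoveToPlayer finishes the pull.
; Character overlap spawns HatClass, hides the cable, destroys the actor and notifies the player's NeedleFunctionality.
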(event OnComponentBeginOverlap(StaticMesh)
  (params (OverlappedComponent :type Primitive%20Component%20Object%20Reference) (OtherActor :type Actor%20Object%20Reference) (OtherComp :type Primitive%20Component%20Object%20Reference) (OtherBodyIndex :type Integer) (bFromSweep :type Boolean) (SweepResult :type Hit%20Result%20Structure%20%28by%20ref%29))
  (bind _player (Variables|Default|GetPlayer))
  (bind _asbp_third_person_character (Utilities|Casting|CastToBP_ThirdPersonCharacter OtherActor))
  (Game|SpawnActorfromClass (Variables|Default|GetHatClass) (Math|Transform|MakeTransform (Transformation|GetWorldLocation (Variables|Default|GetStaticMesh)) "0, 0, 0" "1.000000,1.000000,1.000000") "Undefined" "MultiplyWithRoot" 0 "Lore" 0)
  (Rendering|SetVisibility (Variables|/Game/BP_ThirdPersonCharacter.BP_ThirdPersonCharacter_C|GetCable _asbp_third_person_character) false false)
  (Actor|DestroyActor)
  (Variables|/Game/BP_ThirdPersonCharacter.BP_ThirdPersonCharacter_C|Setpulling _player false)
  (Default|FlyingGrappleDone (Variables|/Game/BP_ThirdPersonCharacter.BP_ThirdPersonCharacter_C|GetNeedleFunctionality _player)))

(event Custom|TravelBetweenAandB
  (if (not (Variables|Default|GetGot%20Caugth))
    (if (Variables|Default|GetGoingtoB)
      (bind _alpha (Timeline|FlyingGrappleTimeline PlayFromStart)
        (:Update
          (if (not (Variables|Default|GetGot%20Caugth))
            (Transformation|SetWorldLocation (Variables|Default|GetStaticMesh) (Utilities|LerpfromGrapple _alpha) false false)
            (else
              (Timeline|FlyingGrappleTimeline Stop))))
        (:Finished
          (Variables|Default|SetGoingtoB (not (Variables|Default|GetGoingtoB)))
          (CallFunction|TravelBetweenAandB)))
      (else
        (Timeline|FlyingGrappleTimeline ReverseFromEnd)))
    (else
      (Timeline|FlyingGrappleTimeline Stop))))

(event Custom|Got%20Caught
  (params (Patch :type BP%20Third%20Person%20Character%20Object%20Reference))
  (Variables|Default|SetPlayer Patch)
  (Utilities|FlowControl|Delay 0.3)
  (Variables|/Script/UMG.Widget|SetVisibility (Variables|/Game/BP_ThirdPersonCharacter.BP_ThirdPersonCharacter_C|GetGameHUD (Variables|Default|GetPlayer)) "Visible")
  (Default|ShowHUD (Variables|/Game/BP_ThirdPersonCharacter.BP_ThirdPersonCharacter_C|GetGameHUD (Variables|Default|GetPlayer)) 3 false)
  (bind _output_get (Variables|Default|SetFlyingGrappleWidget (Variables|/Game/Blueprints_UI/WBP_GameHUD.WBP_GameHUD_C|GetWBP_FlyingGrappleMini (Variables|/Game/BP_ThirdPersonCharacter.BP_ThirdPersonCharacter_C|GetGameHUD (Variables|Default|GetPlayer)))))
  (Variables|/Game/BP_ThirdPersonCharacter.BP_ThirdPersonCharacter_C|SetisActive (Variables|Default|GetPlayer) true)
  (Variables|/Game/Blueprints_UI/WBP_FlyingGrappleMini.WBP_FlyingGrappleMini_C|SetHat _output_get self)
  (Input|SetIgnoreMoveInput (Game|GetPlayerController 0) true)
  (Variables|Default|SetStruggleStart (Transformation|GetWorldLocation (Variables|Default|GetStaticMesh))))

(event Custom|MoveToPlayer
  (bind _staticmesh (Variables|Default|GetStaticMesh))
  (bind _player (Variables|Default|GetPlayer))
  (Timeline|MoveToPlayerTimeline Play
    (:Update
      (Transformation|SetWorldLocation _staticmesh (Math|Interpolation|VInterpTo (Transformation|GetWorldLocation _staticmesh) (Transformation|GetActorLocation (Variables|Default|GetPlayer)) (Utilities|Time|GetWorldDeltaSeconds) 2e+01) false false)
      (Variables|/Script/UMG.Widget|SetVisibility (Variables|/Game/BP_ThirdPersonCharacter.BP_ThirdPersonCharacter_C|GetGameHUD _player) "Hidden")
      (Variables|/Game/BP_ThirdPersonCharacter.BP_ThirdPersonCharacter_C|SetisActive _player false))))

(event Custom|AddProgress
  (bind _flyinggrapplewidget (Variables|Default|GetFlyingGrappleWidget))
  (Development|PrintString "FlyingGrapple")
  (Utilities|IsValid _flyinggrapplewidget
    (:Is%20Valid
      (Default|AddProgress _flyinggrapplewidget))))

(event Custom|Struggle
  (params (Progress :type Float%20%28double-precision%29))
  (bind _alpha (Timeline|StruggleTimeline PlayFromStart)
    (:Update
      (Transformation|SetWorldLocation (Variables|Default|GetStaticMesh) (Math|Vector|Lerp(Vector) (Transformation|GetWorldLocation (Variables|Default|GetStaticMesh)) (Math|Vector|Lerp(Vector) (Variables|Default|GetStruggleStart) (Transformation|GetActorLocation (Variables|Default|GetPlayer)) Progress) _alpha) false false))))

(event Custom|StopStruggle
  (bind _alpha (Timeline|StruggleTimeline Stop)
    (:Update
      (Transformation|SetWorldLocation (Variables|Default|GetStaticMesh) (Math|Vector|Lerp(Vector) (Transformation|GetWorldLocation (Variables|Default|GetStaticMesh)) (Math|Vector|Lerp(Vector) (Variables|Default|GetStruggleStart) (Transformation|GetActorLocation (Variables|Default|GetPlayer)) (stale Custom|Struggle Progress)) _alpha) false false))))

(event Custom|StopMoving
  (Variables|Default|SetGot%20Caugth true))

(event EventBeginPlay
  (Variables|Default|SetCanGrappleHere true)
  (Variables|Default|SetCanPull true)
  (|CallParentFunction)
  (CallFunction|TravelBetweenAandB))

(event Collision|EventActorBeginOverlap
  (params (OtherActor :type Actor%20Object%20Reference))
  (|CallParentFunction OtherActor) ; This node is disabled and will not be called.\nDrag off pins to build functionality.
)

(event EventTick
  (params (DeltaSeconds :type Float%20%28single-precision%29))
  (|CallParentFunction DeltaSeconds))

(fn ConstructionScript
  (|CallParentFunction))