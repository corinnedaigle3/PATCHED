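; BP_Boxes is a droppable box actor that moves by ProjectileMovement and signals through an event dispatcher when it is finished.
; DropBox launches it with a given velocity and enables collision.
; A mesh overlap with a Floor-tagged actor zeroes its velocity via DeactiveBox, then broadcasts OnBoxesDestory after a delay, without destroying the actor itself.
; ResetBox stops and broadcasts immediately, while its timer and the box-to-box overlap check are disconnected.
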(event OnComponentBeginOverlap(BoxesMesh)
  (params (OverlappedComponent :type Primitive%20Component%20Object%20Reference) (OtherActor :type Actor%20Object%20Reference) (OtherComp :type Primitive%20Component%20Object%20Reference) (OtherBodyIndex :type Integer) (bFromSweep :type Boolean) (SweepResult :type Hit%20Result%20Structure%20%28by%20ref%29))
  (if (Actor|ActorHasTag OtherActor "Floor")
    (CallFunction|DeactiveBox)
    (Utilities|FlowControl|Delay 1e+01)
    (Default|CallOnBoxesDestory self)
    (Development|PrintString "BoxDestory")))

(event Custom|DeactiveBox
  (Variables|/Script/Engine.MovementComponent|SetVelocity (Variables|Default|GetProjectileMovement) "0, 0, 0")
  (Collision|SetCollisionEnabled (Variables|Default|GetBoxesMesh) "QueryAndPhysics"))

(event Custom|DropBox
  (params (Velocity :type Vector))
  (Variables|/Script/Engine.MovementComponent|SetVelocity (Variables|Default|GetProjectileMovement) Velocity)
  (Collision|SetCollisionEnabled (Variables|Default|GetBoxesMesh) "QueryAndPhysics"))

(event Custom|ResetBox
  (Default|CallOnBoxesDestory self)
  (Variables|/Script/Engine.MovementComponent|SetVelocity (Variables|Default|GetProjectileMovement) "0, 0, 0"))

(event EventBeginPlay)

(event Collision|EventActorBeginOverlap
  (params (OtherActor :type Actor%20Object%20Reference)))

(event EventTick
  (params (DeltaSeconds :type Float%20%28single-precision%29)))

(fn ConstructionScript)