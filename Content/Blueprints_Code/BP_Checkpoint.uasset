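; Checkpoint actor that records the player's respawn point and level, then saves the game when the character enters its collider.
; It writes the CheckpointTransform world transform and current level name to the player controller, then triggers the save through that controller's game instance reference.
; A DoOnce gate resets 10 seconds after firing to throttle saves; any overlapping actor consumes it because the character cast comes afterwards.
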(event OnComponentBeginOverlap(Collider)
  (params (OverlappedComponent :type Primitive%20Component%20Object%20Reference) (OtherActor :type Actor%20Object%20Reference) (OtherComp :type Primitive%20Component%20Object%20Reference) (OtherBodyIndex :type Integer) (bFromSweep :type Boolean) (SweepResult :type Hit%20Result%20Structure%20%28by%20ref%29))
  (Development|PrintString "Checkpoint Collided")
  (Utilities|FlowControl|DoOnce false
    (:Completed
      (Utilities|FlowControl|Sequence
        (:then_0
          (bind _asbp_third_person_character (Utilities|Casting|CastToBP_ThirdPersonCharacter OtherActor))
          (Variables|Default|SetPatch _asbp_third_person_character)
          (CallFunction|SetCurrentLevelandCoordinates)
          (CallFunction|SaveGame))
        (:then_1
          (Development|PrintString "Checkpoint Logic Finished")
          (Utilities|FlowControl|Delay 1e+01)
          (CallFunction|AllowSave))))))

(event Custom|AllowSave
  (Utilities|FlowControl|DoOnce false) ; enters at Reset
)

(event EventBeginPlay
  (bind _asbp_third_person_player_controller (Utilities|Casting|CastToBP_ThirdPersonPlayerController (Game|GetPlayerController 0)))
  (Variables|Default|SetPlayControllerRef _asbp_third_person_player_controller))

(fn ConstructionScript)

(fn SetCurrentLevelandCoordinates
  (Variables|/Game/ThirdPerson/Blueprints/BP_ThirdPersonPlayerController.BP_ThirdPersonPlayerController_C|SetCheckpoint (Variables|Default|GetPlayControllerRef) (Transformation|GetWorldTransform (Variables|Default|GetCheckpointTransform)))
  (bind _returnvalue (Game|GetCurrentLevelName true))
  (Variables|/Game/ThirdPerson/Blueprints/BP_ThirdPersonPlayerController.BP_ThirdPersonPlayerController_C|SetCurrentLevel (Variables|Default|GetPlayControllerRef) _returnvalue))

(fn SaveGame
  (bind _playcontrollerref (Variables|Default|GetPlayControllerRef))
  (bind _gameinstanceref (Variables|/Game/ThirdPerson/Blueprints/BP_ThirdPersonPlayerController.BP_ThirdPersonPlayerController_C|GetGameInstanceRef _playcontrollerref))
  (Default|RequestSave _gameinstanceref true)
  (Default|SaveGame _gameinstanceref true))