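; Pushable box actor that a player character with an arm can move through an Interact call.
; Box overlap enables interaction and sets the character's push speed by light, medium or heavy flags; leaving restores walking and disables physics.
; MoveObject switches player move state, walk speed and cube physics from the character's interaction flag, applying a forward impulse when pushing.
; Tick plays or stops the push sound from character movement and interaction state.
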(event OnComponentBeginOverlap(Box)
  (params (OverlappedComponent :type Primitive%20Component%20Object%20Reference) (OtherActor :type Actor%20Object%20Reference) (OtherComp :type Primitive%20Component%20Object%20Reference) (OtherBodyIndex :type Integer) (bFromSweep :type Boolean) (SweepResult :type Hit%20Result%20Structure%20%28by%20ref%29))
  (bind _charref (Variables|Default|GetCharREF))
  ;[0.15 0.15 0.15 0.5] Sets if player can interact
  (Utilities|Casting|CastToBP_ThirdPersonCharacter OtherActor)
  (Variables|/Game/BP_ThirdPersonCharacter.BP_ThirdPersonCharacter_C|SetCanInteractBox?? (Variables|Default|GetCharREF) true)
  (if (Variables|Default|GetLightObj)
    (bind _output_get (Variables|/Game/BP_ThirdPersonCharacter.BP_ThirdPersonCharacter_C|SetWalkSpeedPush _charref 8e+01))
    (Development|PrintString (Utilities|String|ToString(Float) _output_get))
    (elif (Variables|Default|GetMediumObj)
      (bind _output_get_2 (Variables|/Game/BP_ThirdPersonCharacter.BP_ThirdPersonCharacter_C|SetWalkSpeedPush _charref 7e+01))
      (Development|PrintString (Utilities|String|ToString(Float) _output_get_2))
      (elif (Variables|Default|GetHeavyObj)
        (bind _output_get_3 (Variables|/Game/BP_ThirdPersonCharacter.BP_ThirdPersonCharacter_C|SetWalkSpeedPush _charref 6e+01))
        (Development|PrintString (Utilities|String|ToString(Float) _output_get_3))
        (else
          (bind _output_get_4 (Variables|/Game/BP_ThirdPersonCharacter.BP_ThirdPersonCharacter_C|SetWalkSpeedPush _charref 8e+01))
          (Development|PrintString (Utilities|String|ToString(Float) _output_get_4)))))))

(event OnComponentEndOverlap(Box)
  (params (OverlappedComponent :type Primitive%20Component%20Object%20Reference) (OtherActor :type Actor%20Object%20Reference) (OtherComp :type Primitive%20Component%20Object%20Reference) (OtherBodyIndex :type Integer))
  (bind _charref (Variables|Default|GetCharREF))
  (bind _charactermovement (Variables|/Script/Engine.Character|GetCharacterMovement _charref))
  ;[0.15 0.15 0.15 0.5] Sets if player can interact
  (Utilities|Casting|CastToBP_ThirdPersonCharacter OtherActor)
  (Variables|/Game/BP_ThirdPersonCharacter.BP_ThirdPersonCharacter_C|SetPlayerMoveState _charref "NewEnumerator0")
  (Variables|/Game/BP_ThirdPersonCharacter.BP_ThirdPersonCharacter_C|SetCanInteractBox?? _charref false)
  (Variables|/Game/BP_ThirdPersonCharacter.BP_ThirdPersonCharacter_C|SetIsNotInteractingBox?? _charref false)
  (if (Variables|/Game/BP_ThirdPersonCharacter.BP_ThirdPersonCharacter_C|GetHasLeg _charref)
    (Variables|/Script/Engine.CharacterMovementComponent|SetMaxWalkSpeed _charactermovement (Variables|/Game/BP_ThirdPersonCharacter.BP_ThirdPersonCharacter_C|GetWalkSpeed _charref))
    (else
      (Variables|/Script/Engine.CharacterMovementComponent|SetMaxWalkSpeed _charactermovement (Variables|/Game/BP_ThirdPersonCharacter.BP_ThirdPersonCharacter_C|GetWalkSpeedNoLeg _charref))))
  (Physics|SetSimulatePhysics (Variables|Default|GetSM_Cube) false))

(event Custom|Move%20Object
  (bind _sm_cube (Variables|Default|GetSM_Cube))
  (bind _charref (Variables|Default|GetCharREF))
  (bind _charactermovement (Variables|/Script/Engine.Character|GetCharacterMovement _charref))
  (bind _relativelocation (Variables|/Script/Engine.SceneComponent|GetRelativeLocation _sm_cube))
  ;[0.15 0.15 0.15 0.5] Sets Simulate Physics On/Off and Player Move State
  (if (Variables|/Game/BP_ThirdPersonCharacter.BP_ThirdPersonCharacter_C|GetHasArm _charref)
    (if (Variables|/Game/BP_ThirdPersonCharacter.BP_ThirdPersonCharacter_C|GetIsNotInteractingBox?? _charref)
      (Variables|/Game/BP_ThirdPersonCharacter.BP_ThirdPersonCharacter_C|SetPlayerMoveState _charref "NewEnumerator0")
      (if (Variables|/Game/BP_ThirdPersonCharacter.BP_ThirdPersonCharacter_C|GetHasLeg _charref)
        (Variables|/Script/Engine.CharacterMovementComponent|SetMaxWalkSpeed _charactermovement (Variables|/Game/BP_ThirdPersonCharacter.BP_ThirdPersonCharacter_C|GetWalkSpeed _charref))
        (else
          (Variables|/Script/Engine.CharacterMovementComponent|SetMaxWalkSpeed _charactermovement (Variables|/Game/BP_ThirdPersonCharacter.BP_ThirdPersonCharacter_C|GetWalkSpeedNoLeg _charref))))
      (Physics|SetSimulatePhysics (Variables|Default|GetSM_Cube) false)
      (else
        (Variables|/Game/BP_ThirdPersonCharacter.BP_ThirdPersonCharacter_C|SetPlayerMoveState _charref "NewEnumerator4")
        (Development|PrintString "Moving Object")
        (Variables|/Script/Engine.CharacterMovementComponent|SetMaxWalkSpeed (Variables|/Script/Engine.Character|GetCharacterMovement _charref) (Variables|/Game/BP_ThirdPersonCharacter.BP_ThirdPersonCharacter_C|GetWalkSpeedPush _charref))
        (Physics|SetSimulatePhysics (Variables|Default|GetSM_Cube) true)
        (Physics|AddImpulse _sm_cube (Math|Interpolation|VInterpTo _relativelocation (+ _relativelocation (* (Transformation|GetActorForwardVector (Variables|Default|GetCharREF)) (Variables|Default|GetFloat))) (Utilities|Time|GetWorldDeltaSeconds) 8.0) "None" false)
        (Audio|Components|Audio|Play (Variables|Default|GetPushSFX) 0.0)))))

(event EventBeginPlay
  (bind _asbp_third_person_character (Utilities|Casting|CastToBP_ThirdPersonCharacter (Game|Player|GetPlayerPawn 0)))
  (Variables|Default|SetCharREF _asbp_third_person_character)
  (bind _returnvalue (AddComponent|AddAudioComponent false))
  (Variables|Default|SetPushSFX _returnvalue))

(event EventTick
  (params (DeltaSeconds :type Float%20%28single-precision%29))
  (bind _charref (Variables|Default|GetCharREF))
  ;[0.15 0.15 0.15 0.5] Plays SFX if player is interacting and moving
  (Utilities|FlowControl|Sequence
    (:then_0
      (if (Variables|/Game/BP_ThirdPersonCharacter.BP_ThirdPersonCharacter_C|GetHasArm _charref)
        (if (Variables|/Game/BP_ThirdPersonCharacter.BP_ThirdPersonCharacter_C|GetIsMoving _charref)
          (if (Variables|/Game/BP_ThirdPersonCharacter.BP_ThirdPersonCharacter_C|GetCanInteractBox?? _charref)
            (if (Variables|/Game/BP_ThirdPersonCharacter.BP_ThirdPersonCharacter_C|GetIsNotInteractingBox?? _charref)
              (Utilities|FlowControl|Delay 2.0)
              (Audio|Components|Audio|Play (Variables|Default|GetPushSFX) 0.0)
              (else
                (Audio|Components|Audio|Stop (Variables|Default|GetPushSFX) :!label _label)))
            (else
              (goto _label)))
          (else
            (goto _label)))
        (else
          (goto _label))))
    (:then_1
      (if (not (> (Variables|/Game/BP_ThirdPersonCharacter.BP_ThirdPersonCharacter_C|GetAction%20Value%20Y (Variables|Default|GetCharREF)) -0.1))
        (Audio|Components|Audio|Stop (Variables|Default|GetPushSFX))))))

(fn ConstructionScript)

(fn Interact
  (params (Character :type BP%20Third%20Person%20Character%20Object%20Reference))
  ;[0.15 0.15 0.15 0.5] Interact - activate event
  (CallFunction|MoveObject)
  (return false))