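; Pushable object, apparently a test version, that the third-person character moves along a referenced spline with sound.
; Interact toggles pushing when the player overlaps MoveBox, has empty hands and has the arm, showing an objective widget if the arm is missing.
; A looping timer polls forward input to play or stop a Timeline that sets position and rotation by spline distance.
; Pulling back, leaving the box or finishing the Timeline restores walking.
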(event OnComponentBeginOverlap(MoveBox)
  (params (OverlappedComponent :type Primitive%20Component%20Object%20Reference) (OtherActor :type Actor%20Object%20Reference) (OtherComp :type Primitive%20Component%20Object%20Reference) (OtherBodyIndex :type Integer) (bFromSweep :type Boolean) (SweepResult :type Hit%20Result%20Structure%20%28by%20ref%29))
  ;[0.15 0.15 0.15 0.5] Set movement speed based on weight of box
  (Utilities|Casting|CastToBP_ThirdPersonCharacter OtherActor)
  (Variables|Default|SetCanInteractCollision true))

(event OnComponentEndOverlap(MoveBox)
  (params (OverlappedComponent :type Primitive%20Component%20Object%20Reference) (OtherActor :type Actor%20Object%20Reference) (OtherComp :type Primitive%20Component%20Object%20Reference) (OtherBodyIndex :type Integer))
  ;[0.15 0.15 0.15 0.5] Set movement speed based on weight of box
  (Utilities|Casting|CastToBP_ThirdPersonCharacter OtherActor)
  (Audio|Components|Audio|Stop (Variables|Default|GetPushSFX))
  (CallFunction|Walking)
  (Variables|Default|SetCanInteractCollision false)
  (Variables|Default|SetCanInteractE false))

(event Custom|CanMoveObj
  ;[0.15 0.15 0.15 0.5] Movement Logic
  (if (Variables|/Game/BP_ThirdPersonCharacter.BP_ThirdPersonCharacter_C|GetHasArm (Variables|Default|GetCharRef))
    (if (Variables|Default|GetCanInteractE)
      (CallFunction|Pushing)
      (Audio|Components|Audio|Play (Variables|Default|GetPushSFX) 0.0)
      (Variables|Default|SetLooping true)
      (bind _returnvalue (Utilities|Time|SetTimerbyEvent (delegate Custom|MoveBW) 0.1 (Variables|Default|GetLooping)))
      (Variables|Default|SetTimer _returnvalue)
      (else
        (CallFunction|Walking)
        (Audio|Components|Audio|Stop (Variables|Default|GetPushSFX))
        (Utilities|Time|ClearandInvalidateTimerbyHandle (Variables|Default|GetTimer))
        (Variables|Default|SetLooping false)))))

(event Custom|Pushing
  (bind _spline_to_follow (Variables|Default|GetSpline%20To%20Follow))
  (bind _spline (Variables|/Game/Blueprints_Code/Hazards/BP_SplineHazards.BP_SplineHazards_C|GetSpline _spline_to_follow))
  ;[0.15 0.15 0.15 0.5] Movement Logic
  (Variables|/Game/BP_ThirdPersonCharacter.BP_ThirdPersonCharacter_C|SetPlayerMoveState (Variables|Default|GetCharRef) "NewEnumerator4")
  (if (> (Variables|/Game/BP_ThirdPersonCharacter.BP_ThirdPersonCharacter_C|GetAction%20Value%20Y (Variables|Default|GetCharRef)) 0.1)
    (CallFunction|PlayMusic)
    (Components|Timeline|SetPlayRate (Variables|Default|GetTimeline) (/ 1.0 (Variables|Default|GetTime%20To%20Complete)))
    (bind _newtrack_1 (Timeline|Timeline Play)
      (:Update
        (Transformation|SetActorLocationAndRotation (Spline|GetLocationatDistanceAlongSpline _spline (Math|Float|Lerp 0.0 (Spline|GetSplineLength _spline) _newtrack_1) "World") (Spline|GetRotationatDistanceAlongSpline _spline (Math|Float|Lerp 0.0 (Spline|GetSplineLength _spline) _newtrack_1) "World")))
      (:Finished
        (Audio|Components|Audio|Stop (Variables|Default|GetPushSFX))
        (Variables|Default|SetCanInteractE false)
        (CallFunction|Walking)))
    (else
      (Utilities|FlowControl|Sequence
        (:then_0
          (Audio|Components|Audio|Stop (Variables|Default|GetPushSFX))
          (Timeline|Timeline Stop))
        (:then_1
          (Utilities|FlowControl|DoOnce false) ; enters at Reset
        )))))

(event Custom|Walking
  (bind _spline_to_follow (Variables|Default|GetSpline%20To%20Follow))
  (bind _spline (Variables|/Game/Blueprints_Code/Hazards/BP_SplineHazards.BP_SplineHazards_C|GetSpline _spline_to_follow))
  ;[0.15 0.15 0.15 0.5] Movement Logic
  (Variables|/Game/BP_ThirdPersonCharacter.BP_ThirdPersonCharacter_C|SetPlayerMoveState (Variables|Default|GetCharRef) "NewEnumerator6")
  (Audio|Components|Audio|Stop (Variables|Default|GetPushSFX))
  (bind _newtrack_1 (Timeline|Timeline Stop)
    (:Update
      (Transformation|SetActorLocationAndRotation (Spline|GetLocationatDistanceAlongSpline _spline (Math|Float|Lerp 0.0 (Spline|GetSplineLength _spline) _newtrack_1) "World") (Spline|GetRotationatDistanceAlongSpline _spline (Math|Float|Lerp 0.0 (Spline|GetSplineLength _spline) _newtrack_1) "World")))
    (:Finished
      (Audio|Components|Audio|Stop (Variables|Default|GetPushSFX))
      (Variables|Default|SetCanInteractE false)
      (CallFunction|Walking))))

(event Custom|PlayMusic
  ;[0.15 0.15 0.15 0.5] Movement Logic
  (Utilities|FlowControl|DoOnce false
    (:Completed
      (Audio|Components|Audio|Play (Variables|Default|GetPushSFX) 0.0))))

(event Custom|MoveBW
  ;[0.15 0.15 0.15 0.5] Movement Logic
  (if (Variables|/Game/BP_ThirdPersonCharacter.BP_ThirdPersonCharacter_C|GetHasArm (Variables|Default|GetCharRef))
    (if (Variables|Default|GetCanInteractE)
      (if (< (Variables|/Game/BP_ThirdPersonCharacter.BP_ThirdPersonCharacter_C|GetAction%20Value%20Y (Variables|Default|GetCharRef)) -0.1)
        (Variables|Default|SetCanInteractCollision false)
        (CallFunction|Walking)
        (else
          (Variables|Default|SetCanInteractCollision true)
          (CallFunction|Pushing))))))

(event EventBeginPlay
  ;[0.15 0.15 0.15 0.5] Refs
  (bind _returnvalue (Actor|GetActorOfClass "/Game/BP_ThirdPersonCharacter.BP_ThirdPersonCharacter_C"))
  (Variables|Default|SetCharRef _returnvalue)
  (bind _returnvalue_2 (AddComponent|AddAudioComponent false))
  (Variables|Default|SetPushSFX _returnvalue_2))

(event Collision|EventHit
  (params (MyComp :type Primitive%20Component%20Object%20Reference) (Other :type Actor%20Object%20Reference) (OtherComp :type Primitive%20Component%20Object%20Reference) (bSelfMoved :type Boolean) (HitLocation :type Vector :default "0, 0, 0") (HitNormal :type Vector :default "0, 0, 0") (NormalImpulse :type Vector :default "0, 0, 0") (Hit :type Hit%20Result%20Structure%20%28by%20ref%29))
  (bind _returnvalue (Transformation|GetActorForwardVector Other))
  (bind (_x _y _z) (Math|Vector|BreakVector _returnvalue))
  ;[0.15 0.15 0.15 0.5] Player Look at Box
  (Utilities|Casting|CastToBP_ThirdPersonCharacter Other)
  (Variables|Default|SetPushableDirection (Math|Vector|MakeVector (Math|Conversions|ToFloat(Integer) (Math|Float|Round _x)) (Math|Conversions|ToFloat(Integer) (Math|Float|Round _y)) (Math|Conversions|ToFloat(Integer) (Math|Float|Round _z)))))

(fn ConstructionScript)

(fn Interact
  (params (Character :type BP%20Third%20Person%20Character%20Object%20Reference))
  ;[0.15 0.15 0.15 0.5] On/Off move obj
  (if (not (Variables|/Game/BP_ThirdPersonCharacter.BP_ThirdPersonCharacter_C|GetHasItemInHand Character))
    (if (Variables|/Game/BP_ThirdPersonCharacter.BP_ThirdPersonCharacter_C|GetHasArm Character)
      (if (Variables|Default|GetCanInteractCollision)
        (Variables|Default|SetCanInteractE (not (Variables|Default|GetCanInteractE)))
        (CallFunction|CanMoveObj)
        (return false))
      (else
        (bind _returnvalue (UserInterface|CreateWidget "/Game/Blueprints_UI/WBP_Ojective.WBP_Ojective_C" 0 "Must have Left ARM"))
        (Default|ObjectiveActive _returnvalue)
        (return false)))))