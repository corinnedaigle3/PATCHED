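; BP_CubeFnB is a cube that the third-person player pushes or pulls along one axis.
; Overlapping the Fwd component marks it movable; leaving clears the character's interaction flags, restores walk speed based on HasLeg and disables cube physics.
; Each tick, while interaction flags allow, it sets the character's NoLR flag and reads forward/back input.
; Speed/Direction then eases the cube along its right vector using VInterpTo, without sweep.
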(event OnComponentBeginOverlap(Fwd)
  (params (OverlappedComponent :type Primitive%20Component%20Object%20Reference) (OtherActor :type Actor%20Object%20Reference) (OtherComp :type Primitive%20Component%20Object%20Reference) (OtherBodyIndex :type Integer) (bFromSweep :type Boolean) (SweepResult :type Hit%20Result%20Structure%20%28by%20ref%29))
  ;[0.15 0.15 0.15 0.5] On/End Overlap Set Bools (Checks if you can move obj)
  (Development|PrintString "Can Interact" true true "(R=0.000000,G=1.000000,B=0.187769,A=1.000000)")
  (Variables|/Game/BP_ThirdPersonCharacter.BP_ThirdPersonCharacter_C|SetCanInteractBox?? (Variables|Default|GetCharREF) true)
  (Variables|Default|SetMoveThisBox1 true))

(event OnComponentEndOverlap(Fwd)
  (params (OverlappedComponent :type Primitive%20Component%20Object%20Reference) (OtherActor :type Actor%20Object%20Reference) (OtherComp :type Primitive%20Component%20Object%20Reference) (OtherBodyIndex :type Integer))
  (bind _charref (Variables|Default|GetCharREF))
  (bind _charactermovement (Variables|/Script/Engine.Character|GetCharacterMovement _charref))
  ;[0.15 0.15 0.15 0.5] On/End Overlap Set Bools (Checks if you can move obj)
  (Development|PrintString "Cannot Interact" true true "(R=1.000000,G=0.005107,B=0.042764,A=1.000000)")
  (Variables|/Game/BP_ThirdPersonCharacter.BP_ThirdPersonCharacter_C|SetPlayerMoveState _charref "NewEnumerator0")
  (Variables|/Game/BP_ThirdPersonCharacter.BP_ThirdPersonCharacter_C|SetCanInteractBox?? _charref false)
  (Variables|/Game/BP_ThirdPersonCharacter.BP_ThirdPersonCharacter_C|SetIsNotInteractingBox?? _charref false)
  (Variables|Default|SetMoveThisBox1 false)
  (Variables|/Game/BP_ThirdPersonCharacter.BP_ThirdPersonCharacter_C|SetNoLR _charref false)
  (if (Variables|/Game/BP_ThirdPersonCharacter.BP_ThirdPersonCharacter_C|GetHasLeg _charref)
    (Variables|/Script/Engine.CharacterMovementComponent|SetMaxWalkSpeed _charactermovement (Variables|/Game/BP_ThirdPersonCharacter.BP_ThirdPersonCharacter_C|GetWalkSpeed _charref))
    (else
      (Variables|/Script/Engine.CharacterMovementComponent|SetMaxWalkSpeed _charactermovement (Variables|/Game/BP_ThirdPersonCharacter.BP_ThirdPersonCharacter_C|GetWalkSpeedNoLeg _charref))))
  (Physics|SetSimulatePhysics (Variables|Default|GetSM_Cube) false))

(event EventBeginPlay
  (bind _asbp_third_person_character (Utilities|Casting|CastToBP_ThirdPersonCharacter (Game|Player|GetPlayerPawn 0)))
  (Variables|Default|SetCharREF _asbp_third_person_character))

(event EventTick
  (params (DeltaSeconds :type Float%20%28single-precision%29))
  (bind _charref (Variables|Default|GetCharREF))
  (bind _charref_2 (Variables|Default|GetCharREF))
  (bind _charref_3 (Variables|Default|GetCharREF))
  (bind _action_value_y (Variables|/Game/BP_ThirdPersonCharacter.BP_ThirdPersonCharacter_C|GetAction%20Value%20Y _charref_2))
  ;[0.15 0.15 0.15 0.5] Move
  (if (Variables|/Game/BP_ThirdPersonCharacter.BP_ThirdPersonCharacter_C|GetCanInteractBox?? _charref)
    (if (Variables|/Game/BP_ThirdPersonCharacter.BP_ThirdPersonCharacter_C|GetIsNotInteractingBox?? _charref)
      (if (Variables|Default|GetMoveThisBox1)
        (Variables|/Game/BP_ThirdPersonCharacter.BP_ThirdPersonCharacter_C|SetNoLR _charref_3 true)
        (Variables|/Game/BP_ThirdPersonCharacter.BP_ThirdPersonCharacter_C|SetInteractingCubeFB?? _charref_3 true)
        (if (== _action_value_y 0.0)
          (Development|PrintString "Is not moving forward or backwards" true true "(R=0.000000,G=0.367746,B=1.000000,A=1.000000)" 2.0 "67456757")
          (elif (>= _action_value_y 0.1)
            (Development|PrintString "is moving forwards" true true "(R=1.000000,G=0.532358,B=0.593024,A=1.000000)" 2.0 "364564356")
            (Utilities|Speed/Direction true -15.0)
            (else
              (Development|PrintString "is moving backwards" true true "(R=1.000000,G=0.532358,B=0.593024,A=1.000000)" 2.0 "55353535")
              (Utilities|Speed/Direction true 15.0))))
        (else
          (Variables|/Game/BP_ThirdPersonCharacter.BP_ThirdPersonCharacter_C|SetNoLR _charref_3 false)
          (Variables|/Game/BP_ThirdPersonCharacter.BP_ThirdPersonCharacter_C|SetInteractingCubeFB?? _charref_3 false))))))

(fn ConstructionScript)

(fn Interact
  (params (Character :type BP%20Third%20Person%20Character%20Object%20Reference))
  (return false))