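; Pushable box that the third-person character slides along a spline, provided the character has an arm and has toggled interaction on.
; Each Tick checks forward input to play or stop a timeline, scaled by TimeToComplete, that sets location and rotation along the spline.
; It also switches the character's move state and walk speed, with push speed set on overlap by weight class.
; Push audio follows movement and input; leaving the box clears interaction.
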(event OnComponentBeginOverlap(Box)
  (params (OverlappedComponent :type Primitive%20Component%20Object%20Reference) (OtherActor :type Actor%20Object%20Reference) (OtherComp :type Primitive%20Component%20Object%20Reference) (OtherBodyIndex :type Integer) (bFromSweep :type Boolean) (SweepResult :type Hit%20Result%20Structure%20%28by%20ref%29))
  (bind _charref (Variables|Default|GetCharREF))
  ;[0.15 0.15 0.15 0.5] Set movement speed based on weight of box
  (Utilities|Casting|CastToBP_ThirdPersonCharacter OtherActor)
  (Development|PrintString "Interact Spline Box")
  (if (Variables|Default|GetLightObj)
    (bind _output_get (Variables|/Game/BP_ThirdPersonCharacter.BP_ThirdPersonCharacter_C|SetWalkSpeedPush _charref 8e+01))
    (Development|PrintString (Utilities|String|ToString(Float) _output_get))
    (elif (Variables|Default|GetMediumObj)
      (bind _output_get_2 (Variables|/Game/BP_ThirdPersonCharacter.BP_ThirdPersonCharacter_C|SetWalkSpeedPush _charref 7e+01))
      (Development|PrintString (Utilities|String|ToString(Float) _output_get_2))
      (elif (Variables|Default|GetHeavyObj)
        (bind _output_get_3 (Variables|/Game/BP_ThirdPersonCharacter.BP_ThirdPersonCharacter_C|SetWalkSpeedPush _charref 6e+01))
        (Development|PrintString (Utilities|String|ToString(Float) _output_get_3))
        (else
          (bind _output_get_4 (Variables|/Game/BP_ThirdPersonCharacter.BP_ThirdPersonCharacter_C|SetWalkSpeedPush _charref 8e+01))
          (Development|PrintString (Utilities|String|ToString(Float) _output_get_4)))))))

(event OnComponentEndOverlap(Box)
  (params (OverlappedComponent :type Primitive%20Component%20Object%20Reference) (OtherActor :type Actor%20Object%20Reference) (OtherComp :type Primitive%20Component%20Object%20Reference) (OtherBodyIndex :type Integer))
  ;[0.15 0.15 0.15 0.5] Movement Logic
  (Utilities|Casting|CastToBP_ThirdPersonCharacter OtherActor)
  (Variables|Default|SetCanInteract false)
  (Utilities|FlowControl|DoOnce false) ; enters at Reset
)

(event Custom|Move%20Obj
  (bind _spline_to_follow (Variables|Default|GetSpline%20To%20Follow))
  (bind _charref (Variables|Default|GetCharRef))
  (bind _charref_2 (Variables|Default|GetCharRef))
  (bind _spline (Variables|/Game/Blueprints_Code/Hazards/BP_SplineHazards.BP_SplineHazards_C|GetSpline _spline_to_follow))
  (bind _charactermovement (Variables|/Script/Engine.Character|GetCharacterMovement _charref_2))
  ;[0.15 0.15 0.15 0.5] Movement Logic
  (Utilities|FlowControl|Sequence
    (:then_0
      (if (Variables|/Game/BP_ThirdPersonCharacter.BP_ThirdPersonCharacter_C|GetHasArm (Variables|Default|GetCharRef))
        (if (Variables|Default|GetCanInteract)
          (Variables|/Game/BP_ThirdPersonCharacter.BP_ThirdPersonCharacter_C|SetPlayerMoveState _charref "NewEnumerator4")
          (Development|PrintString "Moving Object")
          (Variables|/Script/Engine.CharacterMovementComponent|SetMaxWalkSpeed (Variables|/Script/Engine.Character|GetCharacterMovement _charref) (Variables|/Game/BP_ThirdPersonCharacter.BP_ThirdPersonCharacter_C|GetWalkSpeedPush _charref))
          (if (> (Variables|/Game/BP_ThirdPersonCharacter.BP_ThirdPersonCharacter_C|GetAction%20Value%20Y (Variables|Default|GetCharRef)) 0.1)
            (Utilities|FlowControl|Sequence
              (:then_0
                (Components|Timeline|SetPlayRate (Variables|Default|GetTimeline) (/ 1.0 (Variables|Default|GetTime%20To%20Complete)))
                (bind _newtrack_1 (Timeline|Timeline Play)
                  (:Update
                    (Transformation|SetActorLocationAndRotation (Spline|GetLocationatDistanceAlongSpline _spline (Math|Float|Lerp 0.0 (Spline|GetSplineLength _spline) _newtrack_1) "World") (Spline|GetRotationatDistanceAlongSpline _spline (Math|Float|Lerp 0.0 (Spline|GetSplineLength _spline) _newtrack_1) "World")))
                  (:Finished
                    (Audio|Components|Audio|Stop (Variables|Default|GetPushSFX)))))
              (:then_1
                (Utilities|FlowControl|DoOnce false
                  (:Completed
                    (Audio|Components|Audio|Play (Variables|Default|GetPushSFX) 0.0)))))
            (else
              (Timeline|Timeline Stop)))
          (else
            (Variables|/Game/BP_ThirdPersonCharacter.BP_ThirdPersonCharacter_C|SetPlayerMoveState _charref_2 "NewEnumerator0")
            (if (Variables|/Game/BP_ThirdPersonCharacter.BP_ThirdPersonCharacter_C|GetHasLeg _charref_2)
              (Variables|/Script/Engine.CharacterMovementComponent|SetMaxWalkSpeed _charactermovement (Variables|/Game/BP_ThirdPersonCharacter.BP_ThirdPersonCharacter_C|GetWalkSpeed _charref_2))
              (Timeline|Timeline Stop)
              (else
                (Variables|/Script/Engine.CharacterMovementComponent|SetMaxWalkSpeed _charactermovement (Variables|/Game/BP_ThirdPersonCharacter.BP_ThirdPersonCharacter_C|GetWalkSpeedNoLeg _charref_2))
                (Timeline|Timeline Stop)))))))
    (:then_1
      (CallFunction|SFXAudioControl 0.0))))

(event Custom|CanInteractSpline
  ;[0.15 0.15 0.15 0.5] Movement Logic
  ;;[0.15 0.15 0.15 0.5] Variable Hooked up to interaction system
  (Variables|Default|SetCanInteract (not (Variables|Default|GetCanInteract)))
  (Utilities|FlowControl|DoOnce false) ; enters at Reset
)

(event Custom|SFX%20Audio%20Control
  (params (DeltaSeconds :type Float%20%28single-precision%29))
  (bind _charref (Variables|Default|GetCharREF))
  ;[0.15 0.15 0.15 0.5] Plays SFX if player is interacting and moving
  (Utilities|FlowControl|Sequence
    (:then_0
      (if (Variables|/Game/BP_ThirdPersonCharacter.BP_ThirdPersonCharacter_C|GetHasArm _charref)
        (if (Variables|/Game/BP_ThirdPersonCharacter.BP_ThirdPersonCharacter_C|GetIsMoving _charref)
          (if (Variables|Default|GetCanInteract)
            (Utilities|FlowControl|Delay 2.0)
            (Audio|Components|Audio|Play (Variables|Default|GetPushSFX) 0.0)
            (else
              (Audio|Components|Audio|Stop (Variables|Default|GetPushSFX) :!label _label)))
          (else
            (goto _label)))
        (else
          (goto _label))))
    (:then_1
      (if (not (> (Variables|/Game/BP_ThirdPersonCharacter.BP_ThirdPersonCharacter_C|GetAction%20Value%20Y (Variables|Default|GetCharREF)) -0.1))
        (Audio|Components|Audio|Stop (Variables|Default|GetPushSFX))))))

(event EventBeginPlay
  ;[0.15 0.15 0.15 0.5] Refs
  (bind _returnvalue (Actor|GetActorOfClass "/Game/BP_ThirdPersonCharacter.BP_ThirdPersonCharacter_C"))
  (Variables|Default|SetCharRef _returnvalue)
  (bind _returnvalue_2 (AddComponent|AddAudioComponent false))
  (Variables|Default|SetPushSFX _returnvalue_2))

(event EventTick
  (params (DeltaSeconds :type Float%20%28single-precision%29))
  ;[0.15 0.15 0.15 0.5] Movement Logic
  (CallFunction|MoveObj))

(fn ConstructionScript)

(fn Interact
  (params (Character :type BP%20Third%20Person%20Character%20Object%20Reference))
  ;[0.15 0.15 0.15 0.5] On/Off move obj
  (CallFunction|CanInteractSpline)
  (return false))