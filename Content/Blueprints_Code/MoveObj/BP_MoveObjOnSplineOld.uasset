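; Pushable object that the player moves along a spline, provided the character has an arm.
; Interact toggles pushing while the player overlaps MoveBox; leaving it restores the walking state.
; Each Tick, pushing applies the slower push move state and speed, and forward input drives a Timeline that interpolates location and rotation along SplineToFollow over TimeToComplete.
; Push audio follows movement and input, and interacting without the arm shows an objective message.
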(event OnComponentBeginOverlap(MoveBox)
  (params (OverlappedComponent :type Primitive%20Component%20Object%20Reference) (OtherActor :type Actor%20Object%20Reference) (OtherComp :type Primitive%20Component%20Object%20Reference) (OtherBodyIndex :type Integer) (bFromSweep :type Boolean) (SweepResult :type Hit%20Result%20Structure%20%28by%20ref%29))
  ;[0.15 0.15 0.15 0.5] Set movement speed based on weight of box
  (Utilities|Casting|CastToBP_ThirdPersonCharacter OtherActor)
  (Variables|Default|SetCanInteractCollision true)
  (Variables|Default|Set2 true)
  ;;[0.15 0.15 0.15 0.5] This will not happen in final boss fight
  (if (Variables|Default|GetBossAble)
    _))

(event OnComponentEndOverlap(MoveBox)
  (params (OverlappedComponent :type Primitive%20Component%20Object%20Reference) (OtherActor :type Actor%20Object%20Reference) (OtherComp :type Primitive%20Component%20Object%20Reference) (OtherBodyIndex :type Integer))
  ;[0.15 0.15 0.15 0.5] Set movement speed based on weight of box
  (Utilities|Casting|CastToBP_ThirdPersonCharacter OtherActor)
  (CallFunction|Walking)
  (Variables|Default|SetCanInteractCollision false)
  (Variables|Default|SetCanInteractE false)
  (Variables|Default|Set2 false)
  (if (Variables|Default|GetBossAble)
    _))

(event Custom|Move%20Obj
  ;[0.15 0.15 0.15 0.5] Movement Logic
  (Utilities|FlowControl|Sequence
    (:then_0
      (if (Variables|/Game/BP_ThirdPersonCharacter.BP_ThirdPersonCharacter_C|GetHasArm (Variables|Default|GetCharRef))
        (if (Variables|Default|GetCanInteractE)
          (CallFunction|Pushing))))
    (:then_1
      (CallFunction|SFXAudioControl 0.0))))

(event Custom|Pushing
  (bind _charref (Variables|Default|GetCharRef))
  (bind _spline_to_follow (Variables|Default|GetSpline%20To%20Follow))
  (bind _spline (Variables|/Game/Blueprints_Code/Hazards/BP_SplineHazards.BP_SplineHazards_C|GetSpline _spline_to_follow))
  ;[0.15 0.15 0.15 0.5] Movement Logic
  (Variables|/Game/BP_ThirdPersonCharacter.BP_ThirdPersonCharacter_C|SetPlayerMoveState _charref "NewEnumerator4")
  (Variables|/Script/Engine.CharacterMovementComponent|SetMaxWalkSpeed (Variables|/Script/Engine.Character|GetCharacterMovement _charref) (Variables|/Game/BP_ThirdPersonCharacter.BP_ThirdPersonCharacter_C|GetWalkSpeedPush _charref))
  (if (> (Variables|/Game/BP_ThirdPersonCharacter.BP_ThirdPersonCharacter_C|GetAction%20Value%20Y (Variables|Default|GetCharRef)) 0.1)
    (Utilities|FlowControl|Sequence
      (:then_0
        (Components|Timeline|SetPlayRate (Variables|Default|GetTimeline) (/ 1.0 (Variables|Default|GetTime%20To%20Complete)))
        (if (Variables|Default|Get2)
          (bind _newtrack_1 (Timeline|Timeline Play)
            (:Update
              (Transformation|SetActorLocationAndRotation (Spline|GetLocationatDistanceAlongSpline _spline (Math|Float|Lerp 0.0 (Spline|GetSplineLength _spline) _newtrack_1) "World") (Spline|GetRotationatDistanceAlongSpline _spline (Math|Float|Lerp 0.0 (Spline|GetSplineLength _spline) _newtrack_1) "World")))
            (:Finished
              (Audio|Components|Audio|Stop (Variables|Default|GetPushSFX))
              (Variables|Default|SetCanInteractE false)
              (CallFunction|Walking)))
          (else
            (Timeline|Timeline Reverse))))
      (:then_1
        (Utilities|FlowControl|DoOnce false
          (:Completed
            (Audio|Components|Audio|Play (Variables|Default|GetPushSFX) 0.0)))))
    (else
      (Timeline|Timeline Stop))))

(event Custom|Walking
  (bind _spline_to_follow (Variables|Default|GetSpline%20To%20Follow))
  (bind _spline (Variables|/Game/Blueprints_Code/Hazards/BP_SplineHazards.BP_SplineHazards_C|GetSpline _spline_to_follow))
  ;[0.15 0.15 0.15 0.5] Movement Logic
  (Variables|/Game/BP_ThirdPersonCharacter.BP_ThirdPersonCharacter_C|SetPlayerMoveState (Variables|Default|GetCharRef) "NewEnumerator6")
  (Development|PrintString "Hello")
  (bind _newtrack_1 (Timeline|Timeline Stop)
    (:Update
      (Transformation|SetActorLocationAndRotation (Spline|GetLocationatDistanceAlongSpline _spline (Math|Float|Lerp 0.0 (Spline|GetSplineLength _spline) _newtrack_1) "World") (Spline|GetRotationatDistanceAlongSpline _spline (Math|Float|Lerp 0.0 (Spline|GetSplineLength _spline) _newtrack_1) "World")))
    (:Finished
      (Audio|Components|Audio|Stop (Variables|Default|GetPushSFX))
      (Variables|Default|SetCanInteractE false)
      (CallFunction|Walking))))

(event Custom|CanInteractSpline
  ;[0.15 0.15 0.15 0.5] Movement Logic
  ;;[0.15 0.15 0.15 0.5] Variable Hooked up to interaction system
  (if (Variables|Default|GetCanInteractCollision)
    (Variables|Default|SetCanInteractE (not (Variables|Default|GetCanInteractE)))
    (Utilities|FlowControl|DoOnce false) ; enters at Reset
  ))

(event Custom|SFX%20Audio%20Control
  (params (DeltaSeconds :type Float%20%28single-precision%29))
  (bind _charref (Variables|Default|GetCharREF))
  ;[0.15 0.15 0.15 0.5] Plays SFX if player is interacting and moving
  (Utilities|FlowControl|Sequence
    (:then_0
      (if (Variables|/Game/BP_ThirdPersonCharacter.BP_ThirdPersonCharacter_C|GetHasArm _charref)
        (if (Variables|/Game/BP_ThirdPersonCharacter.BP_ThirdPersonCharacter_C|GetIsMoving _charref)
          (if (Variables|Default|GetCanInteractE)
            (Utilities|FlowControl|Delay 2.0)
            (Audio|Components|Audio|Play (Variables|Default|GetPushSFX) 0.0)
            (else
              (Audio|Components|Audio|Stop (Variables|Default|GetPushSFX) :!label _label)))
          (else
            (goto _label)))
        (else
          (goto _label))))
    (:then_1
      (if (< (Variables|/Game/BP_ThirdPersonCharacter.BP_ThirdPersonCharacter_C|GetAction%20Value%20Y (Variables|Default|GetCharREF)) -0.1)
        (Audio|Components|Audio|Stop (Variables|Default|GetPushSFX))))))

(event EventBeginPlay
  ;[0.15 0.15 0.15 0.5] Refs
  (bind _returnvalue (Actor|GetActorOfClass "/Game/BP_ThirdPersonCharacter.BP_ThirdPersonCharacter_C"))
  (Variables|Default|SetCharRef _returnvalue)
  (bind _returnvalue_2 (AddComponent|AddAudioComponent false))
  (Variables|Default|SetPushSFX _returnvalue_2))

(event Collision|EventHit
  (params (MyComp :type Primitive%20Component%20Object%20Reference) (Other :type Actor%20Object%20Reference) (OtherComp :type Primitive%20Component%20Object%20Reference) (bSelfMoved :type Boolean) (HitLocation :type Vector :default "0, 0, 0") (HitNormal :type Vector :default "0, 0, 0") (NormalImpulse :type Vector :default "0, 0, 0") (Hit :type Hit%20Result%20Structure%20%28by%20ref%29))
  (bind _returnvalue (Transformation|GetActorForwardVector Other))
  (bind (_x _y _z) (Math|Vector|BreakVector _returnvalue))
  (Utilities|Casting|CastToBP_ThirdPersonCharacter Other)
  (Variables|Default|SetPushableDirection (Math|Vector|MakeVector (Math|Conversions|ToFloat(Integer) (Math|Float|Round _x)) (Math|Conversions|ToFloat(Integer) (Math|Float|Round _y)) (Math|Conversions|ToFloat(Integer) (Math|Float|Round _z)))))

(event EventTick
  (params (DeltaSeconds :type Float%20%28single-precision%29))
  (bind _charref (Variables|Default|GetCharRef))
  ;[0.15 0.15 0.15 0.5] Movement Logic
  (Utilities|FlowControl|Sequence
    (:then_0
      (CallFunction|MoveObj)
      (if (Variables|/Game/BP_ThirdPersonCharacter.BP_ThirdPersonCharacter_C|GetHasArm (Variables|Default|GetCharRef))
        (if (Variables|Default|GetCanInteractE)
          (if (< (Variables|/Game/BP_ThirdPersonCharacter.BP_ThirdPersonCharacter_C|GetAction%20Value%20Y (Variables|Default|GetCharRef)) -0.1)
            (Variables|/Game/BP_ThirdPersonCharacter.BP_ThirdPersonCharacter_C|SetNoFB _charref true)
            (Utilities|FlowControl|DoOnce false) ; enters at Reset
            (else
              (Variables|/Game/BP_ThirdPersonCharacter.BP_ThirdPersonCharacter_C|SetNoFB _charref false))))))))

(fn ConstructionScript)

(fn Interact
  (params (Character :type BP%20Third%20Person%20Character%20Object%20Reference))
  ;[0.15 0.15 0.15 0.5] On/Off move obj
  (if (not (Variables|/Game/BP_ThirdPersonCharacter.BP_ThirdPersonCharacter_C|GetHasItemInHand Character))
    (if (Variables|/Game/BP_ThirdPersonCharacter.BP_ThirdPersonCharacter_C|GetHasArm Character)
      (CallFunction|CanInteractSpline)
      (else
        (bind _returnvalue (UserInterface|CreateWidget "/Game/Blueprints_UI/WBP_Ojective.WBP_Ojective_C" 0 "Must have Left ARM"))
        (Default|ObjectiveActive _returnvalue)))
    (return false)))