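; BP_CrouchBox is a trigger volume that makes the player's third-person character crouch while inside it.
; On begin overlap, if the cached character is not falling, it shrinks the capsule radius, sets crouched max speed to the character's WalkSpeed and calls Crouch.
; End overlap calls UnCrouch but restores neither radius nor speed, as the radius reset node is left disconnected.
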(event OnComponentBeginOverlap(Box)
  (params (OverlappedComponent :type Primitive%20Component%20Object%20Reference) (OtherActor :type Actor%20Object%20Reference) (OtherComp :type Primitive%20Component%20Object%20Reference) (OtherBodyIndex :type Integer) (bFromSweep :type Boolean) (SweepResult :type Hit%20Result%20Structure%20%28by%20ref%29))
  (if (== OtherActor (Variables|Default|GetCharRef))
    (bind _charref (Variables|Default|GetCharRef)
      (:then
        (if (not (AI|Components|NavMovement|IsFalling (Variables|/Script/Engine.Character|GetCharacterMovement _charref)))
          (Components|Capsule|SetCapsuleRadius (Variables|/Script/Engine.Character|GetCapsuleComponent _charref) 8.731753 false)
          (Variables|/Script/Engine.CharacterMovementComponent|SetMaxWalkSpeedCrouched (Variables|/Script/Engine.Character|GetCharacterMovement _charref) (Variables|/Game/BP_ThirdPersonCharacter.BP_ThirdPersonCharacter_C|GetWalkSpeed _charref))
          (Character|Crouch (Variables|Default|GetCharRef))))
      (:else))))

(event OnComponentEndOverlap(Box)
  (params (OverlappedComponent :type Primitive%20Component%20Object%20Reference) (OtherActor :type Actor%20Object%20Reference) (OtherComp :type Primitive%20Component%20Object%20Reference) (OtherBodyIndex :type Integer))
  (if (== OtherActor (Variables|Default|GetCharRef))
    (bind _charref (Variables|Default|GetCharRef)
      (:then
        (Character|UnCrouch (Variables|Default|GetCharRef)))
      (:else))))

(event EventBeginPlay
  (bind _asbp_third_person_character (Utilities|Casting|CastToBP_ThirdPersonCharacter (Game|Player|GetPlayerPawn 0)))
  (Variables|Default|SetCharRef _asbp_third_person_character))

(fn ConstructionScript)