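; BP_ConveyorButton1 is a button actor that switches off the player's ability to toggle a conveyor belt when interacted with.
; BeginPlay casts player 0's character to BP_ThirdPersonCharacter and stores it.
; Interact prints a debug message, sets CanToggleConverbelt to false on that stored reference rather than the passed-in Character, and returns false.
; Two leftover nodes that set StartStop on the character are unconnected and never run.
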(event EventBeginPlay
  (bind _asbp_third_person_character (Utilities|Casting|CastToBP_ThirdPersonCharacter (Game|GetPlayerCharacter 0)))
  (Variables|Default|SetCharREF _asbp_third_person_character))

(event Collision|EventActorBeginOverlap
  (params (OtherActor :type Actor%20Object%20Reference)))

(event EventTick
  (params (DeltaSeconds :type Float%20%28single-precision%29)))

(fn ConstructionScript)

(fn Interact
  (params (Character :type BP%20Third%20Person%20Character%20Object%20Reference))
  (Development|PrintString "Button Press")
  (Variables|/Game/BP_ThirdPersonCharacter.BP_ThirdPersonCharacter_C|SetCanToggleConverbelt? (Variables|Default|GetCharREF) false)
  (return false))