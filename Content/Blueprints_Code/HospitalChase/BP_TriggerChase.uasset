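; Trigger volume that starts a hospital chase the first time the third-person player character overlaps it.
; SpawnEnemies recursively walks the spawn locations, either relocating existing blind enemies to chase, staggered by short delays, or spawning deaf ones.
; After a delay it opens the assigned doors, greatly raises player footstep loudness and disables trigger collision.
; The enemy-disabling logic is disconnected and never runs.
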(event OnComponentBeginOverlap(Box)
  (params (OverlappedComponent :type Primitive%20Component%20Object%20Reference) (OtherActor :type Actor%20Object%20Reference) (OtherComp :type Primitive%20Component%20Object%20Reference) (OtherBodyIndex :type Integer) (bFromSweep :type Boolean) (SweepResult :type Hit%20Result%20Structure%20%28by%20ref%29))
  (bind _asbp_third_person_character (Utilities|Casting|CastToBP_ThirdPersonCharacter OtherActor))
  (Utilities|FlowControl|DoOnce false
    (:Completed
      (CallFunction|SpawnEnemies)
      (Utilities|FlowControl|Delay (Variables|Default|GetDelay))
      (CallFunction|UnlocksDoors _asbp_third_person_character)
      (bind _boxthing (Variables|Default|GetBoxThing)
        (:then
          (Collision|SetActorEnableCollision _boxthing false))
        (:else
          (Collision|SetCollisionEnabled (Variables|Default|GetBox) "NoCollision"))))))

(event Custom|Disable%20Enemies)

(event Custom|SpawnEnemies
  (if (< (Variables|Default|GetIndexP) (Utilities|Array|Length (Variables|Default|GetEnemySapwnLocation)))
    (if (Variables|Default|GetBlind?)
      (if (Utilities|IsValid (Utilities|Array|Get(acopy) (Variables|Enemies|GetEnemiesBlindChase) (Variables|Default|GetIndexP)))
        (Transformation|SetActorLocation (Utilities|Array|Get(acopy) (Variables|Enemies|GetEnemiesBlindChase) (Variables|Default|GetIndexP)) (.Location (Math|Transform|BreakTransform (Utilities|Array|Get(acopy) (Variables|Default|GetEnemySapwnLocation) (Variables|Default|GetIndexP)))) false false)
        (Utilities|FlowControl|Delay 0.2)
        (Default|ChasePlayer (Utilities|Array|Get(acopy) (Variables|Enemies|GetEnemiesBlindChase) (Variables|Default|GetIndexP)))
        (Variables|Default|SetIndexP (+ (Variables|Default|GetIndexP) 1) :!label _label)
        (CallFunction|SpawnEnemies))
      (else
        (Game|SpawnActorfromClass "/Game/Blueprints_Code/Experimental/BP_NewEnemyDeaf.BP_NewEnemyDeaf_C" (Math|Transform|MakeTransform (.Location (Math|Transform|BreakTransform (Utilities|Array|Get(acopy) (Variables|Default|GetEnemySapwnLocation) (Variables|Default|GetIndexP)))) "0, 0, 0" "1.000000,1.000000,1.000000") "Undefined" "MultiplyWithRoot" 0 0)
        (goto _label)))))

(event EventBeginPlay)

(fn ConstructionScript)

(fn UnlockEnemies)

(fn UnlocksDoors
  (params (Player :type BP%20Third%20Person%20Character%20Object%20Reference))
  (bind _opendoors (Variables|Default|GetOpenDoors))
  (if (Utilities|Array|IsNotEmpty _opendoors)
    (for _array_element _opendoors
      (Default|OpenDoor _array_element)
      (Development|PrintString "trigger open door"))
    (Variables|/Game/BP_ThirdPersonCharacter.BP_ThirdPersonCharacter_C|SetFootStepLoudness Player 1e+03)
    (Development|PrintString "It is now 1000 loud noise ")
    (else
      (Development|PrintString " 
NEED TO ATTACH DOORS TO ARRAY 
" true true "(R=0.447917,G=0.030004,B=0.021864,A=1.000000)" 2e+01))))