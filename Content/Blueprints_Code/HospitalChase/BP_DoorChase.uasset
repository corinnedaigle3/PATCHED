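; BP_DoorChase is a sliding door for the hospital chase that opens after a delay.
; On BeginPlay it creates Locked and Unlocked audio components, which this graph never plays, and adds itself to OpenDoors on its TriggerChase reference.
; OpenDoor waits DelayTime, then plays the OpenCloseDoor timeline, which lerps the SlidingDoor's relative Y position out to SlideDistance.
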(event Custom|OpenDoor
  ;[0.15 0.15 0.15 0.5] Open Door logic
  (Utilities|FlowControl|Delay (Variables|Default|GetDelayTime))
  (bind _doortrack (Timeline|Open/CloseDoor Play)
    (:Update
      (Transformation|SetRelativeLocation (Variables|Default|Getsliding_door) (Math|Vector|MakeVector 0.0 (Math|Float|Lerp 0.0 (Variables|Default|GetSlideDistance) _doortrack) 8.0) false false))))

(event EventBeginPlay
  (bind _returnvalue (AddComponent|AddAudioComponent false))
  (Variables|Default|SetLocked _returnvalue)
  (bind _returnvalue_2 (AddComponent|AddAudioComponent false))
  (Variables|Default|SetUnlocked _returnvalue_2)
  (Utilities|Array|AddUnique (Variables|/Game/Blueprints_Code/HospitalChase/BP_TriggerChase.BP_TriggerChase_C|GetOpenDoors (Variables|SetTriggerChase|GetTriggerChase)) self))

(fn ConstructionScript)