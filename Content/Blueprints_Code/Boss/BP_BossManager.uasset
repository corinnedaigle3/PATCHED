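; Boss manager actor for the DollMaker fight, started by a trigger overlap or interaction and ending in a cutscene, credits and main menu.
; It spawns a BP_BossHandler to run three phases, advanced through a once-guarded NextPhase.
; Timelines move the head and right hand vertically into idle position at fight start.
; ObjectManager attack and box-pool hand finish events drive and reverse the mallet hand's attack timeline.
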(event OnComponentBeginOverlap(BossTrigger)
  (params (OverlappedComponent :type Primitive%20Component%20Object%20Reference) (OtherActor :type Actor%20Object%20Reference) (OtherComp :type Primitive%20Component%20Object%20Reference) (OtherBodyIndex :type Integer) (bFromSweep :type Boolean) (SweepResult :type Hit%20Result%20Structure%20%28by%20ref%29))
  (if (Class|GameplayStatics|ObjectIsA OtherActor "/Game/BP_ThirdPersonCharacter.BP_ThirdPersonCharacter_C")
    (Utilities|FlowControl|DoOnce false
      (:Completed
        (CallFunction|StartBossFight)))))

(event Custom|Start
  (CallFunction|IdleAnimation))

(event Custom|EndBossFight
  (Default|CallBossDead)
  (Development|PrintString "Boss Dead" true true "(R=0.000000,G=0.660000,B=1.000000,A=1.000000)" 2e+01)
  (Default|DestroyPhase3 (Variables|Default|GetBossHandler))
  (Input|DisableInput (Game|GetPlayerController 0))
  (CallFunction|StartFinalCutScene)
  (Utilities|FlowControl|Delay 12.1)
  (bind _returnvalue (Game|ConstructObjectfromClass "/Game/Blueprints_UI/WBP_AltCam.WBP_AltCam_C"))
  (EventDispatchers|BindEventtoCreditsDone _returnvalue (delegate Custom|LoadMainMenu))
  (Default|Credits _returnvalue))

(event Custom|FinishAttack_Event
  (bind _patched_dollmaker_rhand (Variables|Default|GetPATCHED_DollMaker_RHand))
  (bind _returnvalue (Transformation|GetWorldLocation _patched_dollmaker_rhand))
  (Variables|Anim|SetMalletisAttacking false)
  (bind _newtrack_0 (Timeline|Timeline_2 Reverse)
    (:Update
      (Transformation|SetWorldLocation _patched_dollmaker_rhand (Math|Vector|MakeVector (.x _returnvalue) (.y _returnvalue) (Math|Float|Lerp (.z _returnvalue) (Variables|Anim|GetB) _newtrack_0)) false false))
    (:Finished
      (Variables|Anim|SetB -1e+03))))

(event Custom|BossAttack
  (bind _bosshandler (Variables|Default|GetBossHandler))
  (Utilities|FlowControl|Delay 2.0)
  (switch int (Variables|Default|GetPhase)
    (:0
      (Default|Phase1 _bosshandler)
      (Variables|Default|SetObjectManager (Variables|/Game/Blueprints_Code/Boss/BP_BossHandler.BP_BossHandler_C|GetObjectManager _bosshandler)))
    (:1
      (Default|Phase2 (Variables|Default|GetBossHandler)))
    (:2
      (Default|Phase3 (Variables|Default|GetBossHandler)))
    (:3
      (CallFunction|EndBossFight))))

(event Custom|NextPhase
  (bind _phase (Variables|Default|GetPhase))
  (Utilities|FlowControl|DoOnce false
    (:Completed
      (Math|Integer|IncrementInt _phase
        (:%20%20
          (Development|PrintString (Utilities|String|Append "Phase is: " (Utilities|String|ToString(Integer) (+ _phase 1))) true true "(R=0.000000,G=0.660000,B=1.000000,A=1.000000)" 5.0)
          (Utilities|FlowControl|Delay 3.0)
          (CallFunction|BossAttack)
          (CallFunction|AllowAddPhase))))))

(event Custom|AllowAddPhase
  (bind _phase (Variables|Default|GetPhase))
  (Utilities|FlowControl|DoOnce false) ; enters at Reset
)

(event Custom|LoadMainMenu
  (Game|OpenLevel(byName) "MainMenu")
  (Input|EnableInput (Game|GetPlayerController 0)))

(event Custom|StartBossFight
  (Collision|SetCollisionEnabled (Variables|Default|GetBossTrigger) "NoCollision")
  (bind _returnvalue (Game|SpawnActorfromClass "/Game/Blueprints_Code/Boss/BP_BossHandler.BP_BossHandler_C" (Transformation|GetActorTransform self) "Undefined" "MultiplyWithRoot" 0 0))
  (bind _output_get (Variables|Default|SetBossHandler _returnvalue))
  (Variables|/Game/Blueprints_Code/Boss/BP_BossHandler.BP_BossHandler_C|SetBossManager _output_get self)
  (Variables|Default|SetBossAlive true)
  (Default|CallBossStarted)
  (Development|PrintString "Boss Started")
  (CallFunction|BossAttack)
  (EventDispatchers|BindEventtoBossDead (delegate Custom|StartFinalCutScene)))

(event Custom|IdleAnimation
  (bind _patched_dollmaker_rhand (Variables|Default|GetPATCHED_DollMaker_RHand))
  (bind _patched_dollmaker_head (Variables|Default|GetPATCHED_DollMaker_Head))
  (bind _returnvalue (Transformation|GetWorldLocation _patched_dollmaker_head))
  (bind _returnvalue_2 (Transformation|GetWorldLocation _patched_dollmaker_rhand))
  (Utilities|FlowControl|Delay 4.0)
  (Utilities|FlowControl|Sequence
    (:then_0
      ;[0.15 0.15 0.15 0.5] Head Location
      (Components|Timeline|SetPlayRate (Variables|Default|GetTimeline) (/ 1.0 (Utilities|Array|Get(acopy) (Variables|Default|GetCompletedTime))))
      (bind _newtrack_0 (Timeline|Timeline PlayFromStart)
        (:Update
          (Transformation|SetWorldLocation (Variables|Default|GetPATCHED_DollMaker_Head) (Math|Vector|MakeVector (.x _returnvalue) (.y _returnvalue) (Math|Float|Lerp (.z _returnvalue) -7.5e+02 _newtrack_0)) false false))))
    (:then_1
      ;[0.15 0.15 0.15 0.5] Hand Location
      (bind _newtrack_0_2 (Timeline|Timeline_0 Play)
        (:Update
          (Transformation|SetWorldLocation (Variables|Default|GetPATCHED_DollMaker_RHand) (Math|Vector|MakeVector (.x _returnvalue_2) (.y _returnvalue_2) (Math|Float|Lerp (.z _returnvalue_2) -1e+03 _newtrack_0_2)) false false))
        (:Finished
          (Variables|Anim|SetStartIdle true)
          (bind _output_get (Variables|Default|SetHandLocation (Transformation|GetWorldLocation (Variables|Default|GetPATCHED_DollMaker_RHand))))
          (Development|PrintString (Utilities|String|ToString(Vector) _output_get) true true "(R=1.000000,G=0.461342,B=0.000000,A=1.000000)" 1e+01))))))

(event Custom|AttackAnimcation
  (bind _patched_dollmaker_rhand (Variables|Default|GetPATCHED_DollMaker_RHand))
  (bind _returnvalue (Transformation|GetWorldLocation _patched_dollmaker_rhand))
  (Variables|Anim|SetMalletisAttacking true)
  (bind _newtrack_0 (Timeline|Timeline_2 PlayFromStart)
    (:Update
      (Transformation|SetWorldLocation _patched_dollmaker_rhand (Math|Vector|MakeVector (.x _returnvalue) (.y _returnvalue) (Math|Float|Lerp (.z _returnvalue) (Variables|Anim|GetB) _newtrack_0)) false false))
    (:Finished
      (Variables|Anim|SetB -1e+03))))

(event Custom|StartFinalCutScene
  (Class|LevelStreamingDynamic|LoadLevelInstancebySoftObjectPtr (Variables|Default|GetCutSceneLvL) "0, 0, 0" "0, 0, 0" "" 0 false)
  (bind _returnvalue (Actor|GetActorOfClass "/Script/LevelSequence.LevelSequenceActor"))
  (bind _output_get (Variables|Default|SetCutScene _returnvalue))
  (Utilities|IsValid _output_get
    (:Is%20Valid
      (Sequencer|Player|Play (Variables|/Script/LevelSequence.LevelSequenceActor|GetSequencePlayer (Variables|Default|GetCutScene)) :!class /Script/MovieScene.MovieSceneSequencePlayer))))

(event EventBeginPlay
  (bind _objectmanager (Variables|Default|GetObjectManager))
  (bind _bp_boxespool (Variables|/Game/Blueprints_Code/Boss/Objects/BP_ObjectManager.BP_ObjectManager_C|GetBP_BoxesPool _objectmanager))
  (bind _lefthand (Variables|/Game/Blueprints_Code/Boss/Objects/BP_ObjectsPool.BP_ObjectsPool_C|GetLeftHand _bp_boxespool))
  (bind _righthand (Variables|/Game/Blueprints_Code/Boss/Objects/BP_ObjectsPool.BP_ObjectsPool_C|GetRightHand _bp_boxespool))
  (Transformation|AttachComponentToComponent (Variables|Default|GetPATCHED_DollMaker_Mallet) (Variables|Default|GetPATCHED_DollMaker_RHand) "Socket_JNT" "KeepRelative" "KeepRelative" "KeepRelative" true)
  (Variables|Phase1|SetStunIndex 0)
  (bind _asabp_rhand (Utilities|Casting|CastToABP_RHand (Components|SkeletalMesh|GetAnimInstance (Variables|Default|GetPATCHED_DollMaker_RHand))))
  (Variables|/Game/Blueprints_Animations/ABP_RHand.ABP_RHand_C|SetBossManager _asabp_rhand self)
  (EventDispatchers|BindEventtoBossStarted (delegate Custom|Start))
  (Utilities|FlowControl|Delay 5.0)
  (EventDispatchers|BindEventtoOnAttack (Variables|Default|GetObjectManager) (delegate Custom|AttackAnimcation))
  (Variables|Default|SetLeft%20Hand _lefthand)
  (Variables|Default|SetRight%20Hand _righthand)
  (EventDispatchers|BindEventtoFinishAttack _lefthand (delegate Custom|FinishAttack_Event))
  (EventDispatchers|AssignFinishAttack _righthand (delegate Custom|FinishAttack_Event)))

(fn ConstructionScript)

(fn CheckPhase
  (if (> (Variables|Default|GetPhase) 2)
    (return)
    (else
      (CallFunction|EndBossFight))))

(fn Interact
  (params (Character :type BP%20Third%20Person%20Character%20Object%20Reference))
  (CallFunction|StartBossFight)
  (return false))