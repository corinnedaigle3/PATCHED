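; Boss-area repair manager that supplies arm and leg pickups when the player loses a limb.
; On BeginPlay it spawns both pickups, physics off, at random points around itself and binds their destroy events to re-randomize positions.
; The player's limb-loss event triggers a DoOnce-gated, delayed timeline that lerps both pickups' height to TargetZ at the manager's XY.
; A delay chained off the timeline update then re-scatters them and re-arms the gate.
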(event Custom|DropLimb
  (bind _self self)
  (bind _self_2 self)
  (bind _returnvalue (Transformation|GetActorLocation _self))
  (bind _returnvalue_2 (Transformation|GetActorLocation _self_2))
  (Utilities|FlowControl|DoOnce false
    (:Completed
      (Development|PrintString "StartRepair" true true "(R=1.000000,G=0.015998,B=0.000000,A=1.000000)")
      (Utilities|FlowControl|Delay 2e+01)
      (bind _newtrack_0 (Timeline|DropTimeline Play)
        (:Update
          (Transformation|SetActorLocation (Variables|Default|GetLeg) (Math|Vector|MakeVector (.x _returnvalue_2) (.y _returnvalue_2) (Math|Float|Lerp (.z _returnvalue_2) (Variables|Default|GetTargetZ) _newtrack_0)) false false)
          (Transformation|SetActorLocation (Variables|Default|GetArm) (Math|Vector|MakeVector (.x _returnvalue) (.y _returnvalue) (Math|Float|Lerp (.z _returnvalue_2) (Variables|Default|GetTargetZ) _newtrack_0)) false false)
          (Utilities|FlowControl|Delay 15.0)
          (CallFunction|ResetLocation)
          (CallFunction|ResetDropLimb))))))

(event Custom|Reset
  (bind _self self)
  (bind _self_2 self)
  (bind _returnvalue (Transformation|GetActorLocation _self))
  (bind _returnvalue_2 (Transformation|GetActorLocation _self_2))
  (bind _newtrack_0 (Timeline|DropTimeline SetNewTime)
    (:Update
      (Transformation|SetActorLocation (Variables|Default|GetLeg) (Math|Vector|MakeVector (.x _returnvalue_2) (.y _returnvalue_2) (Math|Float|Lerp (.z _returnvalue_2) (Variables|Default|GetTargetZ) _newtrack_0)) false false)
      (Transformation|SetActorLocation (Variables|Default|GetArm) (Math|Vector|MakeVector (.x _returnvalue) (.y _returnvalue) (Math|Float|Lerp (.z _returnvalue_2) (Variables|Default|GetTargetZ) _newtrack_0)) false false)
      (Utilities|FlowControl|Delay 15.0)
      (CallFunction|ResetLocation)
      (CallFunction|ResetDropLimb))))

(event Custom|ResetDropLimb
  (bind _self self)
  (bind _self_2 self)
  (bind _returnvalue (Transformation|GetActorLocation _self))
  (bind _returnvalue_2 (Transformation|GetActorLocation _self_2))
  (Utilities|FlowControl|DoOnce false) ; enters at Reset
)

(event Custom|ResetLocation
  (bind _transformlocation (Utilities|RandomLocation))
  (Transformation|SetActorLocation (Variables|Default|GetArm) _transformlocation false false)
  (bind _transformlocation_2 (Utilities|RandomLocation))
  (Transformation|SetActorLocation (Variables|Default|GetLeg) _transformlocation_2 false false))

(event EventBeginPlay
  (Utilities|FlowControl|Sequence
    (:then_0
      ;[0.15 0.15 0.15 0.5] References
      (bind _asbp_third_person_character (Utilities|Casting|CastToBP_ThirdPersonCharacter (Game|Player|GetPlayerPawn 0)))
      (Variables|Default|SetAs%20BP%20Third%20Person%20Character _asbp_third_person_character))
    (:then_1
      (bind _transformlocation (Utilities|RandomLocation))
      (bind _returnvalue (Game|SpawnActorfromClass "/Game/Blueprints_Code/BP_PickUpEquiptArm.BP_PickUpEquiptArm_C" (Math|Transform|MakeTransform _transformlocation "45.000000,0.000000,0.000000" "1.000000,1.000000,1.000000") "Undefined" "MultiplyWithRoot" 0 0))
      (Variables|Default|SetArm _returnvalue)
      (Physics|SetSimulatePhysics (Variables|/Game/Blueprints_Code/BP_PickUpEquiptArm.BP_PickUpEquiptArm_C|GetArm (Variables|Default|GetArm)) false)
      (bind _transformlocation_2 (Utilities|RandomLocation))
      (bind _returnvalue_2 (Game|SpawnActorfromClass "/Game/Blueprints_Code/BP_PickUpEquiptLeg.BP_PickUpEquiptLeg_C" (Math|Transform|MakeTransform _transformlocation_2 "90.000000,0.000000,0.000000" "1.000000,1.000000,1.000000") "Undefined" "MultiplyWithRoot" 0 0))
      (Variables|Default|SetLeg _returnvalue_2)
      (Physics|SetSimulatePhysics (Variables|/Game/Blueprints_Code/BP_PickUpEquiptLeg.BP_PickUpEquiptLeg_C|GetLeg (Variables|Default|GetLeg)) false)
      (EventDispatchers|BindEventtoArmonDestory (Variables|Default|GetArm) (delegate Custom|ResetLocation))
      (EventDispatchers|BindEventtoLegonDestory (Variables|Default|GetLeg) (delegate Custom|ResetLocation)))
    (:then_2
      (EventDispatchers|BindEventtoPatchLoseLimb (Variables|Default|GetAs%20BP%20Third%20Person%20Character) (delegate Custom|DropLimb)))))

(event Collision|EventActorBeginOverlap
  (params (OtherActor :type Actor%20Object%20Reference)))

(event EventTick
  (params (DeltaSeconds :type Float%20%28single-precision%29)))

(fn ConstructionScript)