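; Phase 3 boss fight manager that runs alternating hand slams and a pimple-popping objective.
; A self-bound HandDone event flip-flops between hands, dropping each by timeline from a randomized spot, pushing the player away and resetting after floor contact.
; Every fourth slam briefly makes pimples hittable and unpauses a polling timer.
; Pops reported by BP_NeedleFunctionality are counted, and reaching the required total advances BossManager to the next phase.
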(event OnComponentBeginOverlap(RightHand)
  (params (OverlappedComponent :type Primitive%20Component%20Object%20Reference) (OtherActor :type Actor%20Object%20Reference) (OtherComp :type Primitive%20Component%20Object%20Reference) (OtherBodyIndex :type Integer) (bFromSweep :type Boolean) (SweepResult :type Hit%20Result%20Structure%20%28by%20ref%29))
  (bind _pushoutforce (Variables|Float|GetPushOutForce))
  (Utilities|FlowControl|Sequence
    (:then_0
      (if (Variables|Boolean|GetRightFalling)
        (bind _asbp_third_person_character (Utilities|Casting|CastToBP_ThirdPersonCharacter OtherActor))
        (bind _output_get (Variables|Default|SetPatch _asbp_third_person_character))
        (Character|LaunchCharacter (Variables|Default|GetPatch) (Math|Vector|MakeVector (.x (* (Math|Vector|Normalize (- (Transformation|GetActorLocation _output_get) (Transformation|GetWorldLocation (Variables|Default|GetRight%20Hand)))) (Math|Vector|MakeVector _pushoutforce _pushoutforce 0.0))) (.y (* (Math|Vector|Normalize (- (Transformation|GetActorLocation _output_get) (Transformation|GetWorldLocation (Variables|Default|GetRight%20Hand)))) (Math|Vector|MakeVector _pushoutforce _pushoutforce 0.0))) 0.0) false false)
        (Utilities|FlowControl|Delay 0.1)
        (Collision|SetCollisionResponsetoChannel (Variables|Default|GetRight%20Hand) "ECC_Pawn" "ECR_Block")))
    (:then_1
      (if (Class|GameplayStatics|ObjectIsA OtherActor "/Game/Blueprints_Code/BP_Floor.BP_Floor_C")
        (CallFunction|StopRight)
        (Math|Integer|IncrementInt (Variables|Default|GetSlamNum)
          (:%20%20
            (if (Utilities|SlamNumCheck)
              (CallFunction|PimpleToggleHit true)
              (Utilities|FlowControl|Delay 8.0)
              (CallFunction|PimpleToggleHit false)
              (else
                (Utilities|FlowControl|Delay 1.0)))
            (Transformation|SetWorldLocation (Variables|Default|GetRight%20Hand) (Variables|Vector|GetRightHandMiddleLocation) false false)
            (Rendering|SetVisibility (Variables|Default|GetRight%20Hand) true true)
            (Default|CallHandDone)))))))

(event OnComponentBeginOverlap(LeftHand)
  (params (OverlappedComponent :type Primitive%20Component%20Object%20Reference) (OtherActor :type Actor%20Object%20Reference) (OtherComp :type Primitive%20Component%20Object%20Reference) (OtherBodyIndex :type Integer) (bFromSweep :type Boolean) (SweepResult :type Hit%20Result%20Structure%20%28by%20ref%29))
  (bind _pushoutforce (Variables|Float|GetPushOutForce))
  (Utilities|FlowControl|Sequence
    (:then_0
      (if (Variables|Boolean|GetLeftFalling)
        (bind _asbp_third_person_character (Utilities|Casting|CastToBP_ThirdPersonCharacter OtherActor))
        (bind _output_get (Variables|Default|SetPatch _asbp_third_person_character))
        (Character|LaunchCharacter (Variables|Default|GetPatch) (Math|Vector|MakeVector (.x (* (Math|Vector|Normalize (- (Transformation|GetActorLocation _output_get) (Transformation|GetWorldLocation (Variables|Default|GetLeft%20Hand)))) (Math|Vector|MakeVector _pushoutforce _pushoutforce 0.0))) (.y (* (Math|Vector|Normalize (- (Transformation|GetActorLocation _output_get) (Transformation|GetWorldLocation (Variables|Default|GetLeft%20Hand)))) (Math|Vector|MakeVector _pushoutforce _pushoutforce 0.0))) 0.0) false false)
        (Utilities|FlowControl|Delay 0.1)
        (Collision|SetCollisionResponsetoChannel (Variables|Default|GetLeft%20Hand) "ECC_Pawn" "ECR_Block")))
    (:then_1
      (if (Class|GameplayStatics|ObjectIsA OtherActor "/Game/Blueprints_Code/BP_Floor.BP_Floor_C")
        (CallFunction|StopLeft)
        (Math|Integer|IncrementInt (Variables|Default|GetSlamNum)
          (:%20%20
            (Utilities|FlowControl|Delay 1.0)
            (Transformation|SetWorldLocation (Variables|Default|GetLeft%20Hand) (Variables|Vector|GetLeftHandMiddleLocation) false false)
            (Rendering|SetVisibility (Variables|Default|GetLeft%20Hand) true true)
            (Default|CallHandDone)))))))

(event Custom|PlayStartRight
  (Variables|Boolean|SetRightFalling true)
  (bind _alpha (Timeline|RightHandTimeline PlayFromStart)
    (:Update
      (Transformation|SetWorldLocation (Variables|Default|GetRight%20Hand) (Utilities|RightHandInterpolate _alpha) false false))
    (:Finished
      (Development|PrintString "The right hand has phased through the BP_Floor, adjust SlamDownDistance or decrease timeline length" true true "(R=0.000000,G=0.660000,B=1.000000,A=1.000000)" 3.0))))

(event Custom|StopRight
  (Variables|Boolean|SetRightFalling false)
  (bind _alpha (Timeline|RightHandTimeline Stop)
    (:Update
      (Transformation|SetWorldLocation (Variables|Default|GetRight%20Hand) (Utilities|RightHandInterpolate _alpha) false false))
    (:Finished
      (Development|PrintString "The right hand has phased through the BP_Floor, adjust SlamDownDistance or decrease timeline length" true true "(R=0.000000,G=0.660000,B=1.000000,A=1.000000)" 3.0))))

(event Custom|PlayStartLeft
  (Variables|Boolean|SetLeftFalling true)
  (bind _alpha (Timeline|LeftHandTimeline PlayFromStart)
    (:Update
      (Transformation|SetWorldLocation (Variables|Default|GetLeft%20Hand) (Utilities|LeftHandInterpolate _alpha) false false))
    (:Finished
      (Development|PrintString "The left hand has phased through the BP_Floor, adjust SlamDownDistance or decrease timeline length" true true "(R=0.000000,G=0.660000,B=1.000000,A=1.000000)" 3.0))))

(event Custom|StopLeft
  (Variables|Boolean|SetLeftFalling false)
  (bind _alpha (Timeline|LeftHandTimeline Stop)
    (:Update
      (Transformation|SetWorldLocation (Variables|Default|GetLeft%20Hand) (Utilities|LeftHandInterpolate _alpha) false false))
    (:Finished
      (Development|PrintString "The left hand has phased through the BP_Floor, adjust SlamDownDistance or decrease timeline length" true true "(R=0.000000,G=0.660000,B=1.000000,A=1.000000)" 3.0))))

(event Custom|PlayLeft
  (Variables|Boolean|SetLeftFalling true)
  (bind _alpha (Timeline|LeftHandTimeline Play)
    (:Update
      (Transformation|SetWorldLocation (Variables|Default|GetLeft%20Hand) (Utilities|LeftHandInterpolate _alpha) false false))
    (:Finished
      (Development|PrintString "The left hand has phased through the BP_Floor, adjust SlamDownDistance or decrease timeline length" true true "(R=0.000000,G=0.660000,B=1.000000,A=1.000000)" 3.0))))

(event Custom|PlayRight
  (Variables|Boolean|SetRightFalling true)
  (bind _alpha (Timeline|RightHandTimeline Play)
    (:Update
      (Transformation|SetWorldLocation (Variables|Default|GetRight%20Hand) (Utilities|RightHandInterpolate _alpha) false false))
    (:Finished
      (Development|PrintString "The right hand has phased through the BP_Floor, adjust SlamDownDistance or decrease timeline length" true true "(R=0.000000,G=0.660000,B=1.000000,A=1.000000)" 3.0))))

(event Custom|Popped
  (Math|Integer|IncrementInt (Variables|Default|GetPimplesPopped)))

(event Custom|EndPhase
  (Default|NextPhase (Variables|Default|GetBossManager)))

(event Custom|PimpleCheck
  (Utilities|FlowControl|Sequence
    (:then_0
      (Utilities|FlowControl|DoOnce false
        (:Completed
          (Development|PrintString "Checking Pimples"))))
    (:then_1
      (if (Utilities|PimpleInt)
        (Utilities|FlowControl|DoOnce false
          (:Completed
            (Variables|Boolean|SetHasPimples false)
            (Default|NextPhase (Variables|Default|GetBossManager))))))))

(event Custom|ResetPimpleString
  (Utilities|FlowControl|DoOnce false) ; enters at Reset
)

(event Custom|Hands
  (if (Variables|Boolean|GetHasPimples)
    (Utilities|FlowControl|FlipFlop
      (:A
        (CallFunction|SetupLeftHand)
        (Utilities|FlowControl|Delay 3.0)
        (CallFunction|PlayStartLeft))
      (:B
        (CallFunction|SetupRightHand)
        (Utilities|FlowControl|Delay 3.0)
        (CallFunction|PlayStartRight)))))

(event EventBeginPlay
  (EventDispatchers|BindEventtoHandDone (delegate Custom|Hands))
  (bind _returnvalue (Actor|GetActorOfClass "/Game/Blueprints_Code/BP_NeedleFunctionality.BP_NeedleFunctionality_C"))
  (bind _output_get (Variables|Default|SetNeedleFunctionality _returnvalue))
  (EventDispatchers|BindEventtoPimpleDestroyed _output_get (delegate Custom|Popped))
  (CallFunction|InitializeHands)
  (bind _returnvalue_2 (Utilities|Time|SetTimerbyFunctionName 0 "PimpleCheck" 0.2 true))
  (bind _output_get_2 (Variables|Default|SetPimpleCheckHandle _returnvalue_2))
  (Utilities|Time|PauseTimerbyHandle _output_get_2)
  (CallFunction|ResetPimpleString)
  (Default|CallHandDone))

(fn ConstructionScript)

(fn SetupLeftHand
  (bind _left_hand (Variables|Default|GetLeft%20Hand))
  (Transformation|SetWorldLocation _left_hand (Utilities|LeftHandSlapLocation) false false)
  (Rendering|SetVisibility _left_hand true true)
  (Collision|SetCollisionResponsetoChannel (Variables|Default|GetLeft%20Hand) "ECC_Pawn" "ECR_Overlap"))

(fn SetupRightHand
  (bind _right_hand (Variables|Default|GetRight%20Hand))
  (Transformation|SetWorldLocation _right_hand (Utilities|RightHandSlapLocation) false false)
  (Rendering|SetVisibility _right_hand true true)
  (Collision|SetCollisionResponsetoChannel (Variables|Default|GetRight%20Hand) "ECC_Pawn" "ECR_Overlap"))

(fn PimpleToggleHit
  (params (PimpleBool :type Boolean))
  (if PimpleBool
    (Utilities|Time|UnpauseTimerbyHandle (Variables|Default|GetPimpleCheckHandle))
    (else
      (Utilities|Time|PauseTimerbyHandle (Variables|Default|GetPimpleCheckHandle))
      (CallFunction|ResetPimpleString)))
  (for _array_element 0
    (Variables|/Game/Blueprints_Code/Boss/Objects/Phase3/BP_Pimple.BP_Pimple_C|SetCanHit _array_element PimpleBool)))

(fn InitializeHands
  (bind _left_hand (Variables|Default|GetLeft%20Hand))
  (bind _right_hand (Variables|Default|GetRight%20Hand))
  (Variables|Vector|SetLeftHandMiddleLocation (Transformation|GetWorldLocation _left_hand))
  (Rendering|SetVisibility _left_hand false true)
  (Variables|Vector|SetRightHandMiddleLocation (Transformation|GetWorldLocation _right_hand))
  (Rendering|SetVisibility _right_hand false true))