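; BP_Pimple is a boss Phase 3 object that is destroyed when its parry detector is overlapped while the player is parrying.
; On BeginPlay it caches the player character as Patch and its parent actor as the Phase 3 manager, which is otherwise unused here.
; The overlap handler checks only Patch's IsParrying flag, not which actor overlapped.
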(event OnComponentBeginOverlap(ParryDetector)
  (params (OverlappedComponent :type Primitive%20Component%20Object%20Reference) (OtherActor :type Actor%20Object%20Reference) (OtherComp :type Primitive%20Component%20Object%20Reference) (OtherBodyIndex :type Integer) (bFromSweep :type Boolean) (SweepResult :type Hit%20Result%20Structure%20%28by%20ref%29))
  (if (Variables|/Game/BP_ThirdPersonCharacter.BP_ThirdPersonCharacter_C|GetisParrying (Variables|Default|GetPatch))
    (Actor|DestroyActor)))

(event OnComponentEndOverlap(ParryDetector)
  (params (OverlappedComponent :type Primitive%20Component%20Object%20Reference) (OtherActor :type Actor%20Object%20Reference) (OtherComp :type Primitive%20Component%20Object%20Reference) (OtherBodyIndex :type Integer)))

(event EventBeginPlay
  (bind _asbp_third_person_character (Utilities|Casting|CastToBP_ThirdPersonCharacter (Game|GetPlayerCharacter 0)))
  (Variables|Default|SetPatch _asbp_third_person_character)
  (bind _asbp_phase_3manager (Utilities|Casting|CastToBP_Phase3Manager (Actor|GetParentActor)))
  (Variables|Default|SetPhase3Manager _asbp_phase_3manager))

(event Collision|EventActorBeginOverlap
  (params (OtherActor :type Actor%20Object%20Reference)))

(event EventTick
  (params (DeltaSeconds :type Float%20%28single-precision%29)))

(fn ConstructionScript)