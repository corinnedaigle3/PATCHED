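; Runs phase 2 of the boss fight, alternating a falling nail and a fist punch aimed at the player character (Patch).
; Timelines chain the loop: the nail tracks Patch, drops and blocks pawns once grounded, then the fist tracks and punches.
; A punch overlapping Patch can cost a life, while one hitting the nail stops and counts toward the required hits.
; Reaching that count destroys the nail and advances BP_BossManager; otherwise the cycle resets.
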(event OnComponentBeginOverlap(FistCollider)
  (params (OverlappedComponent :type Primitive%20Component%20Object%20Reference) (OtherActor :type Actor%20Object%20Reference) (OtherComp :type Primitive%20Component%20Object%20Reference) (OtherBodyIndex :type Integer) (bFromSweep :type Boolean) (SweepResult :type Hit%20Result%20Structure%20%28by%20ref%29))
  (bind _hitnail (Variables|Default|GetHitNail))
  (if (== OtherActor (Variables|Default|GetPatch))
    (if (Variables|Default|GetisPunching)
      (Utilities|FlowControl|DoOnce false
        (:Completed
          (Default|LoseALive (Variables|Default|GetPatch)))))
    (elif (Class|GameplayStatics|ObjectIsA OtherActor "/Game/Blueprints_Code/Boss/Objects/Phase2/BP_NailObject.BP_NailObject_C")
      (CallFunction|StopPunch)
      (Utilities|FlowControl|DoOnce false
        (:Completed
          (Math|Integer|IncrementInt _hitnail
            (:%20%20
              (Development|PrintString (Utilities|String|Append "Hit Nail: " (Utilities|String|ToString(Integer) _hitnail) " Times"))
              (if (Utilities|BoolHitCheck)
                (Actor|DestroyActor (Variables|Default|GetNailObject))
                (Default|NextPhase (Variables|Default|GetBossManager))
                (else
                  (Utilities|ResetFistandNails))))))))))

(event Custom|TrackPatch
  (params (Nails? :type Boolean))
  (CallFunction|SetupTracking Nails?)
  (Timeline|TrackingTimeline PlayFromStart
    (:Update
      (CallFunction|SetLocation Nails?))
    (:Finished
      (if Nails?
        (Utilities|FlowControl|Delay (Variables|Floats|GetFallDelay))
        (CallFunction|NailFall)
        (else
          (Utilities|FlowControl|Delay (Variables|Floats|GetPunchDelay))
          (CallFunction|FistPunch))))))

(event Custom|NailFall
  (Variables|/Game/Blueprints_Code/Boss/Objects/Phase2/BP_NailObject.BP_NailObject_C|SetisFalling (Variables|Default|GetNailObject) true)
  (bind _alpha (Timeline|NailFallTimeline PlayFromStart)
    (:Update
      (Transformation|SetActorLocation (Variables|Default|GetNailObject) (Utilities|LerpFalling _alpha) false false))
    (:Finished
      (CallFunction|TrackPatch false))))

(event Custom|StopFall
  (bind _nailobject (Variables|Default|GetNailObject))
  (Utilities|FlowControl|Sequence
    (:then_0
      (bind _alpha (Timeline|NailFallTimeline Stop)
        (:Update
          (Transformation|SetActorLocation (Variables|Default|GetNailObject) (Utilities|LerpFalling _alpha) false false))
        (:Finished
          (CallFunction|TrackPatch false :!label _label))))
    (:then_1
      (Collision|SetCollisionResponsetoChannel (Variables|/Game/Blueprints_Code/Boss/Objects/Phase2/BP_NailObject.BP_NailObject_C|GetBox _nailobject) "ECC_Pawn" "ECR_Block")
      (Variables|/Game/Blueprints_Code/Boss/Objects/Phase2/BP_NailObject.BP_NailObject_C|SetisFalling _nailobject false)
      (goto _label))))

(event Custom|FistPunch
  (Variables|Default|SetisPunching true)
  (bind _alpha (Timeline|FistTimeline PlayFromStart)
    (:Update
      (Transformation|SetWorldLocation (Variables|Default|GetFistCollider) (Utilities|LerpFist _alpha) false false))
    (:Finished
      (CallFunction|ResetNails)
      (CallFunction|TrackPatch true))))

(event Custom|ResetPunch
  (Utilities|FlowControl|DoOnce false) ; enters at Reset
)

(event Custom|StopPunch
  (Variables|Default|SetisPunching false)
  (bind _alpha (Timeline|FistTimeline Stop)
    (:Update
      (Transformation|SetWorldLocation (Variables|Default|GetFistCollider) (Utilities|LerpFist _alpha) false false))
    (:Finished
      (CallFunction|ResetNails)
      (CallFunction|TrackPatch true))))

(event Custom|ResetNails
  (bind _nailobject (Variables|Default|GetNailObject))
  (Transformation|SetActorLocation _nailobject (Variables|Vectors|GetNailsStartingPos) false false)
  (Rendering|SetVisibility (Variables|/Game/Blueprints_Code/Boss/Objects/Phase2/BP_NailObject.BP_NailObject_C|GetBox _nailobject) false true)
  (Collision|SetCollisionResponsetoChannel (Variables|/Game/Blueprints_Code/Boss/Objects/Phase2/BP_NailObject.BP_NailObject_C|GetBox _nailobject) "ECC_Pawn" "ECR_Overlap"))

(event Custom|ResetFistInc
  (bind _hitnail (Variables|Default|GetHitNail))
  (Utilities|FlowControl|DoOnce false) ; enters at Reset
)

(event EventTick
  (params (DeltaSeconds :type Float%20%28single-precision%29))
  (Variables|Vectors|SetPlayerLocation (Transformation|GetActorLocation (Variables|Default|GetPatch))))

(event EventBeginPlay
  (bind _nailobject (Variables|Default|GetNailObject))
  (bind _returnvalue (Actor|GetActorOfClass "/Game/Blueprints_Code/Boss/BP_BossManager.BP_BossManager_C"))
  (Variables|Default|SetBossManager _returnvalue)
  (CallFunction|SetupFist)
  (CallFunction|InitializeNails)
  (bind _returnvalue_2 (Actor|GetActorOfClass "/Game/BP_ThirdPersonCharacter.BP_ThirdPersonCharacter_C"))
  (bind _output_get (Variables|Default|SetPatch _returnvalue_2))
  (Variables|/Game/Blueprints_Code/Boss/Objects/Phase2/BP_NailObject.BP_NailObject_C|SetPatch _nailobject _output_get)
  (EventDispatchers|BindEventtoGroundHit _nailobject (delegate Custom|StopFall))
  (CallFunction|TrackPatch true))

(fn ConstructionScript)

(fn InitializeNails
  (bind _self self)
  (bind _returnvalue (Transformation|GetActorTransform _self))
  (bind _returnvalue_2 (Game|SpawnActorfromClass "/Game/Blueprints_Code/Boss/Objects/Phase2/BP_NailObject.BP_NailObject_C" (Math|Transform|MakeTransform (Math|Vector|MakeVector (.x (.location _returnvalue)) (.y (.location _returnvalue)) (+ (.z (.location _returnvalue)) 5e+01)) (.rotation _returnvalue) (.scale _returnvalue)) "Undefined" "MultiplyWithRoot" 0 0))
  (bind _output_get (Variables|Default|SetNailObject _returnvalue_2))
  (Rendering|SetVisibility (Variables|/Game/Blueprints_Code/Boss/Objects/Phase2/BP_NailObject.BP_NailObject_C|GetBox _output_get) false true)
  (Variables|Vectors|SetNailsStartingPos (Transformation|GetActorLocation (Variables|Default|GetNailObject))))

(fn SetLocation
  (params (Nail? :type Boolean))
  (bind _playerlocation (Variables|Vectors|GetPlayerLocation))
  (bind _playerlocation_2 (Variables|Vectors|GetPlayerLocation))
  (if Nail?
    (Transformation|SetActorLocation (Variables|Default|GetNailObject) (Math|Vector|MakeVector (.x _playerlocation_2) (.y _playerlocation_2) (.z (Variables|Vectors|GetNailsStartingPos))) false false)
    (else
      (Transformation|SetWorldLocation (Variables|Default|GetFistCollider) (Math|Vector|MakeVector (.x (Transformation|GetWorldLocation (Variables|/Game/Blueprints_Code/Boss/BP_BossManager.BP_BossManager_C|GetPhase2FistStart (Variables|Default|GetBossManager)))) (.y _playerlocation) (.z _playerlocation)) false false))))

(fn SetupTracking
  (params (Condition :type Boolean))
  (if Condition
    (Transformation|SetWorldLocation (Variables|/Game/Blueprints_Code/Boss/Objects/Phase2/BP_NailObject.BP_NailObject_C|GetBox (Variables|Default|GetNailObject)) (Variables|Vectors|GetNailsStartingPos) false false)
    (Rendering|SetVisibility (Variables|/Game/Blueprints_Code/Boss/Objects/Phase2/BP_NailObject.BP_NailObject_C|GetBox (Variables|Default|GetNailObject)) true true)
    (else
      (Transformation|SetWorldLocation (Variables|Default|GetFistCollider) (Transformation|GetWorldLocation (Variables|/Game/Blueprints_Code/Boss/BP_BossManager.BP_BossManager_C|GetPhase2FistStart (Variables|Default|GetBossManager))) false false)
      (Rendering|SetVisibility (Variables|Default|GetFistCollider) true true)))
  (return))

(fn SetupFist
  (bind _fistcollider (Variables|Default|GetFistCollider))
  (Transformation|SetWorldTransform _fistcollider (Transformation|GetWorldTransform (Variables|/Game/Blueprints_Code/Boss/BP_BossManager.BP_BossManager_C|GetPhase2FistStart (Variables|Default|GetBossManager))) false false)
  (Rendering|SetVisibility _fistcollider false true))