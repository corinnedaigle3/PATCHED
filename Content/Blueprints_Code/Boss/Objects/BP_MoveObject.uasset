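; BP_MoveObject is a boss-area object whose Cube switches physics simulation based on overlap between its Box and the third-person character.
; It starts with physics off, enables it on begin overlap through a DoOnce that is never reset, and disables it on end overlap.
; Both overlaps print placeholder debug strings.
; Interact is a stub returning false, and IsPhysic is only initialized, never read.
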(event OnComponentBeginOverlap(Box)
  (params (OverlappedComponent :type Primitive%20Component%20Object%20Reference) (OtherActor :type Actor%20Object%20Reference) (OtherComp :type Primitive%20Component%20Object%20Reference) (OtherBodyIndex :type Integer) (bFromSweep :type Boolean) (SweepResult :type Hit%20Result%20Structure%20%28by%20ref%29))
  (Utilities|Casting|CastToBP_ThirdPersonCharacter OtherActor)
  (Utilities|FlowControl|DoOnce false
    (:Completed
      (Physics|SetSimulatePhysics (Variables|Default|GetCube self) true)
      (Development|PrintString "ssssssssssssssss"))))

(event OnComponentEndOverlap(Box)
  (params (OverlappedComponent :type Primitive%20Component%20Object%20Reference) (OtherActor :type Actor%20Object%20Reference) (OtherComp :type Primitive%20Component%20Object%20Reference) (OtherBodyIndex :type Integer))
  (Utilities|Casting|CastToBP_ThirdPersonCharacter OtherActor)
  (Physics|SetSimulatePhysics (Variables|Default|GetCube self) false)
  (Development|PrintString "ggggggggggggg"))

(event EventBeginPlay
  (Variables|Default|SetisPhysic false)
  (Physics|SetSimulatePhysics (Variables|Default|GetCube self) false))

(event Collision|EventActorBeginOverlap
  (params (OtherActor :type Actor%20Object%20Reference)))

(event EventTick
  (params (DeltaSeconds :type Float%20%28single-precision%29)))

(fn ConstructionScript)

(fn Interact
  (params (Character :type BP%20Third%20Person%20Character%20Object%20Reference))
  (return false))