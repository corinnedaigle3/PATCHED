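; Boss-fight saw hazard that travels along a BP_SplineHazards spline and costs the player a life on contact.
; After a random delay, one timeline drives spline position while another spins pitch, keeping the spline's roll and yaw.
; Overlapping a BP_MoveObjectUpdate box halts travel and sets the boss's swing hand by relative Y; ending the overlap resumes it.
; Path completion or the bound saw-destroy event resets the movement timeline's time.
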(event OnComponentBeginOverlap(Box)
  (params (OverlappedComponent :type Primitive%20Component%20Object%20Reference) (OtherActor :type Actor%20Object%20Reference) (OtherComp :type Primitive%20Component%20Object%20Reference) (OtherBodyIndex :type Integer) (bFromSweep :type Boolean) (SweepResult :type Hit%20Result%20Structure%20%28by%20ref%29))
  (Utilities|FlowControl|Sequence
    (:then_0
      (bind _asbp_move_object_update (Utilities|Casting|CastToBP_MoveObjectUpdate OtherActor))
      (if (== OtherComp (Variables|/Game/Blueprints_Code/Boss/Objects/BP_MoveObjectUpdate.BP_MoveObjectUpdate_C|GetBox _asbp_move_object_update))
        (CallFunction|StopMovement)
        (Variables|/Game/Cutsence/Cutscene_Actors/Bosssss.Bosssss_C|SetLeftHandSwinng (Variables|Default|GetBoss) (> (.y (Transformation|GetActorLocation _asbp_move_object_update)) (.y (Transformation|GetActorLocation))))))
    (:then_1
      (bind _asbp_third_person_character (Utilities|Casting|CastToBP_ThirdPersonCharacter OtherActor))
      (if (== (Variables|/Script/Engine.Character|GetCapsuleComponent _asbp_third_person_character) OtherComp)
        (Default|LoseALive _asbp_third_person_character)))
    (:then_2
      (if (and (Class|GameplayStatics|ObjectIsA OtherActor "/Game/Cutsence/Cutscene_Actors/Bosssss.Bosssss_C") (> (Variables|/Game/Blueprints_Code/Boss/BP_BossManager.BP_BossManager_C|GetStunIndex (Variables|Default|GetBossManager)) 1))
        (Development|PrintString "Mallet gone")))))

(event OnComponentEndOverlap(Box)
  (params (OverlappedComponent :type Primitive%20Component%20Object%20Reference) (OtherActor :type Actor%20Object%20Reference) (OtherComp :type Primitive%20Component%20Object%20Reference) (OtherBodyIndex :type Integer))
  (bind _asbp_move_object_update (Utilities|Casting|CastToBP_MoveObjectUpdate OtherActor))
  (if (== OtherComp (Variables|/Game/Blueprints_Code/Boss/Objects/BP_MoveObjectUpdate.BP_MoveObjectUpdate_C|GetBox _asbp_move_object_update))
    (Variables|Default|SetHittedBox false)
    (CallFunction|Continue)))

(event Custom|StopMovement
  (bind _newtrack_0 (Timeline|SawMovement Stop)
    (:Update
      (Components|Timeline|SetPlayRate (Variables|Default|GetSawMovement) (/ 1.0 (Variables|Default|GetTime%20To%20Complete)))
      (bind _output_get (Variables|Default|SetLocationAlongSpline (Spline|GetLocationatDistanceAlongSpline (Variables|/Game/Blueprints_Code/Hazards/BP_SplineHazards.BP_SplineHazards_C|GetSpline (stale Custom|Boss_MovingSaw _output_get)) (Math|Float|Lerp 0.0 (Spline|GetSplineLength (Variables|/Game/Blueprints_Code/Hazards/BP_SplineHazards.BP_SplineHazards_C|GetSpline (stale Custom|Boss_MovingSaw _output_get))) _newtrack_0) "World")))
      (Transformation|SetActorLocation _output_get false false))
    (:Finished
      (CallFunction|RestartSaw))))

(event Custom|RestartSaw
  (bind _newtrack_0 (Timeline|SawMovement SetNewTime)
    (:Update
      (Components|Timeline|SetPlayRate (Variables|Default|GetSawMovement) (/ 1.0 (Variables|Default|GetTime%20To%20Complete)))
      (bind _output_get (Variables|Default|SetLocationAlongSpline (Spline|GetLocationatDistanceAlongSpline (Variables|/Game/Blueprints_Code/Hazards/BP_SplineHazards.BP_SplineHazards_C|GetSpline (stale Custom|Boss_MovingSaw _output_get)) (Math|Float|Lerp 0.0 (Spline|GetSplineLength (Variables|/Game/Blueprints_Code/Hazards/BP_SplineHazards.BP_SplineHazards_C|GetSpline (stale Custom|Boss_MovingSaw _output_get))) _newtrack_0) "World")))
      (Transformation|SetActorLocation _output_get false false))
    (:Finished
      (CallFunction|RestartSaw))))

(event Custom|Continue
  (bind _newtrack_0 (Timeline|SawMovement Play)
    (:Update
      (Components|Timeline|SetPlayRate (Variables|Default|GetSawMovement) (/ 1.0 (Variables|Default|GetTime%20To%20Complete)))
      (bind _output_get (Variables|Default|SetLocationAlongSpline (Spline|GetLocationatDistanceAlongSpline (Variables|/Game/Blueprints_Code/Hazards/BP_SplineHazards.BP_SplineHazards_C|GetSpline (stale Custom|Boss_MovingSaw _output_get)) (Math|Float|Lerp 0.0 (Spline|GetSplineLength (Variables|/Game/Blueprints_Code/Hazards/BP_SplineHazards.BP_SplineHazards_C|GetSpline (stale Custom|Boss_MovingSaw _output_get))) _newtrack_0) "World")))
      (Transformation|SetActorLocation _output_get false false))
    (:Finished
      (CallFunction|RestartSaw))))

(event Custom|Boss_MovingSaw
  (params (Spline%20To%20Follow :type BP%20Spline%20Hazards%20Object%20Reference))
  (bind _output_get (Variables|Default|SetSpline%20To%20Follow Spline%20To%20Follow))
  (Utilities|FlowControl|Delay (Math|Random|RandomFloatinRange 0.0 5.0))
  (Components|Timeline|SetPlayRate (Variables|Default|GetSawMovement) (/ 1.0 (Variables|Default|GetTime%20To%20Complete)))
  (CallFunction|PlayStartRotateSaw)
  (bind _newtrack_0 (Timeline|SawMovement Play)
    (:Update
      (Components|Timeline|SetPlayRate (Variables|Default|GetSawMovement) (/ 1.0 (Variables|Default|GetTime%20To%20Complete)))
      (bind _output_get_2 (Variables|Default|SetLocationAlongSpline (Spline|GetLocationatDistanceAlongSpline (Variables|/Game/Blueprints_Code/Hazards/BP_SplineHazards.BP_SplineHazards_C|GetSpline _output_get) (Math|Float|Lerp 0.0 (Spline|GetSplineLength (Variables|/Game/Blueprints_Code/Hazards/BP_SplineHazards.BP_SplineHazards_C|GetSpline _output_get)) _newtrack_0) "World")))
      (Transformation|SetActorLocation _output_get_2 false false))
    (:Finished
      (CallFunction|RestartSaw))))

(event Custom|ResetSaws
  (params (Saws :type BP%20Saw%20Child%20Object%20Reference))
  (CallFunction|RestartSaw Saws))

(event Custom|PlayStartRotateSaw
  (bind _newtrack_0 (Timeline|saw_chlid_selfrotate PlayFromStart)
    (:Update
      (Transformation|SetActorRotation (Math|Rotator|MakeRotator (.roll (Spline|GetRotationatDistanceAlongSpline (Variables|/Game/Blueprints_Code/Hazards/BP_SplineHazards.BP_SplineHazards_C|GetSpline (stale Custom|Boss_MovingSaw _output_get)) (Math|Float|Lerp 0.0 (Spline|GetSplineLength (Variables|/Game/Blueprints_Code/Hazards/BP_SplineHazards.BP_SplineHazards_C|GetSpline (stale Custom|Boss_MovingSaw _output_get))) (stale Custom|StopMovement _newtrack_0)) "World")) (.pitch (Math|Rotator|Lerp(Rotator) "0, 0, 0" "360.000000,0.000000,0.000000" _newtrack_0)) (.yaw (Spline|GetRotationatDistanceAlongSpline (Variables|/Game/Blueprints_Code/Hazards/BP_SplineHazards.BP_SplineHazards_C|GetSpline (stale Custom|Boss_MovingSaw _output_get)) (Math|Float|Lerp 0.0 (Spline|GetSplineLength (Variables|/Game/Blueprints_Code/Hazards/BP_SplineHazards.BP_SplineHazards_C|GetSpline (stale Custom|Boss_MovingSaw _output_get))) (stale Custom|StopMovement _newtrack_0)) "World")))))))

(event Custom|StopRotateSaw
  (bind _newtrack_0 (Timeline|saw_chlid_selfrotate Stop)
    (:Update
      (Transformation|SetActorRotation (Math|Rotator|MakeRotator (.roll (Spline|GetRotationatDistanceAlongSpline (Variables|/Game/Blueprints_Code/Hazards/BP_SplineHazards.BP_SplineHazards_C|GetSpline (stale Custom|Boss_MovingSaw _output_get)) (Math|Float|Lerp 0.0 (Spline|GetSplineLength (Variables|/Game/Blueprints_Code/Hazards/BP_SplineHazards.BP_SplineHazards_C|GetSpline (stale Custom|Boss_MovingSaw _output_get))) (stale Custom|StopMovement _newtrack_0)) "World")) (.pitch (Math|Rotator|Lerp(Rotator) "0, 0, 0" "360.000000,0.000000,0.000000" _newtrack_0)) (.yaw (Spline|GetRotationatDistanceAlongSpline (Variables|/Game/Blueprints_Code/Hazards/BP_SplineHazards.BP_SplineHazards_C|GetSpline (stale Custom|Boss_MovingSaw _output_get)) (Math|Float|Lerp 0.0 (Spline|GetSplineLength (Variables|/Game/Blueprints_Code/Hazards/BP_SplineHazards.BP_SplineHazards_C|GetSpline (stale Custom|Boss_MovingSaw _output_get))) (stale Custom|StopMovement _newtrack_0)) "World")))))))

(event Custom|PlayRotateSaw
  (bind _newtrack_0 (Timeline|saw_chlid_selfrotate Play)
    (:Update
      (Transformation|SetActorRotation (Math|Rotator|MakeRotator (.roll (Spline|GetRotationatDistanceAlongSpline (Variables|/Game/Blueprints_Code/Hazards/BP_SplineHazards.BP_SplineHazards_C|GetSpline (stale Custom|Boss_MovingSaw _output_get)) (Math|Float|Lerp 0.0 (Spline|GetSplineLength (Variables|/Game/Blueprints_Code/Hazards/BP_SplineHazards.BP_SplineHazards_C|GetSpline (stale Custom|Boss_MovingSaw _output_get))) (stale Custom|StopMovement _newtrack_0)) "World")) (.pitch (Math|Rotator|Lerp(Rotator) "0, 0, 0" "360.000000,0.000000,0.000000" _newtrack_0)) (.yaw (Spline|GetRotationatDistanceAlongSpline (Variables|/Game/Blueprints_Code/Hazards/BP_SplineHazards.BP_SplineHazards_C|GetSpline (stale Custom|Boss_MovingSaw _output_get)) (Math|Float|Lerp 0.0 (Spline|GetSplineLength (Variables|/Game/Blueprints_Code/Hazards/BP_SplineHazards.BP_SplineHazards_C|GetSpline (stale Custom|Boss_MovingSaw _output_get))) (stale Custom|StopMovement _newtrack_0)) "World")))))))

(event EventBeginPlay
  (bind _asbp_third_person_character (Utilities|Casting|CastToBP_ThirdPersonCharacter (Game|Player|GetPlayerPawn 0)))
  (Variables|Default|SetAs%20BP%20Third%20Person%20Character _asbp_third_person_character)
  (Variables|Default|SetStartPosition (Transformation|GetActorLocation self))
  (bind _returnvalue (Actor|GetActorOfClass "/Game/Cutsence/Cutscene_Actors/Bosssss.Bosssss_C"))
  (Variables|Default|SetBoss _returnvalue)
  (bind _returnvalue_2 (Actor|GetActorOfClass "/Game/Blueprints_Code/Boss/BP_BossManager.BP_BossManager_C"))
  (Variables|Default|SetBossManager _returnvalue_2)
  (bind _returnvalue_3 (Actor|GetActorOfClass "/Game/Blueprints_Code/Hazards/BP_SplineHazards.BP_SplineHazards_C"))
  (bind _output_get (Variables|Default|SetBeginSpline _returnvalue_3))
  (Variables|Default|SetSpline%20To%20Follow _output_get)
  (EventDispatchers|BindEventtoSawonDestory (delegate Custom|ResetSaws)))

(event Collision|EventActorBeginOverlap
  (params (OtherActor :type Actor%20Object%20Reference)))

(event EventTick
  (params (DeltaSeconds :type Float%20%28single-precision%29)))

(fn ConstructionScript
  (|CallParentFunction))