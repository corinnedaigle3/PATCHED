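; BP_RightHand is a boss hand object that swings along the Spline1 path of the BP_swing actor in the level.
; On BeginPlay it finds that actor, aligns itself to its rotation with roll and yaw offsets, and scales the timeline rate from TimeToComplete.
; The timeline moves the hand from spline end to start.
; Custom events start the swing with a whoosh sound, stop it, or resume it.
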(event Custom|HandSwing2
  (bind _spline_to_follow (Variables|Default|GetSpline%20To%20Follow))
  (bind _spline1 (Variables|/Game/Blueprints_Code/Boss/Objects/BP_swing.BP_swing_C|GetSpline1 _spline_to_follow))
  (Audio|PlaySound2D "/Game/Audio/SFX/GameMech/SFX_Whoosh.SFX_Whoosh" 1.0 1.0 0.0 0 0)
  (bind _newtrack_0 (Timeline|Timeline PlayFromStart)
    (:Update
      (Transformation|SetActorLocation (Spline|GetLocationatDistanceAlongSpline _spline1 (Math|Float|Lerp (Spline|GetSplineLength _spline1) 0.0 _newtrack_0) "World") false false))))

(event Custom|StopSwing_RightHand
  (bind _spline_to_follow (Variables|Default|GetSpline%20To%20Follow))
  (bind _spline1 (Variables|/Game/Blueprints_Code/Boss/Objects/BP_swing.BP_swing_C|GetSpline1 _spline_to_follow))
  (bind _newtrack_0 (Timeline|Timeline Stop)
    (:Update
      (Transformation|SetActorLocation (Spline|GetLocationatDistanceAlongSpline _spline1 (Math|Float|Lerp (Spline|GetSplineLength _spline1) 0.0 _newtrack_0) "World") false false))))

(event Custom|ContinuePlay_RightHand
  (bind _spline_to_follow (Variables|Default|GetSpline%20To%20Follow))
  (bind _spline1 (Variables|/Game/Blueprints_Code/Boss/Objects/BP_swing.BP_swing_C|GetSpline1 _spline_to_follow))
  (bind _newtrack_0 (Timeline|Timeline Play)
    (:Update
      (Transformation|SetActorLocation (Spline|GetLocationatDistanceAlongSpline _spline1 (Math|Float|Lerp (Spline|GetSplineLength _spline1) 0.0 _newtrack_0) "World") false false))))

(event EventBeginPlay
  (bind _returnvalue (Actor|GetActorOfClass "/Game/Blueprints_Code/Boss/Objects/BP_swing.BP_swing_C"))
  (bind _output_get (Variables|Default|SetSpline%20To%20Follow _returnvalue))
  (Transformation|SetActorRotation self (Math|Rotator|MakeRotator (+ (.roll (Transformation|GetActorRotation _output_get)) -9e+01) (.pitch (Transformation|GetActorRotation _output_get)) (+ (.yaw (Transformation|GetActorRotation _output_get)) 9e+01)))
  (Components|Timeline|SetPlayRate (Variables|Default|GetTimeline) (/ 1.0 (Variables|Default|GetTime%20To%20Complete))))

(event Collision|EventActorBeginOverlap
  (params (OtherActor :type Actor%20Object%20Reference)))

(event EventTick
  (params (DeltaSeconds :type Float%20%28single-precision%29)))

(fn ConstructionScript)