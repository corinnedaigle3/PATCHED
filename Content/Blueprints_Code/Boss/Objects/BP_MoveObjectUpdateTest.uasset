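; Boss-fight box that lands as a projectile, can be pushed by a one-axis-at-a-time interact, and can stun the boss.
; While airborne, its bottom trigger launches the player away and costs a life; floor contact stops it.
; An armed player toggles pushing, and Tick interpolates the cube along forward or right from input.
; Boss contact counts a stun if overlapping a saw, otherwise physics releases the box as swung.
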(event OnComponentBeginOverlap(BoxInteract)
  (params (OverlappedComponent :type Primitive%20Component%20Object%20Reference) (OtherActor :type Actor%20Object%20Reference) (OtherComp :type Primitive%20Component%20Object%20Reference) (OtherBodyIndex :type Integer) (bFromSweep :type Boolean) (SweepResult :type Hit%20Result%20Structure%20%28by%20ref%29))
  ;[0.15 0.15 0.15 0.5] Overlapping
  ;;[0.15 0.15 0.15 0.5] Box Interact
  (Utilities|Casting|CastToBP_ThirdPersonCharacter OtherActor)
  (if (Variables|/Game/BP_ThirdPersonCharacter.BP_ThirdPersonCharacter_C|GetHasArm (Variables|Default|GetPatch))
    (if (not (Variables|Default|GetBeSwing))
      (Variables|Default|SetCanInteractCollision true)
      (Development|PrintString "Hv arm, didn't being swing, can interact"))
    (else
      (Development|PrintString "Cannot  interact bc no arm"))))

(event OnComponentEndOverlap(BoxInteract)
  (params (OverlappedComponent :type Primitive%20Component%20Object%20Reference) (OtherActor :type Actor%20Object%20Reference) (OtherComp :type Primitive%20Component%20Object%20Reference) (OtherBodyIndex :type Integer))
  (bind _patch (Variables|Default|GetPatch))
  ;[0.15 0.15 0.15 0.5] Overlapping
  ;;[0.15 0.15 0.15 0.5] Box Interact
  (Utilities|Casting|CastToBP_ThirdPersonCharacter OtherActor)
  (Variables|Default|SetCanInteractCollision false)
  (Variables|Default|SetInteractingWIthE false)
  (Physics|SetSimulatePhysics (Variables|Default|GetCube) false)
  (Variables|/Game/BP_ThirdPersonCharacter.BP_ThirdPersonCharacter_C|SetPlayerMoveState _patch "NewEnumerator6")
  (Default|UpdateMovementSpeed _patch)
  (Audio|Components|Audio|Stop (Variables|Default|GetPushSFX)))

(event OnComponentBeginOverlap(BoxBottom)
  (params (OverlappedComponent :type Primitive%20Component%20Object%20Reference) (OtherActor :type Actor%20Object%20Reference) (OtherComp :type Primitive%20Component%20Object%20Reference) (OtherBodyIndex :type Integer) (bFromSweep :type Boolean) (SweepResult :type Hit%20Result%20Structure%20%28by%20ref%29))
  (bind _returnvalue (Transformation|GetActorLocation))
  (bind _patch (Variables|Default|GetPatch))
  (bind _patch_2 (Variables|Default|GetPatch))
  (bind _projectilemovement (Variables|Default|GetProjectileMovement))
  (bind _returnvalue_2 (Transformation|GetActorLocation _patch_2))
  (bind _returnvalue_3 (- _returnvalue_2 _returnvalue))
  (bind _returnvalue_4 (< (.y _returnvalue_3) 0.0))
  ;[0.15 0.15 0.15 0.5] Overlapping
  ;;[0.15 0.15 0.15 0.5] Box Bottom
  (if (not (Variables|Default|GetStopped))
    (if (== OtherActor _patch)
      (Development|PrintString (Utilities|String|ToString(Vector) _returnvalue_2) true true "(R=1.000000,G=0.213229,B=0.000000,A=1.000000)" 1e+01)
      (if (< (.x _returnvalue_3) 0.0)
        (if _returnvalue_4
          (Character|LaunchCharacter _patch "-1500.000000,-1500.000000,-250.000000" false false)
          (else
            (Character|LaunchCharacter _patch "-1500.000000,1500.000000,-250.000000" false false)))
        (elif _returnvalue_4
          (Character|LaunchCharacter _patch "1500.000000,-1500.000000,-250.000000" false false)
          (Development|PrintString "3")
          (else
            (Character|LaunchCharacter _patch "1500.000000,1500.000000,-250.000000" false false))))
      (Components|Activation|SetActive (Variables|Default|GetBoxBottom) false false)
      (Utilities|FlowControl|DoOnce false
        (:Completed
          (Default|LoseALive (Variables|Default|GetPatch))
          (Variables|/Script/Engine.ProjectileMovementComponent|SetbShouldBounce _projectilemovement true)
          (Variables|/Script/Engine.ProjectileMovementComponent|SetProjectileGravityScale _projectilemovement 0.4))))))

(event OnComponentBeginOverlap(Box)
  (params (OverlappedComponent :type Primitive%20Component%20Object%20Reference) (OtherActor :type Actor%20Object%20Reference) (OtherComp :type Primitive%20Component%20Object%20Reference) (OtherBodyIndex :type Integer) (bFromSweep :type Boolean) (SweepResult :type Hit%20Result%20Structure%20%28by%20ref%29))
  (bind _cube (Variables|Default|GetCube))
  (bind _projectilemovement (Variables|Default|GetProjectileMovement))
  (bind _bossmanager (Variables|Default|GetBossManager))
  (bind _cube_2 (Variables|Default|GetCube))
  (bind _stopped (Variables|Default|GetStopped))
  ;[0.15 0.15 0.15 0.5] Overlapping
  ;;[0.15 0.15 0.15 0.5] Box
  (Utilities|FlowControl|Sequence
    (:then_0
      (if (Class|GameplayStatics|ObjectIsA OtherActor "/Game/Blueprints_Code/BP_Floor.BP_Floor_C")
        (CallFunction|DeactiveBoxes)
        (Variables|/Script/Engine.ProjectileMovementComponent|SetbShouldBounce _projectilemovement false)
        (Variables|/Script/Engine.ProjectileMovementComponent|SetProjectileGravityScale _projectilemovement 0.0)))
    (:then_1
      (if (and (Class|GameplayStatics|ObjectIsA OtherActor "/Game/Blueprints_Code/Boss/Objects/BP_Saw_Child.BP_Saw_Child_C") _stopped)
        (Variables|Default|SetwithSaw true)))
    (:then_2
      (if _stopped
        (if (Class|GameplayStatics|ObjectIsA OtherActor "/Game/Cutsence/Cutscene_Actors/Bosssss.Bosssss_C")
          (if (Variables|Default|GetwithSaw)
            (bind _result (Math|Integer|IncrementInt (Variables|/Game/Blueprints_Code/Boss/BP_BossManager.BP_BossManager_C|GetStunIndex _bossmanager))
              (:%20%20
                (Variables|/Game/Blueprints_Code/Boss/BP_BossManager.BP_BossManager_C|SetStunIndex _bossmanager _result)
                (if (== (Math|Integer|%(Integer) (Variables|/Game/Blueprints_Code/Boss/BP_BossManager.BP_BossManager_C|GetStunIndex (Variables|Default|GetBossManager)) 3) 0)
                  _
                  (else
                    (Development|PrintString (Utilities|String|ToString(Integer) (Math|Integer|%(Integer) (Variables|/Game/Blueprints_Code/Boss/BP_BossManager.BP_BossManager_C|GetStunIndex (Variables|Default|GetBossManager)) 3)) true true "(R=0.019819,G=0.000000,B=1.000000,A=1.000000)" 1e+01)
                    (Physics|SetSimulatePhysics (Variables|Default|GetCube) true)
                    (Class|PrimitiveComponent|SetConstraintMode _cube "None")
                    (Class|PrimitiveComponent|SetLinearDamping _cube 0.01)))
                (Default|CallBeStun (Variables|Default|GetBosssss))))
            (else
              (Variables|Default|SetBeSwing true)
              (Physics|SetSimulatePhysics (Variables|Default|GetCube) true)
              (Class|PrimitiveComponent|SetConstraintMode _cube_2 "None")
              (Class|PrimitiveComponent|SetLinearDamping _cube_2 0.01)
              (Utilities|FlowControl|Delay 2.0))))))))

(event OnComponentEndOverlap(Box)
  (params (OverlappedComponent :type Primitive%20Component%20Object%20Reference) (OtherActor :type Actor%20Object%20Reference) (OtherComp :type Primitive%20Component%20Object%20Reference) (OtherBodyIndex :type Integer))
  ;[0.15 0.15 0.15 0.5] Overlapping
  ;;[0.15 0.15 0.15 0.5] Box
  (Utilities|FlowControl|Sequence
    (:then_0
      (if (Class|GameplayStatics|ObjectIsA OtherActor "/Game/Blueprints_Code/Boss/Objects/BP_Saw_Child.BP_Saw_Child_C")
        (Variables|Default|SetwithSaw false)))))

(event Custom|StartInteract
  (bind _patch (Variables|Default|GetPatch))
  (if (Variables|Default|GetCanInteractCollision)
    (Variables|Default|SetInteractingWIthE (not (Variables|Default|GetInteractingWIthE)))
    (if true
      ;[0.15 0.15 0.15 0.5] Update movment
      (Variables|/Game/BP_ThirdPersonCharacter.BP_ThirdPersonCharacter_C|SetPlayerMoveState _patch "NewEnumerator4")
      (Default|UpdateMovementSpeed _patch)
      (Audio|Components|Audio|Play (Variables|Default|GetPushSFX) 0.0)
      (else
        (Audio|Components|Audio|Stop (Variables|Default|GetPushSFX))))))

(event Custom|ChangeVelocity
  (params (Velocity :type Vector))
  (Variables|/Script/Engine.MovementComponent|SetVelocity (Variables|Default|GetProjectileMovement) Velocity)
  (Variables|Default|SetStopped false)
  (Audio|Components|Audio|Stop (Variables|Default|GetPushSFX)))

(event Custom|DeactiveBoxes
  (Variables|/Script/Engine.MovementComponent|SetVelocity (Variables|Default|GetProjectileMovement) "0, 0, 0")
  (Collision|SetCollisionEnabled (Variables|Default|GetBox) "QueryAndPhysics")
  (Variables|Default|SetStopped true)
  (Audio|Components|Audio|Stop (Variables|Default|GetPushSFX)))

(event Custom|Reset
  (bind _cube (Variables|Default|GetCube))
  (Class|PrimitiveComponent|SetConstraintMode _cube "SixDOF")
  (Class|PrimitiveComponent|SetLinearDamping _cube 1e+03)
  (Physics|SetSimulatePhysics (Variables|Default|GetCube) false)
  (Transformation|SetActorRotation "0.000000,90.000000,0.000000")
  (Variables|Default|SetwithSaw false)
  (Variables|Default|SetStopped false)
  (Variables|Default|SetBeSwing false)
  (Components|Activation|SetActive (Variables|Default|GetBoxBottom) true false)
  (CallFunction|ResetBoxBottomDamage)
  (Audio|Components|Audio|Stop (Variables|Default|GetPushSFX)))

(event Custom|ResetBoxBottomDamage
  (bind _projectilemovement (Variables|Default|GetProjectileMovement))
  ;[0.15 0.15 0.15 0.5] Overlapping
  ;;[0.15 0.15 0.15 0.5] Box Bottom
  (Utilities|FlowControl|DoOnce false) ; enters at Reset
)

(event EventBeginPlay
  (bind _asbp_third_person_character (Utilities|Casting|CastToBP_ThirdPersonCharacter (Game|Player|GetPlayerPawn 0)))
  (Variables|Default|SetPatch _asbp_third_person_character)
  (bind _returnvalue (Actor|GetActorOfClass "/Game/Blueprints_Code/Boss/BP_BossManager.BP_BossManager_C"))
  (Variables|Default|SetBossManager _returnvalue)
  (bind _returnvalue_2 (Actor|GetActorOfClass "/Game/Cutsence/Cutscene_Actors/Bosssss.Bosssss_C"))
  (Variables|Default|SetBosssss _returnvalue_2)
  (bind _returnvalue_3 (AddComponent|AddAudioComponent false))
  (Variables|Default|SetPushSFX _returnvalue_3))

(event EventTick
  (params (DeltaSeconds :type Float%20%28single-precision%29))
  (bind _patch (Variables|Default|GetPatch))
  (bind _patch_2 (Variables|Default|GetPatch))
  (bind _action_value_x (Variables|/Game/BP_ThirdPersonCharacter.BP_ThirdPersonCharacter_C|GetAction%20Value%20X _patch))
  (bind _action_value_y (Variables|/Game/BP_ThirdPersonCharacter.BP_ThirdPersonCharacter_C|GetAction%20Value%20Y _patch))
  (bind _action_value_y_2 (Variables|/Game/BP_ThirdPersonCharacter.BP_ThirdPersonCharacter_C|GetAction%20Value%20Y _patch_2))
  (bind _action_value_x_2 (Variables|/Game/BP_ThirdPersonCharacter.BP_ThirdPersonCharacter_C|GetAction%20Value%20X _patch_2))
  (bind _returnvalue (>= _action_value_y_2 0.1))
  (bind _returnvalue_2 (>= _action_value_x 0.1))
  (if (Variables|/Game/BP_ThirdPersonCharacter.BP_ThirdPersonCharacter_C|GetHasArm (Variables|Default|GetPatch))
    (if (Variables|Default|GetCanInteractCollision)
      (if (Variables|Default|GetInteractingWIthE)
        (Utilities|FlowControl|Sequence
          (:then_0
            (if (not (== _action_value_y_2 0.0))
              (if (and _returnvalue (== _action_value_x_2 0.0))
                (if _returnvalue
                  (Utilities|Speed/Direction true -2e+01))
                (elif (and (== _action_value_x_2 0.0) (< _action_value_y_2 0.0))
                  (Development|PrintString "back" true true "(R=1.000000,G=0.232026,B=0.000000,A=1.000000)")
                  (Utilities|Speed/Direction true 2e+01)))))
          (:then_1
            (if (not (== _action_value_x_2 0.0))
              (if (and _returnvalue_2 (== _action_value_y 0.0))
                (if _returnvalue_2
                  (Utilities|Speed/Direction false 2e+01))
                (elif (and (== _action_value_y 0.0) (< _action_value_x 0.0))
                  (Utilities|Speed/Direction false -2e+01)))))
          (:then_2
            ;[0.15 0.15 0.15 0.5] Stop moving
            (if (and (== _action_value_x 0.0) (== _action_value_y 0.0))
              (Utilities|FlowControl|DoOnce false
                (:Completed
                  (Audio|Components|Audio|Stop (Variables|Default|GetPushSFX)))))))))))

(fn ConstructionScript)

(fn Interact
  (params (Character :type BP%20Third%20Person%20Character%20Object%20Reference))
  (bind _patch (Variables|Default|GetPatch))
  (if (not (Variables|/Game/BP_ThirdPersonCharacter.BP_ThirdPersonCharacter_C|GetHasItemInHand Character))
    (if (Variables|/Game/BP_ThirdPersonCharacter.BP_ThirdPersonCharacter_C|GetHasArm Character)
      (if (Variables|Default|GetInteractingWIthE)
        (Variables|Default|SetInteractingWIthE false)
        (Variables|/Game/BP_ThirdPersonCharacter.BP_ThirdPersonCharacter_C|SetPlayerMoveState _patch "NewEnumerator6")
        (Default|UpdateMovementSpeed _patch)
        (Audio|Components|Audio|Stop (Variables|Default|GetPushSFX))
        (else
          (CallFunction|StartInteract)
          (return false)))
      (else
        (Development|PrintString "no arm")))))