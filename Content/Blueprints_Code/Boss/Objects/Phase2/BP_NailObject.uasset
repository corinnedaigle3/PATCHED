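; BP_NailObject is a nail hazard for boss phase 2 that can strike Patch while falling.
; Its Box overlap calls CallGroundHit on contact with BP_Floor.
; Touching Patch while IsFalling launches the character using LaunchDirection, then a DoOnce removes a life after a short delay, once per nail.
; In LaunchDirection, the horizontal push-away calculation from LaunchForce is left unconnected.
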(event OnComponentBeginOverlap(Box)
  (params (OverlappedComponent :type Primitive%20Component%20Object%20Reference) (OtherActor :type Actor%20Object%20Reference) (OtherComp :type Primitive%20Component%20Object%20Reference) (OtherBodyIndex :type Integer) (bFromSweep :type Boolean) (SweepResult :type Hit%20Result%20Structure%20%28by%20ref%29))
  (if (Class|GameplayStatics|ObjectIsA OtherActor "/Game/Blueprints_Code/BP_Floor.BP_Floor_C")
    (Default|CallGroundHit)
    (elif (and (== OtherActor (Variables|Default|GetPatch)) (Variables|Default|GetisFalling))
      (Character|LaunchCharacter (Variables|Default|GetPatch) (Utilities|LaunchDirection) false false)
      (Utilities|FlowControl|DoOnce false
        (:Completed
          (Utilities|FlowControl|Delay 0.5)
          (Default|LoseALive (Variables|Default|GetPatch)))))))

(fn ConstructionScript)