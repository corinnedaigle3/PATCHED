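; BP_ObjectsPool pre-spawns and holds the boss fight's objects: movable boxes, saws and a left and right hand.
; On BeginPlay it fills three arrays, scattering boxes randomly around its owner and parking saws far below it.
; Each box's destroy event is bound to ReturnPool, which resets and re-scatters that box instead of respawning it.
; DestoryPool destroys the pooled actors.
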(event Custom|ReturnPool
  (params (MoveableBox :type BP%20Move%20Object%20Update%20Object%20Reference))
  (bind _returnvalue (Components|GetOwner))
  (bind _returnvalue_2 (Transformation|GetActorLocation _returnvalue))
  (Default|Reset MoveableBox)
  (Transformation|SetActorLocation MoveableBox (Math|Vector|MakeVector (+ (.x _returnvalue_2) (Math|Random|RandomFloatinRange -2e+02 2e+02)) (+ (.y _returnvalue_2) (Math|Random|RandomFloatinRange -3.5e+02 3.5e+02)) (.z _returnvalue_2)) false false))

(event Custom|DestoryPool
  (Utilities|FlowControl|Sequence
    (:then_0
      (for _index (range 0 (Variables|Default|GetAmountOfSaw))
        (Actor|DestroyActor (Utilities|Array|Get(acopy) (Variables|Default|GetSawPool) _index))))
    (:then_1
      (for _index_2 (range 0 (Variables|Default|GetAmountOfBoxes))
        (Actor|DestroyActor (Utilities|Array|Get(acopy) (Variables|Default|GetBoxesPool) _index_2))))
    (:then_2
      (for _index_3 (range 0 1)
        (Actor|DestroyActor (Utilities|Array|Get(acopy) (Variables|Default|GetHandsPool) _index_3))))))

(event EventBeginPlay
  (bind _returnvalue (Components|GetOwner))
  (bind _returnvalue_2 (Components|GetOwner))
  (bind _handspool (Variables|Default|GetHandsPool))
  (bind _returnvalue_3 (Transformation|GetActorLocation _returnvalue_2))
  (bind _returnvalue_4 (Transformation|GetActorLocation _returnvalue))
  (Utilities|FlowControl|Sequence
    (:then_0
      (for _index (range 0 (Variables|Default|GetAmountOfBoxes))
        (bind _returnvalue_5 (Game|SpawnActorfromClass "/Game/Blueprints_Code/Boss/Objects/BP_MoveObjectUpdate.BP_MoveObjectUpdate_C" (Math|Transform|MakeTransform (Math|Vector|MakeVector (+ (.x _returnvalue_3) (Math|Random|RandomFloatinRange -2e+02 2e+02)) (+ (.y _returnvalue_3) (Math|Random|RandomFloatinRange -3.5e+02 3.5e+02)) (.z _returnvalue_3)) (Transformation|GetActorRotation _returnvalue_2) "1.000000,1.000000,1.000000") "AlwaysSpawn" "MultiplyWithRoot" 0 0))
        (Variables|Default|SetMoveableObject _returnvalue_5)
        (Utilities|Array|Add (Variables|Default|GetBoxesPool) (Variables|Default|GetMoveableObject))
        (Utilities|IsValid (Variables|Default|GetMoveableObject)
          (:Is%20Valid
            (EventDispatchers|BindEventtoOnBoxDestory (Variables|Default|GetMoveableObject) (delegate Custom|ReturnPool))))))
    (:then_1
      (for _index_2 (range 0 (Variables|Default|GetAmountOfSaw))
        (bind _returnvalue_6 (Game|SpawnActorfromClass "/Game/Blueprints_Code/Boss/Objects/BP_Saw_Child.BP_Saw_Child_C" (Math|Transform|MakeTransform (Math|Vector|MakeVector (.x _returnvalue_4) (.y _returnvalue_4) (- (.z _returnvalue_4) 1e+04)) "0, 0, 0" "1.000000,1.000000,1.000000") "AlwaysSpawn" "MultiplyWithRoot" 0 0))
        (Variables|Default|SetSawObject _returnvalue_6)
        (Utilities|Array|Add (Variables|Default|GetSawPool) (Variables|Default|GetSawObject))))
    (:then_2
      (bind _returnvalue_7 (Game|SpawnActorfromClass "/Game/Blueprints_Code/Boss/Objects/BP_LeftHand.BP_LeftHand_C" (Math|Transform|MakeTransform (Math|Vector|MakeVector 0.0 0.0 0.0) "0, 0, 0" "1.000000,1.000000,1.000000") "AlwaysSpawn" "MultiplyWithRoot" 0 0))
      (bind _output_get (Variables|Default|SetLeftHand _returnvalue_7))
      (Utilities|Array|Add (Variables|Default|GetHandsPool) _output_get)
      (bind _returnvalue_8 (Game|SpawnActorfromClass "/Game/Blueprints_Code/Boss/Objects/BP_RightHand.BP_RightHand_C" (Math|Transform|MakeTransform (Math|Vector|MakeVector 0.0 0.0 0.0) "0, 0, 0" "1.000000,1.000000,1.000000") "AlwaysSpawn" "MultiplyWithRoot" 0 0))
      (bind _output_get_2 (Variables|Default|SetRightHand _returnvalue_8))
      (Utilities|Array|Add _handspool _output_get_2)
      (Development|PrintString (Utilities|String|Append "Hands Index: " (Utilities|String|ToString(Integer) (Utilities|Array|LastIndex _handspool))) true true "(R=1.000000,G=0.730847,B=0.000000,A=1.000000)"))))