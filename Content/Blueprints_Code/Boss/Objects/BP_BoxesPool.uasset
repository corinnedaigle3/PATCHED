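; Box pool for the boss objects that pre-spawns movable boxes around its owner and recycles them.
; On BeginPlay it spawns BP_MoveObjectUpdate actors at random X/Y offsets from the owner, stores them in BoxesPool and binds each one's OnBoxDestory event to ReturnPool.
; ReturnPool teleports that box back to the owner's position with only a random X offset, so no new actor is spawned.
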(event Custom|ReturnPool
  (params (MoveableBox :type BP%20Move%20Object%20Update%20Object%20Reference))
  (bind _returnvalue (Components|GetOwner))
  (bind _returnvalue_2 (Transformation|GetActorLocation _returnvalue))
  (Transformation|SetActorLocation MoveableBox (Math|Vector|MakeVector (+ (.x _returnvalue_2) (Math|Random|RandomFloatinRange -1.5e+03 1.5e+03)) (.y _returnvalue_2) (.z _returnvalue_2)) false false))

(event EventBeginPlay
  (bind _returnvalue (Components|GetOwner))
  (bind _returnvalue_2 (Transformation|GetActorLocation _returnvalue))
  (Utilities|FlowControl|Sequence
    (:then_0
      (for _index (range 0 (Variables|Default|GetAmountOfBoxes))
        (bind _returnvalue_3 (Game|SpawnActorfromClass "/Game/Blueprints_Code/Boss/Objects/BP_MoveObjectUpdate.BP_MoveObjectUpdate_C" (Math|Transform|MakeTransform (Math|Vector|MakeVector (+ (.x _returnvalue_2) (Math|Random|RandomFloatinRange -1.5e+03 1.5e+03)) (+ (.y _returnvalue_2) (Math|Random|RandomFloatinRange -2e+02 2e+02)) (.z _returnvalue_2)) (Transformation|GetActorRotation _returnvalue) "1.000000,1.000000,1.000000") "Undefined" "MultiplyWithRoot" 0 0))
        (Variables|Default|SetMoveableObject _returnvalue_3)
        (Utilities|Array|Add (Variables|Default|GetBoxesPool) (Variables|Default|GetMoveableObject))
        (Utilities|IsValid (Variables|Default|GetMoveableObject)
          (:Is%20Valid
            (EventDispatchers|BindEventtoOnBoxDestory (Variables|Default|GetMoveableObject) (delegate Custom|ReturnPool))))))))