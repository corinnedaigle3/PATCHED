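; Boss left hand that swings a mallet along a BP_swing spline via timeline, driving its anim blueprint and costing the player a life on hit.
; Overlapping a saw-carrying move object counts a stun, which halts the swing and detaches and lowers the mallet until the swing resumes.
; Saw hits on orientation-matched colliders, gated by Check, slide the mallet away, then raise the hand and end phase 1.
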(event OnComponentBeginOverlap(VerticalCollider)
  (params (OverlappedComponent :type Primitive%20Component%20Object%20Reference) (OtherActor :type Actor%20Object%20Reference) (OtherComp :type Primitive%20Component%20Object%20Reference) (OtherBodyIndex :type Integer) (bFromSweep :type Boolean) (SweepResult :type Hit%20Result%20Structure%20%28by%20ref%29))
  (bind _asbp_saw_child (Utilities|Casting|CastToBP_Saw_Child OtherActor))
  (if (Variables|/Game/Blueprints_Code/Boss/Objects/BP_Saw_Child.BP_Saw_Child_C|GetVertical _asbp_saw_child)
    (if (Utilities|Check)
      (Utilities|FlowControl|DoOnce false
        (:Completed
          (CallFunction|DestoryMalletVertcial))))))

(event OnComponentBeginOverlap(Horizontal2)
  (params (OverlappedComponent :type Primitive%20Component%20Object%20Reference) (OtherActor :type Actor%20Object%20Reference) (OtherComp :type Primitive%20Component%20Object%20Reference) (OtherBodyIndex :type Integer) (bFromSweep :type Boolean) (SweepResult :type Hit%20Result%20Structure%20%28by%20ref%29))
  (if (and (Class|GameplayStatics|ObjectIsA OtherActor "/Game/BP_ThirdPersonCharacter.BP_ThirdPersonCharacter_C") (not (Variables|/Game/Blueprints_Code/Boss/Objects/BP_ObjectManager.BP_ObjectManager_C|GetBossStunned (Variables|Default|GetObjectManager))))
    (Utilities|FlowControl|DoOnce false
      (:Completed
        (Default|LoseALive (Variables|Default|GetAs%20BP%20Third%20Person%20Character))))
    (else
      (bind _asbp_saw_child (Utilities|Casting|CastToBP_Saw_Child OtherActor))
      (if (not (Variables|/Game/Blueprints_Code/Boss/Objects/BP_Saw_Child.BP_Saw_Child_C|GetVertical _asbp_saw_child))
        (if (Utilities|Check)
          (Utilities|FlowControl|DoOnce false
            (:Completed
              (CallFunction|DestoryMalletHorizontal))))))))

(event OnComponentBeginOverlap(Horizontal3)
  (params (OverlappedComponent :type Primitive%20Component%20Object%20Reference) (OtherActor :type Actor%20Object%20Reference) (OtherComp :type Primitive%20Component%20Object%20Reference) (OtherBodyIndex :type Integer) (bFromSweep :type Boolean) (SweepResult :type Hit%20Result%20Structure%20%28by%20ref%29))
  (bind _asbp_saw_child (Utilities|Casting|CastToBP_Saw_Child OtherActor))
  (if (not (Variables|/Game/Blueprints_Code/Boss/Objects/BP_Saw_Child.BP_Saw_Child_C|GetVertical _asbp_saw_child))
    (if (Utilities|Check)
      (Utilities|FlowControl|DoOnce false
        (:Completed
          (CallFunction|DestoryMalletHorizontal))))))

(event Custom|MalletDrop
  (params (MalletLocation :type Vector))
  (bind (_x _y _z) (Math|Vector|BreakVector MalletLocation))
  ;[0.15 0.15 0.15 0.5] Mallet Tmeline for leave hand
  (Components|Timeline|SetPlayRate (Variables|Default|GetTimeline_0) (/ 1.0 (Variables|Default|GetDropDownTime)))
  (bind _newtrack_0 (Timeline|Timeline_0 PlayFromStart)
    (:Update
      (Transformation|SetWorldLocation (Variables|Default|GetPATCHED_DollMaker_Mallet) (Math|Vector|Lerp(Vector) MalletLocation (Math|Vector|MakeVector _x _y (- _z 5e+01)) _newtrack_0) false false))
    (:Finished
      (if (Variables|Default|GetReverse)
        (CallFunction|LHandContinue)))))

(event Custom|StopSwing_LeftHand
  (bind _spline_to_follow (Variables|Default|GetSpline%20To%20Follow))
  (bind _spline1 (Variables|/Game/Blueprints_Code/Boss/Objects/BP_swing.BP_swing_C|GetSpline1 _spline_to_follow))
  ;[0.15 0.15 0.15 0.5] Swing Timeline
  (bind _newtrack_0 (Timeline|Timeline Stop)
    (:Update
      (Transformation|SetActorLocation (Spline|GetLocationatDistanceAlongSpline _spline1 (Math|Float|Lerp 0.0 (Spline|GetSplineLength _spline1) _newtrack_0) "World") false false))
    (:Finished
      (CallFunction|BeStunTime)
      (Variables|/Game/Blueprints_Animations/ABP_RHand.ABP_RHand_C|SetFinishSwing (Variables|Default|GetABP_Hand) true)
      (Variables|/Game/Blueprints_Code/Boss/Objects/BP_MoveObjectUpdate.BP_MoveObjectUpdate_C|SetisSwing (Variables|Default|GetMoveObject) false)
      (Default|CallFinishAttack))))

(event Custom|DestoryMallet_Horizontal
  (bind _patched_dollmaker_mallet (Variables|Default|GetPATCHED_DollMaker_Mallet))
  (bind _returnvalue (Transformation|GetWorldLocation _patched_dollmaker_mallet))
  ;[0.15 0.15 0.15 0.5] Mallet Fly Away Timeline
  (bind _newtrack_0 (Timeline|Timeline_1 PlayFromStart)
    (:Update
      (Transformation|SetWorldLocation _patched_dollmaker_mallet (Math|Vector|Lerp(Vector) (Transformation|GetWorldLocation _patched_dollmaker_mallet) (Math|Vector|MakeVector (.x _returnvalue) (- (.y _returnvalue) 1e+02) (.z _returnvalue)) _newtrack_0) false false))
    (:Finished
      (Default|AnimLHandGoUp (Variables|Default|GetBossManger))
      (Default|CallPhase1End (Variables|Default|GetObjectManager)))))

(event Custom|BeStunTime
  (bind _bossmanger (Variables|Default|GetBossManger))
  (Utilities|FlowControl|DoOnce false) ; enters at Reset
)

(event Custom|LHand_Continue
  ;[0.15 0.15 0.15 0.5] Continue
  (Variables|/Game/Blueprints_Animations/ABP_RHand.ABP_RHand_C|SetisStun (Variables|Default|GetABP_Hand) false)
  (CallFunction|ContinuePlayLeftHand)
  (Transformation|AttachComponentToComponent (Variables|Default|GetPATCHED_DollMaker_Mallet) (Variables|Default|GetPATCHED_DollMaker_LHand) "Socket_JNT" "SnapToTarget" "SnapToTarget" "KeepWorld" true)
  (Components|Animation|PlayAnimation (Variables|Default|GetPATCHED_DollMaker_LHand) "/Game/Animations/DollMaker_Anims/PATCHED_DollMaker_MalletSwing_Freeze.PATCHED_DollMaker_MalletSwing_Freeze" false)
  (CallFunction|ContinuePlayLeftHand))

(event Custom|ContinuePlay_LeftHand
  (bind _spline_to_follow (Variables|Default|GetSpline%20To%20Follow))
  (bind _spline1 (Variables|/Game/Blueprints_Code/Boss/Objects/BP_swing.BP_swing_C|GetSpline1 _spline_to_follow))
  ;[0.15 0.15 0.15 0.5] Swing Timeline
  (bind _newtrack_0 (Timeline|Timeline Play)
    (:Update
      (Transformation|SetActorLocation (Spline|GetLocationatDistanceAlongSpline _spline1 (Math|Float|Lerp 0.0 (Spline|GetSplineLength _spline1) _newtrack_0) "World") false false))
    (:Finished
      (CallFunction|BeStunTime)
      (Variables|/Game/Blueprints_Animations/ABP_RHand.ABP_RHand_C|SetFinishSwing (Variables|Default|GetABP_Hand) true)
      (Variables|/Game/Blueprints_Code/Boss/Objects/BP_MoveObjectUpdate.BP_MoveObjectUpdate_C|SetisSwing (Variables|Default|GetMoveObject) false)
      (Default|CallFinishAttack))))

(event Custom|OnActorBeginOverlap_Event
  (params (OverlappedActor :type Actor%20Object%20Reference) (OtherActor :type Actor%20Object%20Reference))
  (bind _bossmanger (Variables|Default|GetBossManger))
  (bind _asbp_move_object_update (Utilities|Casting|CastToBP_MoveObjectUpdate OtherActor))
  (if (Variables|/Game/Blueprints_Code/Boss/Objects/BP_MoveObjectUpdate.BP_MoveObjectUpdate_C|GetwithSaw _asbp_move_object_update)
    (Utilities|FlowControl|DoOnce false
      (:Completed
        (Variables|/Game/Blueprints_Code/Boss/BP_BossManager.BP_BossManager_C|SetStunIndex _bossmanger (+ (Variables|/Game/Blueprints_Code/Boss/BP_BossManager.BP_BossManager_C|GetStunIndex _bossmanger) 1))
        (Development|PrintString "BossBeingSTUN")
        (Default|CallBossbeStun (Variables|Default|GetObjectManager))))))

(event Custom|HandSwing
  (bind _spline_to_follow (Variables|Default|GetSpline%20To%20Follow))
  (bind _spline1 (Variables|/Game/Blueprints_Code/Boss/Objects/BP_swing.BP_swing_C|GetSpline1 _spline_to_follow))
  ;[0.15 0.15 0.15 0.5] Swing Timeline
  (Variables|/Game/Blueprints_Code/Boss/Objects/BP_MoveObjectUpdate.BP_MoveObjectUpdate_C|SetisSwing (Variables|Default|GetMoveObject) true)
  (Variables|/Game/Blueprints_Animations/ABP_RHand.ABP_RHand_C|SetFinishSwing (Variables|Default|GetABP_Hand) false)
  (CallFunction|ResetDamage)
  (Audio|PlaySound2D "/Game/Audio/SFX/GameMech/SFX_Whoosh1.SFX_Whoosh1" 1.0 1.0 0.0 0 0)
  (bind _newtrack_0 (Timeline|Timeline PlayFromStart)
    (:Update
      (Transformation|SetActorLocation (Spline|GetLocationatDistanceAlongSpline _spline1 (Math|Float|Lerp 0.0 (Spline|GetSplineLength _spline1) _newtrack_0) "World") false false))
    (:Finished
      (CallFunction|BeStunTime)
      (Variables|/Game/Blueprints_Animations/ABP_RHand.ABP_RHand_C|SetFinishSwing (Variables|Default|GetABP_Hand) true)
      (Variables|/Game/Blueprints_Code/Boss/Objects/BP_MoveObjectUpdate.BP_MoveObjectUpdate_C|SetisSwing (Variables|Default|GetMoveObject) false)
      (Default|CallFinishAttack))))

(event Custom|ResetDamage
  (Utilities|FlowControl|DoOnce false) ; enters at Reset
)

(event Custom|MalletBacktoHand
  ;[0.15 0.15 0.15 0.5] Mallet Tmeline for leave hand
  (Variables|Default|SetReverse true)
  (bind _newtrack_0 (Timeline|Timeline_0 Reverse)
    (:Update
      (Transformation|SetWorldLocation (Variables|Default|GetPATCHED_DollMaker_Mallet) (Math|Vector|Lerp(Vector) (stale Custom|MalletDrop MalletLocation) (Math|Vector|MakeVector (.X (Math|Vector|BreakVector (stale Custom|MalletDrop MalletLocation))) (.Y (Math|Vector|BreakVector (stale Custom|MalletDrop MalletLocation))) (- (.Z (Math|Vector|BreakVector (stale Custom|MalletDrop MalletLocation))) 5e+01)) _newtrack_0) false false))
    (:Finished
      (if (Variables|Default|GetReverse)
        (CallFunction|LHandContinue)))))

(event Custom|LHand_BeStun
  ;[0.15 0.15 0.15 0.5] Be Stun
  (Variables|/Game/Blueprints_Animations/ABP_RHand.ABP_RHand_C|SetisStun (Variables|Default|GetABP_Hand) true)
  (CallFunction|StopSwingLeftHand)
  (Transformation|DetachFromComponent (Variables|Default|GetPATCHED_DollMaker_Mallet) "KeepWorld" "KeepWorld" "KeepWorld" true)
  (CallFunction|MalletDrop (Transformation|GetWorldLocation (Variables|Default|GetPATCHED_DollMaker_Mallet))))

(event Custom|DestoryMallet_Vertcial
  (bind _patched_dollmaker_mallet (Variables|Default|GetPATCHED_DollMaker_Mallet))
  (bind _returnvalue (Transformation|GetWorldLocation _patched_dollmaker_mallet))
  ;[0.15 0.15 0.15 0.5] Mallet Fly Away Timeline
  (bind _newtrack_0 (Timeline|Timeline_2 PlayFromStart)
    (:Update
      (Transformation|SetWorldLocation _patched_dollmaker_mallet (Math|Vector|Lerp(Vector) (Transformation|GetWorldLocation _patched_dollmaker_mallet) (Math|Vector|MakeVector (- (.x _returnvalue) 1e+02) (.y _returnvalue) (.z _returnvalue)) _newtrack_0) false false))
    (:Finished
      (Default|AnimLHandGoUp (Variables|Default|GetBossManger))
      (Default|CallPhase1End (Variables|Default|GetObjectManager)))))

(event EventBeginPlay
  (bind _returnvalue (Actor|GetActorOfClass "/Game/Blueprints_Code/Boss/Objects/BP_MoveObjectUpdate.BP_MoveObjectUpdate_C"))
  (Variables|Default|SetMoveObject _returnvalue)
  (bind _returnvalue_2 (Actor|GetActorOfClass "/Game/Blueprints_Code/Boss/BP_BossManager.BP_BossManager_C"))
  (Variables|Default|SetBossManger _returnvalue_2)
  (bind _returnvalue_3 (Actor|GetActorOfClass "/Game/Blueprints_Code/Boss/Objects/BP_ObjectManager.BP_ObjectManager_C"))
  (Variables|Default|SetObjectManager _returnvalue_3)
  (bind _returnvalue_4 (Actor|GetActorOfClass "/Game/Blueprints_Code/Boss/Objects/BP_Saw_Child.BP_Saw_Child_C"))
  (Variables|Default|SetSaw _returnvalue_4)
  (bind _asbp_third_person_character (Utilities|Casting|CastToBP_ThirdPersonCharacter (Game|Player|GetPlayerPawn 0)))
  (Variables|Default|SetAs%20BP%20Third%20Person%20Character _asbp_third_person_character)
  (bind _returnvalue_5 (Actor|GetActorOfClass "/Game/Blueprints_Code/Boss/Objects/BP_swing.BP_swing_C"))
  (bind _output_get (Variables|Default|SetSpline%20To%20Follow _returnvalue_5))
  (Components|Timeline|SetPlayRate (Variables|Default|GetTimeline) (/ 1.0 (Variables|Default|GetTime%20To%20Complete)))
  (EventDispatchers|BindEventtoOnActorBeginOverlap (delegate Custom|OnActorBeginOverlap_Event))
  (bind _asabp_rhand (Utilities|Casting|CastToABP_RHand (Components|SkeletalMesh|GetAnimInstance (Variables|Default|GetPATCHED_DollMaker_LHand))))
  (bind _output_get_2 (Variables|Default|SetABP_Hand _asabp_rhand))
  (Variables|/Game/Blueprints_Animations/ABP_RHand.ABP_RHand_C|SetisSwing _output_get_2 true))

(fn ConstructionScript)