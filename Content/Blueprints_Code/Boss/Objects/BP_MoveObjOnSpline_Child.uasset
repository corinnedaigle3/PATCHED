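; Boss-fight box, derived from the move-on-spline object, that can be dropped via projectile velocity and tracks player interaction range.
; BeginPlay spawns its own BP_SplineHazards as the spline to follow.
; On hitting a Floor-tagged actor, it moves that spline beside itself, stops, and fires OnBoxesDestory after ten seconds.
; Player overlap toggles interaction flags, and Tick still prints the display name for debugging.
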(event OnComponentBeginOverlap(BoxCollider)
  (params (OverlappedComponent :type Primitive%20Component%20Object%20Reference) (OtherActor :type Actor%20Object%20Reference) (OtherComp :type Primitive%20Component%20Object%20Reference) (OtherBodyIndex :type Integer) (bFromSweep :type Boolean) (SweepResult :type Hit%20Result%20Structure%20%28by%20ref%29))
  (Utilities|Casting|CastToBP_ThirdPersonCharacter OtherActor)
  (Variables|Default|SetCanInteractCollision true))

(event OnComponentEndOverlap(BoxCollider)
  (params (OverlappedComponent :type Primitive%20Component%20Object%20Reference) (OtherActor :type Actor%20Object%20Reference) (OtherComp :type Primitive%20Component%20Object%20Reference) (OtherBodyIndex :type Integer))
  (Utilities|Casting|CastToBP_ThirdPersonCharacter OtherActor)
  (CallFunction|Walking)
  (Variables|Default|SetCanInteractCollision false)
  (Variables|Default|SetCanInteractE false))

(event OnComponentBeginOverlap(BossBox)
  (params (OverlappedComponent :type Primitive%20Component%20Object%20Reference) (OtherActor :type Actor%20Object%20Reference) (OtherComp :type Primitive%20Component%20Object%20Reference) (OtherBodyIndex :type Integer) (bFromSweep :type Boolean) (SweepResult :type Hit%20Result%20Structure%20%28by%20ref%29))
  (bind _self self)
  (bind _returnvalue (Transformation|GetActorLocation _self))
  (if (Actor|ActorHasTag OtherActor "Floor")
    (Transformation|SetActorLocation (Variables|Default|GetSpline%20To%20Follow) (Math|Vector|MakeVector (- (.x _returnvalue) 2e+02) (.y _returnvalue) (.z _returnvalue)) false false)
    (CallFunction|DeactiveBox)
    (Utilities|FlowControl|Delay 1e+01)
    (Default|CallOnBoxesDestory self)))

(event Custom|DeactiveBox
  (Variables|/Script/Engine.MovementComponent|SetVelocity (Variables|Default|GetProjectileMovement) "0, 0, 0")
  (Collision|SetCollisionEnabled (Variables|Default|GetBossBox) "QueryAndPhysics"))

(event Custom|DropBox
  (params (Velocity :type Vector))
  (Variables|/Script/Engine.MovementComponent|SetVelocity (Variables|Default|GetProjectileMovement) Velocity))

(event EventBeginPlay
  (bind _self self)
  (bind _returnvalue (Transformation|GetActorLocation _self))
  (|CallParentFunction)
  (bind _returnvalue_2 (Game|SpawnActorfromClass "/Game/Blueprints_Code/Hazards/BP_SplineHazards.BP_SplineHazards_C" (Math|Transform|MakeTransform (Math|Vector|MakeVector (- (.x _returnvalue) 2e+02) (.y _returnvalue) (.z _returnvalue)) "0, 0, 0" "4.000000,1.000000,1.000000") "Undefined" "MultiplyWithRoot" 0 0))
  (bind _output_get (Variables|Default|SetHazard1 _returnvalue_2))
  (Variables|Default|SetSpline%20To%20Follow _output_get))

(event Collision|EventActorBeginOverlap
  (params (OtherActor :type Actor%20Object%20Reference)))

(event EventTick
  (params (DeltaSeconds :type Float%20%28single-precision%29))
  (|CallParentFunction DeltaSeconds)
  (Development|PrintString (Utilities|GetDisplayName 0)))

(fn ConstructionScript
  (|CallParentFunction))