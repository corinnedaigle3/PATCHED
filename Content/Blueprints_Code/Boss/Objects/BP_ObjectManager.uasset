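; BP_ObjectManager runs the first-phase hazards of a boss fight.
; Looping, staggered timers recycle and launch pooled boxes, send pooled saws along shuffled BP_SplineHazards splines, and swing the left or right boss hand.
; On every third boss stun it pauses all timers and the active hand for ten seconds, then resumes them.
; When phase one ends, it destroys the pool and advances BP_BossManager to the next phase.
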(event Custom|Stun
  (bind _bossmanager (Variables|Default|GetBossManager))
  (bind _stunindex (Variables|/Game/Blueprints_Code/Boss/BP_BossManager.BP_BossManager_C|GetStunIndex _bossmanager))
  ;[0.15 0.15 0.15 0.5] BossHand
  (Variables|Default|SetStunned true)
  (if (and (== (Math|Integer|%(Integer) _stunindex 3) 0) (> _stunindex 0))
    (Development|PrintString "Stun more = 3" true true "(R=0.921582,G=1.000000,B=0.896270,A=1.000000)" 5.0)
    (CallFunction|PauseAllTimer)
    (if (Variables|Default|GetLeftHandSwing)
      (Default|StopSwingLeftHand (Variables|/Game/Blueprints_Code/Boss/Objects/BP_ObjectsPool.BP_ObjectsPool_C|GetLeftHand (Variables|Default|GetBP_BoxesPool)))
      (else
        (Default|StopSwingRightHand (Variables|/Game/Blueprints_Code/Boss/Objects/BP_ObjectsPool.BP_ObjectsPool_C|GetRightHand (Variables|Default|GetBP_BoxesPool)))))
    (Utilities|FlowControl|Delay 1e+01)
    (CallFunction|UnPauseAllTimer)
    (if (Variables|Default|GetLeftHandSwing)
      (Default|ContinuePlayLeftHand (Variables|/Game/Blueprints_Code/Boss/Objects/BP_ObjectsPool.BP_ObjectsPool_C|GetLeftHand (Variables|Default|GetBP_BoxesPool)))
      (else
        (Default|ContinuePlayRightHand (Variables|/Game/Blueprints_Code/Boss/Objects/BP_ObjectsPool.BP_ObjectsPool_C|GetRightHand (Variables|Default|GetBP_BoxesPool)))))))

(event Custom|Swing
  ;[0.15 0.15 0.15 0.5] BossHand
  (Variables|Default|SetStunned false)
  (if (Variables|Default|GetLeftHandSwing)
    (Development|PrintString "LeftHand")
    (Default|HandSwing (Variables|/Game/Blueprints_Code/Boss/Objects/BP_ObjectsPool.BP_ObjectsPool_C|GetLeftHand (Variables|Default|GetBP_BoxesPool)))
    (else
      (Development|PrintString "RightHand")
      (Default|HandSwing2 (Variables|/Game/Blueprints_Code/Boss/Objects/BP_ObjectsPool.BP_ObjectsPool_C|GetRightHand (Variables|Default|GetBP_BoxesPool))))))

(event Custom|EndPhase
  ;[0.15 0.15 0.15 0.5] BossHand
  (Default|DestoryPool (Variables|Default|GetBP_BoxesPool))
  (Default|NextPhase (Variables|Default|GetBossManager)))

(event Custom|EndPhase1
  ;[0.15 0.15 0.15 0.5] Never used
  (Utilities|Time|PauseTimerbyHandle (Variables|Default|GetDropBoxHandler))
  (Utilities|Time|PauseTimerbyHandle (Variables|Default|GetSawChildHandler))
  (Default|NextPhase (Variables|Default|GetBossManager)))

(event Custom|StartMoving
  (bind _splinearray (Variables|Default|GetSplineArray))
  ;[0.15 0.15 0.15 0.5] Saw
  (for _array_element (Variables|/Game/Blueprints_Code/Boss/Objects/BP_ObjectsPool.BP_ObjectsPool_C|GetSawPool (Variables|Default|GetBP_BoxesPool))
    (Default|CallSawonDestory _array_element _array_element))
  (Development|PrintString "Start Saw Event")
  (bind _array_element_2 (Utilities|Array|ForEachLoopwithBreak (Variables|/Game/Blueprints_Code/Boss/Objects/BP_ObjectsPool.BP_ObjectsPool_C|GetSawPool (Variables|Default|GetBP_BoxesPool)))
    (:LoopBody
      (Default|BossMovingSaw _array_element_2 (Utilities|Array|Get(acopy) _splinearray (Variables|Default|GetSplineIndex)))
      (Variables|Default|SetSawIndex (+ (Variables|Default|GetSawIndex) 1))
      (Variables|Default|SetSplineIndex (+ (Variables|Default|GetSplineIndex) 1)))
    (:Completed
      (Variables|Default|SetSawIndex 0)
      (Variables|Default|SetSplineIndex 0)
      (Utilities|Array|Shuffle _splinearray))))

(event Custom|DropTheBoxes
  (bind _bp_boxespool (Variables|Default|GetBP_BoxesPool))
  (bind _boxespool (Variables|/Game/Blueprints_Code/Boss/Objects/BP_ObjectsPool.BP_ObjectsPool_C|GetBoxesPool _bp_boxespool))
  (bind _returnvalue (Utilities|Array|Length _boxespool))
  ;[0.15 0.15 0.15 0.5] Moveable Object
  (for _array_element (Variables|/Game/Blueprints_Code/Boss/Objects/BP_ObjectsPool.BP_ObjectsPool_C|GetBoxesPool (Variables|Default|GetBP_BoxesPool))
    (Default|CallOnBoxDestory _array_element _array_element))
  (for _index (range 0 _returnvalue)
    (if (> _returnvalue 0)
      (Utilities|IsValid (Utilities|Array|Get(acopy) _boxespool (Variables|Default|GetBoxIndex))
        (:Is%20Valid
          (Default|ChangeVelocity (Utilities|Array|Get(acopy) _boxespool (Variables|Default|GetBoxIndex)) (* (Transformation|GetActorUpVector (Utilities|Array|Get(acopy) _boxespool (Variables|Default|GetBoxIndex))) (Variables|/Script/Engine.ProjectileMovementComponent|GetInitialSpeed (Variables|/Game/Blueprints_Code/Boss/Objects/BP_MoveObjectUpdate.BP_MoveObjectUpdate_C|GetProjectileMovement (Utilities|Array|Get(acopy) _boxespool (Variables|Default|GetBoxIndex))))))
          (Variables|Default|SetBoxIndex (+ (Variables|Default|GetBoxIndex) 1))))))
  (Variables|Default|SetBoxIndex 0))

(event EventBeginPlay
  (bind _outactors (Actor|GetAllActorsOfClass "/Game/Blueprints_Code/Hazards/BP_SplineHazards.BP_SplineHazards_C"))
  (bind _output_get (Variables|Default|SetSplineArray _outactors))
  (Utilities|Array|Shuffle _output_get)
  (bind _returnvalue (Actor|GetActorOfClass "/Game/Blueprints_Code/Boss/BP_BossManager.BP_BossManager_C"))
  (Variables|Default|SetBossManager _returnvalue)
  (Utilities|FlowControl|Sequence
    (:then_0
      ;[0.15 0.15 0.15 0.5] Moveable Object
      (bind _returnvalue_2 (Utilities|Time|SetTimerbyEvent (delegate Custom|DropTheBoxes) 15.0 true))
      (Variables|Default|SetDropBoxHandler _returnvalue_2))
    (:then_1
      ;[0.15 0.15 0.15 0.5] Saw
      (bind _returnvalue_3 (Utilities|Time|SetTimerbyEvent (delegate Custom|StartMoving) 15.0 true false 2.0))
      (Variables|Default|SetSawChildHandler _returnvalue_3))
    (:then_2
      ;[0.15 0.15 0.15 0.5] BossHand
      (bind _returnvalue_4 (Utilities|Time|SetTimerbyEvent (delegate Custom|Swing) 15.0 true false 12.0))
      (Variables|Default|SetSwingHandler _returnvalue_4)
      (EventDispatchers|BindEventtoBossbeStun (delegate Custom|Stun))
      (EventDispatchers|BindEventtoPhase1End (delegate Custom|EndPhase)))))

(event Collision|EventActorBeginOverlap
  (params (OtherActor :type Actor%20Object%20Reference)))

(event EventTick
  (params (DeltaSeconds :type Float%20%28single-precision%29)))

(fn ConstructionScript)

(fn PauseAllTimer
  (bind (_sawhandler _dropboxhandler _swinghandler) (Utilities|AllHandler))
  (Utilities|Time|PauseTimerbyHandle _sawhandler)
  (Utilities|Time|PauseTimerbyHandle _dropboxhandler)
  (Utilities|Time|PauseTimerbyHandle _swinghandler))

(fn UnPauseAllTimer
  (bind (_sawhandler _dropboxhandler _swinghandler) (Utilities|AllHandler))
  (Utilities|Time|UnpauseTimerbyHandle _sawhandler)
  (Utilities|Time|UnpauseTimerbyHandle _dropboxhandler)
  (Utilities|Time|UnpauseTimerbyHandle _swinghandler))