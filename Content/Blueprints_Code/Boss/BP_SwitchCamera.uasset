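; BP_SwitchCamera is a boss-fight trigger that switches the player's view to a fixed level camera.
; When the third-person character overlaps the Box, it resets control rotation to zero, disables look input and blends to the first CameraActor found.
; BackToNormal restores look input and blends back to the player character, but is not called within this Blueprint.
; The boss reference is cached but unused, so FacingToBoss ignores boss position.
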(event OnComponentBeginOverlap(Box)
  (params (OverlappedComponent :type Primitive%20Component%20Object%20Reference) (OtherActor :type Actor%20Object%20Reference) (OtherComp :type Primitive%20Component%20Object%20Reference) (OtherBodyIndex :type Integer) (bFromSweep :type Boolean) (SweepResult :type Hit%20Result%20Structure%20%28by%20ref%29))
  (bind _returnvalue (Game|GetPlayerController 0))
  (bind _asbp_third_person_character (Utilities|Casting|CastToBP_ThirdPersonCharacter OtherActor))
  (Variables|Default|SetAs%20BP%20Third%20Person%20Character _asbp_third_person_character)
  (CallFunction|FacingtoBoss)
  (Input|SetIgnoreLookInput _returnvalue true)
  (Game|Player|SetViewTargetwithBlend _returnvalue (Variables|Default|GetNewCamera) 0.5 "VTBlend_Linear" 0.0 false))

(event Custom|BackToNormal
  (bind _returnvalue (Game|GetPlayerController 0))
  (Input|SetIgnoreLookInput _returnvalue false)
  (Game|Player|SetViewTargetwithBlend _returnvalue (Game|GetPlayerCharacter 0) 0.5 "VTBlend_Linear" 0.0 false))

(event Custom|FacingToBoss
  (Pawn|SetControlRotation (Game|GetPlayerController 0) (Math|Rotator|MakeRotator 0.0 0.0 0.0)))

(event EventBeginPlay
  (bind _returnvalue (Actor|GetActorOfClass "/Script/Engine.CameraActor"))
  (Variables|Default|SetNewCamera _returnvalue)
  (bind _returnvalue_2 (Actor|GetActorOfClass "/Game/Cutsence/Cutscene_Actors/Bosssss.Bosssss_C"))
  (Variables|Default|SetBoss _returnvalue_2))

(fn ConstructionScript)