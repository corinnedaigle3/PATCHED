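; Test interactable limb actor that the player can pick up and carry in hand.
; BeginPlay caches the third-person character, and Interact calls PickUpTestLeg, which sets the character's HasLimb flag and snaps the limb to the CarryLimbR mesh socket.
; Once held, the cube ignores a custom trace channel and a debug message prints.
; AttachLeg is an empty stub.
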(event Custom|PickUpTestLeg
  (bind _as_bp_third_person_character (Variables|Default|GetAs%20BP%20Third%20Person%20Character))
  (Variables|/Game/BP_ThirdPersonCharacter.BP_ThirdPersonCharacter_C|SetHasLimb _as_bp_third_person_character true)
  (Transformation|AttachComponentToComponent (Variables|/Script/Engine.Character|GetMesh _as_bp_third_person_character) "CarryLimbR" "SnapToTarget" "SnapToTarget" "KeepWorld" false)
  (Collision|SetCollisionResponsetoChannel (Variables|Default|GetCube) "ECC_GameTraceChannel2" "ECR_Ignore")
  (Development|PrintString "LegInHand"))

(event Custom|AttachLeg)

(event EventBeginPlay
  (bind _asbp_third_person_character (Utilities|Casting|CastToBP_ThirdPersonCharacter (Game|Player|GetPlayerPawn 0)))
  (Variables|Default|SetAs%20BP%20Third%20Person%20Character _asbp_third_person_character))

(fn ConstructionScript)

(fn Interact
  (params (Character :type BP%20Third%20Person%20Character%20Object%20Reference))
  (CallFunction|PickUpTestLeg)
  (return false))