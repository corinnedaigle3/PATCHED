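; BP_Trigger is a trigger box that switches the scene's lighting to red when the third-person character walks into it.
; On overlap it destroys the actors in its Light and BPS arrays, then plays a timeline.
; Each timeline update zeroes the Rect lights and makes the RedLight entries visible, with intensity driven by the track.
; The RedLight loop is nested inside the Rect loop, so it depends on Rect having entries.
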(event OnComponentBeginOverlap(Box)
  (params (OverlappedComponent :type Primitive%20Component%20Object%20Reference) (OtherActor :type Actor%20Object%20Reference) (OtherComp :type Primitive%20Component%20Object%20Reference) (OtherBodyIndex :type Integer) (bFromSweep :type Boolean) (SweepResult :type Hit%20Result%20Structure%20%28by%20ref%29))
  (if (Class|GameplayStatics|ObjectIsA OtherActor "/Game/BP_ThirdPersonCharacter.BP_ThirdPersonCharacter_C")
    (for _array_element (Variables|Default|GetLight)
      (if (Utilities|IsValid _array_element)
        (Actor|DestroyActor _array_element)
        (else
          (Development|PrintString "can;t"))))
    (for _array_element_2 (Variables|Default|GetBP_S)
      (Utilities|IsValid _array_element_2
        (:Is%20Valid
          (Actor|DestroyActor _array_element_2))))
    (bind _newtrack_0 (Timeline|Timeline Play)
      (:Update
        (for _array_element_3 (Variables|Default|GetRect)
          (Rendering|Components|Light|SetIntensity (Variables|/Script/Engine.Light|GetLightComponent _array_element_3) 0.0)
          (for _array_element_4 (Variables|Default|GetRedLight)
            (Rendering|SetVisibility (Variables|/Script/Engine.Light|GetLightComponent _array_element_4) true false)
            (Rendering|Components|Light|SetIntensity (Variables|/Script/Engine.Light|GetLightComponent _array_element_4) (* _newtrack_0 3.0))))))))

(fn ConstructionScript)