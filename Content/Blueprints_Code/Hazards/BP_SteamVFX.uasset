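; Steam hazard effect actor that travels along a spline and affects the player character while inside its box.
; On BeginPlay a timeline, rate-scaled by TimeToComplete, lerps distance along SplineToFollow's spline to set location and rotation.
; Box overlap with BP_ThirdPersonCharacter clears Deactivated on the BP_SteamCollision found at BeginPlay and shows the WBP_SteamScreen overlay.
; End overlap sets Deactivated again and removes the overlay.
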(event OnComponentBeginOverlap(Box)
  (params (OverlappedComponent :type Primitive%20Component%20Object%20Reference) (OtherActor :type Actor%20Object%20Reference) (OtherComp :type Primitive%20Component%20Object%20Reference) (OtherBodyIndex :type Integer) (bFromSweep :type Boolean) (SweepResult :type Hit%20Result%20Structure%20%28by%20ref%29))
  (Utilities|Casting|CastToBP_ThirdPersonCharacter OtherActor)
  (Variables|/Game/Blueprints_Code/Hazards/BP_SteamCollision.BP_SteamCollision_C|SetDeactivated (Variables|Default|GetSteamCollision) false)
  (UserInterface|Viewport|AddtoViewport (Variables|Default|GetSteamScreen) 0))

(event OnComponentEndOverlap(Box)
  (params (OverlappedComponent :type Primitive%20Component%20Object%20Reference) (OtherActor :type Actor%20Object%20Reference) (OtherComp :type Primitive%20Component%20Object%20Reference) (OtherBodyIndex :type Integer))
  (Utilities|Casting|CastToBP_ThirdPersonCharacter OtherActor)
  (Variables|/Game/Blueprints_Code/Hazards/BP_SteamCollision.BP_SteamCollision_C|SetDeactivated (Variables|Default|GetSteamCollision) true)
  (Widget|RemovefromParent (Variables|Default|GetSteamScreen)))

(event EventBeginPlay
  (bind _spline_to_follow (Variables|Default|GetSpline%20To%20Follow))
  (bind _spline (Variables|/Game/Blueprints_Code/Hazards/BP_SplineHazards.BP_SplineHazards_C|GetSpline _spline_to_follow))
  ;[0.15 0.15 0.15 0.5] Moves the steam
  (bind _returnvalue (Actor|GetActorOfClass "/Game/Blueprints_Code/Hazards/BP_SteamCollision.BP_SteamCollision_C"))
  (Variables|Default|SetSteamCollision _returnvalue)
  (bind _returnvalue_2 (UserInterface|CreateWidget "/Game/Blueprints_UI/WBP_SteamScreen.WBP_SteamScreen_C"))
  (Variables|Default|SetSteamScreen _returnvalue_2)
  (Components|Timeline|SetPlayRate (Variables|Default|GetT_MSteam) (/ 1.0 (Variables|Default|GetTime%20To%20Complete)))
  (bind _newtrack_1 (Timeline|T_MSteam Play)
    (:Update
      (Transformation|SetActorLocationAndRotation (Spline|GetLocationatDistanceAlongSpline _spline (Math|Float|Lerp 0.0 (Spline|GetSplineLength _spline) _newtrack_1) "World") (Spline|GetRotationatDistanceAlongSpline _spline (Math|Float|Lerp 0.0 (Spline|GetSplineLength _spline) _newtrack_1) "World")))))

(fn ConstructionScript)