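; BP_Saw is a saw hazard actor that travels along a referenced spline when its MoveSaw event fires.
; BeginPlay adds an audio component, which MoveSaw plays as it starts a timeline with play rate scaled by TimeToComplete.
; Each timeline update maps the track alpha to distance along SplineToFollow's spline, setting the actor's world location and rotation from that point.
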(event Custom|MoveSaw
  (bind _spline_to_follow (Variables|Default|GetSpline%20To%20Follow))
  (bind _spline (Variables|/Game/Blueprints_Code/Hazards/BP_SplineHazards.BP_SplineHazards_C|GetSpline _spline_to_follow))
  ;[0.15 0.15 0.15 0.5] Move saw
  (Audio|Components|Audio|Play (Variables|Default|GetSaw) 0.0)
  (Components|Timeline|SetPlayRate (Variables|Default|GetT_MSaw) (/ 1.0 (Variables|Default|GetTime%20To%20Complete)))
  (bind _newtrack_1 (Timeline|T_MSaw Play)
    (:Update
      (Transformation|SetActorLocationAndRotation (Spline|GetLocationatDistanceAlongSpline _spline (Math|Float|Lerp 0.0 (Spline|GetSplineLength _spline) _newtrack_1) "World") (Spline|GetRotationatDistanceAlongSpline _spline (Math|Float|Lerp 0.0 (Spline|GetSplineLength _spline) _newtrack_1) "World")))))

(event EventBeginPlay
  (bind _returnvalue (AddComponent|AddAudioComponent false))
  (Variables|Default|SetSaw _returnvalue))

(fn ConstructionScript)