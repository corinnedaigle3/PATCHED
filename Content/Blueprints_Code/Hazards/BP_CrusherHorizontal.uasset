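; Horizontal crusher hazard that slides two blocks in opposite directions and can kill the player.
; StartSensor overlaps activate the Tick-driven stroke, which repeats after a pause while anything remains inside and otherwise stops once retracted.
; PlayerSensor arms a kill flag via timer, and HazardDeath fires when that flag and both crusher collision overlaps are set.
; Item and player sensors call conveyor start/stop events, whose loops currently perform no action.
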(event OnComponentBeginOverlap(PlayerSensor)
  (params (OverlappedComponent :type Primitive%20Component%20Object%20Reference) (OtherActor :type Actor%20Object%20Reference) (OtherComp :type Primitive%20Component%20Object%20Reference) (OtherBodyIndex :type Integer) (bFromSweep :type Boolean) (SweepResult :type Hit%20Result%20Structure%20%28by%20ref%29))
  ;[0.15 0.15 0.15 0.5] Start/Stop Conveyors
  (Utilities|Casting|CastToBP_ThirdPersonCharacter OtherActor)
  (bind _returnvalue (Utilities|Time|SetTimerbyEvent (delegate Custom|CustomEvent_0) (Variables|Default|GetTimeTillCrushed)))
  (Variables|Default|SetTimer _returnvalue)
  (if (not (Variables|Default|GetItem))
    (Utilities|FlowControl|Delay 0.2)
    (CallFunction|StopConveyors)))

(event OnComponentBeginOverlap(ItemSensor)
  (params (OverlappedComponent :type Primitive%20Component%20Object%20Reference) (OtherActor :type Actor%20Object%20Reference) (OtherComp :type Primitive%20Component%20Object%20Reference) (OtherBodyIndex :type Integer) (bFromSweep :type Boolean) (SweepResult :type Hit%20Result%20Structure%20%28by%20ref%29))
  ;[0.15 0.15 0.15 0.5] Start/Stop Conveyors
  (Utilities|Casting|CastToBP_ConveyorItem OtherActor)
  (Variables|Default|SetItem true)
  (Utilities|FlowControl|Delay 0.2)
  (CallFunction|StopConveyors))

(event OnComponentBeginOverlap(StartSensor)
  (params (OverlappedComponent :type Primitive%20Component%20Object%20Reference) (OtherActor :type Actor%20Object%20Reference) (OtherComp :type Primitive%20Component%20Object%20Reference) (OtherBodyIndex :type Integer) (bFromSweep :type Boolean) (SweepResult :type Hit%20Result%20Structure%20%28by%20ref%29))
  ;[0.15 0.15 0.15 0.5] Item Detection
  (Variables|Default|SetOverlapCount (+ 1 (Variables|Default|GetOverlapCount)))
  (Variables|Default|SetActivated true))

(event OnComponentEndOverlap(StartSensor)
  (params (OverlappedComponent :type Primitive%20Component%20Object%20Reference) (OtherActor :type Actor%20Object%20Reference) (OtherComp :type Primitive%20Component%20Object%20Reference) (OtherBodyIndex :type Integer))
  ;[0.15 0.15 0.15 0.5] Item Detection
  (Variables|Default|SetOverlapCount (Math|Integer|Clamp(Integer) (- (Variables|Default|GetOverlapCount) 1) 0 100)))

(event OnComponentBeginOverlap(CollisionR)
  (params (OverlappedComponent :type Primitive%20Component%20Object%20Reference) (OtherActor :type Actor%20Object%20Reference) (OtherComp :type Primitive%20Component%20Object%20Reference) (OtherBodyIndex :type Integer) (bFromSweep :type Boolean) (SweepResult :type Hit%20Result%20Structure%20%28by%20ref%29))
  ;[0.15 0.15 0.15 0.5] Crushers hit object
  (Variables|Default|SetHitObjR true))

(event OnComponentBeginOverlap(CollisionL)
  (params (OverlappedComponent :type Primitive%20Component%20Object%20Reference) (OtherActor :type Actor%20Object%20Reference) (OtherComp :type Primitive%20Component%20Object%20Reference) (OtherBodyIndex :type Integer) (bFromSweep :type Boolean) (SweepResult :type Hit%20Result%20Structure%20%28by%20ref%29))
  ;[0.15 0.15 0.15 0.5] Crushers hit object
  (Variables|Default|SetHitObjL true))

(event OnComponentEndOverlap(CollisionR)
  (params (OverlappedComponent :type Primitive%20Component%20Object%20Reference) (OtherActor :type Actor%20Object%20Reference) (OtherComp :type Primitive%20Component%20Object%20Reference) (OtherBodyIndex :type Integer))
  ;[0.15 0.15 0.15 0.5] Crushers hit object
  (Variables|Default|SetHitObjR false))

(event OnComponentEndOverlap(CollisionL)
  (params (OverlappedComponent :type Primitive%20Component%20Object%20Reference) (OtherActor :type Actor%20Object%20Reference) (OtherComp :type Primitive%20Component%20Object%20Reference) (OtherBodyIndex :type Integer))
  ;[0.15 0.15 0.15 0.5] Crushers hit object
  (Variables|Default|SetHitObjL false))

(event OnComponentEndOverlap(PlayerSensor)
  (params (OverlappedComponent :type Primitive%20Component%20Object%20Reference) (OtherActor :type Actor%20Object%20Reference) (OtherComp :type Primitive%20Component%20Object%20Reference) (OtherBodyIndex :type Integer))
  (Utilities|Casting|CastToBP_ThirdPersonCharacter OtherActor)
  (Utilities|Time|ClearandInvalidateTimerbyHandle (Variables|Default|GetTimer))
  (Utilities|FlowControl|Delay 0.2)
  (CallFunction|StartConveyors))

(event Custom|StartConveyors
  ;[0.15 0.15 0.15 0.5] Start Conveyors
  (Utilities|FlowControl|Delay 0.2)
  (Utilities|FlowControl|Sequence
    (:then_0
      (for _array_element 0
        (Utilities|IsValid _array_element)))
    (:then_1
      (for _array_element_2 0
        (Utilities|IsValid _array_element_2)))))

(event Custom|CustomEvent_0
  ;[0.15 0.15 0.15 0.5] Start/Stop Conveyors
  (Variables|Default|SetPlayer true)
  (CallFunction|KillPlayer))

(event Custom|Kill%20Player
  ;[0.15 0.15 0.15 0.5] Check if player is dead / Reset conveyors
  (if (Variables|Default|GetHitObjL)
    (if (Variables|Default|GetHitObjR)
      (if (Variables|Default|GetPlayer)
        (Variables|Default|SetPlayer false)
        (Utilities|FlowControl|Delay 0.2)
        (Default|HazardDeath (Variables|Default|GetCharREF))))))

(event Custom|StopConveyors
  ;[0.15 0.15 0.15 0.5] Stop Conveyors
  (Utilities|FlowControl|Sequence
    (:then_0
      (for _array_element 0
        (Utilities|IsValid _array_element)))
    (:then_1
      (for _array_element_2 0
        (Utilities|IsValid _array_element_2)))))

(event EventBeginPlay
  ;[0.15 0.15 0.15 0.5] Refs
  (bind _asbp_third_person_character (Utilities|Casting|CastToBP_ThirdPersonCharacter (Game|Player|GetPlayerPawn 0)))
  (Variables|Default|SetCharREF _asbp_third_person_character))

(event EventTick
  (params (DeltaSeconds :type Float%20%28single-precision%29))
  (bind _crusherr (Variables|Default|GetCrusherR))
  (bind _crusherr_2 (Variables|Default|GetCrusherR))
  (bind _crusherl (Variables|Default|GetCrusherL))
  (bind _crusherl_2 (Variables|Default|GetCrusherL))
  (bind _relativelocation (Variables|/Script/Engine.SceneComponent|GetRelativeLocation _crusherr_2))
  (bind _relativelocation_2 (Variables|/Script/Engine.SceneComponent|GetRelativeLocation _crusherl))
  (bind _relativelocation_3 (Variables|/Script/Engine.SceneComponent|GetRelativeLocation _crusherl_2))
  (bind _relativelocation_4 (Variables|/Script/Engine.SceneComponent|GetRelativeLocation _crusherr))
  ;[0.15 0.15 0.15 0.5] Crusher moving logic
  (Utilities|FlowControl|Sequence
    (:then_0
      (if (Variables|Default|GetActivated)
        (if (Variables|Default|GetGoingBack)
          (Transformation|SetRelativeLocation _crusherr (Math|Vector|MakeVector (- (.x _relativelocation_4) (Variables|Default|GetSpeed)) (.y _relativelocation_4) (.z _relativelocation_4)) false false)
          (Transformation|SetRelativeLocation _crusherl_2 (Math|Vector|MakeVector (+ (.x _relativelocation_3) (Variables|Default|GetSpeed)) (.y _relativelocation_3) (.z _relativelocation_3)) false false)
          (if (<= (.x _relativelocation_4) (Variables|Default|GetStartPoint))
            (Variables|Default|SetGoingBack false)
            (if (<= (Variables|Default|GetOverlapCount) 0)
              (Variables|Default|SetActivated false)
              (Development|PrintString "StopCrush")
              (else
                (Variables|Default|SetActivated false)
                (Utilities|FlowControl|Delay 1.5)
                (Variables|Default|SetActivated true)
                (Development|PrintString "ContinueCrush"))))
          (else
            (Transformation|SetRelativeLocation _crusherr_2 (Math|Vector|MakeVector (+ (.x _relativelocation) (Variables|Default|GetSpeed)) (.y _relativelocation) (.z _relativelocation)) false false)
            (Transformation|SetRelativeLocation _crusherl (Math|Vector|MakeVector (- (.x _relativelocation_2) (Variables|Default|GetSpeed)) (.y _relativelocation_2) (.z _relativelocation_2)) false false)
            (if (<= (Variables|Default|GetEndPoint) (.x _relativelocation))
              (Variables|Default|SetGoingBack true))))))
    (:then_1
      (CallFunction|KillPlayer))))

(fn ConstructionScript)