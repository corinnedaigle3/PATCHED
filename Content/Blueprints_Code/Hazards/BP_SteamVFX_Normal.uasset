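; Steam vent hazard that cycles on and off, obscuring the screen and pushing the player who enters it.
; A looping delay cycle in SteamActive toggles the particle effect and collider, restarting the audio component on each burst.
; Player overlap shows the steam screen widget and starts a repeating timer that calls LaunchCharacter while steam is active; leaving clears both.
; An older offset-based push for overlapping actors remains as unused logic.
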(event OnComponentBeginOverlap(Collider)
  (params (OverlappedComponent :type Primitive%20Component%20Object%20Reference) (OtherActor :type Actor%20Object%20Reference) (OtherComp :type Primitive%20Component%20Object%20Reference) (OtherBodyIndex :type Integer) (bFromSweep :type Boolean) (SweepResult :type Hit%20Result%20Structure%20%28by%20ref%29))
  ;[0.15 0.15 0.15 0.5] Visual Steam Widget
  (Utilities|Casting|CastToBP_ThirdPersonCharacter OtherActor)
  (UserInterface|Viewport|AddtoViewport (Variables|Default|GetSteamScreen) 0)
  (Variables|Default|SetLooping true)
  (bind _returnvalue (Utilities|Time|SetTimerbyEvent (delegate Custom|SteamMovePlayer) 0.1 (Variables|Default|GetLooping)))
  (Variables|Default|SetTimer _returnvalue))

(event OnComponentEndOverlap(Collider)
  (params (OverlappedComponent :type Primitive%20Component%20Object%20Reference) (OtherActor :type Actor%20Object%20Reference) (OtherComp :type Primitive%20Component%20Object%20Reference) (OtherBodyIndex :type Integer))
  ;[0.15 0.15 0.15 0.5] Visual Steam Widget
  (Utilities|Casting|CastToBP_ThirdPersonCharacter OtherActor)
  (Widget|RemovefromParent (Variables|Default|GetSteamScreen))
  (Variables|Default|SetLooping false)
  (Utilities|Time|ClearandInvalidateTimerbyHandle (Variables|Default|GetTimer)))

(event Custom|SteamMovePlayer
  ;[0.15 0.15 0.15 0.5] Push items in steam
  (if (Variables|Default|GetSteamActivated)
    (Character|LaunchCharacter (Variables|Default|GetCharRef) (Variables|Default|GetLaunch%20Velocity) true true)))

(event Custom|SteamActive
  ;[0.15 0.15 0.15 0.5] SteamState
  (Audio|Components|Audio|Play (Variables|Default|GetSteam) 0.0 :!label _label)
  (CallFunction|SteamStart)
  (Variables|Default|SetSteamActivated true)
  (Utilities|FlowControl|Delay (Variables|Default|GetSteamDuration))
  (CallFunction|SteamStop)
  (Utilities|FlowControl|Delay (Variables|Default|GetTimeBetweenSteam))
  (Rendering|SetVisibility (Variables|Default|GetFXE_Steam) true false)
  (goto _label))

(event Custom|SteamStop
  ;[0.15 0.15 0.15 0.5] Steam Start/Stop logic
  (Components|Activation|Deactivate (Variables|Default|GetFXE_Steam))
  (Collision|SetCollisionEnabled (Variables|Default|GetCollider) "NoCollision")
  (Variables|Default|SetSteamActivated false)
  (Rendering|SetVisibility (Variables|Default|GetFXE_Steam) false false))

(event Custom|SteamStart
  ;[0.15 0.15 0.15 0.5] Steam Start/Stop logic
  (Collision|SetCollisionEnabled (Variables|Default|GetCollider) "QueryOnly")
  (Components|Activation|Activate (Variables|Default|GetFXE_Steam) false))

(event EventBeginPlay
  (bind _returnvalue (UserInterface|CreateWidget "/Game/Blueprints_UI/WBP_SteamScreen.WBP_SteamScreen_C"))
  (Variables|Default|SetSteamScreen _returnvalue)
  (bind _returnvalue_2 (AddComponent|AddAudioComponent false))
  (Variables|Default|SetSteam _returnvalue_2)
  (CallFunction|SteamActive)
  (bind _asbp_third_person_character (Utilities|Casting|CastToBP_ThirdPersonCharacter (Game|Player|GetPlayerPawn 0)))
  (Variables|Default|SetCharRef _asbp_third_person_character))

(fn ConstructionScript)