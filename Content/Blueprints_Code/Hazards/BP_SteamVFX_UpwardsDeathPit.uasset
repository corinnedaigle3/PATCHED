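; BP_SteamVFX_UpwardsDeathPit is a steam hazard effect that raises its SteamWidget component vertically for a death pit.
; Three events, Area, Area1 and Area2, each play their own timeline, which lerps the widget's relative Z from zero toward a matching billboard marker.
; The target height is the billboard's world Z, applied as a relative location.
; Nothing in this Blueprint calls the events or handles damage.
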(event Custom|Area
  (bind _area (Timeline|Timeline_Area Play)
    (:Update
      (Transformation|SetRelativeLocation (Variables|Default|GetSteamWidget) (Math|Vector|MakeVector 0.0 0.0 (Math|Float|Lerp 0.0 (.z (Transformation|GetWorldLocation (Variables|Default|GetBillboard))) _area)) false false))))

(event Custom|Area1
  (bind _doortrack (Timeline|Timeline_Area1 Play)
    (:Update
      (Transformation|SetRelativeLocation (Variables|Default|GetSteamWidget) (Math|Vector|MakeVector 0.0 0.0 (Math|Float|Lerp 0.0 (.z (Transformation|GetWorldLocation (Variables|Default|GetBillboard1))) _doortrack)) false false))))

(event Custom|Area2
  (bind _doortrack (Timeline|Timeline_Area2 Play)
    (:Update
      (Transformation|SetRelativeLocation (Variables|Default|GetSteamWidget) (Math|Vector|MakeVector 0.0 0.0 (Math|Float|Lerp 0.0 (.z (Transformation|GetWorldLocation (Variables|Default|GetBillboard2))) _doortrack)) false false))))

(event EventBeginPlay
  (|CallParentFunction) ; This node is disabled and will not be called.\nDrag off pins to build functionality.
)

(fn ConstructionScript
  (|CallParentFunction))