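; Steam hazard actor that cycles a steam jet on and off, pushing actors along its collider's forward vector.
; BeginPlay starts a DoOnce-gated timer that launches an endless delay loop toggling effect and collision, replaying audio each cycle.
; Player overlap shows a steam screen widget and runs a timer that offsets every overlapping actor while steam is active.
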(event OnComponentBeginOverlap(Collider)
  (params (OverlappedComponent :type Primitive%20Component%20Object%20Reference) (OtherActor :type Actor%20Object%20Reference) (OtherComp :type Primitive%20Component%20Object%20Reference) (OtherBodyIndex :type Integer) (bFromSweep :type Boolean) (SweepResult :type Hit%20Result%20Structure%20%28by%20ref%29))
  ;[0.15 0.15 0.15 0.5] Visual Steam Widget
  (Utilities|Casting|CastToBP_ThirdPersonCharacter OtherActor)
  (UserInterface|Viewport|AddtoViewport (Variables|Default|GetSteamScreen) 0)
  (Variables|Default|SetLooping true)
  (bind _returnvalue (Utilities|Time|SetTimerbyEvent (delegate Custom|SteamMovePlayer) 0.1 (Variables|Default|GetLooping)))
  (Variables|Default|SetTimer _returnvalue))

(event OnComponentEndOverlap(Collider)
  (params (OverlappedComponent :type Primitive%20Component%20Object%20Reference) (OtherActor :type Actor%20Object%20Reference) (OtherComp :type Primitive%20Component%20Object%20Reference) (OtherBodyIndex :type Integer))
  ;[0.15 0.15 0.15 0.5] Visual Steam Widget
  (Utilities|Casting|CastToBP_ThirdPersonCharacter OtherActor)
  (Widget|RemovefromParent (Variables|Default|GetSteamScreen))
  (Variables|Default|SetLooping false)
  (Utilities|Time|ClearandInvalidateTimerbyHandle (Variables|Default|GetTimer)))

(event Custom|SteamMovePlayer
  ;[0.15 0.15 0.15 0.5] Push items in steam
  (if (Variables|Default|GetSteamActivated)
    (Development|PrintString "Player Overlap Move" true true "(R=0.000000,G=1.000000,B=0.126237,A=1.000000)")
    (Variables|Default|SetSpeed (Variables|Default|GetSetSpeed))
    (for _array_element (Collision|GetOverlappingActors (Variables|Default|GetCollider) 0 :!class /Script/Engine.PrimitiveComponent)
      (Transformation|AddActorWorldOffset _array_element (* (Math|Vector|GetForwardVector (Transformation|GetWorldRotation (Variables|Default|GetCollider))) (* (Utilities|Time|GetWorldDeltaSeconds) (Variables|Default|GetSpeed)))))
    (else
      (Development|PrintString "Player Overlap No Move" true true "(R=1.000000,G=0.000000,B=0.040983,A=1.000000)")
      (Variables|Default|SetSpeed 0.0))))

(event Custom|SteamNearPlayer
  ;[0.15 0.15 0.15 0.5] Steam Start up logic
  (if (Variables|Default|GetSteamActivated)
    (Utilities|FlowControl|DoOnce false
      (:Completed
        (CallFunction|SteamActive)))))

(event Custom|SteamActive
  ;[0.15 0.15 0.15 0.5] SteamState
  (Audio|Components|Audio|Play (Variables|Default|GetSteam) 0.0 :!label _label)
  (Collision|SetCollisionEnabled (Variables|Default|GetCollider) "QueryOnly")
  (Components|Activation|Activate (Variables|Default|GetFXE_SteamReverse) false)
  (Variables|Default|SetSteamActivated true)
  (Utilities|FlowControl|Delay (Variables|Default|GetSteamDuration))
  (Components|Activation|Deactivate (Variables|Default|GetFXE_SteamReverse))
  (Collision|SetCollisionEnabled (Variables|Default|GetCollider) "NoCollision")
  (Variables|Default|SetSteamActivated false)
  (Rendering|SetVisibility (Variables|Default|GetFXE_SteamReverse) false false)
  (Utilities|FlowControl|Delay (Variables|Default|GetTimeBetweenSteam))
  (Rendering|SetVisibility (Variables|Default|GetFXE_SteamReverse) true false)
  (goto _label))

(event Custom|SteamStart
  ;[0.15 0.15 0.15 0.5] Steam Start up logic
  (Variables|Default|SetSteamActivated true)
  (Variables|Default|SetLooping1 true)
  (bind _returnvalue (Utilities|Time|SetTimerbyEvent (delegate Custom|SteamNearPlayer) 0.05 (Variables|Default|GetLooping1)))
  (Variables|Default|SetTimer1 _returnvalue))

(event EventBeginPlay
  (bind _returnvalue (UserInterface|CreateWidget "/Game/Blueprints_UI/WBP_SteamScreen.WBP_SteamScreen_C"))
  (Variables|Default|SetSteamScreen _returnvalue)
  (bind _returnvalue_2 (AddComponent|AddAudioComponent false))
  (Variables|Default|SetSteam _returnvalue_2)
  (CallFunction|SteamStart))

(fn ConstructionScript)