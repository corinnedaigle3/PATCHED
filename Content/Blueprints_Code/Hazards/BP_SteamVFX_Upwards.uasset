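; BP_SteamVFX_Upwards is a timed hazard that shoots an upward steam jet and costs the player a life on contact.
; An endless delay loop started on BeginPlay alternates two seconds of active effect and box collision with an off period set by TimeBetweenSteam.
; Overlapping while active shows a steam screen widget and calls LoseALive on the character, and ending overlap removes the widget.
; A BP_SteamCollision reference is cached but unused here.
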(event OnComponentBeginOverlap(Box)
  (params (OverlappedComponent :type Primitive%20Component%20Object%20Reference) (OtherActor :type Actor%20Object%20Reference) (OtherComp :type Primitive%20Component%20Object%20Reference) (OtherBodyIndex :type Integer) (bFromSweep :type Boolean) (SweepResult :type Hit%20Result%20Structure%20%28by%20ref%29))
  (Utilities|Casting|CastToBP_ThirdPersonCharacter OtherActor)
  (if (Variables|Default|GetActivated)
    (UserInterface|Viewport|AddtoViewport (Variables|Default|GetSteamScreen) 0)
    (Default|LoseALive (Variables|Default|GetCharRef))))

(event OnComponentEndOverlap(Box)
  (params (OverlappedComponent :type Primitive%20Component%20Object%20Reference) (OtherActor :type Actor%20Object%20Reference) (OtherComp :type Primitive%20Component%20Object%20Reference) (OtherBodyIndex :type Integer))
  (Utilities|Casting|CastToBP_ThirdPersonCharacter OtherActor)
  (Widget|RemovefromParent (Variables|Default|GetSteamScreen)))

(event Custom|SteamStart
  ;[0.15 0.15 0.15 0.5] SteamState
  (Variables|Default|SetActivated true :!label _label)
  (Collision|SetCollisionEnabled (Variables|Default|GetBox) "QueryOnly")
  (Components|Activation|Activate (Variables|Default|GetFXE_Steam_Upwards) false)
  (Utilities|FlowControl|Delay 2.0)
  (Variables|Default|SetActivated false)
  (Components|Activation|Deactivate (Variables|Default|GetFXE_Steam_Upwards))
  (Collision|SetCollisionEnabled (Variables|Default|GetBox) "NoCollision")
  (Utilities|FlowControl|Delay (Variables|Default|GetTimeBetweenSteam))
  (goto _label))

(event EventBeginPlay
  (bind _asbp_third_person_character (Utilities|Casting|CastToBP_ThirdPersonCharacter (Game|Player|GetPlayerPawn 0)))
  (Variables|Default|SetCharRef _asbp_third_person_character)
  (bind _returnvalue (Actor|GetActorOfClass "/Game/Blueprints_Code/Hazards/BP_SteamCollision.BP_SteamCollision_C"))
  (Variables|Default|SetSteamCollision _returnvalue)
  (bind _returnvalue_2 (UserInterface|CreateWidget "/Game/Blueprints_UI/WBP_SteamScreen.WBP_SteamScreen_C"))
  (Variables|Default|SetSteamScreen _returnvalue_2)
  (CallFunction|SteamStart))

(fn ConstructionScript)