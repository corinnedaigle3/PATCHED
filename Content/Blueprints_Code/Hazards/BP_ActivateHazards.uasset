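; BP_ActivateHazards is a trigger that switches on linked hazards when the third-person character overlaps its Box.
; The overlap loops through the Saw, CrusherH and CrusherV arrays, skipping invalid entries.
; Saws get their Activate flag set and MoveSaw called, while both crusher types only get Activated set.
; Nothing resets the hazards, as the branch that stops the saws is never run.
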(event OnComponentBeginOverlap(Box)
  (params (OverlappedComponent :type Primitive%20Component%20Object%20Reference) (OtherActor :type Actor%20Object%20Reference) (OtherComp :type Primitive%20Component%20Object%20Reference) (OtherBodyIndex :type Integer) (bFromSweep :type Boolean) (SweepResult :type Hit%20Result%20Structure%20%28by%20ref%29))
  (Utilities|Casting|CastToBP_ThirdPersonCharacter OtherActor)
  (Utilities|FlowControl|Sequence
    (:then_0
      (for _array_element (Variables|Default|GetSaw)
        (Utilities|IsValid _array_element
          (:Is%20Valid
            (Variables|/Game/Blueprints_Code/Hazards/BP_Saw.BP_Saw_C|SetActivate _array_element true)
            (Default|MoveSaw _array_element)))))
    (:then_1
      (for _array_element_2 (Variables|Default|GetCrusherH)
        (Utilities|IsValid _array_element_2
          (:Is%20Valid
            (Variables|/Game/Blueprints_Code/Hazards/BP_CrusherHorizontal.BP_CrusherHorizontal_C|SetActivated _array_element_2 true)))))
    (:then_2
      (for _array_element_3 (Variables|Default|GetCrusherV)
        (Utilities|IsValid _array_element_3
          (:Is%20Valid
            (Variables|/Game/Blueprints_Code/Hazards/BP_CrusherVertical.BP_CrusherVertical_C|SetActivated _array_element_3 true)))))))

(fn ConstructionScript)