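; Interactable button that switches the level's crusher hazard on and off.
; On BeginPlay it caches the BP_Crusher found by GetActorOfClass, so it has no per-instance link, and adds button and beep audio components.
; Interact fires the CrusherButton event, which plays both sounds and toggles the crusher's Activated flag if the reference is valid, then returns false.
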(event Custom|CrusherButton
  (bind _crusher (Variables|Default|GetCrusher))
  ;[0.15 0.15 0.15 0.5] On/Off crusher button
  (Audio|Components|Audio|Play (Variables|Default|GetButton) 0.0)
  (Audio|Components|Audio|Play (Variables|Default|GetBeep) 0.0)
  (Utilities|IsValid _crusher
    (:Is%20Valid
      (if (Variables|/Game/Blueprints_Code/Hazards/BP_Crusher.BP_Crusher_C|GetActivated _crusher)
        (Variables|/Game/Blueprints_Code/Hazards/BP_Crusher.BP_Crusher_C|SetActivated _crusher false)
        (else
          (Variables|/Game/Blueprints_Code/Hazards/BP_Crusher.BP_Crusher_C|SetActivated _crusher true))))))

(event EventBeginPlay
  (bind _returnvalue (Actor|GetActorOfClass "/Game/Blueprints_Code/Hazards/BP_Crusher.BP_Crusher_C"))
  (Variables|Default|SetCrusher _returnvalue)
  (bind _returnvalue_2 (AddComponent|AddAudioComponent false))
  (Variables|Default|SetButton _returnvalue_2)
  (bind _returnvalue_3 (AddComponent|AddAudioComponent false))
  (Variables|Default|SetBeep _returnvalue_3))

(fn ConstructionScript)

(fn Interact
  (params (Character :type BP%20Third%20Person%20Character%20Object%20Reference))
  ;[0.15 0.15 0.15 0.5] Turn on/off the crusher
  (CallFunction|CrusherButton)
  (return false))