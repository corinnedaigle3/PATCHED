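; Child saw hazard that travels along a referenced spline when its Boss_MovingSaw event is called, apparently for a boss encounter.
; The event scales the SawMovement timeline's play rate by TimeToComplete, then each update maps the track onto the spline's length to set world location and rotation.
; BeginPlay starts no movement, and leftover timer and move calls are unconnected.
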(event Custom|Boss_MovingSaw
  (bind _spline_to_follow (Variables|Default|GetSpline%20To%20Follow))
  (bind _spline (Variables|/Game/Blueprints_Code/Hazards/BP_SplineHazards.BP_SplineHazards_C|GetSpline _spline_to_follow))
  (Components|Timeline|SetPlayRate (Variables|Default|GetSawMovement) (/ 1.0 (Variables|Default|GetTime%20To%20Complete)))
  (bind _newtrack_0 (Timeline|SawMovement Play)
    (:Update
      (Transformation|SetActorLocationAndRotation (Spline|GetLocationatDistanceAlongSpline _spline (Math|Float|Lerp 0.0 (Spline|GetSplineLength _spline) _newtrack_0) "World") (Spline|GetRotationatDistanceAlongSpline _spline (Math|Float|Lerp 0.0 (Spline|GetSplineLength _spline) _newtrack_0) "World")))))

(event EventBeginPlay)

(event Collision|EventActorBeginOverlap
  (params (OtherActor :type Actor%20Object%20Reference)))

(event EventTick
  (params (DeltaSeconds :type Float%20%28single-precision%29)))

(fn ConstructionScript
  (|CallParentFunction))