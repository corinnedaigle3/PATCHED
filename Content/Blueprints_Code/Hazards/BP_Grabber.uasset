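; BP_Grabber is a robotic arm hazard that seizes the third-person player character on overlap and holds them for a set time.
; The trigger disables its collision, sets Activate, blocks move input, then after a short delay attaches the character to the rig's "Grabbed" socket.
; It flags the character's AnimBP and records the grabber achievement, then detaches and restores control after HoldTime.
; The trigger is never re-enabled here.
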(event OnComponentBeginOverlap(ArmGrabber)
  (params (OverlappedComponent :type Primitive%20Component%20Object%20Reference) (OtherActor :type Actor%20Object%20Reference) (OtherComp :type Primitive%20Component%20Object%20Reference) (OtherBodyIndex :type Integer) (bFromSweep :type Boolean) (SweepResult :type Hit%20Result%20Structure%20%28by%20ref%29))
  (bind _returnvalue (Game|GetPlayerController 0))
  (bind _armgrabber (Variables|Default|GetArmGrabber))
  (bind _charref (Variables|Default|GetCharREF))
  ;[0.15 0.15 0.15 0.5] Activate grabber
  (Utilities|Casting|CastToBP_ThirdPersonCharacter OtherActor)
  (Components|Activation|Deactivate _armgrabber)
  (Collision|SetCollisionEnabled _armgrabber "NoCollision")
  (Variables|Default|SetActivate true)
  (Input|SetIgnoreMoveInput (Game|GetPlayerController 0) true)
  (Utilities|FlowControl|Delay 0.5)
  (Transformation|AttachComponentToComponent (Variables|Default|GetCharREF) (Variables|Default|Getrobo_arm_rigged) "Grabbed" "KeepRelative" "KeepWorld" "KeepWorld" true)
  (Transformation|SetActorRelativeLocation _charref)
  (Variables|/Game/Blueprints_Animations/ABP_Patched.ABP_Patched_C|SetGrabbed (Variables|/Game/BP_ThirdPersonCharacter.BP_ThirdPersonCharacter_C|GetAnimationBP _charref) true)
  (|CacheAchievements _returnvalue
    (:OnSuccess
      (|WriteProgress _returnvalue "ACH_Grabber" 1.0
        (:then
          _)))
    (:OnFailure
      _))
  (Utilities|FlowControl|Delay (Variables|Default|GetHoldTime))
  (Transformation|DetachFromActor (Variables|Default|GetCharREF) "KeepWorld" "KeepWorld" "KeepWorld")
  (Variables|Default|SetActivate false)
  (Variables|/Game/Blueprints_Animations/ABP_Patched.ABP_Patched_C|SetGrabbed (Variables|/Game/BP_ThirdPersonCharacter.BP_ThirdPersonCharacter_C|GetAnimationBP (Variables|Default|GetCharREF)) false)
  (Input|SetIgnoreMoveInput (Game|GetPlayerController 0) false))

(event EventBeginPlay
  (bind _asbp_third_person_character (Utilities|Casting|CastToBP_ThirdPersonCharacter (Game|Player|GetPlayerPawn 0)))
  (Variables|Default|SetCharREF _asbp_third_person_character)
  (AddComponent|AddAudioComponent false))

(fn ConstructionScript)