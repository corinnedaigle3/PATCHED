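; BP_SteamCollision is a steam hazard volume that pushes actors inside it sideways.
; Each tick, it offsets every actor overlapping BoxSteam along the box's right vector at PushSpeed, scaled by delta time and without sweeping.
; When any overlap with the box ends, it sets Deactivated, which stops the push; nothing in this graph clears that flag.
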(event OnComponentEndOverlap(BoxSteam)
  (params (OverlappedComponent :type Primitive%20Component%20Object%20Reference) (OtherActor :type Actor%20Object%20Reference) (OtherComp :type Primitive%20Component%20Object%20Reference) (OtherBodyIndex :type Integer))
  (Variables|Default|SetDeactivated true))

(event EventTick
  (params (DeltaSeconds :type Float%20%28single-precision%29))
  (if (Variables|Default|GetDeactivated)
    (Variables|Default|SetSpeed 0.0)
    (else
      (Variables|Default|SetSpeed (Variables|Default|GetPushSpeed))
      (for _array_element (Collision|GetOverlappingActors (Variables|Default|GetBoxSteam) 0 :!class /Script/Engine.PrimitiveComponent)
        (Transformation|AddActorWorldOffset _array_element (* (Math|Vector|GetRightVector (Transformation|GetWorldRotation (Variables|Default|GetBoxSteam))) (* (Utilities|Time|GetWorldDeltaSeconds) (Variables|Default|GetSpeed))))))))

(fn ConstructionScript)