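; Test steam vent hazard that cycles its effect on and off, pushing overlapping actors and showing a steam screen overlay to the player.
; SteamStart uses Delays to toggle box collision and FX, and Tick re-calls it whenever SteamActivated is false.
; While active, Tick offsets overlapping actors along the box's forward vector without sweep.
; Box overlaps add or remove the widget; the looping timer they set has no bound event.
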(event OnComponentBeginOverlap(Box)
  (params (OverlappedComponent :type Primitive%20Component%20Object%20Reference) (OtherActor :type Actor%20Object%20Reference) (OtherComp :type Primitive%20Component%20Object%20Reference) (OtherBodyIndex :type Integer) (bFromSweep :type Boolean) (SweepResult :type Hit%20Result%20Structure%20%28by%20ref%29))
  (Utilities|Casting|CastToBP_ThirdPersonCharacter OtherActor)
  (if (Variables|Default|GetMoveActivated)
    (UserInterface|Viewport|AddtoViewport (Variables|Default|GetSteamScreen) 0)
    (Variables|Default|SetLooping true)
    (Utilities|Time|SetTimerbyEvent 0 0.1 (Variables|Default|GetLooping))))

(event OnComponentEndOverlap(Box)
  (params (OverlappedComponent :type Primitive%20Component%20Object%20Reference) (OtherActor :type Actor%20Object%20Reference) (OtherComp :type Primitive%20Component%20Object%20Reference) (OtherBodyIndex :type Integer))
  (Utilities|Casting|CastToBP_ThirdPersonCharacter OtherActor)
  (Widget|RemovefromParent (Variables|Default|GetSteamScreen))
  (Variables|Default|SetLooping false))

(event Custom|SteamStart
  ;[0.15 0.15 0.15 0.5] SteamState
  (Variables|Default|SetMoveActivated true)
  (Collision|SetCollisionEnabled (Variables|Default|GetBox) "QueryOnly")
  (Components|Activation|Activate (Variables|Default|GetFXE_Steam) false)
  (Development|PrintString "SteamOn")
  (Utilities|FlowControl|Delay (Variables|Default|GetTimeBetweenSteam))
  (Components|Activation|Deactivate (Variables|Default|GetFXE_Steam))
  (Utilities|FlowControl|Delay 0.7)
  (Collision|SetCollisionEnabled (Variables|Default|GetBox) "NoCollision")
  (Variables|Default|SetMoveActivated false)
  (Development|PrintString "SteamOff")
  (Variables|Default|SetSteamActivated true)
  (Utilities|FlowControl|Delay (Variables|Default|GetTimeBetweenSteam))
  (Development|PrintString "Reset")
  (Variables|Default|SetSteamActivated false))

(event EventBeginPlay
  (bind _asbp_third_person_character (Utilities|Casting|CastToBP_ThirdPersonCharacter (Game|Player|GetPlayerPawn 0)))
  (Variables|Default|SetCharRef _asbp_third_person_character)
  (bind _returnvalue (UserInterface|CreateWidget "/Game/Blueprints_UI/WBP_SteamScreen.WBP_SteamScreen_C"))
  (Variables|Default|SetSteamScreen _returnvalue)
  (CallFunction|SteamStart)
  (Collision|SetCollisionEnabled (Variables|Default|GetBox) "NoCollision")
  (Components|Activation|Deactivate (Variables|Default|GetFXE_Steam)))

(event EventTick
  (params (DeltaSeconds :type Float%20%28single-precision%29))
  (Utilities|FlowControl|Sequence
    (:then_0
      (if (Variables|Default|GetMoveActivated)
        (Variables|Default|SetSpeed (Variables|Default|GetSetSpeed))
        (for _array_element (Collision|GetOverlappingActors (Variables|Default|GetBox) 0 :!class /Script/Engine.PrimitiveComponent)
          (Transformation|AddActorWorldOffset _array_element (* (Math|Vector|GetForwardVector (Transformation|GetWorldRotation (Variables|Default|GetBox))) (* (Utilities|Time|GetWorldDeltaSeconds) (Variables|Default|GetSpeed)))))
        (else
          (Variables|Default|SetSpeed 0.0))))
    (:then_1
      (if (not (Variables|Default|GetSteamActivated))
        (CallFunction|SteamStart)))))

(fn ConstructionScript)