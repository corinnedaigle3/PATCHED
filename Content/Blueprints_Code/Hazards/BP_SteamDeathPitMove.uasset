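; Trigger volume that tells the level's upward steam death pit to respond to one of four areas.
; On BeginPlay it caches the first BP_SteamVFX_UpwardsDeathPit found in the world.
; Any overlap with its box calls the matching Area function on that pit, chosen by a priority chain of boolean flags, or prints "No Movement" if none is set.
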(event OnComponentBeginOverlap(Box)
  (params (OverlappedComponent :type Primitive%20Component%20Object%20Reference) (OtherActor :type Actor%20Object%20Reference) (OtherComp :type Primitive%20Component%20Object%20Reference) (OtherBodyIndex :type Integer) (bFromSweep :type Boolean) (SweepResult :type Hit%20Result%20Structure%20%28by%20ref%29))
  (bind _steamdeath (Variables|Default|GetSteamDeath))
  (if (Variables|Default|GetArea)
    (Default|Area _steamdeath)
    (elif (Variables|Default|GetArea1)
      (Default|Area1 _steamdeath)
      (elif (Variables|Default|GetArea2)
        (Default|Area2 _steamdeath)
        (elif (Variables|Default|GetArea3)
          (Default|Area3 _steamdeath)
          (else
            (Development|PrintString "No Movement")))))))

(event EventBeginPlay
  (bind _returnvalue (Actor|GetActorOfClass "/Game/Blueprints_Code/Hazards/BP_SteamVFX_UpwardsDeathPit.BP_SteamVFX_UpwardsDeathPit_C"))
  (Variables|Default|SetSteamDeath _returnvalue))

(fn ConstructionScript)