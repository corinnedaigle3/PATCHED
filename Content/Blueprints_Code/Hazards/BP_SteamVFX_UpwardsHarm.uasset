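; Steam vent hazard that, when activated, cycles upward steam bursts on and off, costing the player a life on contact.
; A looping delay chain toggles the Niagara-style effect and collider together, playing audio as each burst starts.
; Overlap starts a polling timer that removes one life and shows a steam screen widget, then clears itself and disarms until the next burst.
; Ending the overlap removes the widget and also disarms the vent.
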(event OnComponentBeginOverlap(Collider)
  (params (OverlappedComponent :type Primitive%20Component%20Object%20Reference) (OtherActor :type Actor%20Object%20Reference) (OtherComp :type Primitive%20Component%20Object%20Reference) (OtherBodyIndex :type Integer) (bFromSweep :type Boolean) (SweepResult :type Hit%20Result%20Structure%20%28by%20ref%29))
  ;[0.15 0.15 0.15 0.5] On Player Overlap
  (Utilities|Casting|CastToBP_ThirdPersonCharacter OtherActor)
  (Variables|Default|SetLooping true)
  (if (not (Utilities|Time|IsTimerActivebyHandle (Variables|Default|GetTimer)))
    (bind _returnvalue (Utilities|Time|SetTimerbyEvent (delegate Custom|SteamLoseALife) 0.1 (Variables|Default|GetLooping)))
    (Variables|Default|SetTimer _returnvalue)))

(event OnComponentEndOverlap(Collider)
  (params (OverlappedComponent :type Primitive%20Component%20Object%20Reference) (OtherActor :type Actor%20Object%20Reference) (OtherComp :type Primitive%20Component%20Object%20Reference) (OtherBodyIndex :type Integer))
  ;[0.15 0.15 0.15 0.5] On Player End Overlap
  (Widget|RemovefromParent (Variables|Default|GetSteamScreen))
  (Variables|Default|SetLooping false)
  (Utilities|Time|ClearandInvalidateTimerbyHandle (Variables|Default|GetTimer))
  (Variables|Default|SetCanSteamEffectPlayer false))

(event Custom|SteamLoseALife
  ;[0.15 0.15 0.15 0.5] On Player Overlap
  (if (Variables|Default|GetCanSteamEffectPlayer)
    (UserInterface|Viewport|AddtoViewport (Variables|Default|GetSteamScreen) 0)
    (Default|LoseALive (Variables|Default|GetCharRef))
    ;[0.15 0.15 0.15 0.5] On Player End Overlap
    (Variables|Default|SetLooping false)
    (Utilities|Time|ClearandInvalidateTimerbyHandle (Variables|Default|GetTimer))
    (Variables|Default|SetCanSteamEffectPlayer false)))

(event Custom|SteamStart
  ;[0.15 0.15 0.15 0.5] SteamState
  (Audio|Components|Audio|Play (Variables|Default|GetSteam) 0.0 :!label _label)
  (Collision|SetCollisionEnabled (Variables|Default|GetCollider) "QueryOnly")
  (Components|Activation|Activate (Variables|Default|GetFXE_Steam_Upwards) false)
  (Variables|Default|SetCanSteamEffectPlayer true)
  (Utilities|FlowControl|Delay (Variables|Default|GetSteamDurnation))
  (Components|Activation|Deactivate (Variables|Default|GetFXE_Steam_Upwards))
  (Collision|SetCollisionEnabled (Variables|Default|GetCollider) "NoCollision")
  (Variables|Default|SetCanSteamEffectPlayer false)
  (Utilities|FlowControl|Delay (Variables|Default|GetTimeBetweenSteam))
  (goto _label))

(event EventBeginPlay
  (bind _asbp_third_person_character (Utilities|Casting|CastToBP_ThirdPersonCharacter (Game|Player|GetPlayerPawn 0)))
  (Variables|Default|SetCharRef _asbp_third_person_character)
  (bind _returnvalue (AddComponent|AddAudioComponent false))
  (Variables|Default|SetSteam _returnvalue)
  (bind _returnvalue_2 (UserInterface|CreateWidget "/Game/Blueprints_UI/WBP_SteamScreen.WBP_SteamScreen_C"))
  (Variables|Default|SetSteamScreen _returnvalue_2)
  (Components|Activation|Deactivate (Variables|Default|GetFXE_Steam_Upwards))
  (Collision|SetCollisionEnabled (Variables|Default|GetCollider) "NoCollision")
  (if (Variables|Default|GetSteamActivated)
    (CallFunction|SteamStart)))

(fn ConstructionScript)