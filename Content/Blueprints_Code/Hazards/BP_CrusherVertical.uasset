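; Vertical crusher hazard that kills the player caught beneath or within it.
; While activated, Tick moves the Crusher up and down between height limits at a set per-frame speed.
; PlayerSensor arms the kill after the player stays for TimeTillCrushed, cancelling the timer on exit.
; Death fires through the character's HazardDeath after a short delay, once armed and the Collision component registers an overlap.
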(event OnComponentBeginOverlap(PlayerSensor)
  (params (OverlappedComponent :type Primitive%20Component%20Object%20Reference) (OtherActor :type Actor%20Object%20Reference) (OtherComp :type Primitive%20Component%20Object%20Reference) (OtherBodyIndex :type Integer) (bFromSweep :type Boolean) (SweepResult :type Hit%20Result%20Structure%20%28by%20ref%29))
  ;[0.15 0.15 0.15 0.5] Player Kill Sensor
  (Utilities|Casting|CastToBP_ThirdPersonCharacter OtherActor)
  (bind _returnvalue (Utilities|Time|SetTimerbyEvent (delegate Custom|CustomEvent_0) (Variables|Default|GetTimeTillCrushed)))
  (Variables|Default|SetTimer _returnvalue)
  (if (not (Variables|Default|GetItem))
    (Utilities|FlowControl|Delay 0.2)))

(event OnComponentBeginOverlap(Collision)
  (params (OverlappedComponent :type Primitive%20Component%20Object%20Reference) (OtherActor :type Actor%20Object%20Reference) (OtherComp :type Primitive%20Component%20Object%20Reference) (OtherBodyIndex :type Integer) (bFromSweep :type Boolean) (SweepResult :type Hit%20Result%20Structure%20%28by%20ref%29))
  ;[0.15 0.15 0.15 0.5] Check if hit
  (Variables|Default|SetHitObj true))

(event OnComponentEndOverlap(Collision)
  (params (OverlappedComponent :type Primitive%20Component%20Object%20Reference) (OtherActor :type Actor%20Object%20Reference) (OtherComp :type Primitive%20Component%20Object%20Reference) (OtherBodyIndex :type Integer))
  ;[0.15 0.15 0.15 0.5] Check if hit
  (Variables|Default|SetHitObj false))

(event OnComponentEndOverlap(PlayerSensor)
  (params (OverlappedComponent :type Primitive%20Component%20Object%20Reference) (OtherActor :type Actor%20Object%20Reference) (OtherComp :type Primitive%20Component%20Object%20Reference) (OtherBodyIndex :type Integer))
  ;[0.15 0.15 0.15 0.5] Player Kill Sensor
  (Utilities|Casting|CastToBP_ThirdPersonCharacter OtherActor)
  (Utilities|Time|ClearandInvalidateTimerbyHandle (Variables|Default|GetTimer))
  (Utilities|FlowControl|Delay 0.2))

(event Custom|CustomEvent_0
  ;[0.15 0.15 0.15 0.5] Player Kill Sensor
  (Variables|Default|SetPlayer true)
  (CallFunction|KillPlayer))

(event Custom|Kill%20Player
  ;[0.15 0.15 0.15 0.5] Check if player is dead / Reset conveyors
  (if (Variables|Default|GetHitObj)
    (if (Variables|Default|GetPlayer)
      (Variables|Default|SetPlayer false)
      (Utilities|FlowControl|Delay 0.2)
      (Default|HazardDeath (Variables|Default|GetCharREF)))))

(event EventBeginPlay
  ;[0.15 0.15 0.15 0.5] Refs
  (bind _asbp_third_person_character (Utilities|Casting|CastToBP_ThirdPersonCharacter (Game|Player|GetPlayerPawn 0)))
  (Variables|Default|SetCharREF _asbp_third_person_character))

(event EventTick
  (params (DeltaSeconds :type Float%20%28single-precision%29))
  (bind _speed (Variables|Default|GetSpeed))
  (bind _speed_2 (Variables|Default|GetSpeed))
  (bind _crusher (Variables|Default|GetCrusher))
  (bind _crusher_2 (Variables|Default|GetCrusher))
  (bind _relativelocation (Variables|/Script/Engine.SceneComponent|GetRelativeLocation _crusher))
  (bind _relativelocation_2 (Variables|/Script/Engine.SceneComponent|GetRelativeLocation _crusher_2))
  (bind _returnvalue (+ (.z _relativelocation) _speed))
  (bind _returnvalue_2 (- (.z _relativelocation_2) _speed_2))
  ;[0.15 0.15 0.15 0.5] Crusher moving logic
  (Utilities|FlowControl|Sequence
    (:then_0
      (if (Variables|Default|GetActivated)
        (if (Variables|Default|GetGoingBack)
          (Transformation|SetRelativeLocation _crusher_2 (Math|Vector|MakeVector (.x _relativelocation_2) (.y _relativelocation_2) _returnvalue_2) false false)
          (if (<= _returnvalue_2 (Variables|Default|GetLowestPoint))
            (Variables|Default|SetGoingBack false))
          (else
            (Transformation|SetRelativeLocation _crusher (Math|Vector|MakeVector (.x _relativelocation) (.y _relativelocation) _returnvalue) false false)
            (if (<= (Variables|Default|GetHighestPoint) _returnvalue)
              (Variables|Default|SetGoingBack true))))))
    (:then_1
      (CallFunction|KillPlayer))))

(fn ConstructionScript)