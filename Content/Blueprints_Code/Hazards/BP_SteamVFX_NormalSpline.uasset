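; A steam hazard actor that travels along a referenced spline and pushes overlapping actors along its collider's forward vector.
; A timeline, scaled by completion time, sets location and rotation along the spline, while Tick applies the push offset.
; At the end of each run it toggles the small steam effect and disables collision during a cooldown, then restarts, restoring both a second later.
; BeginPlay also creates and stores a steam screen widget.
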(event Custom|MoveSteam
  (bind _splinetofollow (Variables|Default|GetSplineToFollow))
  (bind _spline (Variables|/Game/Blueprints_Code/Hazards/BP_SplineHazards.BP_SplineHazards_C|GetSpline _splinetofollow))
  (if (not (Variables|Default|GetSteamCoolDown))
    (Components|Timeline|SetPlayRate (Variables|Default|GetT_MSteam) (/ 1.0 (Variables|Default|GetTimeToComplete)))
    (bind _move_grabber (Timeline|T_MSteam Play)
      (:Update
        (Transformation|SetActorLocationAndRotation (Spline|GetLocationatDistanceAlongSpline _spline (Math|Float|Lerp 0.0 (Spline|GetSplineLength _spline) _move_grabber) "World") (Spline|GetRotationatDistanceAlongSpline _spline (Math|Float|Lerp 0.0 (Spline|GetSplineLength _spline) _move_grabber) "World"))
        (Utilities|FlowControl|Delay 1.0))
      (:Finished
        (Variables|Default|SetSteamCoolDown true)
        (Rendering|ToggleVisibility (Variables|Default|GetFXE_SteamSmall) true)
        (Collision|SetCollisionEnabled (Variables|Default|GetCollider) "NoCollision")
        (Utilities|FlowControl|Delay (Variables|Default|GetSteamCoolDownControl))
        (Development|PrintString "Cool Down Done")
        (Variables|Default|SetSteamCoolDown false)
        (Utilities|FlowControl|Sequence
          (:then_0
            (Timeline|T_MSteam PlayFromStart))
          (:then_1
            (Utilities|FlowControl|Delay 1.0)
            (Rendering|ToggleVisibility (Variables|Default|GetFXE_SteamSmall) true)
            (Collision|SetCollisionEnabled (Variables|Default|GetCollider) "QueryOnly")))))))

(event EventBeginPlay
  (CallFunction|MoveSteam)
  (bind _returnvalue (UserInterface|CreateWidget "/Game/Blueprints_UI/WBP_SteamScreen.WBP_SteamScreen_C"))
  (Variables|Default|SetSteamScreen _returnvalue))

(event EventTick
  (params (DeltaSeconds :type Float%20%28single-precision%29))
  (Variables|Default|SetSpeed (Variables|Default|GetSpeedMoveControl))
  (for _array_element (Collision|GetOverlappingActors (Variables|Default|GetCollider) 0 :!class /Script/Engine.PrimitiveComponent)
    (Transformation|AddActorWorldOffset _array_element (* (Math|Vector|GetForwardVector (Transformation|GetWorldRotation (Variables|Default|GetCollider))) (* DeltaSeconds (Variables|Default|GetSpeed))))))

(fn ConstructionScript)