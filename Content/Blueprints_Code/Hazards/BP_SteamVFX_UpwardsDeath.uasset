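; Upward steam hazard that kills the player and shows a steam screen overlay when they are near it.
; BeginPlay caches the player character and creates a WBP_SteamScreen widget.
; The Box trigger adds or removes that widget as the character enters or leaves.
; The DEATH trigger calls HazardDeath on the cached character for any overlapping actor, without checking what entered.
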(event OnComponentBeginOverlap(DEATH)
  (params (OverlappedComponent :type Primitive%20Component%20Object%20Reference) (OtherActor :type Actor%20Object%20Reference) (OtherComp :type Primitive%20Component%20Object%20Reference) (OtherBodyIndex :type Integer) (bFromSweep :type Boolean) (SweepResult :type Hit%20Result%20Structure%20%28by%20ref%29))
  (Default|HazardDeath (Variables|Default|GetCharRef)))

(event OnComponentBeginOverlap(Box)
  (params (OverlappedComponent :type Primitive%20Component%20Object%20Reference) (OtherActor :type Actor%20Object%20Reference) (OtherComp :type Primitive%20Component%20Object%20Reference) (OtherBodyIndex :type Integer) (bFromSweep :type Boolean) (SweepResult :type Hit%20Result%20Structure%20%28by%20ref%29))
  (Utilities|Casting|CastToBP_ThirdPersonCharacter OtherActor)
  (UserInterface|Viewport|AddtoViewport (Variables|Default|GetSteamScreen) 0))

(event OnComponentEndOverlap(Box)
  (params (OverlappedComponent :type Primitive%20Component%20Object%20Reference) (OtherActor :type Actor%20Object%20Reference) (OtherComp :type Primitive%20Component%20Object%20Reference) (OtherBodyIndex :type Integer))
  (Utilities|Casting|CastToBP_ThirdPersonCharacter OtherActor)
  (Widget|RemovefromParent (Variables|Default|GetSteamScreen)))

(event EventBeginPlay
  (bind _asbp_third_person_character (Utilities|Casting|CastToBP_ThirdPersonCharacter (Game|Player|GetPlayerPawn 0)))
  (Variables|Default|SetCharRef _asbp_third_person_character)
  (bind _returnvalue (UserInterface|CreateWidget "/Game/Blueprints_UI/WBP_SteamScreen.WBP_SteamScreen_C"))
  (Variables|Default|SetSteamScreen _returnvalue))

(fn ConstructionScript)