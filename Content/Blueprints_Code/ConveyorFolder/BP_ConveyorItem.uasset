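; BP_ConveyorItem is a conveyor item that gets "crushed" by BP_Crusher, which here means being teleported rather than destroyed.
; BeginPlay caches the first crusher and BP_TeleportLocationCrusher found in the level.
; Tick polls the crusher's two hit flags and Item flag, teleporting to that location while all are true.
; After a short Delay it restarts the conveyors and clears Item; the DestroyActor node is unconnected.
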(event EventBeginPlay
  (bind _returnvalue (Actor|GetActorOfClass "/Game/Blueprints_Code/Hazards/BP_Crusher.BP_Crusher_C"))
  (Variables|Default|SetCrusher _returnvalue)
  (bind _returnvalue_2 (Actor|GetActorOfClass "/Game/Blueprints_Code/Hazards/BP_TeleportLocationCrusher.BP_TeleportLocationCrusher_C"))
  (Variables|Default|SetTeleportLocationCrusher _returnvalue_2))

(event Collision|EventActorBeginOverlap
  (params (OtherActor :type Actor%20Object%20Reference)))

(event EventTick
  (params (DeltaSeconds :type Float%20%28single-precision%29))
  (bind _crusher (Variables|Default|GetCrusher))
  (Utilities|IsValid (Variables|Default|GetCube)
    (:Is%20Valid
      (if (Variables|/Game/Blueprints_Code/Hazards/BP_Crusher.BP_Crusher_C|GetHitObjL _crusher)
        (if (Variables|/Game/Blueprints_Code/Hazards/BP_Crusher.BP_Crusher_C|GetHitObjR _crusher)
          (if (Variables|/Game/Blueprints_Code/Hazards/BP_Crusher.BP_Crusher_C|GetItem _crusher)
            (Development|PrintString "Crush")
            (Transformation|Teleport (Transformation|GetActorLocation (Variables|Default|GetTeleportLocationCrusher)) "0, 0, 0")
            (Utilities|FlowControl|Delay 1.5)
            (Default|StartConveyors _crusher)
            (Variables|/Game/Blueprints_Code/Hazards/BP_Crusher.BP_Crusher_C|SetItem _crusher false)))))))

(fn ConstructionScript)