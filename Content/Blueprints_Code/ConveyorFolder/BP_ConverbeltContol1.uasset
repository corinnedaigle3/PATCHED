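; Conveyor belt actor that carries any overlapping actors along a path of Start, BoxM, End and numbered curve sections.
; Each Tick, it offsets actors in every section along that component's forward vector, scaled by delta time, without sweep, with curves at half speed.
; The Deactivated flag halts movement, but nothing here sets it.
; BeginPlay caches the player character without using it, and Interact only returns false.
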(event EventBeginPlay
  (bind _asbp_third_person_character (Utilities|Casting|CastToBP_ThirdPersonCharacter (Game|GetPlayerCharacter 0)))
  (Variables|Default|SetCharREF _asbp_third_person_character))

(event Collision|EventActorBeginOverlap
  (params (OtherActor :type Actor%20Object%20Reference)))

(event EventTick
  (params (DeltaSeconds :type Float%20%28single-precision%29))
  (if (Variables|Default|GetDeactivated)
    (Variables|Default|SetspeedConver 0.0)
    (else
      (Utilities|FlowControl|Sequence
        (:then_0
          ;[0.15 0.15 0.15 0.5] Conveyor Logic On/Off
          (Variables|Default|SetspeedConver 2.5e+02)
          (for _array_element (Collision|GetOverlappingActors (Variables|Default|GetEnd) 0 :!class /Script/Engine.PrimitiveComponent)
            (Transformation|AddActorWorldOffset _array_element (* (Math|Vector|GetForwardVector (Transformation|GetWorldRotation (Variables|Default|GetEnd))) (* DeltaSeconds (Variables|Default|GetspeedConver))))))
        (:then_1
          (Variables|Default|SetspeedConver 125.0)
          (for _array_element_2 (Collision|GetOverlappingActors (Variables|Default|GetCurve2_2) 0 :!class /Script/Engine.PrimitiveComponent)
            (Transformation|AddActorWorldOffset _array_element_2 (* (Math|Vector|GetForwardVector (Transformation|GetWorldRotation (Variables|Default|GetCurve2_2))) (* DeltaSeconds (Variables|Default|GetspeedConver))))))
        (:then_2
          (Variables|Default|SetspeedConver 125.0)
          (for _array_element_3 (Collision|GetOverlappingActors (Variables|Default|GetCurve2_3) 0 :!class /Script/Engine.PrimitiveComponent)
            (Transformation|AddActorWorldOffset _array_element_3 (* (Math|Vector|GetForwardVector (Transformation|GetWorldRotation (Variables|Default|GetCurve2_3))) (* DeltaSeconds (Variables|Default|GetspeedConver))))))
        (:then_3
          (Variables|Default|SetspeedConver 2.5e+02)
          (for _array_element_4 (Collision|GetOverlappingActors (Variables|Default|GetBoxM) 0 :!class /Script/Engine.PrimitiveComponent)
            (Transformation|AddActorWorldOffset _array_element_4 (* (Math|Vector|GetForwardVector (Transformation|GetWorldRotation (Variables|Default|GetBoxM))) (* DeltaSeconds (Variables|Default|GetspeedConver))))))
        (:then_4
          (Variables|Default|SetspeedConver 125.0)
          (for _array_element_5 (Collision|GetOverlappingActors (Variables|Default|GetCurve2_1) 0 :!class /Script/Engine.PrimitiveComponent)
            (Transformation|AddActorWorldOffset _array_element_5 (* (Math|Vector|GetForwardVector (Transformation|GetWorldRotation (Variables|Default|GetCurve2_1))) (* DeltaSeconds (Variables|Default|GetspeedConver))))))
        (:then_5
          (Variables|Default|SetspeedConver 125.0)
          (for _array_element_6 (Collision|GetOverlappingActors (Variables|Default|GetCurve2_4) 0 :!class /Script/Engine.PrimitiveComponent)
            (Transformation|AddActorWorldOffset _array_element_6 (* (Math|Vector|GetForwardVector (Transformation|GetWorldRotation (Variables|Default|GetCurve2_4))) (* DeltaSeconds (Variables|Default|GetspeedConver))))))
        (:then_6
          (Variables|Default|SetspeedConver 125.0)
          (for _array_element_7 (Collision|GetOverlappingActors (Variables|Default|GetCurve2_5) 0 :!class /Script/Engine.PrimitiveComponent)
            (Transformation|AddActorWorldOffset _array_element_7 (* (Math|Vector|GetForwardVector (Transformation|GetWorldRotation (Variables|Default|GetCurve2_5))) (* DeltaSeconds (Variables|Default|GetspeedConver))))))
        (:then_7
          (Variables|Default|SetspeedConver 125.0)
          (for _array_element_8 (Collision|GetOverlappingActors (Variables|Default|GetCurve1_7) 0 :!class /Script/Engine.PrimitiveComponent)
            (Transformation|AddActorWorldOffset _array_element_8 (* (Math|Vector|GetForwardVector (Transformation|GetWorldRotation (Variables|Default|GetCurve1_7))) (* DeltaSeconds (Variables|Default|GetspeedConver))))))
        (:then_8
          (Variables|Default|SetspeedConver 2.5e+02)
          (for _array_element_9 (Collision|GetOverlappingActors (Variables|Default|GetStart) 0 :!class /Script/Engine.PrimitiveComponent)
            (Transformation|AddActorWorldOffset _array_element_9 (* (Math|Vector|GetForwardVector (Transformation|GetWorldRotation (Variables|Default|GetStart))) (* DeltaSeconds (Variables|Default|GetspeedConver))))))
        (:then_9
          (Variables|Default|SetspeedConver 125.0)
          (for _array_element_10 (Collision|GetOverlappingActors (Variables|Default|GetCurve2_6) 0 :!class /Script/Engine.PrimitiveComponent)
            (Transformation|AddActorWorldOffset _array_element_10 (* (Math|Vector|GetForwardVector (Transformation|GetWorldRotation (Variables|Default|GetCurve2_6))) (* DeltaSeconds (Variables|Default|GetspeedConver))))))
        (:then_10
          (Variables|Default|SetspeedConver 125.0)
          (for _array_element_11 (Collision|GetOverlappingActors (Variables|Default|GetCurve1_6) 0 :!class /Script/Engine.PrimitiveComponent)
            (Transformation|AddActorWorldOffset _array_element_11 (* (Math|Vector|GetForwardVector (Transformation|GetWorldRotation (Variables|Default|GetCurve1_6))) (* DeltaSeconds (Variables|Default|GetspeedConver))))))
        (:then_11
          (Variables|Default|SetspeedConver 125.0)
          (for _array_element_12 (Collision|GetOverlappingActors (Variables|Default|GetCurve1_1) 0 :!class /Script/Engine.PrimitiveComponent)
            (Transformation|AddActorWorldOffset _array_element_12 (* (Math|Vector|GetForwardVector (Transformation|GetWorldRotation (Variables|Default|GetCurve1_1))) (* DeltaSeconds (Variables|Default|GetspeedConver))))))
        (:then_12
          (Variables|Default|SetspeedConver 125.0)
          (for _array_element_13 (Collision|GetOverlappingActors (Variables|Default|GetCurve2_7) 0 :!class /Script/Engine.PrimitiveComponent)
            (Transformation|AddActorWorldOffset _array_element_13 (* (Math|Vector|GetForwardVector (Transformation|GetWorldRotation (Variables|Default|GetCurve2_7))) (* DeltaSeconds (Variables|Default|GetspeedConver))))))
        (:then_13
          (Variables|Default|SetspeedConver 125.0)
          (for _array_element_14 (Collision|GetOverlappingActors (Variables|Default|GetCurve1_5) 0 :!class /Script/Engine.PrimitiveComponent)
            (Transformation|AddActorWorldOffset _array_element_14 (* (Math|Vector|GetForwardVector (Transformation|GetWorldRotation (Variables|Default|GetCurve1_5))) (* DeltaSeconds (Variables|Default|GetspeedConver))))))
        (:then_14
          (Variables|Default|SetspeedConver 125.0)
          (for _array_element_15 (Collision|GetOverlappingActors (Variables|Default|GetCurve1_2) 0 :!class /Script/Engine.PrimitiveComponent)
            (Transformation|AddActorWorldOffset _array_element_15 (* (Math|Vector|GetForwardVector (Transformation|GetWorldRotation (Variables|Default|GetCurve1_2))) (* DeltaSeconds (Variables|Default|GetspeedConver))))))
        (:then_15
          (Variables|Default|SetspeedConver 125.0)
          (for _array_element_16 (Collision|GetOverlappingActors (Variables|Default|GetCurve1_4) 0 :!class /Script/Engine.PrimitiveComponent)
            (Transformation|AddActorWorldOffset _array_element_16 (* (Math|Vector|GetForwardVector (Transformation|GetWorldRotation (Variables|Default|GetCurve1_4))) (* DeltaSeconds (Variables|Default|GetspeedConver))))))
        (:then_16
          (Variables|Default|SetspeedConver 125.0)
          (for _array_element_17 (Collision|GetOverlappingActors (Variables|Default|GetCurve1_3) 0 :!class /Script/Engine.PrimitiveComponent)
            (Transformation|AddActorWorldOffset _array_element_17 (* (Math|Vector|GetForwardVector (Transformation|GetWorldRotation (Variables|Default|GetCurve1_3))) (* DeltaSeconds (Variables|Default|GetspeedConver))))))))))

(fn ConstructionScript)

(fn Interact
  (params (Character :type Character%20Object%20Reference))
  (return false))