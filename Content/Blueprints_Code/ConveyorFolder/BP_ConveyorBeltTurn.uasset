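; BP_ConveyorBeltTurn is a conveyor belt turn piece that carries overlapping actors along while active.
; Each Tick, two box volumes push their overlapping actors along their own forward vectors at a fixed, frame-rate-independent speed, using unswept world offsets.
; The Deactivated flag zeroes the speed and skips movement.
; BeginPlay caches the player character reference, and Interact simply returns false.
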(event EventBeginPlay
  (bind _asbp_third_person_character (Utilities|Casting|CastToBP_ThirdPersonCharacter (Game|GetPlayerCharacter 0)))
  (Variables|Default|SetCharREF _asbp_third_person_character))

(event EventTick
  (params (DeltaSeconds :type Float%20%28single-precision%29))
  ;[0.15 0.15 0.15 0.5] Conveyor Logic On/Off
  (Utilities|FlowControl|Sequence
    (:then_0
      (if (Variables|Default|GetDeactivated)
        (Variables|Default|SetspeedConver 0.0)
        (else
          (Variables|Default|SetspeedConver 2.5e+02)
          (for _array_element (Collision|GetOverlappingActors (Variables|Default|GetBox) 0 :!class /Script/Engine.PrimitiveComponent)
            (Transformation|AddActorWorldOffset _array_element (* (Math|Vector|GetForwardVector (Transformation|GetWorldRotation (Variables|Default|GetBox))) (* DeltaSeconds (Variables|Default|GetspeedConver))))))))
    (:then_1
      (if (Variables|Default|GetDeactivated)
        (Variables|Default|SetspeedConver 0.0)
        (else
          (Variables|Default|SetspeedConver 2.5e+02)
          (for _array_element_2 (Collision|GetOverlappingActors (Variables|Default|GetBox1) 0 :!class /Script/Engine.PrimitiveComponent)
            (Transformation|AddActorWorldOffset _array_element_2 (* (Math|Vector|GetForwardVector (Transformation|GetWorldRotation (Variables|Default|GetBox1))) (* DeltaSeconds (Variables|Default|GetspeedConver))))))))))

(fn ConstructionScript)

(fn Interact
  (params (Character :type Character%20Object%20Reference))
  (return false))