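; A turning conveyor belt actor that carries whatever overlaps its two collision boxes around a corner.
; Each tick it offsets actors in the long box along that box's right vector and actors in the short box along that box's forward vector, scaled by delta time and speed.
; A Deactivated flag zeroes the speed and stops the movement, and BeginPlay caches a player character reference that is otherwise unused here.
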(event EventBeginPlay
  (bind _asbp_third_person_character (Utilities|Casting|CastToBP_ThirdPersonCharacter (Game|GetPlayerCharacter 0)))
  (Variables|Default|SetCharRef _asbp_third_person_character))

(event EventTick
  (params (DeltaSeconds :type Float%20%28single-precision%29))
  ;[0.15 0.15 0.15 0.5] Conveyor Logic On/Off
  (Utilities|FlowControl|Sequence
    (:then_0
      (if (Variables|Default|GetDeactivated)
        (Variables|Default|SetSpeed 0.0)
        (else
          (Variables|Default|SetSpeed (Variables|Default|GetSpeedControl))
          (for _array_element (Collision|GetOverlappingActors (Variables|Default|GetBoxCollisionLong) 0 :!class /Script/Engine.PrimitiveComponent)
            (Transformation|AddActorWorldOffset _array_element (* (Math|Vector|GetRightVector (Transformation|GetWorldRotation (Variables|Default|GetBoxCollisionLong))) (* DeltaSeconds (Variables|Default|GetSpeed))))))))
    (:then_1
      (if (Variables|Default|GetDeactivated)
        (Variables|Default|SetSpeed 0.0)
        (else
          (Variables|Default|SetSpeed (Variables|Default|GetSpeedControl))
          (for _array_element_2 (Collision|GetOverlappingActors (Variables|Default|GetBoxCollisionShort) 0 :!class /Script/Engine.PrimitiveComponent)
            (Transformation|AddActorWorldOffset _array_element_2 (* (Math|Vector|GetForwardVector (Transformation|GetWorldRotation (Variables|Default|GetBoxCollisionShort))) (* DeltaSeconds (Variables|Default|GetSpeed))))))))))

(fn ConstructionScript)