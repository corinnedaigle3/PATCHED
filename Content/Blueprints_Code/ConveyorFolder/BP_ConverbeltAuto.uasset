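; BP_ConverbeltAuto is a conveyor belt actor that carries overlapping actors along while it is active.
; Every tick it moves each actor overlapping its Box along the Box's forward vector at a fixed, frame-rate-independent speed.
; The offset is applied without sweep, so collisions along the path are ignored.
; The Deactivated flag zeroes Speed and skips the movement.
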(event EventBeginPlay)

(event Collision|EventActorBeginOverlap
  (params (OtherActor :type Actor%20Object%20Reference)))

(event EventTick
  (params (DeltaSeconds :type Float%20%28single-precision%29))
  ;[0.15 0.15 0.15 0.5] Conveyor Logic On/Off
  (if (Variables|Default|GetDeactivated)
    (Variables|Default|Setspeed 0.0)
    (else
      (Variables|Default|Setspeed 2.5e+02)
      (for _array_element (Collision|GetOverlappingActors (Variables|Default|GetBox) 0 :!class /Script/Engine.PrimitiveComponent)
        (Transformation|AddActorWorldOffset _array_element (* (Math|Vector|GetForwardVector (Transformation|GetWorldRotation (Variables|Default|GetBox))) (* DeltaSeconds (Variables|Default|Getspeed))))))))

(fn ConstructionScript)