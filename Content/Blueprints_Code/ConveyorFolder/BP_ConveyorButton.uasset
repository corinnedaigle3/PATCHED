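; BP_ConveyorButton is an interactable button that toggles linked conveyors on and off when the character has no item in hand.
; Interact calls Start/StopConveyor, which plays button and beep audio components created at BeginPlay.
; It then flips the Deactivated flag on each valid entry in the Spline array.
; Three further loops do nothing, and debug prints for straight, turn and curved conveyors are unreachable.
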(event Custom|Start/Stop%20Conveyor
  ;[0.15 0.15 0.15 0.5] Which Conveyor the Button is Hooked Up to
  (Audio|Components|Audio|Play (Variables|Default|GetButton) 0.0)
  (Audio|Components|Audio|Play (Variables|Default|GetBeep) 0.0)
  (Utilities|FlowControl|Sequence
    (:then_0
      (for _array_element (Variables|Default|GetSpline)
        (Utilities|IsValid _array_element
          (:Is%20Valid
            (if (Variables|/Game/Blueprints_Code/ConveyorFolder/BP_ConveyorSpline.BP_ConveyorSpline_C|Getdeactivated _array_element)
              (Variables|/Game/Blueprints_Code/ConveyorFolder/BP_ConveyorSpline.BP_ConveyorSpline_C|Setdeactivated _array_element false)
              (else
                (Variables|/Game/Blueprints_Code/ConveyorFolder/BP_ConveyorSpline.BP_ConveyorSpline_C|Setdeactivated _array_element true)))
            (Development|PrintString "SplineOn/Off")))))
    (:then_2
      (for _array_element_2 0
        (Utilities|IsValid _array_element_2
          (:Is%20Valid
            (if true
              _)))))
    (:then_3
      (for _array_element_3 0
        (Utilities|IsValid _array_element_3
          (:Is%20Valid
            (if true
              _)))))
    (:then_4
      (for _array_element_4 0
        (Utilities|IsValid _array_element_4
          (:Is%20Valid
            (if true
              _)))))))

(event EventBeginPlay
  (bind _returnvalue (AddComponent|AddAudioComponent false))
  (Variables|Default|SetButton _returnvalue)
  (bind _returnvalue_2 (AddComponent|AddAudioComponent false))
  (Variables|Default|SetBeep _returnvalue_2))

(fn ConstructionScript)

(fn Interact
  (params (Character :type BP%20Third%20Person%20Character%20Object%20Reference))
  ;[0.15 0.15 0.15 0.5] Call Start/Stop
  (if (not (Variables|/Game/BP_ThirdPersonCharacter.BP_ThirdPersonCharacter_C|GetHasItemInHand Character))
    (CallFunction|Start/StopConveyor)
    (return false)))