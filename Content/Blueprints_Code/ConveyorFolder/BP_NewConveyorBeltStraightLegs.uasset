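; Straight conveyor belt actor with legs that carries actors along while it is active.
; Each Tick, it copies SpeedControl into Speed and offsets every actor overlapping its BoxCollision along the box's right vector, scaled by delta time.
; Movement is a direct world offset without sweep, so carried actors ignore blocking collision.
; The Deactivated flag zeroes Speed and skips the movement.
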(event EventTick
  (params (DeltaSeconds :type Float%20%28single-precision%29))
  ;[0.15 0.15 0.15 0.5] Conveyor Logic On/Off
  (if (Variables|Default|GetDeactivated)
    (Variables|Default|SetSpeed 0.0)
    (else
      (Variables|Default|SetSpeed (Variables|Default|GetSpeedControl))
      (for _array_element (Collision|GetOverlappingActors (Variables|Default|GetBoxCollision) 0 :!class /Script/Engine.PrimitiveComponent)
        (Transformation|AddActorWorldOffset _array_element (* (Math|Vector|GetRightVector (Transformation|GetWorldRotation (Variables|Default|GetBoxCollision))) (* DeltaSeconds (Variables|Default|GetSpeed))))))))

(fn ConstructionScript)