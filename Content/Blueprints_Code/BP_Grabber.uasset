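; BP_Grabber is a hazard actor that moves along a referenced spline and temporarily immobilizes the third-person character it touches.
; A timeline, rate-scaled by TimeToComplete, drives its position and rotation along the spline.
; Box overlap runs a delayed sequence inside a conveyor loop, toggling conveyor deactivation and player movement, then disabling the box.
; Tick polls every saw's ResetOtherHazards flag to return the grabber to the spline start, re-enable the box and restart the timeline.
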(event OnComponentBeginOverlap(BoxGrabber)
  (params (OverlappedComponent :type Primitive%20Component%20Object%20Reference) (OtherActor :type Actor%20Object%20Reference) (OtherComp :type Primitive%20Component%20Object%20Reference) (OtherBodyIndex :type Integer) (bFromSweep :type Boolean) (SweepResult :type Hit%20Result%20Structure%20%28by%20ref%29))
  (bind _charref (Variables|Default|GetCharREF))
  (bind _boxgrabber (Variables|Default|GetBoxGrabber))
  (bind _charactermovement (Variables|/Script/Engine.Character|GetCharacterMovement _charref))
  (Utilities|Casting|CastToBP_ThirdPersonCharacter OtherActor)
  (bind _array_element (Utilities|Array|ForEachLoopwithBreak (Variables|Default|GetConveyor))
    (:LoopBody
      (Utilities|FlowControl|Delay 0.2)
      (Variables|/Game/Blueprints_Code/ConveyorFolder/BP_ConverbeltContol.BP_ConverbeltContol_C|SetDeactivated _array_element true)
      (Pawn|Components|CharacterMovement|SetMovementMode _charactermovement "MOVE_None" 0)
      (Utilities|FlowControl|Delay 2.0)
      (Variables|/Game/Blueprints_Code/ConveyorFolder/BP_ConverbeltContol.BP_ConverbeltContol_C|SetDeactivated _array_element false)
      (Pawn|Components|CharacterMovement|SetMovementMode _charactermovement "MOVE_Walking" 0)
      (Components|Activation|Deactivate _boxgrabber)
      (Collision|SetCollisionEnabled _boxgrabber "NoCollision"))))

(event Custom|MoveGrabber
  (bind _spline_to_follow (Variables|Default|GetSpline%20To%20Follow))
  (bind _spline (Variables|/Game/Blueprints_Code/BP_SplineHazards.BP_SplineHazards_C|GetSpline _spline_to_follow))
  (Components|Timeline|SetPlayRate (Variables|Default|GetT_MGrabber) (/ 1.0 (Variables|Default|GetTime%20To%20Complete)))
  (bind _move_grabber (Timeline|T_MGrabber Play)
    (:Update
      (Transformation|SetActorLocationAndRotation (Spline|GetLocationatDistanceAlongSpline _spline (Math|Float|Lerp 0.0 (Spline|GetSplineLength _spline) _move_grabber) "World") (Spline|GetRotationatDistanceAlongSpline _spline (Math|Float|Lerp 0.0 (Spline|GetSplineLength _spline) _move_grabber) "World")))))

(event EventTick
  (params (DeltaSeconds :type Float%20%28single-precision%29))
  (bind _spline_to_follow (Variables|Default|GetSpline%20To%20Follow))
  (bind _boxgrabber (Variables|Default|GetBoxGrabber))
  (bind _spline (Variables|/Game/Blueprints_Code/BP_SplineHazards.BP_SplineHazards_C|GetSpline _spline_to_follow))
  (bind _array_element (Utilities|Array|ForEachLoopwithBreak (Variables|Default|GetSawREF))
    (:LoopBody
      (if (Variables|/Game/Blueprints_Code/BP_Saw.BP_Saw_C|GetResetOtherHazards _array_element)
        (Audio|Components|Audio|Stop (Variables|Default|GetT_MGrabber))
        (Transformation|SetActorLocationAndRotation (Spline|GetLocationatDistanceAlongSpline _spline 0.0 "World") (Spline|GetRotationatDistanceAlongSpline _spline 0.0 "World"))
        (Components|Activation|Activate _boxgrabber false)
        (Collision|SetCollisionEnabled _boxgrabber "QueryAndPhysics")
        (Components|Timeline|PlayfromStart (Variables|Default|GetT_MGrabber))))))

(event EventBeginPlay
  (bind _asbp_third_person_character (Utilities|Casting|CastToBP_ThirdPersonCharacter (Game|Player|GetPlayerPawn 0)))
  (Variables|Default|SetCharREF _asbp_third_person_character)
  (bind _outactors (Actor|GetAllActorsOfClass "/Game/Blueprints_Code/ConveyorFolder/BP_ConverbeltContol.BP_ConverbeltContol_C"))
  (Variables|Default|SetConveyor _outactors)
  (bind _outactors_2 (Actor|GetAllActorsOfClass "/Game/Blueprints_Code/BP_Saw.BP_Saw_C"))
  (Variables|Default|SetSawREF _outactors_2))

(fn ConstructionScript)