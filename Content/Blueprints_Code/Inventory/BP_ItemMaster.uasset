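; Master pickup actor for inventory items that show a lore widget when the player interacts with them.
; The first Interact adds the item to the character's inventory, shows a HUD notification, opens the item's widget and notifies BP_LoreManager, unlocking its VB word.
; A second Interact, also triggered when the character leaves the box, closes the widget and destroys the actor.
; Sphere overlaps toggle the outline's visibility.
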(event OnComponentBeginOverlap(Sphere)
  (params (OverlappedComponent :type Primitive%20Component%20Object%20Reference) (OtherActor :type Actor%20Object%20Reference) (OtherComp :type Primitive%20Component%20Object%20Reference) (OtherBodyIndex :type Integer) (bFromSweep :type Boolean) (SweepResult :type Hit%20Result%20Structure%20%28by%20ref%29))
  ;[0.15 0.15 0.15 0.5] Outline Visailbity
  (Rendering|ToggleVisibility (Variables|Default|GetOutline) false))

(event OnComponentEndOverlap(Sphere)
  (params (OverlappedComponent :type Primitive%20Component%20Object%20Reference) (OtherActor :type Actor%20Object%20Reference) (OtherComp :type Primitive%20Component%20Object%20Reference) (OtherBodyIndex :type Integer))
  ;[0.15 0.15 0.15 0.5] Outline Visailbity
  (Rendering|ToggleVisibility (Variables|Default|GetOutline) true))

(event OnComponentEndOverlap(Box)
  (params (OverlappedComponent :type Primitive%20Component%20Object%20Reference) (OtherActor :type Actor%20Object%20Reference) (OtherComp :type Primitive%20Component%20Object%20Reference) (OtherBodyIndex :type Integer))
  ;[0.15 0.15 0.15 0.5] Close when you leave
  (Utilities|Casting|CastToBP_ThirdPersonCharacter OtherActor)
  (if (Variables|Internal|GetIsLoreShowing)
    (CallFunction|Interact)))

(event EventBeginPlay
  (Utilities|FlowControl|Delay 0.2)
  ;[0.15 0.15 0.15 0.5] Store references
  (bind _asbp_third_person_character (Utilities|Casting|CastToBP_ThirdPersonCharacter (Game|Player|GetPlayerPawn 0)))
  (Variables|PlayerRefs|SetInventoryComponent (Variables|/Game/BP_ThirdPersonCharacter.BP_ThirdPersonCharacter_C|GetBP_InventoryComponent _asbp_third_person_character))
  (Variables|PlayerRefs|SetPlayer%20HUD (Variables|/Game/BP_ThirdPersonCharacter.BP_ThirdPersonCharacter_C|GetPlayerHUD _asbp_third_person_character))
  (bind _returnvalue (Actor|GetActorOfClass "/Game/Blueprints_Code/LoreCollection/BP_LoreManager.BP_LoreManager_C"))
  (Variables|Internal|SetLore%20Manager _returnvalue))

(fn ConstructionScript)

(fn FirstTimeItemInteract
  (bind _addeditem (Default|AddItem (Variables|PlayerRefs|GetInventoryComponent) (Variables|Default|GetItemIndex) "NewEnumerator1"))
  (Default|AddItemNotification (Variables|PlayerRefs|GetPlayer%20HUD) (Variables|Default|GetItemNotifName) (.itemicon _addeditem))
  (bind _returnvalue (UserInterface|CreateWidget (.itemwidget _addeditem)))
  (Variables|Internal|SetWidgetSelf _returnvalue)
  (Utilities|FlowControl|DoOnce false
    (:Completed
      (Default|FirstLoreEncounter (Variables|Internal|GetLore%20Manager))
      (CallFunction|VBUnlock (.vbunlock _addeditem)))))

(fn LorePopUp
  (params (DoTurnOn :type Boolean))
  (bind _widgetself (Variables|Internal|GetWidgetSelf))
  (if DoTurnOn
    (UserInterface|Viewport|AddtoViewport _widgetself 0)
    (Default|PlayLoreSFX (Variables|Internal|GetLore%20Manager))
    (else
      (Widget|RemovefromParent _widgetself)))
  (Variables|/Script/Engine.PlayerController|SetbShowMouseCursor (Game|GetPlayerController 0) DoTurnOn))

(fn VBUnlock
  (params (VBUnlock :type Enum_VoiceBox%20Enum :default "NewEnumerator2"))
  (bind _lore_manager (Variables|Internal|GetLore%20Manager))
  ;[0.15 0.15 0.15 0.5] This handles the unlock of the VB words
  (switch Utilities|FlowControl|Switch|SwitchonEnum_VoiceBox VBUnlock
    (:NewEnumerator2
      (Variables|/Game/Blueprints_Code/LoreCollection/BP_LoreManager.BP_LoreManager_C|SetUnlocksApple _lore_manager true))
    (:NewEnumerator1
      (Variables|/Game/Blueprints_Code/LoreCollection/BP_LoreManager.BP_LoreManager_C|SetUnlockButterscotch _lore_manager true))
    (:NewEnumerator3
      (Variables|/Game/Blueprints_Code/LoreCollection/BP_LoreManager.BP_LoreManager_C|SetUnlocksHello _lore_manager true))
    (:NewEnumerator4
      (Variables|/Game/Blueprints_Code/LoreCollection/BP_LoreManager.BP_LoreManager_C|SetUnlocksPaperwork _lore_manager true))
    (:NewEnumerator5
      (Variables|/Game/Blueprints_Code/LoreCollection/BP_LoreManager.BP_LoreManager_C|SetUnlocksRevolution _lore_manager false)))
  (Default|CallVB (Math|Conversions|ToInteger(Byte) VBUnlock)))

(fn Interact
  (params (Character :type BP%20Third%20Person%20Character%20Object%20Reference))
  (bind _player_hud (Variables|PlayerRefs|GetPlayer%20HUD))
  (Development|PrintString "Interacting")
  (if (Variables|Internal|GetIsLoreShowing)
    (CallFunction|LorePopUp false)
    (bind _output_get (Variables|Internal|SetIsLoreShowing false))
    (Variables|/Game/Blueprints_Code/Inventory/WBP_PlayerHUD.WBP_PlayerHUD_C|SetIsNewItemOnDisplay _player_hud _output_get)
    (Actor|DestroyActor)
    (return true)
    (else
      (CallFunction|FirstTimeItemInteract)
      (CallFunction|LorePopUp true)
      (bind _output_get_2 (Variables|Internal|SetIsLoreShowing true))
      (Variables|/Game/Blueprints_Code/Inventory/WBP_PlayerHUD.WBP_PlayerHUD_C|SetIsNewItemOnDisplay _player_hud _output_get_2)
      (return false))))