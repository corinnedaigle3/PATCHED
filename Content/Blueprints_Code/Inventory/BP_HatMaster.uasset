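; BP_HatMaster is a hat pickup actor that adds a hat to the player's inventory.
; After a short delay on BeginPlay, it caches the third-person character, its inventory component and its HUD.
; Any actor overlap, with no check on the other actor, adds the item by index, shows a HUD notification with name and icon, destroys the pickup and calls EquipUnequipHat on the character.
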(event EventBeginPlay
  (Utilities|FlowControl|Delay 0.2)
  (bind _asbp_third_person_character (Utilities|Casting|CastToBP_ThirdPersonCharacter (Game|Player|GetPlayerPawn 0)))
  (Variables|Default|SetAs%20BP%20Third%20Person%20Character _asbp_third_person_character)
  (Variables|Default|SetInventoryComponent (Variables|/Game/BP_ThirdPersonCharacter.BP_ThirdPersonCharacter_C|GetBP_InventoryComponent _asbp_third_person_character))
  (Variables|Default|SetPlayer%20HUD (Variables|/Game/BP_ThirdPersonCharacter.BP_ThirdPersonCharacter_C|GetPlayerHUD _asbp_third_person_character)))

(event Collision|EventActorBeginOverlap
  (params (OtherActor :type Actor%20Object%20Reference))
  (Development|PrintString "Hat collected")
  (bind _addedhat (Default|AddItem (Variables|Default|GetInventoryComponent) (Variables|Default|GetItemIndex)))
  (Default|AddItemNotification (Variables|Default|GetPlayer%20HUD) (Variables|Default|GetItem%20Notif%20Name) (.haticon _addedhat))
  (Actor|DestroyActor)
  (Default|Equip/UnequipHat (Variables|Default|GetAs%20BP%20Third%20Person%20Character) true))

(fn ConstructionScript)