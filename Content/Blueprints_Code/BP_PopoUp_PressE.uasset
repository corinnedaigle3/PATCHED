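; BP_PopoUp_PressE is an actor that shows a world pop-up prompt, likely "Press E", when the player character is nearby.
; On BeginPlay it creates a WBP_WorldPopUp, assigns it to its widget component and hides it.
; Box overlaps by BP_ThirdPersonCharacter show and hide the widget.
; When IsPickable is set, the prompt only appears while TargeActor is still valid.
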(event OnComponentBeginOverlap(Box)
  (params (OverlappedComponent :type Primitive%20Component%20Object%20Reference) (OtherActor :type Actor%20Object%20Reference) (OtherComp :type Primitive%20Component%20Object%20Reference) (OtherBodyIndex :type Integer) (bFromSweep :type Boolean) (SweepResult :type Hit%20Result%20Structure%20%28by%20ref%29))
  (if (not (Class|WidgetComponent|IsWidgetVisible (Variables|Default|GetWidget)))
    (if (Class|GameplayStatics|ObjectIsA OtherActor "/Game/BP_ThirdPersonCharacter.BP_ThirdPersonCharacter_C")
      (if (Variables|Default|GetisPickable)
        (Variables|Default|GetTargeActor
          (:then
            _)
          (:else)))
      (Rendering|SetVisibility (Variables|Default|GetWidget) true false))))

(event OnComponentEndOverlap(Box)
  (params (OverlappedComponent :type Primitive%20Component%20Object%20Reference) (OtherActor :type Actor%20Object%20Reference) (OtherComp :type Primitive%20Component%20Object%20Reference) (OtherBodyIndex :type Integer))
  (if (Class|GameplayStatics|ObjectIsA OtherActor "/Game/BP_ThirdPersonCharacter.BP_ThirdPersonCharacter_C")
    (if (Class|WidgetComponent|IsWidgetVisible (Variables|Default|GetWidget))
      (Rendering|SetVisibility (Variables|Default|GetWidget) false false))))

(event EventBeginPlay
  (bind _widget (Variables|Default|GetWidget))
  (bind _returnvalue (UserInterface|CreateWidget "/Game/Blueprints_UI/WBP_WorldPopUp.WBP_WorldPopUp_C"))
  (UserInterface|SetWidget _widget _returnvalue)
  (Rendering|SetVisibility _widget false false))

(event Collision|EventActorBeginOverlap
  (params (OtherActor :type Actor%20Object%20Reference)))

(event EventTick
  (params (DeltaSeconds :type Float%20%28single-precision%29)))

(fn ConstructionScript)