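; BP_NoVbLore1 is an interactable lore pickup that toggles a WBP_NoVbLore1 popup widget on screen.
; BeginPlay creates the widget and finds the level's BP_LoreManager.
; Interact calls LorePopUp, which adds or removes the widget; showing it also sets the manager's NoVbLore1 flag and calls FirstLoreEncounter.
; Leaving the Box overlap hides the popup.
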(event OnComponentEndOverlap(Box)
  (params (OverlappedComponent :type Primitive%20Component%20Object%20Reference) (OtherActor :type Actor%20Object%20Reference) (OtherComp :type Primitive%20Component%20Object%20Reference) (OtherBodyIndex :type Integer))
  ;[0.15 0.15 0.15 0.5] Turn on/off Lore Pop Up
  (Widget|RemovefromParent (Variables|Default|GetLore))
  (Variables|Default|SetShowLore false))

(event Custom|LorePopUp
  ;[0.15 0.15 0.15 0.5] Turn on/off Lore Pop Up
  (if (Variables|Default|GetShowLore)
    (Widget|RemovefromParent (Variables|Default|GetLore))
    (Variables|Default|SetShowLore false)
    (Development|PrintString "Turn Off Lore")
    (else
      (UserInterface|Viewport|AddtoViewport (Variables|Default|GetLore) 0)
      (Variables|Default|SetShowLore true)
      ;;[0.15 0.15 0.15 0.5] Switch out for lore number
      (Variables|/Game/Blueprints_Code/LoreCollection/BP_LoreManager.BP_LoreManager_C|SetNoVbLore_1 (Variables|Default|GetLoreManager) true)
      (Default|FirstLoreEncounter (Variables|Default|GetLoreManager))
      (Development|PrintString "Turn On Lore"))))

(event EventBeginPlay
  ;[0.15 0.15 0.15 0.5] Reffs
  (bind _returnvalue (UserInterface|CreateWidget "/Game/Blueprints_Code/LoreCollection/WBP_NoVbLore1.WBP_NoVbLore1_C"))
  (Variables|Default|SetLore _returnvalue)
  (bind _returnvalue_2 (Actor|GetActorOfClass "/Game/Blueprints_Code/LoreCollection/BP_LoreManager.BP_LoreManager_C"))
  (Variables|Default|SetLoreManager _returnvalue_2))

(fn ConstructionScript)

(fn Interact
  (params (Character :type BP%20Third%20Person%20Character%20Object%20Reference))
  (Development|PrintString "InteractLore")
  (CallFunction|LorePopUp)
  (return false))