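; BP_Lore1Zack is an interactable lore pickup that toggles a popup widget and adds its item to the player's inventory until an add succeeds.
; Opening the popup passes the first enabled voice-line unlock flag to BP_LoreManager and plays its SFX.
; If the player has a voice box, it also triggers the manager's first-encounter event once.
; Leaving the box closes the popup, and sphere overlaps toggle outline visibility.
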(event OnComponentBeginOverlap(Sphere)
  (params (OverlappedComponent :type Primitive%20Component%20Object%20Reference) (OtherActor :type Actor%20Object%20Reference) (OtherComp :type Primitive%20Component%20Object%20Reference) (OtherBodyIndex :type Integer) (bFromSweep :type Boolean) (SweepResult :type Hit%20Result%20Structure%20%28by%20ref%29))
  ;[0.15 0.15 0.15 0.5] Outline Visailbity
  (Rendering|ToggleVisibility (Variables|Default|GetOutline) false))

(event OnComponentEndOverlap(Box)
  (params (OverlappedComponent :type Primitive%20Component%20Object%20Reference) (OtherActor :type Actor%20Object%20Reference) (OtherComp :type Primitive%20Component%20Object%20Reference) (OtherBodyIndex :type Integer))
  ;[0.15 0.15 0.15 0.5] Turn on/off Lore Pop Up
  (Widget|RemovefromParent (Variables|DoNOTTOUCH|GetLoreWidget))
  (Variables|Default|SetShowLore false)
  (Development|PrintString "Hello" true true "(R=1.000000,G=0.304933,B=0.805635,A=1.000000)"))

(event OnComponentEndOverlap(Sphere)
  (params (OverlappedComponent :type Primitive%20Component%20Object%20Reference) (OtherActor :type Actor%20Object%20Reference) (OtherComp :type Primitive%20Component%20Object%20Reference) (OtherBodyIndex :type Integer))
  ;[0.15 0.15 0.15 0.5] Outline Visailbity
  (Rendering|ToggleVisibility (Variables|Default|GetOutline) true))

(event Custom|LorePopUp
  ;[0.15 0.15 0.15 0.5] Turn on/off Lore Pop Up
  (if (Variables|Default|GetShowLore)
    (Widget|RemovefromParent (Variables|DoNOTTOUCH|GetLoreWidget))
    (Variables|Default|SetShowLore false)
    (else
      (UserInterface|Viewport|AddtoViewport (Variables|DoNOTTOUCH|GetLoreWidget) 0)
      (CallFunction|UnlockVBLine)
      (Variables|Default|SetShowLore true)
      (if (Variables|/Game/BP_ThirdPersonCharacter.BP_ThirdPersonCharacter_C|GethasVoiceBox (Variables|Default|GetCHarRef))
        (Utilities|FlowControl|DoOnce false
          (:Completed
            (Default|FirstLoreEncounter (Variables|Default|GetLoreManager))))))))

(event EventBeginPlay
  ;[0.15 0.15 0.15 0.5] Reffs
  (bind _returnvalue (UserInterface|CreateWidget (Variables|Default|GetYourWIdgetHere)))
  (Variables|DoNOTTOUCH|SetLoreWidget _returnvalue)
  (bind _returnvalue_2 (Actor|GetActorOfClass "/Game/Blueprints_Code/LoreCollection/BP_LoreManager.BP_LoreManager_C"))
  (Variables|Default|SetLoreManager _returnvalue_2)
  (bind _asbp_third_person_character (Utilities|Casting|CastToBP_ThirdPersonCharacter (Game|Player|GetPlayerPawn 0)))
  (Variables|Default|SetCHarRef _asbp_third_person_character))

(fn ConstructionScript)

(fn InitializeItemDataStructure
  (bind _returnvalue (Utilities|GetDataTableRow "/Game/Blueprints_Code/Inventory/DT_InventoryItemData.DT_InventoryItemData" (Utilities|String|StringToName (Variables|Default|GetItemID)))
    (:then
      (Variables|Default|SetItemDataStruct _returnvalue))))

(fn UnlockVBLine
  (bind _unlocksbutterscotch (Variables|VoicboxUnlocks|GetUnlocksButterscotch))
  (if (Variables|VoicboxUnlocks|GetUnlocksApple)
    (bind _loremanager (Variables|Default|GetLoreManager)
      (:then
        (Variables|/Game/Blueprints_Code/LoreCollection/BP_LoreManager.BP_LoreManager_C|SetUnlocksApple _loremanager (Variables|VoicboxUnlocks|GetUnlocksApple))
        (Default|PlayLoreSFX (Variables|Default|GetLoreManager) :!label _label))
      (:else
        (Development|PrintString "LORE NOT SET UP PROPERLY  
 
 
 
 
 
 
 
 
 
 
" true true "(R=0.000000,G=0.660000,B=1.000000,A=1.000000)" 2e+03 :!label _label_2)))
    (elif _unlocksbutterscotch
      (bind _loremanager_2 (Variables|Default|GetLoreManager)
        (:then
          (Variables|/Game/Blueprints_Code/LoreCollection/BP_LoreManager.BP_LoreManager_C|SetUnlockButterscotch _loremanager_2 _unlocksbutterscotch)
          (goto _label))
        (:else
          (goto _label_2)))
      (elif (Variables|VoicboxUnlocks|GetUnlocksHello)
        (bind _loremanager_3 (Variables|Default|GetLoreManager)
          (:then
            (Variables|/Game/Blueprints_Code/LoreCollection/BP_LoreManager.BP_LoreManager_C|SetUnlocksHello _loremanager_3 (Variables|VoicboxUnlocks|GetUnlocksHello))
            (goto _label))
          (:else
            (goto _label_2)))
        (elif (Variables|VoicboxUnlocks|GetUnlocksPaperwork)
          (bind _loremanager_4 (Variables|Default|GetLoreManager)
            (:then
              (Variables|/Game/Blueprints_Code/LoreCollection/BP_LoreManager.BP_LoreManager_C|SetUnlocksPaperwork _loremanager_4 (Variables|VoicboxUnlocks|GetUnlocksPaperwork))
              (goto _label))
            (:else
              (goto _label_2)))
          (elif (Variables|VoicboxUnlocks|GetUnlocksRevolution)
            (bind _loremanager_5 (Variables|Default|GetLoreManager)
              (:then
                (Variables|/Game/Blueprints_Code/LoreCollection/BP_LoreManager.BP_LoreManager_C|SetUnlocksRevolution _loremanager_5 (Variables|VoicboxUnlocks|GetUnlocksRevolution))
                (goto _label))
              (:else
                (goto _label_2)))
            (else
              (Development|PrintString "only show regular lore, there are no unlicks")
              (goto _label))))))))

(fn Interact
  (params (Character :type BP%20Third%20Person%20Character%20Object%20Reference))
  (bind _itemid (Variables|Default|GetItemID))
  (Development|PrintString "Hello")
  (CallFunction|LorePopUp)
  (if (not (Variables|Default|GetHasLoreBeenInteracted))
    (Development|PrintString _itemid true true "(R=1.000000,G=0.000000,B=0.014605,A=1.000000)")
    (bind _success (Default|AddItem (Variables|/Game/BP_ThirdPersonCharacter.BP_ThirdPersonCharacter_C|GetBP_InventoryComponent Character) "NewEnumerator0" 0 0 _itemid))
    (if _success
      (Default|AddItemNotification (Variables|/Game/BP_ThirdPersonCharacter.BP_ThirdPersonCharacter_C|GetPlayerHUD Character) "" 0 (Variables|Default|GetItemDataStruct))
      (Variables|Default|SetHasLoreBeenInteracted true)
      (return false))))