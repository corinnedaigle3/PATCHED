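; BP_Lore4 is an interactable lore pickup, the fourth in the lore collection, that shows a lore pop-up widget.
; On BeginPlay it creates a WBP_Lore widget and finds the BP_LoreManager in the level.
; Interacting toggles the widget; showing it sets the manager's LoreBool4 flag and calls FirstLoreEncounter.
; Ending overlap with its Box component removes the widget.
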(event OnComponentEndOverlap(Box)
  (params (OverlappedComponent :type Primitive%20Component%20Object%20Reference) (OtherActor :type Actor%20Object%20Reference) (OtherComp :type Primitive%20Component%20Object%20Reference) (OtherBodyIndex :type Integer))
  ;[0.15 0.15 0.15 0.5] Turn on/off Lore Pop Up
  (Widget|RemovefromParent (Variables|Default|GetLore4))
  (Variables|Default|SetShowLore false))

(event Custom|LorePopUp
  ;[0.15 0.15 0.15 0.5] Turn on/off Lore Pop Up
  (if (Variables|Default|GetShowLore)
    (Widget|RemovefromParent (Variables|Default|GetLore4))
    (Variables|Default|SetShowLore false)
    (else
      (UserInterface|Viewport|AddtoViewport (Variables|Default|GetLore4) 0)
      (Variables|Default|SetShowLore true)
      ;;[0.15 0.15 0.15 0.5] Switch out for lore number
      (Variables|/Game/Blueprints_Code/LoreCollection/BP_LoreManager.BP_LoreManager_C|SetLoreBool_4 (Variables|Default|GetLoreManager) true)
      (Default|FirstLoreEncounter (Variables|Default|GetLoreManager)))))

(event EventBeginPlay
  ;[0.15 0.15 0.15 0.5] Reffs
  (bind _returnvalue (UserInterface|CreateWidget "/Game/Blueprints_UI/Lore/WBP_Lore.WBP_Lore_C"))
  (Variables|Default|SetLore4 _returnvalue)
  (bind _returnvalue_2 (Actor|GetActorOfClass "/Game/Blueprints_Code/LoreCollection/BP_LoreManager.BP_LoreManager_C"))
  (Variables|Default|SetLoreManager _returnvalue_2))

(fn ConstructionScript)

(fn Interact
  (params (Character :type BP%20Third%20Person%20Character%20Object%20Reference))
  (Development|PrintString "Hello")
  (CallFunction|LorePopUp)
  (return false))