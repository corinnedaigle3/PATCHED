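; BP_LoreJacob is an interactable lore object that toggles a WBP_Lore popup on screen and hides it when an overlap with its Box ends.
; Showing the popup sets UnlockButterscotch on BP_LoreManager, plays the lore sound and fires FirstLoreEncounter once per instance.
; Interact also tries to add its item to the player's inventory until one add succeeds, then shows a HUD notification using data-table item data.
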(event OnComponentEndOverlap(Box)
  (params (OverlappedComponent :type Primitive%20Component%20Object%20Reference) (OtherActor :type Actor%20Object%20Reference) (OtherComp :type Primitive%20Component%20Object%20Reference) (OtherBodyIndex :type Integer))
  ;[0.15 0.15 0.15 0.5] Turn on/off Lore Pop Up
  (Widget|RemovefromParent (Variables|Default|GetLore))
  (Variables|Default|SetShowLore false))

(event Custom|LorePopUp
  (bind _loremanager (Variables|Default|GetLoreManager))
  ;[0.15 0.15 0.15 0.5] Turn on/off Lore Pop Up
  (if (Variables|Default|GetShowLore)
    (Widget|RemovefromParent (Variables|Default|GetLore))
    (Variables|Default|SetShowLore false)
    (Development|PrintString "Turn Off Lore")
    (else
      (UserInterface|Viewport|AddtoViewport (Variables|Default|GetLore) 0)
      (Variables|/Game/Blueprints_Code/LoreCollection/BP_LoreManager.BP_LoreManager_C|SetUnlockButterscotch _loremanager true)
      (Default|PlayLoreSFX _loremanager)
      (Variables|Default|SetShowLore true)
      (Utilities|FlowControl|DoOnce false
        (:Completed
          (Default|FirstLoreEncounter (Variables|Default|GetLoreManager)))))))

(event EventBeginPlay
  ;[0.15 0.15 0.15 0.5] Reffs
  (bind _returnvalue (UserInterface|CreateWidget "/Game/Blueprints_UI/Lore/WBP_Lore.WBP_Lore_C"))
  (Variables|Default|SetLore _returnvalue)
  (bind _returnvalue_2 (Actor|GetActorOfClass "/Game/Blueprints_Code/LoreCollection/BP_LoreManager.BP_LoreManager_C"))
  (Variables|Default|SetLoreManager _returnvalue_2))

(fn ConstructionScript)

(fn InitializeItemDataStructure
  (bind _returnvalue (Utilities|GetDataTableRow "/Game/Blueprints_Code/Inventory/DT_InventoryItemData.DT_InventoryItemData" (Utilities|String|StringToName (Variables|Default|GetItemID)))
    (:then
      (Variables|Default|SetItemDataStruct _returnvalue))))

(fn Interact
  (params (Character :type BP%20Third%20Person%20Character%20Object%20Reference))
  (Development|PrintString "InteractLore")
  (CallFunction|LorePopUp)
  (if (not (Variables|Default|GetHasLoreBeenInteracted))
    (bind _asbp_third_person_character (Utilities|Casting|CastToBP_ThirdPersonCharacter Character))
    (bind _success (Default|AddItem (Variables|/Game/BP_ThirdPersonCharacter.BP_ThirdPersonCharacter_C|GetBP_InventoryComponent _asbp_third_person_character) (Variables|Default|GetItemID) (Variables|Default|GetAmount)))
    (if _success
      (Default|AddItemNotification (Variables|/Game/BP_ThirdPersonCharacter.BP_ThirdPersonCharacter_C|GetPlayerHUD _asbp_third_person_character) (Variables|Default|GetItemDataStruct) (Variables|Default|GetAmount))
      (Variables|Default|SetHasLoreBeenInteracted true)
      (return false))))