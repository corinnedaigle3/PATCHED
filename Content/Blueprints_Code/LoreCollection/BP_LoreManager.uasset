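; BP_LoreManager tracks lore collection, holding per-entry lore flags and unlock slot states, and plays the lore interaction sound.
; BeginPlay adds the audio component and caches the game instance.
; SaveData packs the individual variables into save-game arrays, and LoadData restores them by index through switch functions.
; FirstLoreEncounter increments and logs the lore count, but its check for a full count of twelve triggers nothing.
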(event Custom|FirstLoreEncounter
  ;[0.15 0.15 0.15 0.5] Lore Encounter Tracker
  (Variables|Default|SetLoreCount (+ (Variables|Default|GetLoreCount) 1))
  (Development|PrintString "AddedToLore")
  (if (== (Variables|Default|GetLoreCount) 12)
    _))

(event Custom|PlayLoreSFX
  ;[0.15 0.15 0.15 0.5] Lore Encounter Tracker
  (Audio|Components|Audio|Play (Variables|Default|GetLoreInteraction) 0.0))

(event EventBeginPlay
  ;[0.15 0.15 0.15 0.5] Add audio compent to scene
  (bind _returnvalue (AddComponent|AddAudioComponent false))
  (Variables|Default|SetLoreInteraction _returnvalue)
  (bind _asbp_game_instance (Utilities|Casting|CastToBP_GameInstance (Game|GetGameInstance)))
  (Variables|Default|SetGame%20Instance%20Ref _asbp_game_instance))

(event EventLoadData
  (params (SaveGameRef :type BP%20Save%20Game%20Object%20Reference))
  ;[0.15 0.15 0.15 0.5] Saving Lore
  (for (_array_element _array_index) (Variables|/Game/Blueprints_Code/SaveData/BP_SaveGame.BP_SaveGame_C|GetLoreBools SaveGameRef)
    (CallFunction|LoadNoVB _array_element _array_index))
  (for (_array_element_2 _array_index_2) (Variables|/Game/Blueprints_Code/SaveData/BP_SaveGame.BP_SaveGame_C|GetUnlockSlotLMs SaveGameRef)
    (CallFunction|LoadUnlockSlots _array_element_2 _array_index_2)))

(event EventSaveData
  (params (SaveGameRef :type BP%20Save%20Game%20Object%20Reference))
  ;[0.15 0.15 0.15 0.5] Saving Lore
  (Variables|/Game/Blueprints_Code/SaveData/BP_SaveGame.BP_SaveGame_C|SetLoreBools SaveGameRef (Utilities|NoVBIntoArray))
  (Variables|/Game/Blueprints_Code/SaveData/BP_SaveGame.BP_SaveGame_C|SetUnlockSlotLMs SaveGameRef (Utilities|UnlockSlotsIntoArray)))

(fn ConstructionScript)

(fn LoadNoVB
  (params (InputPin :type Boolean) (Selection :type Integer))
  (switch int Selection
    (:0
      (Variables|Default|SetNoVbLore InputPin))
    (:1
      (Variables|Default|SetNoVbLore_1 InputPin))
    (:2
      (Variables|Default|SetNoVbLore_2 InputPin))
    (:3
      (Variables|Default|SetNoVbLore_3 InputPin))
    (:4
      (Variables|Default|SetNoVbLore_4 InputPin))
    (:5
      (Variables|Default|SetNoVbLore_5 InputPin))
    (:6
      (Variables|Default|SetNoVbLore_6 InputPin))
    (:7
      (Variables|Default|SetNoVbLore_7 InputPin))
    (:8
      (Variables|Default|SetNoVbLore_8 InputPin))
    (:9
      (Variables|Default|SetNoVbLore_9 InputPin))
    (:10
      (Variables|Default|SetNoVbLore_10 InputPin))
    (:11
      (Variables|Default|SetNoVbLore_11 InputPin))))

(fn LoadUnlockSlots
  (params (InputPin :type Boolean) (Selection :type Integer))
  (switch int Selection
    (:0
      (Variables|Default|SetUnlockSlotLM InputPin))
    (:1
      (Variables|Default|SetUnlockSlotLM_1 InputPin))
    (:2
      (Variables|Default|SetUnlockSlotLM_2 InputPin))
    (:3
      (Variables|Default|SetUnlockSlotLM_3 InputPin))
    (:4
      (Variables|Default|SetUnlockSlotLM_4 InputPin))))