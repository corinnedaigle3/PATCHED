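; BP_Crusher is a crusher hazard with two cubes that oscillate along relative X in mirrored motion.
; Tick shifts both cubes by a fixed per-frame step unless OFF is set, flipping GoingBack on exact CubeL position matches, so speed depends on frame rate.
; Two box overlaps detect BP_ThirdPersonCharacter, print a debug "DIE" and increment HitsRemaining, with no damage applied here.
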(event OnComponentBeginOverlap(Box)
  (params (OverlappedComponent :type Primitive%20Component%20Object%20Reference) (OtherActor :type Actor%20Object%20Reference) (OtherComp :type Primitive%20Component%20Object%20Reference) (OtherBodyIndex :type Integer) (bFromSweep :type Boolean) (SweepResult :type Hit%20Result%20Structure%20%28by%20ref%29))
  (Utilities|Casting|CastToBP_ThirdPersonCharacter OtherActor)
  (Development|PrintString "DIE")
  (Variables|Default|SetHitsRemaining (+ 1 (Variables|Default|GetHitsRemaining))))

(event OnComponentBeginOverlap(Box1)
  (params (OverlappedComponent :type Primitive%20Component%20Object%20Reference) (OtherActor :type Actor%20Object%20Reference) (OtherComp :type Primitive%20Component%20Object%20Reference) (OtherBodyIndex :type Integer) (bFromSweep :type Boolean) (SweepResult :type Hit%20Result%20Structure%20%28by%20ref%29))
  (Utilities|Casting|CastToBP_ThirdPersonCharacter OtherActor)
  (Development|PrintString "DIE")
  (Variables|Default|SetHitsRemaining (+ 1 (Variables|Default|GetHitsRemaining))))

(event EventBeginPlay)

(event Collision|EventActorBeginOverlap
  (params (OtherActor :type Actor%20Object%20Reference)))

(event EventTick
  (params (DeltaSeconds :type Float%20%28single-precision%29))
  (bind _cubel (Variables|Default|GetCubeL))
  (bind _cuber (Variables|Default|GetCubeR))
  (bind _cuber_2 (Variables|Default|GetCubeR))
  (bind _cubel_2 (Variables|Default|GetCubeL))
  (bind _relativelocation (Variables|/Script/Engine.SceneComponent|GetRelativeLocation _cuber))
  (bind _relativelocation_2 (Variables|/Script/Engine.SceneComponent|GetRelativeLocation _cubel_2))
  (bind _relativelocation_3 (Variables|/Script/Engine.SceneComponent|GetRelativeLocation _cuber_2))
  (bind _relativelocation_4 (Variables|/Script/Engine.SceneComponent|GetRelativeLocation _cubel))
  (bind _returnvalue (- (.x _relativelocation_2) 2.0))
  (Utilities|FlowControl|Sequence
    (:then_0
      (if (not (Variables|Default|GetOFF))
        (if (Variables|Default|GetGoingBack)
          (Transformation|SetRelativeLocation _cubel (Math|Vector|MakeVector (+ (.x _relativelocation_4) 2.0) (.y _relativelocation_4) (.z _relativelocation_4)) false false)
          (Transformation|SetRelativeLocation _cuber_2 (Math|Vector|MakeVector (- (.x _relativelocation_3) 2.0) (.y _relativelocation_3) (.z _relativelocation_3)) false false)
          (if (== (.x _relativelocation_4) 1.2e+02)
            (Variables|Default|SetGoingBack false))
          (else
            (Transformation|SetRelativeLocation _cubel_2 (Math|Vector|MakeVector _returnvalue (.y _relativelocation_2) (.z _relativelocation_2)) false false)
            (Transformation|SetRelativeLocation _cuber (Math|Vector|MakeVector (+ (.x _relativelocation) 2.0) (.y _relativelocation) (.z _relativelocation)) false false)
            (if (== _returnvalue 2e+01)
              (Variables|Default|SetGoingBack true))))))
    (:then_1
      (bind _output_get (Variables|Default|SetHitsRemaining (Variables|Default|GetHitsRemaining))))))

(fn ConstructionScript)