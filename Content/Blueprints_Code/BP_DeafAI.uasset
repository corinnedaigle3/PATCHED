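; Deaf enemy AI that spots the player by sight, then screams and chases at a changed speed.
; Pawn sensing halts current movement and starts an AI MoveTo toward the player, returning to path following on success.
; Retriggerable delays detect lost sight, then fade the scream, restore normal speed and resume the path.
; A DoOnce with a timed reset limits how often the scream replays.
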(event OnSeePawn(PawnSensing)
  (params (Pawn :type Pawn%20Object%20Reference))
  (bind _charactermovement (Variables|Character|GetCharacterMovement))
  ;[0.15 0.15 0.15 0.5] Sensing Player
  (Utilities|FlowControl|Sequence
    (:then_0
      (if (not (Variables|Default|GetCanSeePlayer))
        (Utilities|Casting|CastToBP_ThirdPersonCharacter Pawn)
        (Variables|Default|SetCanSeePlayer true)
        (Class|NavMovementInterface|StopActiveMovement _charactermovement)
        (Components|Movement|StopMovementImmediately _charactermovement)
        (CallFunction|ChasePlayer)))
    (:then_1
      (Utilities|FlowControl|RetriggerableDelay 1.0)
      (Variables|Default|SetCanSeePlayer false)
      (Utilities|FlowControl|RetriggerableDelay 1.5)
      (if (not (Variables|Default|GetCanSeePlayer))
        (CallFunction|StopScream)
        (Variables|/Script/Engine.CharacterMovementComponent|SetMaxWalkSpeed (Variables|Character|GetCharacterMovement) (Variables|Default|GetDeafEnemySpeed))
        (CallFunction|FollowPath)))))

(event Custom|ChasePlayer
  ;[0.15 0.15 0.15 0.5] Chasing Player
  (CallFunction|PlayScream)
  (Variables|/Script/Engine.CharacterMovementComponent|SetMaxWalkSpeed (Variables|Character|GetCharacterMovement) (Variables|Default|GetUpdatedDeafEnemySpeed))
  (AI|AIMoveTo self "0, 0, 0" (Game|Player|GetPlayerPawn 0) 15.0 false
    (:OnSuccess
      (Variables|Default|SetCanSeePlayer false)
      (CallFunction|FollowPath))))

(event Custom|PlayScream
  ;[0.15 0.15 0.15 0.5] Plays Enemy Audio Scream
  (Utilities|FlowControl|DoOnce false :!label _label
    (:Completed
      (Audio|Components|Audio|Play (Variables|Default|GetScream) 0.0)
      (Utilities|FlowControl|Delay 5.5)
      (goto _label Reset))))

(event Custom|StopScream
  ;[0.15 0.15 0.15 0.5] Fades Enemy Audio Scream
  (Development|PrintString "Stop scream")
  (Audio|Components|Audio|FadeOut (Variables|Default|GetScream) 2.0 0.0 "Linear" :!class /Script/Engine.AudioComponent))

(event EventBeginPlay
  (bind _returnvalue (AddComponent|AddAudioComponent false))
  (Audio|Components|Audio|Stop _returnvalue)
  (Variables|Default|SetScream _returnvalue)
  (|CallParentFunction))

(fn ConstructionScript
  (|CallParentFunction))