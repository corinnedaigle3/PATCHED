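; BP_Switch is an interactable switch that toggles a referenced spot light on and off.
; Its Interact function flips the IsLightOn flag, sets the SpotLightComponent intensity of the Light reference to a lit value or zero, and prints the new state.
; Interact always returns false and does not use its Character input; the event graph and construction script are empty.
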(event EventBeginPlay)

(event Collision|EventActorBeginOverlap
  (params (OtherActor :type Actor%20Object%20Reference)))

(event EventTick
  (params (DeltaSeconds :type Float%20%28single-precision%29)))

(fn ConstructionScript)

(fn Interact
  (params (Character :type BP%20Third%20Person%20Character%20Object%20Reference))
  (bind _light (Variables|Default|GetLight))
  (bind _spotlightcomponent (Variables|/Script/Engine.SpotLight|GetSpotLightComponent _light))
  (if (not (Variables|Default|GetIsLightOn???))
    (Variables|Default|SetIsLightOn??? true)
    (Development|PrintString "On")
    (Rendering|Components|Light|SetIntensity _spotlightcomponent 8.0)
    (else
      (Variables|Default|SetIsLightOn??? false)
      (Development|PrintString "Off")
      (Rendering|Components|Light|SetIntensity _spotlightcomponent 0.0)))
  (return false))