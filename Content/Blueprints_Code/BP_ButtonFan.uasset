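; Interactable one-shot button that starts fans and toggles steam, usable only by an empty-handed character with a shield.
; Interacting plays a cutscene, slides the button via a timeline and costs shield life, then activates linked fans, followed after delays by the steam gauge, steam actors and boiler sounds.
; An overlap sphere toggles the outline until use.
; The pressed state is saved, and loading it re-applies fans, steam and sounds.
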(event OnComponentBeginOverlap(Sphere)
  (params (OverlappedComponent :type Primitive%20Component%20Object%20Reference) (OtherActor :type Actor%20Object%20Reference) (OtherComp :type Primitive%20Component%20Object%20Reference) (OtherBodyIndex :type Integer) (bFromSweep :type Boolean) (SweepResult :type Hit%20Result%20Structure%20%28by%20ref%29))
  (bind _outline (Variables|Default|GetOutline))
  ;[0.15 0.15 0.15 0.5] Start Fans
  ;;[0.15 0.15 0.15 0.5] Outline
  (Utilities|IsValid _outline
    (:Is%20Valid
      (Rendering|ToggleVisibility _outline false))))

(event OnComponentEndOverlap(Sphere)
  (params (OverlappedComponent :type Primitive%20Component%20Object%20Reference) (OtherActor :type Actor%20Object%20Reference) (OtherComp :type Primitive%20Component%20Object%20Reference) (OtherBodyIndex :type Integer))
  (bind _outline (Variables|Default|GetOutline))
  ;[0.15 0.15 0.15 0.5] Start Fans
  ;;[0.15 0.15 0.15 0.5] Outline
  (Utilities|IsValid _outline
    (:Is%20Valid
      (Rendering|ToggleVisibility _outline true))))

(event Custom|Start/StopFans
  ;[0.15 0.15 0.15 0.5] Start Fans
  (Audio|Components|Audio|Play (Variables|Default|GetPress) 0.0)
  (Audio|Components|Audio|Play (Variables|Default|GetButton) 0.0)
  (Default|ShieldLoseLife (Variables|/Game/BP_ThirdPersonCharacter.BP_ThirdPersonCharacter_C|GetShield (Variables|Default|GetCharRef)))
  (CallFunction|ActivateFans)
  (Utilities|FlowControl|Delay 2.2)
  (Default|StartActive (Variables|Default|GetSteamGauge))
  (Utilities|FlowControl|Delay 5.0)
  (CallFunction|ActivateSteam)
  (CallFunction|BoilerSFX))

(event Custom|Button%20Pressed
  ;[0.15 0.15 0.15 0.5] Start Fans
  (bind _newtrack_0 (Timeline|Timeline Play)
    (:Update
      (Transformation|SetRelativeLocation (Variables|Default|Getpressable_button) (Math|Vector|MakeVector 0.0 0.0 (Math|Float|Lerp 0.0 (Variables|Default|GetSlideDistance) _newtrack_0)) false false))))

(event Custom|ActivateFans
  ;[0.15 0.15 0.15 0.5] Start Fans
  (for _array_element (Variables|Default|GetFans)
    (Utilities|IsValid _array_element
      (:Is%20Valid
        (Variables|/Game/Blueprints_Code/BP_Fan.BP_Fan_C|SetFanActivate _array_element true)))))

(event Custom|ActivateSteam
  ;[0.15 0.15 0.15 0.5] Start Fans
  (for _array_element (Variables|Default|GetSteam)
    (Utilities|IsValid _array_element
      (:Is%20Valid
        (if (Variables|/Game/Blueprints_Code/Hazards/BP_SteamVFX_UpwardsHarm.BP_SteamVFX_UpwardsHarm_C|GetSteamActivated _array_element)
          (Variables|/Game/Blueprints_Code/Hazards/BP_SteamVFX_UpwardsHarm.BP_SteamVFX_UpwardsHarm_C|SetSteamActivated _array_element false)
          (else
            (Variables|/Game/Blueprints_Code/Hazards/BP_SteamVFX_UpwardsHarm.BP_SteamVFX_UpwardsHarm_C|SetSteamActivated _array_element true)
            (Default|SteamStart _array_element)))))))

(event Custom|BoilerSFX
  ;[0.15 0.15 0.15 0.5] Start Fans
  (for _array_element (Variables|Default|GetSFXBoiler)
    (Utilities|IsValid _array_element
      (:Is%20Valid
        (Default|PlaySFX _array_element)))))

(event Custom|InitializeData
  (if (Variables|Default|GetInteracted)
    (CallFunction|ActivateFans)
    (CallFunction|ActivateSteam)
    (CallFunction|BoilerSFX)))

(event EventBeginPlay
  (bind _returnvalue (AddComponent|AddAudioComponent false))
  (Variables|Default|SetPress _returnvalue)
  (bind _returnvalue_2 (AddComponent|AddAudioComponent false))
  (Variables|Default|SetButton _returnvalue_2)
  (bind _asbp_third_person_character (Utilities|Casting|CastToBP_ThirdPersonCharacter (Game|Player|GetPlayerPawn 0)))
  (Variables|Default|SetCharRef _asbp_third_person_character)
  (bind _returnvalue_3 (Actor|GetActorOfClass "/Game/Cutsence/BP_CutSceneManager.BP_CutSceneManager_C"))
  (Variables|Default|SetCutsceneManager _returnvalue_3))

(event EventSaveData
  (params (SaveGameRef :type BP%20Save%20Game%20Object%20Reference))
  (Variables|/Game/Blueprints_Code/SaveData/BP_SaveGame.BP_SaveGame_C|SetButtonPressed SaveGameRef (Variables|Default|GetInteracted)))

(event EventLoadData
  (params (SaveGameRef :type BP%20Save%20Game%20Object%20Reference))
  (Variables|Default|SetInteracted (Variables|/Game/Blueprints_Code/SaveData/BP_SaveGame.BP_SaveGame_C|GetButtonPressed SaveGameRef))
  (CallFunction|InitializeData))

(fn ConstructionScript)

(fn Interact
  (params (Character :type BP%20Third%20Person%20Character%20Object%20Reference))
  ;[0.15 0.15 0.15 0.5] Button Interaction
  (if (not (Variables|/Game/BP_ThirdPersonCharacter.BP_ThirdPersonCharacter_C|GetHasItemInHand Character))
    (if (Variables|/Game/BP_ThirdPersonCharacter.BP_ThirdPersonCharacter_C|GetHasShield Character)
      (if (not (Variables|Default|GetInteracted))
        (Variables|Default|SetInteracted true)
        (Default|PlayCutscene (Variables|Default|GetCutsceneManager))
        (Components|DestroyComponent (Variables|Default|GetOutline))
        (CallFunction|ButtonPressed)
        (CallFunction|Start/StopFans)
        (return false))
      (else
        (Audio|Components|Audio|Play (Variables|Default|GetPress) 0.0)))))