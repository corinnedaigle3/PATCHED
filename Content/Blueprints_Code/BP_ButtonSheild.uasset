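; Button shield pickup that gives the third-person character a one-use parry against deaf and blind enemies.
; Interacting without a shield attaches it to the ShieldR socket, sets HasShield, ignores a trace channel on its mesh and shows a parry objective prompt.
; Box overlaps with either enemy type toggle CanParry.
; Parrying then raises IsParrying for a second before removing and destroying the shield, with only a printed placeholder for animation.
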(event OnComponentBeginOverlap(Box)
  (params (OverlappedComponent :type Primitive%20Component%20Object%20Reference) (OtherActor :type Actor%20Object%20Reference) (OtherComp :type Primitive%20Component%20Object%20Reference) (OtherBodyIndex :type Integer) (bFromSweep :type Boolean) (SweepResult :type Hit%20Result%20Structure%20%28by%20ref%29))
  ;[0.15 0.15 0.15 0.5] Check if overlaping enemy
  (Utilities|FlowControl|Sequence
    (:then_0
      (Utilities|Casting|CastToBP_NewEnemyDeaf OtherActor))
    (:then_1
      (Utilities|Casting|CastToBP_NewEnemyBlind OtherActor)))
  (Variables|Default|SetCanParry true)
  (Development|PrintString "Can Parry"))

(event OnComponentEndOverlap(Box)
  (params (OverlappedComponent :type Primitive%20Component%20Object%20Reference) (OtherActor :type Actor%20Object%20Reference) (OtherComp :type Primitive%20Component%20Object%20Reference) (OtherBodyIndex :type Integer))
  ;[0.15 0.15 0.15 0.5] Check if overlaping enemy
  (Utilities|FlowControl|Sequence
    (:then_0
      (Utilities|Casting|CastToBP_NewEnemyDeaf OtherActor))
    (:then_1
      (Utilities|Casting|CastToBP_NewEnemyBlind OtherActor)))
  (Variables|Default|SetCanParry false)
  (Development|PrintString "Can't Parry"))

(event Custom|PickupShield
  (bind _charref (Variables|Default|GetCharRef))
  ;[0.15 0.15 0.15 0.5] Adding and removeing shield and shield collisions
  (Variables|/Game/BP_ThirdPersonCharacter.BP_ThirdPersonCharacter_C|SetHasShield _charref true)
  (Transformation|AttachComponentToComponent (Variables|/Script/Engine.Character|GetMesh _charref) "ShieldR" "SnapToTarget" "SnapToTarget" "SnapToTarget" false)
  (Collision|SetCollisionResponsetoChannel (Variables|Default|GetPATCHED_ButtonShield_WIP) "ECC_GameTraceChannel2" "ECR_Ignore")
  (bind _returnvalue (UserInterface|CreateWidget "/Game/Blueprints_UI/WBP_Ojective.WBP_Ojective_C" 0 "Press X/E to Parry"))
  (Default|ObjectiveActive _returnvalue))

(event Custom|RemoveShield
  ;[0.15 0.15 0.15 0.5] Adding and removeing shield and shield collisions
  (Variables|/Game/BP_ThirdPersonCharacter.BP_ThirdPersonCharacter_C|SetHasShield (Variables|Default|GetCharRef) false)
  (Variables|Default|SetCanParry false)
  (Development|PrintString "Shield Removed")
  (Transformation|DetachFromComponent (Variables|Default|GetPATCHED_ButtonShield_WIP) "KeepRelative" "KeepRelative" "KeepRelative" false)
  (Collision|SetCollisionResponsetoChannel (Variables|Default|GetPATCHED_ButtonShield_WIP) "ECC_GameTraceChannel2" "ECR_Block")
  (Actor|DestroyActor))

(event Custom|Parrying
  ;[0.15 0.15 0.15 0.5] Parrying Logic
  (if (Variables|/Game/BP_ThirdPersonCharacter.BP_ThirdPersonCharacter_C|GetHasShield (Variables|Default|GetCharRef))
    (if (Variables|Default|GetCanParry)
      (Variables|Default|SetIsParrying true)
      (Development|PrintText "Parry Animation")
      (Utilities|FlowControl|Delay 1.0)
      (Variables|Default|SetIsParrying false)
      (CallFunction|RemoveShield))))

(event EventBeginPlay
  (bind _asbp_third_person_character (Utilities|Casting|CastToBP_ThirdPersonCharacter (Game|Player|GetPlayerPawn 0)))
  (Variables|Default|SetCharRef _asbp_third_person_character))

(fn ConstructionScript)

(fn Interact
  (params (Character :type BP%20Third%20Person%20Character%20Object%20Reference))
  (if (not (Variables|/Game/BP_ThirdPersonCharacter.BP_ThirdPersonCharacter_C|GetHasShield (Variables|Default|GetCharRef)))
    (CallFunction|PickupShield)
    (return false)))