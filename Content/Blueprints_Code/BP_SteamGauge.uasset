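; Steam gauge actor whose needle sweeps to a fixed angle once StartActive is called.
; StartActive stores the needle's current world pitch, then plays a timeline with its play rate set to the inverse of TimeToFinsh, so that variable controls the sweep time.
; Each timeline update lerps the pitch from the stored value toward the hard-coded target, keeping roll and yaw unchanged.
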(event Custom|StartActive
  (bind _needle (Variables|Default|GetNeedle))
  (bind _returnvalue (Transformation|GetWorldRotation _needle))
  (Variables|Default|SetOriginalY (.pitch _returnvalue))
  (Components|Timeline|SetPlayRate (Variables|Default|GetTimeline) (/ 1.0 (Variables|Default|GetTimeToFinsh)))
  (bind _newtrack_0 (Timeline|Timeline Play)
    (:Update
      (Transformation|SetWorldRotation _needle (Math|Rotator|MakeRotator (.roll _returnvalue) (Math|Float|Lerp (Variables|Default|GetOriginalY) 2.5e+02 _newtrack_0) (.yaw _returnvalue)) false false))))

(fn ConstructionScript)