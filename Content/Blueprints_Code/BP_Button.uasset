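; BP_Button is an interactable button that toggles an outline and plays press and beep sounds when approached.
; BeginPlay adds both audio components and caches the player's BP_ThirdPersonCharacter.
; Sphere overlaps toggle the outline and set NearButton; entering also starts a short one-shot timer that plays both sounds if the character's CanPressButton is true.
; The Interact function is a stub returning false, and the NearButton check is unwired.
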(event OnComponentBeginOverlap(Sphere)
  (params (OverlappedComponent :type Primitive%20Component%20Object%20Reference) (OtherActor :type Actor%20Object%20Reference) (OtherComp :type Primitive%20Component%20Object%20Reference) (OtherBodyIndex :type Integer) (bFromSweep :type Boolean) (SweepResult :type Hit%20Result%20Structure%20%28by%20ref%29))
  (Rendering|ToggleVisibility (Variables|Default|GetOutline) false)
  (Variables|Default|SetNearButton true)
  (Utilities|Time|SetTimerbyEvent (delegate Custom|CustomEvent) 0.1))

(event OnComponentEndOverlap(Sphere)
  (params (OverlappedComponent :type Primitive%20Component%20Object%20Reference) (OtherActor :type Actor%20Object%20Reference) (OtherComp :type Primitive%20Component%20Object%20Reference) (OtherBodyIndex :type Integer))
  (Rendering|ToggleVisibility (Variables|Default|GetOutline) true)
  (Variables|Default|SetNearButton false))

(event Custom|CustomEvent
  (if (Variables|/Game/BP_ThirdPersonCharacter.BP_ThirdPersonCharacter_C|GetCanPressButton (Variables|Default|GetCharRef))
    (Development|PrintString "PlaySFX")
    (Audio|Components|Audio|Play (Variables|Default|GetPress) 0.0)
    (Audio|Components|Audio|Play (Variables|Default|GetBeep) 0.0)))

(event EventBeginPlay
  (bind _returnvalue (AddComponent|AddAudioComponent false))
  (Variables|Default|SetPress _returnvalue)
  (bind _returnvalue_2 (AddComponent|AddAudioComponent false))
  (Variables|Default|SetBeep _returnvalue_2)
  (bind _asbp_third_person_character (Utilities|Casting|CastToBP_ThirdPersonCharacter (Game|Player|GetPlayerPawn 0)))
  (Variables|Default|SetCharRef _asbp_third_person_character))

(fn ConstructionScript)

(fn Interact
  (params (Character :type BP%20Third%20Person%20Character%20Object%20Reference))
  ;[0.15 0.15 0.15 0.5] Button Interaction
  (return false))