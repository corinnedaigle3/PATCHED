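; BP_SaveGame is a save game object that coordinates saving and loading by handing itself to saveable objects.
; SaveAllData and LoadDataForAll loop over the supplied objects and send each a save or load message, while LoadDataForRequester loads a single object.
; Each receiver handles its own data in its SaveDataMessage and LoadDataMessage implementations, so these functions hold no object-specific logic.
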(fn SaveAllData
  (params (NewParam :type Array%20of%20Object%20Object%20References))
  (for _array_element NewParam
    (Class|BPISaveable|SaveData(Message) _array_element self))
  (return))

(fn LoadDataforRequester
  (params (Requester :type Object%20Object%20Reference))
  (Class|BPISaveable|LoadData(Message) Requester self)
  (return))

(fn LoadDataforAll
  (params (Saveables :type Array%20of%20Object%20Object%20References))
  (for _array_element Saveables
    (Class|BPISaveable|LoadData(Message) _array_element self))
  (return))