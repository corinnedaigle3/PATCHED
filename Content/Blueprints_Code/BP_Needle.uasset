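; BP_Needle is an interactable needle item that the third-person character can carry in hand or wear on the hip, where it grants grapple.
; Interact calls PickUpNeedle when hands are free, playing audio, disabling physics and collision responses, and snapping to a carry socket.
; AttachNeedle moves it to the hip socket and sets the character's needle and grapple flags; its call within Interact is unreachable.
; DropNeedle detaches it and restores blocking, but leaves physics simulation off.
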(event Custom|AttachNeedle
  (bind _charref (Variables|Default|GetCharRef))
  (Variables|/Game/BP_ThirdPersonCharacter.BP_ThirdPersonCharacter_C|SetHasItemInHand _charref false)
  (Variables|/Game/BP_ThirdPersonCharacter.BP_ThirdPersonCharacter_C|SetNeedleInHand _charref false)
  (bind _output_get (Variables|/Game/BP_ThirdPersonCharacter.BP_ThirdPersonCharacter_C|SetHasNeedle _charref true))
  (Variables|/Game/BP_ThirdPersonCharacter.BP_ThirdPersonCharacter_C|SetHasGrapple _charref _output_get)
  (Transformation|DetachFromComponent (Variables|Default|GetNeedle) "KeepWorld" "KeepWorld" "KeepWorld" false)
  (Transformation|AttachComponentToComponent (Variables|/Script/Engine.Character|GetMesh _charref) "AttachNeedleL" "SnapToTarget" "SnapToTarget" "SnapToTarget" false)
  (Development|PrintString "NeedleOnHip"))

(event Custom|PickUpNeedle
  (bind _charref (Variables|Default|GetCharRef))
  (bind _charref_2 (Variables|Default|GetCharRef))
  ;[0.15 0.15 0.15 0.5] Pick up voicebox
  (if (not (Variables|/Game/BP_ThirdPersonCharacter.BP_ThirdPersonCharacter_C|GetHasItemInHand _charref_2))
    (Variables|/Game/BP_ThirdPersonCharacter.BP_ThirdPersonCharacter_C|SetPickUpNeedle _charref_2 self)
    (Variables|Default|SetNeedlePicked true)
    (Audio|Components|Audio|Play (Variables|Default|GetPickUp) 0.0)
    (Physics|SetSimulatePhysics (Variables|Default|GetNeedle) false)
    (Variables|/Game/BP_ThirdPersonCharacter.BP_ThirdPersonCharacter_C|SetHasItemInHand _charref true)
    (Variables|/Game/BP_ThirdPersonCharacter.BP_ThirdPersonCharacter_C|SetNeedleInHand _charref true)
    (Transformation|AttachComponentToComponent (Variables|/Script/Engine.Character|GetMesh _charref) "CarryLegR" "SnapToTarget" "SnapToTarget" "SnapToTarget" false)
    (Collision|SetCollisionResponsetoChannel (Variables|Default|GetNeedle) "ECC_GameTraceChannel2" "ECR_Ignore")
    (Collision|SetCollisionResponsetoChannel (Variables|Default|GetNeedle) "ECC_Pawn" "ECR_Ignore")))

(event Custom|DropNeedle
  (bind _charref (Variables|Default|GetCharRef))
  (Transformation|DetachFromComponent (Variables|Default|GetNeedle) "KeepRelative" "KeepRelative" "KeepRelative" false)
  (Collision|SetCollisionResponsetoChannel (Variables|Default|GetNeedle) "ECC_GameTraceChannel2" "ECR_Block")
  (Collision|SetCollisionResponsetoChannel (Variables|Default|GetNeedle) "ECC_Pawn" "ECR_Block")
  (Physics|SetSimulatePhysics (Variables|Default|GetNeedle) false)
  (Variables|/Game/BP_ThirdPersonCharacter.BP_ThirdPersonCharacter_C|SetHasItemInHand _charref false)
  (Variables|/Game/BP_ThirdPersonCharacter.BP_ThirdPersonCharacter_C|SetNeedleInHand _charref false))

(event EventBeginPlay
  (bind _asbp_third_person_character (Utilities|Casting|CastToBP_ThirdPersonCharacter (Game|Player|GetPlayerPawn 0)))
  (Variables|Default|SetCharRef _asbp_third_person_character)
  (bind _returnvalue (AddComponent|AddAudioComponent false))
  (Variables|Default|SetPickUp _returnvalue))

(fn ConstructionScript)

(fn Interact
  (params (Character :type BP%20Third%20Person%20Character%20Object%20Reference))
  (if (not (Variables|/Game/BP_ThirdPersonCharacter.BP_ThirdPersonCharacter_C|GetHasItemInHand (Variables|Default|GetCharRef)))
    (CallFunction|PickUpNeedle)
    (return false)))