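; Interactable arm pickup that the player character carries in hand and can later attach to recover a body part.
; Interact calls PickUpArm if no limb is held, which plays audio, disables physics, snaps to the CarryLimbR socket and sets the character's carry flags.
; AttachArm, not called within this Blueprint, passes BodyPartType to the character's RecoverALive, destroys the actor and clears those flags.
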(event Custom|AttachArm
  (bind _bodyparttype (Variables|Default|GetBodyPartType))
  (bind _charref (Variables|Default|GetCharRef))
  ;[0.15 0.15 0.15 0.5] Attach arm to body
  (Default|RecoverALive (Variables|Default|GetCharRef) _bodyparttype)
  (Development|PrintString (Utilities|String|EnumtoString _bodyparttype))
  (Actor|DestroyActor)
  (Variables|/Game/BP_ThirdPersonCharacter.BP_ThirdPersonCharacter_C|SetHasLimbInHand _charref false)
  (Variables|/Game/BP_ThirdPersonCharacter.BP_ThirdPersonCharacter_C|SetArmInHand _charref false)
  (Development|PrintString "destroy" true true "(R=1.000000,G=0.000000,B=0.054998,A=1.000000)"))

(event Custom|PickUpArm
  (bind _charref (Variables|Default|GetCharRef))
  ;[0.15 0.15 0.15 0.5] Pick up arm
  (if (not (Variables|/Game/BP_ThirdPersonCharacter.BP_ThirdPersonCharacter_C|GetHasLimbInHand (Variables|Default|GetCharRef)))
    (Variables|Default|SetpickedUp true)
    (Audio|Components|Audio|Play (Variables|Default|GetPickUp) 0.0)
    (Physics|SetSimulatePhysics (Variables|Default|GetArm) false)
    (Variables|/Game/BP_ThirdPersonCharacter.BP_ThirdPersonCharacter_C|SetHasLimbInHand _charref true)
    (Variables|/Game/BP_ThirdPersonCharacter.BP_ThirdPersonCharacter_C|SetArmInHand _charref true)
    (Transformation|AttachComponentToComponent (Variables|/Script/Engine.Character|GetMesh _charref) "CarryLimbR" "SnapToTarget" "SnapToTarget" "SnapToTarget" false)
    (Collision|SetCollisionResponsetoChannel (Variables|Default|GetArm) "ECC_GameTraceChannel2" "ECR_Ignore")
    (Development|PrintString "PickedUpArm" true true "(R=0.839272,G=1.000000,B=0.000000,A=1.000000)")))

(event EventBeginPlay
  (bind _asbp_third_person_character (Utilities|Casting|CastToBP_ThirdPersonCharacter (Game|Player|GetPlayerPawn 0)))
  (Variables|Default|SetCharRef _asbp_third_person_character)
  (bind _returnvalue (AddComponent|AddAudioComponent false))
  (Variables|Default|SetPickUp _returnvalue))

(fn ConstructionScript)

(fn Interact
  (params (Character :type BP%20Third%20Person%20Character%20Object%20Reference))
  ;[0.15 0.15 0.15 0.5] Interact
  (if (not (Variables|/Game/BP_ThirdPersonCharacter.BP_ThirdPersonCharacter_C|GetHasLimbInHand (Variables|Default|GetCharRef)))
    (CallFunction|PickUpArm)
    (return false)))