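; Sliding door that unlocks when the player enters three correct voice box choices in order.
; While the player is in the trigger box, a timer polls the character's choice through three chained lock checks, each lighting a bulb green.
; The first two steps start a reset timer that clears progress on expiry; the third slides the door open via timeline.
; First overlap can trigger a tutorial page.
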(event OnComponentBeginOverlap(Box)
  (params (OverlappedComponent :type Primitive%20Component%20Object%20Reference) (OtherActor :type Actor%20Object%20Reference) (OtherComp :type Primitive%20Component%20Object%20Reference) (OtherBodyIndex :type Integer) (bFromSweep :type Boolean) (SweepResult :type Hit%20Result%20Structure%20%28by%20ref%29))
  ;[0.15 0.15 0.15 0.5] Near Door Check
  (Utilities|Casting|CastToBP_ThirdPersonCharacter OtherActor)
  (if (Variables|Default|GetTutorial)
    (Utilities|FlowControl|DoOnce false
      (:Completed
        (bind _returnvalue (Actor|GetActorOfClass "/Game/Blueprints_Code/UI/BP_TutorialTrigger.BP_TutorialTrigger_C"))
        (Variables|Default|SetTutorialRef _returnvalue)
        (Variables|/Game/Blueprints_Code/UI/BP_TutorialTrigger.BP_TutorialTrigger_C|SetTutorialInstance (Variables|Default|GetTutorialRef) 1)
        (Default|TriggerWBPTutorialPage (Variables|Default|GetTutorialRef))
        (Variables|Default|SetTutorial false))))
  (if (not (Variables|Default|GetDOOR%20OPENED))
    (Variables|/Game/BP_ThirdPersonCharacter.BP_ThirdPersonCharacter_C|SetNearVADoor (Variables|Default|GetCharRef) true)
    (Variables|Default|SetLooping true)
    (Utilities|Time|SetTimerbyEvent (delegate Custom|PlayerIsNear) 0.08 (Variables|Default|GetLooping))))

(event OnComponentEndOverlap(Box)
  (params (OverlappedComponent :type Primitive%20Component%20Object%20Reference) (OtherActor :type Actor%20Object%20Reference) (OtherComp :type Primitive%20Component%20Object%20Reference) (OtherBodyIndex :type Integer))
  (bind _charref (Variables|Default|GetCharRef))
  ;[0.15 0.15 0.15 0.5] Near Door Check
  (Utilities|Casting|CastToBP_ThirdPersonCharacter OtherActor)
  (if (not (Variables|Default|GetDOOR%20OPENED))
    (Variables|/Game/BP_ThirdPersonCharacter.BP_ThirdPersonCharacter_C|SetNearVADoor _charref false)
    (Variables|/Game/BP_ThirdPersonCharacter.BP_ThirdPersonCharacter_C|SetCanOpenDoor _charref false)
    (Variables|Default|SetLooping false)))

(event Custom|TimeIsUp
  ;[0.15 0.15 0.15 0.5] Lock Check
  (Variables|/Game/BP_ThirdPersonCharacter.BP_ThirdPersonCharacter_C|SetVoiceBoxChoice (Variables|Default|GetCharRef) "NewEnumerator6")
  (Audio|PlaySound2D "/Game/Audio/SFX/GameMech/SFX_LockedDoor.SFX_LockedDoor" 1.0 1.0 0.0 0 0)
  (Variables|Default|SetUnlock1 false)
  (Variables|Default|SetUnlock2 false)
  (CallFunction|SetBulbDefault)
  (Utilities|FlowControl|Sequence
    (:then_0
      (Utilities|FlowControl|DoOnce false) ; enters at Reset
    )
    (:then_1
      (Utilities|FlowControl|DoOnce false) ; enters at Reset
    )))

(event Custom|SlideDoor
  ;[0.15 0.15 0.15 0.5] Open Door
  (if (Variables|Default|GetDOOR%20OPENED)
    (Utilities|FlowControl|Delay 1.0)
    (Audio|PlaySound2D "/Game/Audio/SFX/GameMech/SFX_UnlockOpenDoor.SFX_UnlockOpenDoor" 1.0 1.0 0.0 0 0)
    (bind _newtrack_0 (Timeline|Open/CloseDoor Play)
      (:Update
        (Transformation|SetRelativeLocation (Variables|Default|Getsliding_door) (Math|Vector|MakeVector 0.0 (Math|Float|Lerp 0.0 (Variables|Default|GetSlideDistance) _newtrack_0) 8.0) false false)))))

(event Custom|Lock
  ;[0.15 0.15 0.15 0.5] Lock Check
  (if (Utilities|Enum|Equal(Enum) (Variables|/Game/BP_ThirdPersonCharacter.BP_ThirdPersonCharacter_C|GetVoiceBoxChoice (Variables|Default|GetCharRef)) (Variables|Default|GetCorrectChoice))
    (Rendering|Material|SetMaterial (Variables|Default|GetSphere) 0 "/Game/Levels/Emissive/GreenLight.GreenLight")
    (bind _returnvalue (Utilities|Time|SetTimerbyEvent (delegate Custom|TimeIsUp) (Variables|Default|GetResetTimer)))
    (Variables|Default|SetTimer _returnvalue)
    (Variables|Default|SetUnlock1 true)
    (Utilities|FlowControl|DoOnce false
      (:Completed
        (Variables|/Game/BP_ThirdPersonCharacter.BP_ThirdPersonCharacter_C|SetVoiceBoxChoice (Variables|Default|GetCharRef) "NewEnumerator6")))
    (else
      (CallFunction|WrongChoice))))

(event Custom|Lock1
  ;[0.15 0.15 0.15 0.5] Lock Check
  (if (Variables|Default|GetUnlock1)
    (if (Utilities|Enum|Equal(Enum) (Variables|/Game/BP_ThirdPersonCharacter.BP_ThirdPersonCharacter_C|GetVoiceBoxChoice (Variables|Default|GetCharRef)) (Variables|Default|GetCorrectChoice_1))
      (Utilities|Time|ClearandInvalidateTimerbyHandle (Variables|Default|GetTimer))
      (Rendering|Material|SetMaterial (Variables|Default|GetSphere1) 0 "/Game/Levels/Emissive/GreenLight.GreenLight")
      (bind _returnvalue (Utilities|Time|SetTimerbyEvent (delegate Custom|TimeIsUp) (Variables|Default|GetResetTimer)))
      (Variables|Default|SetTimer1 _returnvalue)
      (Variables|Default|SetUnlock2 true)
      (Utilities|FlowControl|DoOnce false
        (:Completed
          (Variables|/Game/BP_ThirdPersonCharacter.BP_ThirdPersonCharacter_C|SetVoiceBoxChoice (Variables|Default|GetCharRef) "NewEnumerator6")))
      (else
        (CallFunction|WrongChoice)))))

(event Custom|Lock2
  ;[0.15 0.15 0.15 0.5] Lock Check
  (if (Variables|Default|GetUnlock2)
    (if (Utilities|Enum|Equal(Enum) (Variables|/Game/BP_ThirdPersonCharacter.BP_ThirdPersonCharacter_C|GetVoiceBoxChoice (Variables|Default|GetCharRef)) (Variables|Default|GetCorrectChoice_2))
      (Utilities|Time|ClearandInvalidateTimerbyHandle (Variables|Default|GetTimer1))
      (Rendering|Material|SetMaterial (Variables|Default|GetSphere2) 0 "/Game/Levels/Emissive/GreenLight.GreenLight")
      (Variables|Default|SetDOOR%20OPENED true)
      (Collision|SetCollisionEnabled (Variables|Default|GetBox) "NoCollision")
      (Variables|/Game/BP_ThirdPersonCharacter.BP_ThirdPersonCharacter_C|SetVoiceBoxChoice (Variables|Default|GetCharRef) "NewEnumerator6")
      (CallFunction|SlideDoor)
      (else
        (CallFunction|WrongChoice)))))

(event Custom|SetBulbDefault
  ;[0.15 0.15 0.15 0.5] Lock Check
  (Rendering|Material|SetMaterial (Variables|Default|GetSphere) 0 "/Game/Art/M_Outline.M_Outline")
  (Rendering|Material|SetMaterial (Variables|Default|GetSphere1) 0 "/Game/Art/M_Outline.M_Outline")
  (Rendering|Material|SetMaterial (Variables|Default|GetSphere2) 0 "/Game/Art/M_Outline.M_Outline"))

(event Custom|PlayerIsNear
  ;[0.15 0.15 0.15 0.5] Lock Check
  (if (Utilities|Enum|NotEqual(Enum) "NewEnumerator6" (Variables|/Game/BP_ThirdPersonCharacter.BP_ThirdPersonCharacter_C|GetVoiceBoxChoice (Variables|Default|GetCharRef)))
    (if (Variables|/Game/BP_ThirdPersonCharacter.BP_ThirdPersonCharacter_C|GetNearVADoor (Variables|Default|GetCharRef))
      (if (not (Variables|Default|GetDOOR%20OPENED))
        (if (Variables|/Game/BP_ThirdPersonCharacter.BP_ThirdPersonCharacter_C|GetCanOpenDoor (Variables|Default|GetCharRef))
          (CallFunction|Lock)
          (CallFunction|Lock1)
          (CallFunction|Lock2))))))

(event Custom|WrongChoice
  ;[0.15 0.15 0.15 0.5] Wrong choice
  (if (Variables|/Game/BP_ThirdPersonCharacter.BP_ThirdPersonCharacter_C|GetVoiceBoxOpen (Variables|Default|GetCharRef))
    (Utilities|FlowControl|DoOnce false :!label _label
      (:Completed
        (Audio|PlaySound2D "/Game/Audio/SFX/GameMech/SFX_LockedDoor.SFX_LockedDoor" 1.0 1.0 0.0 0 0)))
    (else
      (goto _label Reset))))

(event EventBeginPlay
  (bind _asbp_third_person_character (Utilities|Casting|CastToBP_ThirdPersonCharacter (Game|Player|GetPlayerPawn 0)))
  (Variables|Default|SetCharRef _asbp_third_person_character)
  (CallFunction|SetBulbDefault))

(fn ConstructionScript)