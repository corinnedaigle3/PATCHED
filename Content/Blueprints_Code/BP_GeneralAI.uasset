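; BP_GeneralAI is an enemy character that patrols a looping list of waypoints and costs the player a life on contact.
; A recursive FollowPath event waits, then uses AIMoveTo to reach each waypoint in turn.
; A Box overlap with BP_ThirdPersonCharacter calls LoseALive, stops movement and sets a timed CatchedPlayer flag.
; While that flag is set, FollowPath keeps retrying after its delay instead of moving.
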(event OnComponentBeginOverlap(Box)
  (params (OverlappedComponent :type Primitive%20Component%20Object%20Reference) (OtherActor :type Actor%20Object%20Reference) (OtherComp :type Primitive%20Component%20Object%20Reference) (OtherBodyIndex :type Integer) (bFromSweep :type Boolean) (SweepResult :type Hit%20Result%20Structure%20%28by%20ref%29))
  (bind _charactermovement (Variables|Character|GetCharacterMovement))
  ;[0.15 0.15 0.15 0.5] Behavior for when the player loses a life
  (bind _asbp_third_person_character (Utilities|Casting|CastToBP_ThirdPersonCharacter OtherActor))
  (Default|LoseALive _asbp_third_person_character)
  (Class|NavMovementInterface|StopActiveMovement _charactermovement)
  (Components|Movement|StopMovementImmediately _charactermovement)
  (CallFunction|CatchedthePlayer 5.0))

(event Custom|Follow%20Path
  ;[0.15 0.15 0.15 0.5] Waypoint system
  (Variables|/Script/Engine.CharacterMovementComponent|SetMaxWalkSpeed (Variables|Character|GetCharacterMovement) 3e+02)
  (Utilities|FlowControl|Delay 3.0)
  (if (not (Variables|Default|GetCatchedPlayer))
    (AI|AIMoveTo self "0, 0, 0" (Utilities|Array|Get(acopy) (Variables|Default|Getwaypoints) (Variables|Default|GetcurrentWaypoint)) 5.0 false
      (:OnSuccess
        (Math|Integer|IncrementInt (Variables|Default|GetcurrentWaypoint)
          (:%20%20
            (if (>= (Variables|Default|GetcurrentWaypoint) (Utilities|Array|Length (Variables|Default|Getwaypoints)))
              (Variables|Default|SetcurrentWaypoint 0))
            (Utilities|FlowControl|Delay 0.1)
            (CallFunction|FollowPath)))))
    (else
      (CallFunction|FollowPath))))

(event Custom|CatchedThePlayer
  (params (WaitForSeconds :type Float%20%28double-precision%29))
  ;[0.15 0.15 0.15 0.5] Determines if the player has been caught or not
  (Variables|Default|SetCatchedPlayer true)
  (Utilities|FlowControl|Delay WaitForSeconds)
  (Variables|Default|SetCatchedPlayer false))

(event EventBeginPlay
  (CallFunction|FollowPath))

(fn ConstructionScript)