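; BP_ObjectivePoint is a trigger volume that announces an objective to the player on screen.
; It creates a WBP_Ojective widget at BeginPlay and sizes its box from ObjectiveBoxSize in the construction script.
; The first player overlap plays a sound, fades the objective text in and out, then clears ObjectiveInProgress.
; A CompletedObjective event reuses the widget to flash a completion message.
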(event OnComponentBeginOverlap(ObjectiveBox)
  (params (OverlappedComponent :type Primitive%20Component%20Object%20Reference) (OtherActor :type Actor%20Object%20Reference) (OtherComp :type Primitive%20Component%20Object%20Reference) (OtherBodyIndex :type Integer) (bFromSweep :type Boolean) (SweepResult :type Hit%20Result%20Structure%20%28by%20ref%29))
  (bind _wbp_objectivewidgetref (Variables|Default|GetWBP_ObjectiveWidgetRef))
  (bind _wbp_objectivewidgetref_2 (Variables|Default|GetWBP_ObjectiveWidgetRef))
  (if (== OtherActor (Game|GetPlayerCharacter 0))
    (Utilities|FlowControl|DoOnce false
      (:Completed
        (Variables|/Game/Blueprints_UI/WBP_Ojective.WBP_Ojective_C|SetObjectiveContentText (Variables|Default|GetWBP_ObjectiveWidgetRef) (Variables|Default|GetObjectiveContentTest))
        (Audio|PlaySound2D "/Game/Audio/SFX/sfx_placeHolder.SFX_placeHolder" 1.0 1.0 0.0 0 0)
        (UserInterface|Viewport|AddtoViewport _wbp_objectivewidgetref 0)
        (UserInterface|Animation|PlayAnimation _wbp_objectivewidgetref (Variables|/Game/Blueprints_UI/WBP_Ojective.WBP_Ojective_C|GetObjectiveFade _wbp_objectivewidgetref) 0.0 1 "Forward" 1.0 false)
        (Utilities|FlowControl|Delay 2.0)
        (UserInterface|Animation|PlayAnimation _wbp_objectivewidgetref_2 (Variables|/Game/Blueprints_UI/WBP_Ojective.WBP_Ojective_C|GetObjectiveFade _wbp_objectivewidgetref_2) 0.0 1 "Reverse" 1.0 false)
        (Variables|Default|SetObjectiveInProgress false)))))

(event Custom|CompletedObjective
  (bind _wbp_objectivewidgetref (Variables|Default|GetWBP_ObjectiveWidgetRef))
  (bind _wbp_objectivewidgetref_2 (Variables|Default|GetWBP_ObjectiveWidgetRef))
  (Variables|/Game/Blueprints_UI/WBP_Ojective.WBP_Ojective_C|SetObjectiveContentText (Variables|Default|GetWBP_ObjectiveWidgetRef) "Completed Objective")
  (Audio|PlaySound2D "/Game/Audio/SFX/sfx_placeHolder.SFX_placeHolder" 1.0 1.0 0.0 0 0)
  (UserInterface|Viewport|AddtoViewport _wbp_objectivewidgetref_2 0)
  (UserInterface|Animation|PlayAnimation _wbp_objectivewidgetref_2 (Variables|/Game/Blueprints_UI/WBP_Ojective.WBP_Ojective_C|GetObjectiveFade _wbp_objectivewidgetref_2) 0.0 1 "Forward" 1.0 false)
  (Utilities|FlowControl|Delay 0.5)
  (UserInterface|Animation|PlayAnimation _wbp_objectivewidgetref (Variables|/Game/Blueprints_UI/WBP_Ojective.WBP_Ojective_C|GetObjectiveFade _wbp_objectivewidgetref) 0.0 1 "Reverse" 1.0 false))

(event EventBeginPlay
  (bind _returnvalue (UserInterface|CreateWidget "/Game/Blueprints_UI/WBP_Ojective.WBP_Ojective_C" 0 (Variables|Default|GetObjectiveContentTest)))
  (Variables|Default|SetWBP_ObjectiveWidgetRef _returnvalue))

(event Collision|EventActorBeginOverlap
  (params (OtherActor :type Actor%20Object%20Reference)))

(event EventTick
  (params (DeltaSeconds :type Float%20%28single-precision%29)))

(fn ConstructionScript
  (Components|Box|SetBoxExtent (Variables|Default|GetObjectiveBox) (Variables|Default|GetObjectiveBoxSize) true))