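; Vertical moving platform that starts when the player interacts empty-handed with its button, a one-time press that slides in and removes its highlight outline.
; Once active, Tick moves the cube between height limits, pausing at each end and toggling conveyor audio through paired DoOnce nodes.
; An overlap box attaches and detaches the riding character, while a Kill volume calls HazardDeath on the player.
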(event OnComponentEndOverlap(Box)
  (params (OverlappedComponent :type Primitive%20Component%20Object%20Reference) (OtherActor :type Actor%20Object%20Reference) (OtherComp :type Primitive%20Component%20Object%20Reference) (OtherBodyIndex :type Integer))
  ;[0.15 0.15 0.15 0.5] If Player Overlaps - Activate
  (bind _asbp_third_person_character (Utilities|Casting|CastToBP_ThirdPersonCharacter OtherActor))
  (Transformation|DetachFromActor _asbp_third_person_character "KeepRelative" "KeepRelative" "KeepRelative"))

(event OnComponentBeginOverlap(Kill)
  (params (OverlappedComponent :type Primitive%20Component%20Object%20Reference) (OtherActor :type Actor%20Object%20Reference) (OtherComp :type Primitive%20Component%20Object%20Reference) (OtherBodyIndex :type Integer) (bFromSweep :type Boolean) (SweepResult :type Hit%20Result%20Structure%20%28by%20ref%29))
  ;[0.15 0.15 0.15 0.5] Move Platform Logic
  (Default|HazardDeath (Variables|Default|GetCharREF)))

(event OnComponentBeginOverlap(Box)
  (params (OverlappedComponent :type Primitive%20Component%20Object%20Reference) (OtherActor :type Actor%20Object%20Reference) (OtherComp :type Primitive%20Component%20Object%20Reference) (OtherBodyIndex :type Integer) (bFromSweep :type Boolean) (SweepResult :type Hit%20Result%20Structure%20%28by%20ref%29))
  ;[0.15 0.15 0.15 0.5] If Player Overlaps - Activate
  (bind _asbp_third_person_character (Utilities|Casting|CastToBP_ThirdPersonCharacter OtherActor))
  (Transformation|AttachComponentToComponent _asbp_third_person_character 0 "None" "KeepWorld" "KeepWorld" "KeepWorld" true))

(event OnComponentBeginOverlap(Sphere)
  (params (OverlappedComponent :type Primitive%20Component%20Object%20Reference) (OtherActor :type Actor%20Object%20Reference) (OtherComp :type Primitive%20Component%20Object%20Reference) (OtherBodyIndex :type Integer) (bFromSweep :type Boolean) (SweepResult :type Hit%20Result%20Structure%20%28by%20ref%29))
  ;[0.15 0.15 0.15 0.5] Button
  ;;[0.15 0.15 0.15 0.5] Outline visablity of button
  (Utilities|IsValid (Variables|Default|GetOutline)
    (:Is%20Valid
      (Rendering|ToggleVisibility (Variables|Default|GetOutline) false))))

(event OnComponentEndOverlap(Sphere)
  (params (OverlappedComponent :type Primitive%20Component%20Object%20Reference) (OtherActor :type Actor%20Object%20Reference) (OtherComp :type Primitive%20Component%20Object%20Reference) (OtherBodyIndex :type Integer))
  ;[0.15 0.15 0.15 0.5] Button
  ;;[0.15 0.15 0.15 0.5] Outline visablity of button
  (Utilities|IsValid (Variables|Default|GetOutline)
    (:Is%20Valid
      (Rendering|ToggleVisibility (Variables|Default|GetOutline) true))))

(event Custom|PlaySFX
  (bind _sfx_conveyor (Variables|Default|GetSFX_Conveyor))
  ;[0.15 0.15 0.15 0.5] SFX
  (Utilities|FlowControl|DoOnce false
    (:Completed
      (Audio|Components|Audio|Play _sfx_conveyor 0.0)
      (Utilities|FlowControl|DoOnce false) ; enters at Reset
    )))

(event Custom|StopSFX
  (bind _sfx_conveyor (Variables|Default|GetSFX_Conveyor))
  ;[0.15 0.15 0.15 0.5] SFX
  (Utilities|FlowControl|DoOnce false
    (:Completed
      (Audio|Components|Audio|Stop _sfx_conveyor)
      (Utilities|FlowControl|DoOnce false) ; enters at Reset
    )))

(event Custom|PlatformButtonActivate
  ;[0.15 0.15 0.15 0.5] Button
  (Variables|Default|SetActivated true)
  (Audio|Components|Audio|Play (Variables|Default|GetPress) 0.0)
  (Audio|Components|Audio|Play (Variables|Default|GetBeep) 0.0)
  (Components|DestroyComponent (Variables|Default|GetOutline)))

(event Custom|Button%20Pressed
  ;[0.15 0.15 0.15 0.5] Button
  (bind _newtrack_0 (Timeline|Timeline Play)
    (:Update
      (Transformation|SetRelativeLocation (Variables|Default|Getpressable_button) (Math|Vector|MakeVector -3e+01 3e+01 (Math|Float|Lerp 0.0 (Variables|Default|GetSlide%20distance) _newtrack_0)) false false))))

(event EventBeginPlay
  ;[0.15 0.15 0.15 0.5] Player REF
  (bind _asbp_third_person_character (Utilities|Casting|CastToBP_ThirdPersonCharacter (Game|GetPlayerCharacter 0)))
  (Variables|Default|SetCharREF _asbp_third_person_character)
  (bind _returnvalue (AddComponent|AddAudioComponent false))
  (Variables|Default|SetPress _returnvalue)
  (bind _returnvalue_2 (AddComponent|AddAudioComponent false))
  (Variables|Default|SetBeep _returnvalue_2))

(event EventTick
  (params (DeltaSeconds :type Float%20%28single-precision%29))
  (bind _speed (Variables|Default|GetSpeed))
  (bind _speed_2 (Variables|Default|GetSpeed))
  (bind _cube (Variables|Default|GetCube))
  (bind _cube_2 (Variables|Default|GetCube))
  (bind _relativelocation (Variables|/Script/Engine.SceneComponent|GetRelativeLocation _cube_2))
  (bind _relativelocation_2 (Variables|/Script/Engine.SceneComponent|GetRelativeLocation _cube))
  (bind _returnvalue (+ (.z _relativelocation) _speed_2))
  (bind _returnvalue_2 (- (.z _relativelocation_2) _speed))
  ;[0.15 0.15 0.15 0.5] Move Platform Logic
  (if (Variables|Default|GetActivated)
    (CallFunction|PlaySFX)
    (if (Variables|Default|GetGoingBack)
      (Transformation|SetRelativeLocation _cube (Math|Vector|MakeVector (.x _relativelocation_2) (.y _relativelocation_2) _returnvalue_2) false false)
      (if (<= _returnvalue_2 (Variables|Default|GetLowestPoint))
        (Variables|Default|SetActivated false)
        (CallFunction|StopSFX)
        (Utilities|FlowControl|Delay (Variables|Default|GetStopDelay))
        (Variables|Default|SetGoingBack false)
        (Variables|Default|SetActivated true))
      (else
        (Transformation|SetRelativeLocation _cube_2 (Math|Vector|MakeVector (.x _relativelocation) (.y _relativelocation) _returnvalue) false false)
        (if (<= (Variables|Default|GetHighestPoint) _returnvalue)
          (Variables|Default|SetActivated false)
          (CallFunction|StopSFX)
          (Utilities|FlowControl|Delay (Variables|Default|GetStopDelay))
          (Variables|Default|SetGoingBack true)
          (Variables|Default|SetActivated true))))))

(fn ConstructionScript)

(fn Interact
  (params (Character :type BP%20Third%20Person%20Character%20Object%20Reference))
  (if (not (Variables|/Game/BP_ThirdPersonCharacter.BP_ThirdPersonCharacter_C|GetHasItemInHand Character))
    (if (not (Variables|Default|GetInteracted))
      (Variables|Default|SetInteracted true)
      (CallFunction|ButtonPressed)
      (CallFunction|PlatformButtonActivate)
      (return false))))