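; Vertical moving platform that travels between a lowest and highest point, pausing at each end before reversing.
; PlatformActivate starts it through a DoOnce that resets at the bottom, and Tick moves the cube by a fixed per-frame step while Activated.
; One trigger box attaches the player character on overlap and detaches it on exit.
; A second box halts movement while overlapped and resumes it afterwards.
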(event OnComponentEndOverlap(Box)
  (params (OverlappedComponent :type Primitive%20Component%20Object%20Reference) (OtherActor :type Actor%20Object%20Reference) (OtherComp :type Primitive%20Component%20Object%20Reference) (OtherBodyIndex :type Integer))
  ;[0.15 0.15 0.15 0.5] If Player Overlaps - Activate
  (bind _asbp_third_person_character (Utilities|Casting|CastToBP_ThirdPersonCharacter OtherActor))
  (Transformation|DetachFromActor _asbp_third_person_character "KeepRelative" "KeepRelative" "KeepRelative"))

(event OnComponentBeginOverlap(Box1)
  (params (OverlappedComponent :type Primitive%20Component%20Object%20Reference) (OtherActor :type Actor%20Object%20Reference) (OtherComp :type Primitive%20Component%20Object%20Reference) (OtherBodyIndex :type Integer) (bFromSweep :type Boolean) (SweepResult :type Hit%20Result%20Structure%20%28by%20ref%29))
  (Variables|Default|SetActivated false))

(event OnComponentBeginOverlap(Box)
  (params (OverlappedComponent :type Primitive%20Component%20Object%20Reference) (OtherActor :type Actor%20Object%20Reference) (OtherComp :type Primitive%20Component%20Object%20Reference) (OtherBodyIndex :type Integer) (bFromSweep :type Boolean) (SweepResult :type Hit%20Result%20Structure%20%28by%20ref%29))
  ;[0.15 0.15 0.15 0.5] If Player Overlaps - Activate
  (bind _asbp_third_person_character (Utilities|Casting|CastToBP_ThirdPersonCharacter OtherActor))
  (Transformation|AttachComponentToComponent _asbp_third_person_character 0 "None" "KeepWorld" "KeepWorld" "KeepWorld" true))

(event OnComponentEndOverlap(Box1)
  (params (OverlappedComponent :type Primitive%20Component%20Object%20Reference) (OtherActor :type Actor%20Object%20Reference) (OtherComp :type Primitive%20Component%20Object%20Reference) (OtherBodyIndex :type Integer))
  (Variables|Default|SetActivated true))

(event Custom|PlatformActivate
  ;[0.15 0.15 0.15 0.5] Move Platform Logic
  (Utilities|FlowControl|DoOnce false
    (:Completed
      (Variables|Default|SetActivated true))))

(event EventBeginPlay
  ;[0.15 0.15 0.15 0.5] Player REF
  (bind _asbp_third_person_character (Utilities|Casting|CastToBP_ThirdPersonCharacter (Game|GetPlayerCharacter 0)))
  (Variables|Default|SetCharREF _asbp_third_person_character))

(event EventTick
  (params (DeltaSeconds :type Float%20%28single-precision%29))
  (bind _speed (Variables|Default|GetSpeed))
  (bind _speed_2 (Variables|Default|GetSpeed))
  (bind _cube (Variables|Default|GetCube))
  (bind _cube_2 (Variables|Default|GetCube))
  (bind _relativelocation (Variables|/Script/Engine.SceneComponent|GetRelativeLocation _cube_2))
  (bind _relativelocation_2 (Variables|/Script/Engine.SceneComponent|GetRelativeLocation _cube))
  (bind _returnvalue (+ (.z _relativelocation) _speed_2))
  (bind _returnvalue_2 (- (.z _relativelocation_2) _speed))
  ;[0.15 0.15 0.15 0.5] Move Platform Logic
  (if (Variables|Default|GetActivated)
    (if (Variables|Default|GetGoingBack)
      (Transformation|SetRelativeLocation _cube (Math|Vector|MakeVector (.x _relativelocation_2) (.y _relativelocation_2) _returnvalue_2) false false)
      (if (<= _returnvalue_2 (Variables|Default|GetLowestPoint))
        (Variables|Default|SetActivated false)
        (Utilities|FlowControl|Delay (Variables|Default|GetStopDelay))
        (Variables|Default|SetGoingBack false)
        (Variables|Default|SetActivated true)
        (Utilities|FlowControl|DoOnce false) ; enters at Reset
      )
      (else
        (Transformation|SetRelativeLocation _cube_2 (Math|Vector|MakeVector (.x _relativelocation) (.y _relativelocation) _returnvalue) false false)
        (if (<= (Variables|Default|GetHighestPoint) _returnvalue)
          (Variables|Default|SetActivated false)
          (Utilities|FlowControl|Delay (Variables|Default|GetStopDelay))
          (Variables|Default|SetGoingBack true)
          (Variables|Default|SetActivated true))))))

(fn ConstructionScript)

(fn Interact
  (params (Character :type BP%20Third%20Person%20Character%20Object%20Reference))
  (return false))