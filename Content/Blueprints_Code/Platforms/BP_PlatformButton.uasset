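; Interactable platform button that switches linked moving platforms on or off.
; Interact calls StartPlatform only for a character with a shield and empty hands, playing press sounds and removing the cached player's shield.
; After a delay it flips Activated on each valid OnOffMoving entry, playing conveyor audio for those switched on.
; Sphere overlap begin and end toggle the outline's visibility.
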(event OnComponentBeginOverlap(Sphere)
  (params (OverlappedComponent :type Primitive%20Component%20Object%20Reference) (OtherActor :type Actor%20Object%20Reference) (OtherComp :type Primitive%20Component%20Object%20Reference) (OtherBodyIndex :type Integer) (bFromSweep :type Boolean) (SweepResult :type Hit%20Result%20Structure%20%28by%20ref%29))
  ;[0.15 0.15 0.15 0.5] Outline
  (Rendering|ToggleVisibility (Variables|Default|GetOutline) false))

(event OnComponentEndOverlap(Sphere)
  (params (OverlappedComponent :type Primitive%20Component%20Object%20Reference) (OtherActor :type Actor%20Object%20Reference) (OtherComp :type Primitive%20Component%20Object%20Reference) (OtherBodyIndex :type Integer))
  ;[0.15 0.15 0.15 0.5] Outline
  (Rendering|ToggleVisibility (Variables|Default|GetOutline) true))

(event Custom|StartPlatform
  ;[0.15 0.15 0.15 0.5] Start Platforms
  (Audio|Components|Audio|Play (Variables|Default|GetPress) 0.0)
  (Audio|Components|Audio|Play (Variables|Default|GetButton) 0.0)
  (Default|RemoveShield (Variables|/Game/BP_ThirdPersonCharacter.BP_ThirdPersonCharacter_C|GetPickUpShield (Variables|Default|GetCharRef)))
  (Utilities|FlowControl|Delay (Variables|Default|GetStopDelay))
  (for _array_element (Variables|Default|GetOnOffMoving)
    (Utilities|IsValid _array_element
      (:Is%20Valid
        (if (Variables|/Game/Blueprints_Code/Platforms/BP_OnOffMovingPlatform.BP_OnOffMovingPlatform_C|GetActivated _array_element)
          (Variables|/Game/Blueprints_Code/Platforms/BP_OnOffMovingPlatform.BP_OnOffMovingPlatform_C|SetActivated _array_element false)
          (else
            (Variables|/Game/Blueprints_Code/Platforms/BP_OnOffMovingPlatform.BP_OnOffMovingPlatform_C|SetActivated _array_element true)
            (Audio|Components|Audio|Play (Variables|/Game/Blueprints_Code/Platforms/BP_OnOffMovingPlatform.BP_OnOffMovingPlatform_C|GetSFX_Conveyor _array_element) 0.0)))))))

(event EventBeginPlay
  (bind _returnvalue (AddComponent|AddAudioComponent false))
  (Variables|Default|SetPress _returnvalue)
  (bind _returnvalue_2 (AddComponent|AddAudioComponent false))
  (Variables|Default|SetButton _returnvalue_2)
  (bind _asbp_third_person_character (Utilities|Casting|CastToBP_ThirdPersonCharacter (Game|Player|GetPlayerPawn 0)))
  (Variables|Default|SetCharRef _asbp_third_person_character))

(fn ConstructionScript)

(fn Interact
  (params (Character :type BP%20Third%20Person%20Character%20Object%20Reference))
  ;[0.15 0.15 0.15 0.5] Button Checks
  (if (not (Variables|/Game/BP_ThirdPersonCharacter.BP_ThirdPersonCharacter_C|GetHasItemInHand Character))
    (if (Variables|/Game/BP_ThirdPersonCharacter.BP_ThirdPersonCharacter_C|GetHasShield Character)
      (CallFunction|StartPlatform)
      (return false))))