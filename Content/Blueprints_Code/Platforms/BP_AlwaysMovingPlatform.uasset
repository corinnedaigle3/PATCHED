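; Moving platform Blueprint that travels between its placed position and a configurable MoveToPos offset.
; The construction script adds both relative control points to an InterpToMovement component, which drives the motion without event graph logic.
; A Box overlap attaches BP_ThirdPersonCharacter with world transform kept on entry and detaches it on exit, so the character can ride along.
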(event OnComponentBeginOverlap(Box)
  (params (OverlappedComponent :type Primitive%20Component%20Object%20Reference) (OtherActor :type Actor%20Object%20Reference) (OtherComp :type Primitive%20Component%20Object%20Reference) (OtherBodyIndex :type Integer) (bFromSweep :type Boolean) (SweepResult :type Hit%20Result%20Structure%20%28by%20ref%29))
  (bind _asbp_third_person_character (Utilities|Casting|CastToBP_ThirdPersonCharacter OtherActor))
  (Transformation|AttachComponentToComponent _asbp_third_person_character 0 "None" "KeepWorld" "KeepWorld" "KeepWorld" true))

(event OnComponentEndOverlap(Box)
  (params (OverlappedComponent :type Primitive%20Component%20Object%20Reference) (OtherActor :type Actor%20Object%20Reference) (OtherComp :type Primitive%20Component%20Object%20Reference) (OtherBodyIndex :type Integer))
  (bind _asbp_third_person_character (Utilities|Casting|CastToBP_ThirdPersonCharacter OtherActor))
  (Transformation|DetachFromActor _asbp_third_person_character "KeepRelative" "KeepRelative" "KeepRelative"))

(fn ConstructionScript
  ;[0.15 0.15 0.15 0.5] Move Between Points
  (Class|InterptoMovementComponent|AddControlPointPosition (Variables|Default|GetInterpToMovement) "0, 0, 0" true)
  (Class|InterptoMovementComponent|AddControlPointPosition (Variables|Default|GetInterpToMovement) (Variables|Default|GetMoveToPos) true))