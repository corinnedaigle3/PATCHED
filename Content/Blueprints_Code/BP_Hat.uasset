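; BP_Hat is a wearable hat pickup that attaches to the third-person character when interacted with.
; BeginPlay caches the character, and PickupHat snaps the hat to the mesh's "Hat" socket, disables the Cube's physics and collision, and sets HasHat.
; Interact calls PickupHat on both HasHat branches, ignoring its Character input.
; UnequipHat, marked in progress, detaches and restores physics but not collision, and is never called here.
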(event Custom|PickupHat
  ;[0.15 0.15 0.15 0.5] Pick Up Hat
  (Transformation|AttachComponentToComponent (Variables|/Script/Engine.Character|GetMesh (Variables|Default|GetCharRef)) "Hat" "SnapToTarget" "SnapToTarget" "KeepWorld" false)
  (Physics|SetSimulatePhysics (Variables|Default|GetCube) false)
  (Collision|SetCollisionEnabled (Variables|Default|GetCube) "NoCollision")
  (Variables|/Game/BP_ThirdPersonCharacter.BP_ThirdPersonCharacter_C|SetHasHat (Variables|Default|GetCharRef) true))

(event Custom|UnequipHat
  ;[0.15 0.15 0.15 0.5] Unequip Hat (In Progress)
  (Transformation|DetachFromComponent (Variables|Default|GetCube) "KeepRelative" "KeepRelative" "KeepRelative" false)
  (Physics|SetSimulatePhysics (Variables|Default|GetCube) true)
  (Variables|/Game/BP_ThirdPersonCharacter.BP_ThirdPersonCharacter_C|SetHasHat (Variables|Default|GetCharRef) false))

(event EventBeginPlay
  (bind _returnvalue (Actor|GetActorOfClass "/Game/BP_ThirdPersonCharacter.BP_ThirdPersonCharacter_C"))
  (Variables|Default|SetCharRef _returnvalue))

(fn ConstructionScript)

(fn Interact
  (params (Character :type BP%20Third%20Person%20Character%20Object%20Reference))
  (if (Variables|/Game/BP_ThirdPersonCharacter.BP_ThirdPersonCharacter_C|GetHasHat (Variables|Default|GetCharRef))
    (CallFunction|PickupHat)
    (else
      (CallFunction|PickupHat)))
  (return false))