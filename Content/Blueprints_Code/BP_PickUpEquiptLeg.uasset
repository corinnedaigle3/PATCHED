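; Pickup actor for a severed leg that the player carries and reattaches to recover a body part.
; Interact, with empty hands, plays a sound and snaps the leg to the character's CarryLegR socket.
; AttachLeg requires a needle to restore the part and destroy the actor, firing an extra destroy call in FinalOfficeBoss; otherwise it drops the leg with physics.
; Sphere overlaps toggle the outline, and shared character flags track the held item.
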(event OnComponentBeginOverlap(Sphere)
  (params (OverlappedComponent :type Primitive%20Component%20Object%20Reference) (OtherActor :type Actor%20Object%20Reference) (OtherComp :type Primitive%20Component%20Object%20Reference) (OtherBodyIndex :type Integer) (bFromSweep :type Boolean) (SweepResult :type Hit%20Result%20Structure%20%28by%20ref%29))
  ;[0.15 0.15 0.15 0.5] Outline Visibility
  (Rendering|ToggleVisibility (Variables|Default|GetPatch_RightLegDROP) false))

(event OnComponentEndOverlap(Sphere)
  (params (OverlappedComponent :type Primitive%20Component%20Object%20Reference) (OtherActor :type Actor%20Object%20Reference) (OtherComp :type Primitive%20Component%20Object%20Reference) (OtherBodyIndex :type Integer))
  ;[0.15 0.15 0.15 0.5] Outline Visibility
  (Rendering|ToggleVisibility (Variables|Default|GetPatch_RightLegDROP) true))

(event Custom|AttachLeg
  (bind _bodyparttype (Variables|Default|GetBodyPartType))
  (bind _charref (Variables|Default|GetCharRef))
  (bind _charref_2 (Variables|Default|GetCharRef))
  ;[0.15 0.15 0.15 0.5] Attach leg to body
  (if (Variables|/Game/BP_ThirdPersonCharacter.BP_ThirdPersonCharacter_C|GetHasNeedle _charref)
    (Variables|/Game/BP_ThirdPersonCharacter.BP_ThirdPersonCharacter_C|SetHasItemInHand _charref false)
    (Variables|/Game/BP_ThirdPersonCharacter.BP_ThirdPersonCharacter_C|SetLegInHand _charref false)
    (Default|RecoverALive _charref_2 _bodyparttype)
    (Default|CallUnattachNeedle _charref_2)
    (Development|PrintString (Utilities|String|EnumtoString _bodyparttype))
    (CallFunction|NoIteminHand)
    (bind _returnvalue (Game|GetCurrentLevelName true))
    (if (not (== (Utilities|String|StringToName _returnvalue) "FinalOfficeBoss"))
      _
      (else
        (Default|CallLegonDestory)))
    (Actor|DestroyActor)
    (else
      (CallFunction|DropLeg))))

(event Custom|NoItemInHand
  (bind _charref (Variables|Default|GetCharRef))
  ;[0.15 0.15 0.15 0.5] Set item in hand Bools false
  (Variables|/Game/BP_ThirdPersonCharacter.BP_ThirdPersonCharacter_C|SetHasItemInHand _charref false)
  (Variables|/Game/BP_ThirdPersonCharacter.BP_ThirdPersonCharacter_C|SetLegInHand _charref false))

(event Custom|DropLeg
  (bind _leg (Variables|Default|GetLeg))
  ;[0.15 0.15 0.15 0.5] Drop leg from hand
  (Transformation|DetachFromComponent (Variables|Default|GetLeg) "KeepRelative" "KeepRelative" "KeepRelative" false)
  (Collision|SetCollisionResponsetoChannel _leg "ECC_GameTraceChannel2" "ECR_Block")
  (Collision|SetCollisionResponsetoChannel _leg "ECC_Pawn" "ECR_Block")
  (Collision|SetCollisionResponsetoChannel _leg "ECC_WorldStatic" "ECR_Block")
  (Physics|SetSimulatePhysics _leg true)
  (Rendering|ToggleVisibility (Variables|Default|GetPatch_RightLegDROP) false)
  (CallFunction|NoIteminHand))

(event Custom|PickUpLeg
  (bind _charref (Variables|Default|GetCharRef))
  (bind _charref_2 (Variables|Default|GetCharRef))
  ;[0.15 0.15 0.15 0.5] Pick up leg
  (if (not (Variables|/Game/BP_ThirdPersonCharacter.BP_ThirdPersonCharacter_C|GetHasItemInHand _charref_2))
    (Variables|/Game/BP_ThirdPersonCharacter.BP_ThirdPersonCharacter_C|SetPickUpLeg _charref_2 self)
    (Rendering|ToggleVisibility (Variables|Default|GetPatch_RightLegDROP) true)
    (Variables|Default|SetLegPicked true)
    (Audio|Components|Audio|Play (Variables|Default|GetPickUp) 0.0)
    (Physics|SetSimulatePhysics (Variables|Default|GetLeg) false)
    (Variables|/Game/BP_ThirdPersonCharacter.BP_ThirdPersonCharacter_C|SetHasItemInHand _charref true)
    (Variables|/Game/BP_ThirdPersonCharacter.BP_ThirdPersonCharacter_C|SetLegInHand _charref true)
    (Transformation|AttachComponentToComponent self (Variables|/Script/Engine.Character|GetMesh _charref) "CarryLegR" "SnapToTarget" "SnapToTarget" "SnapToTarget" false)
    (Collision|SetCollisionResponsetoChannel (Variables|Default|GetLeg) "ECC_GameTraceChannel2" "ECR_Ignore")
    (Collision|SetCollisionResponsetoChannel (Variables|Default|GetLeg) "ECC_Pawn" "ECR_Ignore")))

(event EventBeginPlay
  (bind _asbp_third_person_character (Utilities|Casting|CastToBP_ThirdPersonCharacter (Game|Player|GetPlayerPawn 0)))
  (Variables|Default|SetCharRef _asbp_third_person_character)
  (bind _returnvalue (AddComponent|AddAudioComponent false))
  (Variables|Default|SetPickUp _returnvalue))

(fn ConstructionScript)

(fn Interact
  (params (Character :type BP%20Third%20Person%20Character%20Object%20Reference))
  ;[0.15 0.15 0.15 0.5] Interact
  (if (not (Variables|/Game/BP_ThirdPersonCharacter.BP_ThirdPersonCharacter_C|GetHasItemInHand (Variables|Default|GetCharRef)))
    (CallFunction|PickUpLeg)
    (return false)))