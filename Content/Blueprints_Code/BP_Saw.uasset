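; BP_Saw is a moving saw hazard that costs the player a life and teleports them away on contact.
; MoveSaw plays a timeline, rate-scaled by TimeToComplete, that moves and rotates the saw along the SplineToFollow actor's spline.
; Overlapping BoxSaw calls LoseALive on the third-person character, then after a brief delay teleports them to the BP_TeleportLocationHazard found at BeginPlay.
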(event OnComponentBeginOverlap(BoxSaw)
  (params (OverlappedComponent :type Primitive%20Component%20Object%20Reference) (OtherActor :type Actor%20Object%20Reference) (OtherComp :type Primitive%20Component%20Object%20Reference) (OtherBodyIndex :type Integer) (bFromSweep :type Boolean) (SweepResult :type Hit%20Result%20Structure%20%28by%20ref%29))
  (bind _asbp_third_person_character (Utilities|Casting|CastToBP_ThirdPersonCharacter OtherActor))
  (Default|LoseALive _asbp_third_person_character)
  (Utilities|FlowControl|Delay 0.2)
  (Transformation|Teleport _asbp_third_person_character (Transformation|GetActorLocation (Variables|Default|GetTeleportLocation)) "0, 0, 0"))

(event Custom|MoveSaw
  (bind _spline_to_follow (Variables|Default|GetSpline%20To%20Follow))
  (bind _spline (Variables|/Game/Blueprints_Code/BP_SplineHazards.BP_SplineHazards_C|GetSpline _spline_to_follow))
  (Components|Timeline|SetPlayRate (Variables|Default|GetT_MSaw) (/ 1.0 (Variables|Default|GetTime%20To%20Complete)))
  (bind _newtrack_1 (Timeline|T_MSaw Play)
    (:Update
      (Transformation|SetActorLocationAndRotation (Spline|GetLocationatDistanceAlongSpline _spline (Math|Float|Lerp 0.0 (Spline|GetSplineLength _spline) _newtrack_1) "World") (Spline|GetRotationatDistanceAlongSpline _spline (Math|Float|Lerp 0.0 (Spline|GetSplineLength _spline) _newtrack_1) "World")))))

(event EventBeginPlay
  (bind _returnvalue (Actor|GetActorOfClass "/Game/Blueprints_Code/BP_TeleportLocationHazard.BP_TeleportLocationHazard_C"))
  (Variables|Default|SetTeleportLocation _returnvalue))

(fn ConstructionScript)