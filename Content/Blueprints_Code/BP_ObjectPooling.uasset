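; BP_ObjectPooling is an actor that periodically launches a batch of boxes from the pool held by BPBoxesPool.
; A looping timer started on BeginPlay fires DropTheBoxes, which calls DropBox on pooled boxes along the actor's up vector at their projectile initial speed, then detaches them.
; The index resets after each batch, so every wave reuses boxes from the front of the array instead of spawning new ones.
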(event Custom|DropTheBoxes
  (bind _bp_boxespool (Variables|Default|GetBP_BoxesPool))
  (bind _boxespool (Variables|/Game/Blueprints_Code/BP_BoxesPool.BP_BoxesPool_C|GetBoxesPool _bp_boxespool))
  (bind _returnvalue (Utilities|Array|Length _boxespool))
  (for _index (range 0 4)
    (if (> _returnvalue 0)
      (Variables|Default|SetMaxBoxes _returnvalue)
      (Utilities|IsValid (Utilities|Array|Get(acopy) _boxespool (Variables|Default|GetBoxIndex))
        (:Is%20Valid
          (Default|DropBox (Utilities|Array|Get(acopy) _boxespool (Variables|Default|GetBoxIndex)) (* (Transformation|GetActorUpVector) (Variables|/Script/Engine.ProjectileMovementComponent|GetInitialSpeed (Variables|/Game/Blueprints_Code/BP_Boxes.BP_Boxes_C|GetProjectileMovement (Utilities|Array|Get(acopy) _boxespool (Variables|Default|GetBoxIndex))))))
          (Transformation|DetachFromActor (Utilities|Array|Get(acopy) _boxespool (Variables|Default|GetBoxIndex)) "KeepWorld" "KeepWorld" "KeepWorld")
          (Variables|Default|SetBoxIndex (+ (Variables|Default|GetBoxIndex) 1))))))
  (Variables|Default|SetBoxIndex 0))

(event EventBeginPlay
  (Utilities|Time|SetTimerbyEvent (delegate Custom|DropTheBoxes) 3e+01 true))

(event Collision|EventActorBeginOverlap
  (params (OtherActor :type Actor%20Object%20Reference)))

(event EventTick
  (params (DeltaSeconds :type Float%20%28single-precision%29)))

(fn ConstructionScript)