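; Runs the player's needle grappling hook, which pulls in limb pickups or moves the player to grappable objects.
; OnGrapple sphere-traces from the camera on two channels: limbs first, then grappables, which either pull the capsule via MoveComponentTo or trigger a flying grapple's catch.
; Timelines with VInterpTo animate the character's detached needle and cable outward, retracting on a miss.
; A cooldown gates firing, while input locks and socket reattachment manage each shot.
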(event Custom|RecoverNeedle
  ;[0.15 0.15 0.15 0.5] Hendles the needle projectile first launch, it also does the get back projectile for when you do not hit any grappable object
  (Timeline|RecoverNeedleTimeline PlayFromStart
    (:Update
      (CallFunction|SmoothMoveto (Transformation|GetSocketLocation (Variables|/Script/Engine.Character|GetMesh (Variables|Default|GetPlayerRef)) (Variables|Default|GetNeedleHandScoket)) 7.0))
    (:Finished
      (CallFunction|ResetNeedletoSocekt (Variables|Default|GetNeedleHipSocket))
      (Variables|Default|SetGrapplingCooldown false)
      (CallFunction|IgnoreInputs false))))

(event Custom|GrappleMechanic
  (params (Start :type Vector) (End :type Vector))
  ;[0.15 0.15 0.15 0.5] Handles the execution of the traces and the cooldown functionality
  (if (not (Variables|Default|GetGrapplingCooldown))
    (CallFunction|IgnoreInputs true)
    (Audio|PlaySound2D "/Game/Audio/SFX/GameMech/SFX_Whoosh1.SFX_Whoosh1" 1.0 1.0 0.0 0 0)
    (Variables|Default|SetGrapplingCooldown true)
    (bind (_out_hit _return_value) (CallFunction|TracingforGrapple Start End "TraceTypeQuery4" "ForDuration" 1.0))
    (if _return_value
      (bind _hit_is_arm_or_leg (CallFunction|PullingLimbs _out_hit))
      (if _hit_is_arm_or_leg
        (Variables|Default|SetPulling _hit_is_arm_or_leg)
        (CallFunction|LimbGetClose _hit_is_arm_or_leg)
        (CallFunction|IgnoreInputs false)
        (Utilities|FlowControl|Delay 1.0)
        (CallFunction|SetNeedleEnd "0, 0, 0" 0 false true)
        (else
          (bind (_out_hit_2 _return_value_2) (CallFunction|TracingforGrapple Start End "TraceTypeQuery3" "ForDuration" 1.0 :!label _label))
          (if _return_value_2
            (bind _asbp_grappable_3d (Utilities|Casting|CastToBP_Grappable3D (.HitActor (Collision|BreakHitResult _out_hit_2)))
              (:then
                (if (not (Variables|/Game/Blueprints_Code/BP_Grappable3D.BP_Grappable3D_C|GetCanPull _asbp_grappable_3d))
                  (if (Variables|/Game/Blueprints_Code/BP_Grappable3D.BP_Grappable3D_C|GetCanGrappleHere _asbp_grappable_3d)
                    (Variables|Default|SetHItMoveTo true)
                    (CallFunction|HandleCable true)
                    (CallFunction|SetNeedleEnd (.ImpactPoint (Collision|BreakHitResult _out_hit_2)) (.HitActor (Collision|BreakHitResult _out_hit_2)) true false)
                    (Utilities|FlowControl|Delay 1.0)
                    (CallFunction|GrappleMoveT (.HitActor (Collision|BreakHitResult _out_hit_2)) (.ImpactPoint (Collision|BreakHitResult _out_hit_2))))
                  (else
                    (bind _asbp_flying_grapple (Utilities|Casting|CastToBP_FlyingGrapple (.HitActor (Collision|BreakHitResult _out_hit_2))))
                    (CallFunction|HandleCable true)
                    (CallFunction|SetNeedleEnd (.ImpactPoint (Collision|BreakHitResult _out_hit_2)) 0 false false)
                    (Variables|Default|Setpulling true)
                    (Utilities|FlowControl|Delay 1.0)
                    (Development|PrintString "Got Caught")
                    (Default|GotCaught _asbp_flying_grapple (Variables|Default|GetPlayerRef)))))
              (:CastFailed
                (CallFunction|SetNeedleEnd (.TraceEnd (Collision|BreakHitResult _out_hit_2)) 0 false false :!label _label_2)
                (CallFunction|RecoverNeedle)))
            (else
              (goto _label_2)))))
      (else
        (goto _label)))
    (else
      (Development|PrintString "grappling cooldown"))))

(event Custom|Set%20Needle%20end
  (params (End%20point :type Vector) (hit%20actor :type Actor%20Object%20Reference) (HitSomething :type Boolean) (OnlyRetract :type Boolean))
  ;[0.15 0.15 0.15 0.5] Hendles the needle projectile first launch, it also does the get back projectile for when you do not hit any grappable object
  (if (not HitSomething)
    (if (not OnlyRetract)
      (Transformation|DetachFromComponent (Variables|/Game/BP_ThirdPersonCharacter.BP_ThirdPersonCharacter_C|GetNeedle (Variables|Default|GetPlayerRef)) "KeepWorld" "KeepWorld" "KeepWorld" true)
      (CallFunction|ResetNeedletoSocekt (Variables|Default|GetNeedleHandScoket))
      (Transformation|DetachFromComponent (Variables|/Game/BP_ThirdPersonCharacter.BP_ThirdPersonCharacter_C|GetNeedle (Variables|Default|GetPlayerRef)) "KeepWorld" "KeepWorld" "KeepWorld" true)
      (CallFunction|HandleCable true)
      (Timeline|ShootNeedleTimeline PlayFromStart
        (:Update
          (CallFunction|SmoothMoveto End%20point 7.0)))
      (else
        (Timeline|RecoverNeedleTimeline PlayFromStart
          (:Update
            (CallFunction|SmoothMoveto (Transformation|GetSocketLocation (Variables|/Script/Engine.Character|GetMesh (Variables|Default|GetPlayerRef)) (Variables|Default|GetNeedleHandScoket)) 7.0))
          (:Finished
            (CallFunction|ResetNeedletoSocekt (Variables|Default|GetNeedleHipSocket))
            (Variables|Default|SetGrapplingCooldown false)
            (CallFunction|IgnoreInputs false)))))
    (else
      (Transformation|DetachFromComponent (Variables|/Game/BP_ThirdPersonCharacter.BP_ThirdPersonCharacter_C|GetNeedle (Variables|Default|GetPlayerRef)) "KeepWorld" "KeepWorld" "KeepWorld" true)
      (CallFunction|ResetNeedletoSocekt (Variables|Default|GetNeedleHandScoket))
      (Transformation|DetachFromComponent (Variables|/Game/BP_ThirdPersonCharacter.BP_ThirdPersonCharacter_C|GetNeedle (Variables|Default|GetPlayerRef)) "KeepWorld" "KeepWorld" "KeepWorld" true)
      (bind _objectvector (CallFunction|DetermineNeedleEndPoint hit%20actor))
      (CallFunction|HandleCable true)
      (Timeline|ShootNeeddelToObject PlayFromStart
        (:Update
          (CallFunction|SmoothMoveto _objectvector 2.0))
        (:Finished
          (CallFunction|HandleCable false))))))

(event Custom|FlyingGrappleDone
  ;[0.15 0.15 0.15 0.5] Handles the execution of the traces and the cooldown functionality
  (CallFunction|SetNeedleEnd "0, 0, 0" 0 false true)
  (CallFunction|HandleCable false)
  (CallFunction|RecoverNeedle))

(event Custom|limbGetClose
  (params (hit%20arm%20or%20leg :type Boolean))
  (bind _pickuplongdistance (Variables|Default|GetPickUpLongDistance))
  (bind _returnvalue (Components|GetOwner _pickuplongdistance))
  ;[0.15 0.15 0.15 0.5] pulls limb closer
  (if hit%20arm%20or%20leg
    (Variables|Default|Setpulling true)
    (CallFunction|HandleCable true)
    (bind _asbp_pick_up_equipt_leg (Utilities|Casting|CastToBP_PickUpEquiptLeg _returnvalue)
      (:then
        (bind _output_get (Variables|Default|SetPick%20Up%20Leg _asbp_pick_up_equipt_leg))
        (Default|MovetoPlayer _output_get)
        (Development|PrintString "She does not give a fuck "))
      (:CastFailed
        (bind _asbp_pick_up_equipt_arm (Utilities|Casting|CastToBP_PickUpEquiptArm _returnvalue))
        (bind _output_get_2 (Variables|Default|SetPick%20Up%20Arm _asbp_pick_up_equipt_arm))
        (Default|MovetoPlayer _output_get_2)))
    (Variables|Default|Setpulling false)))

(event Custom|GrappleMoveT
  (params (Hit%20Actor :type Actor%20Object%20Reference) (Impact%20point :type Vector))
  (bind _returnvalue (Transformation|GetActorLocation))
  (bind _returnvalue_2 (Math|Rotator|FindLookatRotation _returnvalue Impact%20point))
  ;[0.15 0.15 0.15 0.5] handles the movement towards grappable object
  (Class|BPIGrapple|OnGrapple(Message) Hit%20Actor)
  (Audio|PlaySound2D "/Game/Audio/SFX/GameMech/SFX_Whoosh.SFX_Whoosh" 1.0 1.0 0.0 0 0)
  (Components|MoveComponentTo (Variables|/Script/Engine.Character|GetCapsuleComponent (Variables|Default|GetPlayerRef)) Impact%20point (Math|Rotator|MakeRotator (.roll _returnvalue_2) 0.0 (.yaw _returnvalue_2)) true false 0.5 true)
  (Development|PrintString "should be idl")
  (Transformation|SetWorldLocation (Variables|/Game/BP_ThirdPersonCharacter.BP_ThirdPersonCharacter_C|GetNeedle (Variables|Default|GetPlayerRef)) (Transformation|GetSocketLocation (Variables|/Script/Engine.Character|GetMesh (Variables|Default|GetPlayerRef)) (Variables|Default|GetNeedleHipSocket)) false false)
  (CallFunction|HandleCable false)
  (CallFunction|IgnoreInputs false)
  (CallFunction|ResetNeedletoSocekt (Variables|Default|GetNeedleHipSocket))
  (Variables|Default|SetGrapplingCooldown false))

(event EventBeginPlay
  (bind _returnvalue (Actor|GetActorOfClass "/Game/BP_ThirdPersonCharacter.BP_ThirdPersonCharacter_C"))
  (Variables|Default|SetPlayerRef _returnvalue))

(event Collision|EventActorBeginOverlap
  (params (OtherActor :type Actor%20Object%20Reference)))

(event EventTick
  (params (DeltaSeconds :type Float%20%28single-precision%29))
  (Utilities|FlowControl|Sequence
    (:then_0
      (if (== (== (Variables|Default|GetGrapplingCooldown) false) (== (Variables|Default|GetPulling) true))
        (Variables|Default|SetPulling false)))
    (:then_1
      (if (not (Variables|Default|GetGrapplingCooldown))
        (if (not (Variables|Default|GetPulling))
          (if (Utilities|Operators|NotEqual(!=) :A (Variables|/Script/Engine.SceneComponent|GetRelativeLocation (Variables|/Game/BP_ThirdPersonCharacter.BP_ThirdPersonCharacter_C|GetNeedle (Variables|Default|GetPlayerRef))) :ErrorTolerance 0.1)
            (Development|PrintString "not relative location 0 ")
            (Transformation|SetRelativeLocation (Variables|/Game/BP_ThirdPersonCharacter.BP_ThirdPersonCharacter_C|GetNeedle (Variables|Default|GetPlayerRef)) "0, 0, 0" false false)))))))

(event EventOnGrapple
  (bind (_start _end) (CallFunction|DetermineAimGrapple))
  (CallFunction|GrappleMechanic _start _end))

(fn ConstructionScript)

(fn TracingforGrapple
  (params (Start :type Vector) (End :type Vector) (TaraceChannel :type ETraceTypeQuery%20Enum :default "TraceTypeQuery1") (DrawDebugType :type EDrawDebugTrace%20Enum :default "None") (DrawTime :type Float%20%28double-precision%29))
  (bind (_outhit _returnvalue) (Collision|SphereTraceByChannel Start (+ Start (* End (Variables|Default|GetGrappleRange))) (Variables|Default|GetGrapplerRadius) TaraceChannel true 0 DrawDebugType true "(R=1.000000,G=0.000000,B=0.000000,A=1.000000)" "(R=0.000000,G=1.000000,B=0.000000,A=1.000000)" DrawTime))
  (return _outhit _returnvalue))

(fn PullingLimbs
  (params (hit%20 :type Hit%20Result%20Structure))
  (bind (_bblockinghit _binitialoverlap _time _distance _location _impactpoint _normal _impactnormal _physmat _hitactor _hitcomponent _hitbonename _bonename _hititem _elementindex _faceindex _tracestart _traceend) (Collision|BreakHitResult hit%20))
  (bind _asbp_pick_up_equipt_arm (Utilities|Casting|CastToBP_PickUpEquiptArm _hitactor)
    (:then
      (CallFunction|HandleCable true)
      (CallFunction|SetNeedleEnd _traceend _asbp_pick_up_equipt_arm true false)
      (Variables|Default|SetPickUpLongDistance (Variables|/Game/Blueprints_Code/BP_PickUpEquiptArm.BP_PickUpEquiptArm_C|GetArm _asbp_pick_up_equipt_arm))
      (Development|PrintString "Hello")
      (return true))
    (:CastFailed
      (bind _asbp_pick_up_equipt_leg (Utilities|Casting|CastToBP_PickUpEquiptLeg _hitactor)
        (:then
          (CallFunction|HandleCable true)
          (CallFunction|SetNeedleEnd _traceend _asbp_pick_up_equipt_leg true false)
          (Variables|Default|SetPickUpLongDistance (Variables|/Game/Blueprints_Code/BP_PickUpEquiptLeg.BP_PickUpEquiptLeg_C|GetLeg _asbp_pick_up_equipt_leg))
          (return true))
        (:CastFailed
          (Development|PrintString "GOTTTTTTTTTTTTTTTTTTTTTTTTTTTTTTTTTTTTTTTTTTTTTTTTTTTTTTTTTTTTTTTTTTTTTTTTTT" true true "(R=1.000000,G=0.101258,B=0.000000,A=1.000000)")
          (return false))))))

(fn HandleCable
  (params (set%20visibility%20 :type Boolean))
  (bind _playerref (Variables|Default|GetPlayerRef))
  (bind _cable (Variables|/Game/BP_ThirdPersonCharacter.BP_ThirdPersonCharacter_C|GetCable _playerref))
  (Rendering|SetVisibility _cable set%20visibility%20 false)
  (Class|CableComponent|SetAttachEndtoComponent _cable (Variables|/Game/BP_ThirdPersonCharacter.BP_ThirdPersonCharacter_C|GetNeedle (Variables|Default|GetPlayerRef)) "None")
  (Development|PrintString "HandleCable"))

(fn DetermineAimGrapple
  (bind _returnvalue (Game|GetPlayerCameraManager 0))
  (if (Variables|/Game/BP_ThirdPersonCharacter.BP_ThirdPersonCharacter_C|GetisSplineCam (Variables|Default|GetPlayerRef))
    (return "0, 0, 0" "0, 0, 0")
    (else
      (return (Camera|GetCameraLocation _returnvalue) (Math|Vector|GetForwardVector (Camera|GetCameraRotation _returnvalue))))))

(fn DetermineNeedleEndPoint
  (params (Actor :type Actor%20Object%20Reference))
  (bind _asbp_grappable_3d (Utilities|Casting|CastToBP_Grappable3D Actor)
    (:then
      (Development|PrintString (Utilities|String|ToString(Vector) (Transformation|GetWorldLocation (Variables|/Game/Blueprints_Code/BP_Grappable3D.BP_Grappable3D_C|GetStaticMesh _asbp_grappable_3d))) true true "(R=0.000000,G=0.660000,B=1.000000,A=1.000000)" 1e+01)
      (return (Transformation|GetWorldLocation (Variables|/Game/Blueprints_Code/BP_Grappable3D.BP_Grappable3D_C|GetStaticMesh _asbp_grappable_3d))))
    (:CastFailed
      (bind _asbp_pick_up_equipt_arm (Utilities|Casting|CastToBP_PickUpEquiptArm Actor)
        (:then
          (return (Transformation|GetWorldLocation (Variables|/Game/Blueprints_Code/BP_PickUpEquiptArm.BP_PickUpEquiptArm_C|GetArm _asbp_pick_up_equipt_arm))))
        (:CastFailed
          (bind _asbp_pick_up_equipt_leg (Utilities|Casting|CastToBP_PickUpEquiptLeg Actor))
          (return (Transformation|GetWorldLocation (Variables|/Game/Blueprints_Code/BP_PickUpEquiptLeg.BP_PickUpEquiptLeg_C|GetLeg _asbp_pick_up_equipt_leg))))))))

(fn SmoothMoveto
  (params (VectorMoveTo :type Vector) (InterpSpeed :type Float%20%28double-precision%29))
  (bind _playerref (Variables|Default|GetPlayerRef))
  (bind _needle (Variables|/Game/BP_ThirdPersonCharacter.BP_ThirdPersonCharacter_C|GetNeedle _playerref))
  (Transformation|SetWorldLocation _needle (Math|Interpolation|VInterpTo (Transformation|GetWorldLocation _needle) VectorMoveTo (Utilities|Time|GetWorldDeltaSeconds) InterpSpeed) false false))

(fn IgnoreInputs
  (params (Remove%20input? :type Boolean))
  (bind _returnvalue (Game|GetPlayerController 0))
  (Input|SetIgnoreMoveInput _returnvalue Remove%20input?)
  (Input|SetIgnoreLookInput _returnvalue Remove%20input?)
  (Development|PrintString "input issssssssssssssssssssssssssssssssssssssssssssssssss"))

(fn ResetNeedletoSocekt
  (params (SocketName :type Name))
  (bind _playerref (Variables|Default|GetPlayerRef))
  (bind _playerref_2 (Variables|Default|GetPlayerRef))
  (bind _needle (Variables|/Game/BP_ThirdPersonCharacter.BP_ThirdPersonCharacter_C|GetNeedle _playerref))
  (Transformation|AttachComponentToComponent (Variables|/Game/BP_ThirdPersonCharacter.BP_ThirdPersonCharacter_C|GetNeedle _playerref_2) (Variables|/Script/Engine.Character|GetMesh _playerref_2) SocketName "KeepRelative" "KeepRelative" "KeepRelative" true)
  (Transformation|SetRelativeLocation _needle "0, 0, 0" false false)
  (Transformation|SetRelativeRotation _needle "0, 0, 0" false false)
  (CallFunction|HandleCable false))