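; Spline-shaped conveyor belt that carries overlapping actors along its path.
; The construction script builds a visual and an overlap spline mesh per segment, scaling the visual material's XScale by segment length.
; A fast looping timer offsets each overlapping actor once per pass by DynamicSpeed along the nearest spline direction, without sweeping.
; Movement pauses while the player ThirdPersonCharacter's StartStop flag is true.
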(event Custom|MoveObj
  (if (not (Variables|/Game/BP_ThirdPersonCharacter.BP_ThirdPersonCharacter_C|GetStart/%20Stop (Variables|Default|GetCharREF)))
    (Variables|Default|SetMovedActors (Utilities|Array|MakeArray self))
    (for _array_element (Variables|Default|GetOverlapComponets)
      (for _array_element_2 (Collision|GetOverlappingActors _array_element 0 :!class /Script/Engine.PrimitiveComponent)
        (if (== (Utilities|Array|FindItem (Variables|Default|GetMovedActors) _array_element_2) -1)
          (Transformation|AddActorWorldOffset _array_element_2 (Math|Vector|RotateVector (* (Spline|FindDirectionClosesttoWorldLocation (Variables|Default|GetSpline) (Transformation|GetActorLocation _array_element_2) "Local") (Variables|Default|GetDynamicSpeed)) (Transformation|GetWorldRotation (Variables|Default|GetDefaultSceneRoot))))
          (Utilities|Array|Add (Variables|Default|GetMovedActors) _array_element_2))))))

(event EventBeginPlay
  (bind _asbp_third_person_character (Utilities|Casting|CastToBP_ThirdPersonCharacter (Game|GetPlayerCharacter 0)))
  (Variables|Default|SetCharREF _asbp_third_person_character)
  (Utilities|Time|SetTimerbyEvent (delegate Custom|MoveObj) 0.01 true))

(event Collision|EventActorBeginOverlap
  (params (OtherActor :type Actor%20Object%20Reference)))

(event EventTick
  (params (DeltaSeconds :type Float%20%28single-precision%29)))

(fn ConstructionScript
  (bind _spline (Variables|Default|GetSpline))
  (bind _spline_2 (Variables|Default|GetSpline))
  (for _index (range 0 (- (Spline|GetNumberOfSplinePoints (Variables|Default|GetSpline)) 2))
    (bind _returnvalue (AddComponent|AddSplineMeshComponent false))
    (Utilities|Array|Add (Variables|Default|GetMeshComponets) _returnvalue)
    (SplineMesh|SetStartandEnd _returnvalue (.Location (Spline|GetLocationandTangentatSplinePoint _spline _index "Local")) (.Tangent (Spline|GetLocationandTangentatSplinePoint _spline _index "Local")) (.Location (Spline|GetLocationandTangentatSplinePoint _spline (+ _index 1) "Local")) (.Tangent (Spline|GetLocationandTangentatSplinePoint _spline (+ _index 1) "Local")) true :!class /Script/Engine.SplineMeshComponent)
    (Rendering|Material|SetScalarParameterValueonMaterials _returnvalue "XScale" (/ (- (Spline|GetDistanceAlongSplineatSplinePoint _spline_2 (+ _index 1)) (Spline|GetDistanceAlongSplineatSplinePoint _spline_2 _index)) 2e+02))
    (bind _returnvalue_2 (AddComponent|AddSplineMeshComponent false))
    (Utilities|Array|Add (Variables|Default|GetOverlapComponets) _returnvalue_2)
    (SplineMesh|SetStartandEnd _returnvalue_2 (.Location (Spline|GetLocationandTangentatSplinePoint _spline _index "Local")) (.Tangent (Spline|GetLocationandTangentatSplinePoint _spline _index "Local")) (.Location (Spline|GetLocationandTangentatSplinePoint _spline (+ _index 1) "Local")) (.Tangent (Spline|GetLocationandTangentatSplinePoint _spline (+ _index 1) "Local")) true :!class /Script/Engine.SplineMeshComponent)))