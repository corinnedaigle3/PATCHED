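; Door actor that opens or closes based on the overlapping player's VoiceBoxChoice.
; Box overlap caches the third-person character, and Tick polls its choice, clearing the cube mesh for Choice 1 and restoring it otherwise.
; Leaving the box drops the player reference only while closed, so an open door keeps tracking the choice.
; Locked and Unlocked audio components are created at BeginPlay, but their Play calls are unwired.
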(event OnComponentBeginOverlap(Box)
  (params (OverlappedComponent :type Primitive%20Component%20Object%20Reference) (OtherActor :type Actor%20Object%20Reference) (OtherComp :type Primitive%20Component%20Object%20Reference) (OtherBodyIndex :type Integer) (bFromSweep :type Boolean) (SweepResult :type Hit%20Result%20Structure%20%28by%20ref%29))
  (bind _asbp_third_person_character (Utilities|Casting|CastToBP_ThirdPersonCharacter OtherActor))
  (Variables|Default|SetPlayerRef _asbp_third_person_character)
  (Development|PrintString "Hello"))

(event OnComponentEndOverlap(Box)
  (params (OverlappedComponent :type Primitive%20Component%20Object%20Reference) (OtherActor :type Actor%20Object%20Reference) (OtherComp :type Primitive%20Component%20Object%20Reference) (OtherBodyIndex :type Integer))
  (if (not (Variables|Default|GetDOOR%20OPENED))
    (Variables|Default|SetPlayerRef 0)))

(event EventBeginPlay
  (bind _returnvalue (AddComponent|AddAudioComponent false))
  (Variables|Default|SetLocked _returnvalue)
  (bind _returnvalue_2 (AddComponent|AddAudioComponent false))
  (Variables|Default|SetUnlocked _returnvalue_2))

(event Collision|EventActorBeginOverlap
  (params (OtherActor :type Actor%20Object%20Reference)))

(event EventTick
  (params (DeltaSeconds :type Float%20%28single-precision%29))
  (bind _cube (Variables|Default|GetCube))
  (bind _playerref (Variables|Default|GetPlayerRef)
    (:then
      (switch Utilities|FlowControl|Switch|SwitchonEnum_VoiceBox (Variables|/Game/BP_ThirdPersonCharacter.BP_ThirdPersonCharacter_C|GetVoiceBoxChoice _playerref)
        (:NewEnumerator0
          (Components|StaticMesh|SetStaticMesh _cube "/Engine/BasicShapes/Cube.Cube" :!label _label)
          (Development|PrintString "CHOICE ONE DONE")
          (if (Variables|Default|GetDOOR%20OPENED)
            (Variables|Default|SetDOOR%20OPENED false)))
        (:NewEnumerator1
          (Components|StaticMesh|SetStaticMesh _cube 0)
          (Variables|Default|SetDOOR%20OPENED true))
        (:NewEnumerator2
          (goto _label))
        (:NewEnumerator3
          (goto _label))
        (:NewEnumerator4
          (goto _label))
        (:NewEnumerator5
          (goto _label))))
    (:else)))

(fn ConstructionScript)