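; Test pickup actor for a severed leg that the third-person character can carry and reattach.
; Interact calls PickUpLeg if no limb is held, stopping physics, playing audio, snapping to the CarryLimbR socket and setting the character's carry flags.
; AttachLeg, not called within this Blueprint, clears those flags, recovers the body part, restores walk speed and destroys the actor.
; An objective widget hint for running is left unwired.
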(event Custom|AttachLeg
  (bind _bodyparttype (Variables|Default|GetBodyPartType))
  (bind _charref (Variables|Default|GetCharRef))
  (bind _charref_2 (Variables|Default|GetCharRef))
  ;[0.15 0.15 0.15 0.5] Attach leg to body
  (Rendering|SetVisibility (Variables|Default|GetLeg) false false)
  (Variables|/Game/BP_ThirdPersonCharacter.BP_ThirdPersonCharacter_C|SetHasLimbInHand _charref false)
  (Variables|/Game/BP_ThirdPersonCharacter.BP_ThirdPersonCharacter_C|SetLegInHand _charref false)
  (Transformation|DetachFromComponent (Variables|/Script/Engine.Character|GetMesh _charref) "KeepRelative" "KeepRelative" "KeepRelative" false)
  (Physics|SetSimulatePhysics (Variables|Default|GetLeg) true)
  (Default|RecoverALive (Variables|Default|GetCharRef) _bodyparttype)
  (Development|PrintString (Utilities|String|EnumtoString _bodyparttype))
  (Variables|/Script/Engine.CharacterMovementComponent|SetMaxWalkSpeed (Variables|/Script/Engine.Character|GetCharacterMovement _charref_2) (Variables|/Game/BP_ThirdPersonCharacter.BP_ThirdPersonCharacter_C|GetWalkSpeed _charref_2))
  (Development|PrintString "Attached Leg")
  (Actor|DestroyActor))

(event Custom|PickUpLeg
  (bind _charref (Variables|Default|GetCharRef))
  ;[0.15 0.15 0.15 0.5] Pick up leg
  (Variables|Default|SetLegPicked true)
  (Audio|Components|Audio|Play (Variables|Default|GetPickUp) 0.0)
  (Physics|SetSimulatePhysics (Variables|Default|GetLeg) false)
  (Variables|/Game/BP_ThirdPersonCharacter.BP_ThirdPersonCharacter_C|SetHasLimbInHand _charref true)
  (Variables|/Game/BP_ThirdPersonCharacter.BP_ThirdPersonCharacter_C|SetLegInHand _charref true)
  (Transformation|AttachComponentToComponent (Variables|/Script/Engine.Character|GetMesh _charref) "CarryLimbR" "SnapToTarget" "SnapToTarget" "SnapToTarget" false)
  (Collision|SetCollisionResponsetoChannel (Variables|Default|GetLeg) "ECC_GameTraceChannel2" "ECR_Ignore")
  (Development|PrintString "PickedUoLeg"))

(event EventBeginPlay
  (bind _asbp_third_person_character (Utilities|Casting|CastToBP_ThirdPersonCharacter (Game|Player|GetPlayerPawn 0)))
  (Variables|Default|SetCharRef _asbp_third_person_character)
  (bind _returnvalue (AddComponent|AddAudioComponent false))
  (Variables|Default|SetPickUp _returnvalue))

(fn ConstructionScript)

(fn Interact
  (params (Character :type BP%20Third%20Person%20Character%20Object%20Reference))
  ;[0.15 0.15 0.15 0.5] Interact
  (if (not (Variables|/Game/BP_ThirdPersonCharacter.BP_ThirdPersonCharacter_C|GetHasLimbInHand (Variables|Default|GetCharRef)))
    (CallFunction|PickUpLeg)
    (return false)))