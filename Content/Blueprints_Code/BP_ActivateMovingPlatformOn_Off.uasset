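; Moving platform actor that switches its InterpToMovement component on and off through a Box overlap volume.
; BeginPlay caches the player's BP_ThirdPersonCharacter, and only that character entering the box activates the movement.
; Activation passes through a DoOnce that is never reset, so it fires only on the first entry.
; Any end overlap on the box deactivates the movement, with no check on which actor left.
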(event OnComponentBeginOverlap(Box)
  (params (OverlappedComponent :type Primitive%20Component%20Object%20Reference) (OtherActor :type Actor%20Object%20Reference) (OtherComp :type Primitive%20Component%20Object%20Reference) (OtherBodyIndex :type Integer) (bFromSweep :type Boolean) (SweepResult :type Hit%20Result%20Structure%20%28by%20ref%29))
  ;[0.15 0.15 0.15 0.5] If Player Overlaps - Activate
  (if (== OtherActor (Variables|Default|GetCharREF))
    (Utilities|FlowControl|DoOnce false
      (:Completed
        (Components|Activation|Activate (Variables|Default|GetInterpToMovement) false)))))

(event OnComponentEndOverlap(Box)
  (params (OverlappedComponent :type Primitive%20Component%20Object%20Reference) (OtherActor :type Actor%20Object%20Reference) (OtherComp :type Primitive%20Component%20Object%20Reference) (OtherBodyIndex :type Integer))
  (Components|Activation|Deactivate (Variables|Default|GetInterpToMovement)))

(event EventBeginPlay
  ;[0.15 0.15 0.15 0.5] Player REF
  (bind _asbp_third_person_character (Utilities|Casting|CastToBP_ThirdPersonCharacter (Game|GetPlayerCharacter 0)))
  (Variables|Default|SetCharREF _asbp_third_person_character))

(event Collision|EventActorBeginOverlap
  (params (OtherActor :type Actor%20Object%20Reference)))

(event EventTick
  (params (DeltaSeconds :type Float%20%28single-precision%29)))

(fn ConstructionScript)