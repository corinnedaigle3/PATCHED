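; Blind enemy AI that hunts the player by sound, using PawnSensing hearing.
; A noise from the player character stops movement and starts an AIMoveTo chase at blind-enemy speed.
; The move's immediate Then output clears the hearing flag and calls FollowPath, which is defined outside this file.
; Each noise also restarts retriggerable delays that clear the flag and resume path following once things stay quiet.
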(event OnHearNoise(PawnSensing)
  (params (Instigator :type Pawn%20Object%20Reference) (Location :type Vector%20%28by%20ref%29 :default "0, 0, 0") (Volume :type Float%20%28single-precision%29))
  (bind _charactermovement (Variables|Character|GetCharacterMovement))
  ;[0.15 0.15 0.15 0.5] Sensing Player
  (Utilities|FlowControl|Sequence
    (:then_0
      (if (not (Variables|Default|GetCanHearPlayer))
        (Utilities|Casting|CastToBP_ThirdPersonCharacter Instigator)
        (Variables|Default|SetCanHearPlayer true)
        (Class|NavMovementInterface|StopActiveMovement _charactermovement)
        (Components|Movement|StopMovementImmediately _charactermovement)
        (CallFunction|ChasePlayer)))
    (:then_1
      (Utilities|FlowControl|RetriggerableDelay 1.0)
      (Variables|Default|SetCanHearPlayer false)
      (Utilities|FlowControl|RetriggerableDelay 1.5)
      (if (not (Variables|Default|GetCanHearPlayer))
        (Variables|/Script/Engine.CharacterMovementComponent|SetMaxWalkSpeed (Variables|Character|GetCharacterMovement) (Variables|Default|GetBlindEnemySpeed))
        (CallFunction|FollowPath)))))

(event Custom|ChasePlayer
  ;[0.15 0.15 0.15 0.5] Chasing Player
  (Variables|/Script/Engine.CharacterMovementComponent|SetMaxWalkSpeed (Variables|Character|GetCharacterMovement) (Variables|Default|GetBlindEnemySpeed))
  (AI|AIMoveTo self "0, 0, 0" (Game|Player|GetPlayerPawn 0) 15.0 false
    (:then
      (Variables|Default|SetCanHearPlayer false)
      (CallFunction|FollowPath))))

(event Custom|Event%20BeginPlay
  (|CallParentFunction))

(fn ConstructionScript
  (|CallParentFunction))