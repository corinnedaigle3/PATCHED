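; BP_Shield is an interactable shield that the player carries, attaches and uses to parry.
; Interact picks it up into a carry socket if the left arm is present, and AttachShield moves it to the shield socket, swapping the mesh and showing a parry hint.
; RemoveShield decrements Lives, then drops and destroys the shield once none remain; Tick also calls it while a shielded player lacks the arm.
; Dropping restores physics and collision.
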(event Custom|PickupShield
  (bind _charref (Variables|Default|GetCharRef))
  (bind _charref_2 (Variables|Default|GetCharRef))
  ;[0.15 0.15 0.15 0.5] Adding and removeing shield and shield collisions
  (if (Variables|/Game/BP_ThirdPersonCharacter.BP_ThirdPersonCharacter_C|GetHasArm _charref_2)
    (if (not (Variables|/Game/BP_ThirdPersonCharacter.BP_ThirdPersonCharacter_C|GetHasItemInHand _charref_2))
      (Variables|/Game/BP_ThirdPersonCharacter.BP_ThirdPersonCharacter_C|SetPickUpShield _charref_2 self)
      (Audio|Components|Audio|Play (Variables|Default|GetPickUp) 0.0)
      (Physics|SetSimulatePhysics (Variables|Default|GetButtonShield) false)
      (Variables|/Game/BP_ThirdPersonCharacter.BP_ThirdPersonCharacter_C|SetHasItemInHand _charref true)
      (Variables|/Game/BP_ThirdPersonCharacter.BP_ThirdPersonCharacter_C|SetShieldInHand _charref true)
      (Transformation|AttachComponentToComponent (Variables|/Script/Engine.Character|GetMesh _charref) "CarryShieldR" "SnapToTarget" "SnapToTarget" "SnapToTarget" false)
      (Collision|SetCollisionResponsetoChannel (Variables|Default|GetButtonShield) "ECC_GameTraceChannel2" "ECR_Ignore")
      (Collision|SetCollisionResponsetoChannel (Variables|Default|GetButtonShield) "ECC_Pawn" "ECR_Ignore"))
    (else
      (bind _returnvalue (UserInterface|CreateWidget "/Game/Blueprints_UI/WBP_Ojective.WBP_Ojective_C" 0 "Must have Left ARM"))
      (Default|ObjectiveActive _returnvalue))))

(event Custom|RemoveShield
  ;[0.15 0.15 0.15 0.5] Adding and removeing shield and shield collisions
  (if (<= (Variables|Default|Getlives) 0)
    (Variables|/Game/BP_ThirdPersonCharacter.BP_ThirdPersonCharacter_C|SetHasShield (Variables|Default|GetCharRef) false)
    (CallFunction|DropShield)
    (Actor|DestroyActor)
    (else
      (bind _output_get (Variables|Default|Setlives (- (Variables|Default|Getlives) 1)))
      (Development|PrintString (Utilities|String|ToString(Integer) _output_get))
      (Development|PrintString "Shield lives are Bellow 
"))))

(event Custom|DropShield
  (bind _charref (Variables|Default|GetCharRef))
  ;[0.15 0.15 0.15 0.5] Adding and removeing shield and shield collisions
  (Variables|/Game/BP_ThirdPersonCharacter.BP_ThirdPersonCharacter_C|SetStartParry (Variables|Default|GetCharRef) false)
  (Development|PrintString "Shield Removed")
  (Transformation|DetachFromComponent (Variables|Default|GetButtonShield) "KeepRelative" "KeepRelative" "KeepRelative" false)
  (Collision|SetCollisionResponsetoChannel (Variables|Default|GetButtonShield) "ECC_GameTraceChannel2" "ECR_Block")
  (Collision|SetCollisionResponsetoChannel (Variables|Default|GetButtonShield) "ECC_Pawn" "ECR_Block")
  (Physics|SetSimulatePhysics (Variables|Default|GetButtonShield) true)
  (Variables|/Game/BP_ThirdPersonCharacter.BP_ThirdPersonCharacter_C|SetHasShield _charref false)
  (Variables|/Game/BP_ThirdPersonCharacter.BP_ThirdPersonCharacter_C|SetHasItemInHand _charref false)
  (Variables|/Game/BP_ThirdPersonCharacter.BP_ThirdPersonCharacter_C|SetShieldInHand _charref false))

(event Custom|AttachShield
  (bind _charref (Variables|Default|GetCharRef))
  ;[0.15 0.15 0.15 0.5] Adding and removeing shield and shield collisions
  (Variables|/Game/BP_ThirdPersonCharacter.BP_ThirdPersonCharacter_C|SetHasItemInHand _charref false)
  (Variables|/Game/BP_ThirdPersonCharacter.BP_ThirdPersonCharacter_C|SetShieldInHand _charref false)
  (Variables|/Game/BP_ThirdPersonCharacter.BP_ThirdPersonCharacter_C|SetHasShield _charref true)
  (Transformation|AttachComponentToComponent (Variables|/Script/Engine.Character|GetMesh _charref) "ShieldL" "SnapToTarget" "SnapToTarget" "SnapToTarget" false)
  (bind _returnvalue (UserInterface|CreateWidget "/Game/Blueprints_UI/WBP_Ojective.WBP_Ojective_C" 0 "Press LB/T to Parry"))
  (Default|ObjectiveActive _returnvalue)
  (Components|StaticMesh|SetStaticMesh (Variables|Default|GetButtonShield) "/Game/Art/Patch/PATCHED_ButtonShield.PATCHED_ButtonShield"))

(event EventBeginPlay
  (bind _asbp_third_person_character (Utilities|Casting|CastToBP_ThirdPersonCharacter (Game|Player|GetPlayerPawn 0)))
  (Variables|Default|SetCharRef _asbp_third_person_character)
  (bind _returnvalue (AddComponent|AddAudioComponent false))
  (Variables|Default|SetPickUp _returnvalue)
  (bind _returnvalue_2 (AddComponent|AddAudioComponent false))
  (Variables|Default|Sethit _returnvalue_2))

(event EventTick
  (params (DeltaSeconds :type Float%20%28single-precision%29))
  (bind _charref (Variables|Default|GetCharRef))
  (if (not (Variables|/Game/BP_ThirdPersonCharacter.BP_ThirdPersonCharacter_C|GetHasArm _charref))
    (if (Variables|/Game/BP_ThirdPersonCharacter.BP_ThirdPersonCharacter_C|GetHasShield _charref)
      (CallFunction|RemoveShield))))

(fn ConstructionScript)

(fn Interact
  (params (Character :type BP%20Third%20Person%20Character%20Object%20Reference))
  (if (not (Variables|/Game/BP_ThirdPersonCharacter.BP_ThirdPersonCharacter_C|GetHasItemInHand (Variables|Default|GetCharRef)))
    (CallFunction|PickupShield)
    (return false)))