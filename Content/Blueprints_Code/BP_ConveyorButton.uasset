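; BP_ConveyorButton is an interactable button that switches a hooked-up conveyor on or off.
; Box overlaps set CanInteract, which is copied to the player character's CanToggleConverbelt only when an actor overlap begins.
; Interact flips Deactivated on the first valid Spline entry and returns, reaching the nested Control and Auto fallbacks only through invalid entries.
; The GetAllActorsOfClass lookups are unwired, so this graph never fills those arrays.
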(event OnComponentBeginOverlap(Box)
  (params (OverlappedComponent :type Primitive%20Component%20Object%20Reference) (OtherActor :type Actor%20Object%20Reference) (OtherComp :type Primitive%20Component%20Object%20Reference) (OtherBodyIndex :type Integer) (bFromSweep :type Boolean) (SweepResult :type Hit%20Result%20Structure%20%28by%20ref%29))
  (Variables|Default|SetCanInteract true))

(event OnComponentEndOverlap(Box)
  (params (OverlappedComponent :type Primitive%20Component%20Object%20Reference) (OtherActor :type Actor%20Object%20Reference) (OtherComp :type Primitive%20Component%20Object%20Reference) (OtherBodyIndex :type Integer))
  (Variables|Default|SetCanInteract false))

(event EventBeginPlay
  (bind _asbp_third_person_character (Utilities|Casting|CastToBP_ThirdPersonCharacter (Game|GetPlayerCharacter 0)))
  (Variables|Default|SetCharREF _asbp_third_person_character))

(event Collision|EventActorBeginOverlap
  (params (OtherActor :type Actor%20Object%20Reference))
  (bind _charref (Variables|Default|GetCharREF))
  (if (Variables|Default|GetCanInteract)
    (Variables|/Game/BP_ThirdPersonCharacter.BP_ThirdPersonCharacter_C|SetCanToggleConverbelt? _charref true)
    (else
      (Variables|/Game/BP_ThirdPersonCharacter.BP_ThirdPersonCharacter_C|SetCanToggleConverbelt? _charref false))))

(event EventTick
  (params (DeltaSeconds :type Float%20%28single-precision%29)))

(fn ConstructionScript)

(fn Interact
  (params (Character :type BP%20Third%20Person%20Character%20Object%20Reference))
  ;[0.15 0.15 0.15 0.5] Which Conveyor the Button is Hooked Up to
  (bind _array_element (Utilities|Array|ForEachLoopwithBreak (Variables|Default|GetSpline))
    (:LoopBody
      (Utilities|IsValid _array_element
        (:Is%20Valid
          (if (Variables|/Game/Blueprints_Code/BP_ConveyorSpline.BP_ConveyorSpline_C|Getdeactivated _array_element)
            (Variables|/Game/Blueprints_Code/BP_ConveyorSpline.BP_ConveyorSpline_C|Setdeactivated _array_element false)
            (else
              (Variables|/Game/Blueprints_Code/BP_ConveyorSpline.BP_ConveyorSpline_C|Setdeactivated _array_element true))))
        (:Is%20Not%20Valid
          (bind _array_element_2 (Utilities|Array|ForEachLoopwithBreak (Variables|Default|GetControl))
            (:LoopBody
              (Utilities|IsValid _array_element_2
                (:Is%20Valid
                  (if (Variables|/Game/Blueprints_Code/BP_ConverbeltContol.BP_ConverbeltContol_C|GetDeactivated _array_element_2)
                    (Variables|/Game/Blueprints_Code/BP_ConverbeltContol.BP_ConverbeltContol_C|SetDeactivated _array_element_2 false)
                    (else
                      (Variables|/Game/Blueprints_Code/BP_ConverbeltContol.BP_ConverbeltContol_C|SetDeactivated _array_element_2 true))))
                (:Is%20Not%20Valid
                  (bind _array_element_3 (Utilities|Array|ForEachLoopwithBreak (Variables|Default|GetAuto) :!label _label)
                    (:LoopBody
                      (Utilities|IsValid _array_element_3
                        (:Is%20Valid
                          (if (Variables|/Game/Blueprints_Code/BP_ConverbeltAuto.BP_ConverbeltAuto_C|GetDeactivated _array_element_3)
                            (Variables|/Game/Blueprints_Code/BP_ConverbeltAuto.BP_ConverbeltAuto_C|SetDeactivated _array_element_3 false)
                            (else
                              (Variables|/Game/Blueprints_Code/BP_ConverbeltAuto.BP_ConverbeltAuto_C|SetDeactivated _array_element_3 true))))
                        (:Is%20Not%20Valid
                          (goto _label Break)))))))))))
      (Development|PrintString "Button Press")
      (return false))))