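; Voice-activated sliding door that opens when the player character's voice box choice matches the door's CorrectChoice.
; Entering the box shows an objective widget and starts a looping timer that polls the character's choice and door flags.
; A match plays a timeline that slides the door open for good and disables box collision, while a mismatch resets the choice and plays a locked sound.
; A sphere overlap toggles the outline until opened.
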(event OnComponentBeginOverlap(Sphere)
  (params (OverlappedComponent :type Primitive%20Component%20Object%20Reference) (OtherActor :type Actor%20Object%20Reference) (OtherComp :type Primitive%20Component%20Object%20Reference) (OtherBodyIndex :type Integer) (bFromSweep :type Boolean) (SweepResult :type Hit%20Result%20Structure%20%28by%20ref%29))
  (if (not (Variables|Default|GetDOOR%20OPENED))
    ;[0.15 0.15 0.15 0.5] Outline Visibility
    (Rendering|ToggleVisibility (Variables|Default|GetOutline) false)))

(event OnComponentBeginOverlap(Box)
  (params (OverlappedComponent :type Primitive%20Component%20Object%20Reference) (OtherActor :type Actor%20Object%20Reference) (OtherComp :type Primitive%20Component%20Object%20Reference) (OtherBodyIndex :type Integer) (bFromSweep :type Boolean) (SweepResult :type Hit%20Result%20Structure%20%28by%20ref%29))
  (Utilities|Casting|CastToBP_ThirdPersonCharacter OtherActor)
  (bind _returnvalue (UserInterface|CreateWidget "/Game/Blueprints_UI/WBP_Ojective.WBP_Ojective_C" 0 "Voice Activated Door"))
  (Default|ObjectiveActive _returnvalue)
  (Variables|/Game/BP_ThirdPersonCharacter.BP_ThirdPersonCharacter_C|SetNearVADoor (Variables|Default|GetCharRef) true)
  (Variables|Default|SetLooping true)
  (Utilities|Time|SetTimerbyEvent (delegate Custom|PlayerIsNear) 0.1 (Variables|Default|GetLooping)))

(event OnComponentEndOverlap(Box)
  (params (OverlappedComponent :type Primitive%20Component%20Object%20Reference) (OtherActor :type Actor%20Object%20Reference) (OtherComp :type Primitive%20Component%20Object%20Reference) (OtherBodyIndex :type Integer))
  (bind _charref (Variables|Default|GetCharRef))
  (Utilities|Casting|CastToBP_ThirdPersonCharacter OtherActor)
  (if (not (Variables|Default|GetDOOR%20OPENED))
    (Variables|/Game/BP_ThirdPersonCharacter.BP_ThirdPersonCharacter_C|SetNearVADoor _charref false)
    (Variables|/Game/BP_ThirdPersonCharacter.BP_ThirdPersonCharacter_C|SetCanOpenDoor _charref false)
    (Variables|Default|SetLooping false)))

(event OnComponentEndOverlap(Sphere)
  (params (OverlappedComponent :type Primitive%20Component%20Object%20Reference) (OtherActor :type Actor%20Object%20Reference) (OtherComp :type Primitive%20Component%20Object%20Reference) (OtherBodyIndex :type Integer))
  (if (not (Variables|Default|GetDOOR%20OPENED))
    ;[0.15 0.15 0.15 0.5] Outline Visibility
    (Rendering|ToggleVisibility (Variables|Default|GetOutline) true)))

(event Custom|PlayerIsNear
  ;[0.15 0.15 0.15 0.5] Open Door logic
  (if (Utilities|Enum|NotEqual(Enum) "NewEnumerator0" (Variables|/Game/BP_ThirdPersonCharacter.BP_ThirdPersonCharacter_C|GetVoiceBoxChoice (Variables|Default|GetCharRef)))
    (if (Variables|/Game/BP_ThirdPersonCharacter.BP_ThirdPersonCharacter_C|GetNearVADoor (Variables|Default|GetCharRef))
      (if (not (Variables|Default|GetDOOR%20OPENED))
        (if (Variables|/Game/BP_ThirdPersonCharacter.BP_ThirdPersonCharacter_C|GetCanOpenDoor (Variables|Default|GetCharRef))
          (if (Utilities|Enum|Equal(Enum) (Variables|/Game/BP_ThirdPersonCharacter.BP_ThirdPersonCharacter_C|GetVoiceBoxChoice (Variables|Default|GetCharRef)) (Variables|Default|GetCorrectChoice))
            (Rendering|ToggleVisibility (Variables|Default|GetOutline) true)
            (Variables|Default|SetDOOR%20OPENED true)
            (Utilities|FlowControl|Delay 0.8)
            (Audio|PlaySound2D "/Game/Audio/SFX/GameMech/SFX_UnlockOpenDoor.SFX_UnlockOpenDoor" 1.0 1.0 0.0 0 0)
            (bind _doortrack (Timeline|Open/CloseDoor Play)
              (:Update
                (Transformation|SetRelativeLocation (Variables|Default|Getsliding_door) (Math|Vector|MakeVector 0.0 (Math|Float|Lerp 0.0 (Variables|Default|GetSlideDistance) _doortrack) 8.0) false false)
                (Collision|SetCollisionEnabled (Variables|Default|GetBox) "NoCollision")
                (Variables|/Game/BP_ThirdPersonCharacter.BP_ThirdPersonCharacter_C|SetVoiceBoxChoice (Variables|Default|GetCharRef) "NewEnumerator0")))
            (else
              (Variables|/Game/BP_ThirdPersonCharacter.BP_ThirdPersonCharacter_C|SetVoiceBoxChoice (Variables|Default|GetCharRef) "NewEnumerator0")
              (Utilities|FlowControl|Delay 1.0)
              (Audio|PlaySound2D "/Game/Audio/SFX/GameMech/SFX_LockedDoor.SFX_LockedDoor" 1.0 1.0 0.0 0 0)))
          (Utilities|FlowControl|Delay 1.0))))))

(event EventBeginPlay
  (bind _asbp_third_person_character (Utilities|Casting|CastToBP_ThirdPersonCharacter (Game|Player|GetPlayerPawn 0)))
  (Variables|Default|SetCharRef _asbp_third_person_character))

(fn ConstructionScript)