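; BP_MutatedAI is an enemy AI child Blueprint that chases the player on overlap.
; Player overlap starts a looping timer on CheckPlayerInRadius, which raises walk speed and issues AIMoveTo targeting the player controller rather than the pawn.
; End overlap clears PlayerTimer, though the timer's handle is never shown being stored there.
; It then lowers walk speed and re-runs the parent's BeginPlay, whose behavior lives outside this file.
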(event Custom|CheckPlayerInRadius
  (Variables|/Script/Engine.CharacterMovementComponent|SetMaxWalkSpeed (Variables|Character|GetCharacterMovement) 4e+02)
  (AI|AIMoveTo self "0, 0, 0" (Game|GetPlayerController 0) 15.0 false))

(event EventBeginPlay
  (|CallParentFunction))

(event Collision|EventActorBeginOverlap
  (params (OtherActor :type Actor%20Object%20Reference))
  (Utilities|Casting|CastToBP_ThirdPersonCharacter OtherActor)
  (Utilities|Time|SetTimerbyFunctionName 0 "CheckPlayerInRadius" 5.0 true))

(event Collision|EventActorEndOverlap
  (params (OtherActor :type Actor%20Object%20Reference))
  (Utilities|Casting|CastToBP_ThirdPersonCharacter OtherActor)
  (Utilities|Time|ClearandInvalidateTimerbyHandle (Variables|Default|GetPlayerTimer))
  (Variables|/Script/Engine.CharacterMovementComponent|SetMaxWalkSpeed (Variables|Character|GetCharacterMovement) 3.5e+02)
  (|CallParentFunction))

(fn ConstructionScript
  (|CallParentFunction))