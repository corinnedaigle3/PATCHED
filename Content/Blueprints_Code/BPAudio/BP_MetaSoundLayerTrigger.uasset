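; BP_MetaSoundLayerTrigger is a trigger actor that adds and removes a bells layer in the level's MetaSound as the player enters and leaves its volume.
; On BeginPlay it finds and caches the BP_LvlMetaSounds actor.
; Overlaps on its MetaSoundChecker component by BP_ThirdPersonCharacter send AddBells on enter and RemoveBells on exit as trigger parameters, after validity checks on the actor and its MetaSound.
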(event OnComponentBeginOverlap(MetaSoundChecker)
  (params (OverlappedComponent :type Primitive%20Component%20Object%20Reference) (OtherActor :type Actor%20Object%20Reference) (OtherComp :type Primitive%20Component%20Object%20Reference) (OtherBodyIndex :type Integer) (bFromSweep :type Boolean) (SweepResult :type Hit%20Result%20Structure%20%28by%20ref%29))
  (Utilities|Casting|CastToBP_ThirdPersonCharacter OtherActor)
  (bind _lvl_meta_sounds (Variables|Default|GetLvl%20Meta%20Sounds)
    (:then
      (bind _metasound (Variables|/Game/Blueprints_Code/BPAudio/BP_LvlMetaSounds.BP_LvlMetaSounds_C|GetMetaSound _lvl_meta_sounds)
        (:then
          (Class|AudioParameterControllerInterface|SetTriggerParameter _metasound "AddBells"))
        (:else)))
    (:else)))

(event OnComponentEndOverlap(MetaSoundChecker)
  (params (OverlappedComponent :type Primitive%20Component%20Object%20Reference) (OtherActor :type Actor%20Object%20Reference) (OtherComp :type Primitive%20Component%20Object%20Reference) (OtherBodyIndex :type Integer))
  (Utilities|Casting|CastToBP_ThirdPersonCharacter OtherActor)
  (bind _lvl_meta_sounds (Variables|Default|GetLvl%20Meta%20Sounds)
    (:then
      (bind _metasound (Variables|/Game/Blueprints_Code/BPAudio/BP_LvlMetaSounds.BP_LvlMetaSounds_C|GetMetaSound _lvl_meta_sounds)
        (:then
          (Class|AudioParameterControllerInterface|SetTriggerParameter _metasound "RemoveBells"))
        (:else)))
    (:else)))

(event EventBeginPlay
  (bind _returnvalue (Actor|GetActorOfClass "/Game/Blueprints_Code/BPAudio/BP_LvlMetaSounds.BP_LvlMetaSounds_C"))
  (Variables|Default|SetLvl%20Meta%20Sounds _returnvalue))

(fn ConstructionScript)