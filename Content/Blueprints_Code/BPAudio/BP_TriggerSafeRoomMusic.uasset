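; BP_TriggerSafeRoomMusic is a trigger actor that switches safe room music on and off as the player passes through it.
; On actor overlap it checks whether the player pawn is in the enter box or, failing that, the exit box.
; A MusicIsOn flag prevents repeat triggers.
; Entering plays the audio from an offset at full volume, while exiting starts a long linear fade-out and clears the flag immediately.
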(event Custom|Play%20Music
  (bind _saferoommusic (Variables|Default|GetSafeRoomMusic))
  ;[0.15 0.15 0.15 0.5] Play Music
  (Audio|Components|Audio|Play _saferoommusic 4.0)
  (Audio|Components|Audio|AdjustVolume _saferoommusic 0.0 1.0 "Linear" :!class /Script/Engine.AudioComponent)
  (Variables|Default|SetMusicIsOn true)
  (Development|PrintString "Turned music on"))

(event Custom|Turn%20Off%20Music
  ;[0.15 0.15 0.15 0.5] Turn Off music
  (Development|PrintString "Music Fading out")
  (Variables|Default|SetMusicIsOn false)
  (Audio|Components|Audio|AdjustVolume (Variables|Default|GetSafeRoomMusic) 15.0 -1.0 "Linear" :!class /Script/Engine.AudioComponent)
  (Development|PrintString "Turned music off"))

(event Collision|EventActorBeginOverlap
  (params (OtherActor :type Actor%20Object%20Reference))
  ;[0.15 0.15 0.15 0.5] Overlap Enter Box
  (if (Collision|IsOverlappingActor (Variables|Default|GetEnterBox) (Game|Player|GetPlayerPawn 0) :!class /Script/Engine.PrimitiveComponent)
    (if (not (Variables|Default|GetMusicIsOn))
      (CallFunction|PlayMusic))
    (else
      ;[0.15 0.15 0.15 0.5] Overlap Exit Box
      (if (Collision|IsOverlappingActor (Variables|Default|GetExitBox) (Game|Player|GetPlayerPawn 0) :!class /Script/Engine.PrimitiveComponent)
        (if (Variables|Default|GetMusicIsOn)
          (CallFunction|TurnOffMusic))))))

(fn ConstructionScript)