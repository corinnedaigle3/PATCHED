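; BP_BulletMagic is a short-lived bullet actor that acts as a grapple shot for the third-person character.
; On BeginPlay it caches the player and destroys itself after a brief delay.
; Sphere1 overlaps attach the player's Cable end to arm pickups or other actors, then destroy the bullet.
; Leg pickups only print a debug message, while other non-arm actors also receive OnGrappleMessage before attachment.
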(event OnComponentBeginOverlap(Sphere)
  (params (OverlappedComponent :type Primitive%20Component%20Object%20Reference) (OtherActor :type Actor%20Object%20Reference) (OtherComp :type Primitive%20Component%20Object%20Reference) (OtherBodyIndex :type Integer) (bFromSweep :type Boolean) (SweepResult :type Hit%20Result%20Structure%20%28by%20ref%29)))

(event OnComponentBeginOverlap(Sphere1)
  (params (OverlappedComponent :type Primitive%20Component%20Object%20Reference) (OtherActor :type Actor%20Object%20Reference) (OtherComp :type Primitive%20Component%20Object%20Reference) (OtherBodyIndex :type Integer) (bFromSweep :type Boolean) (SweepResult :type Hit%20Result%20Structure%20%28by%20ref%29))
  (bind _asbp_pick_up_equipt_arm (Utilities|Casting|CastToBP_PickUpEquiptArm OtherActor)
    (:then
      (Class|CableComponent|SetAttachEndto (Variables|/Game/BP_ThirdPersonCharacter.BP_ThirdPersonCharacter_C|GetCable (Variables|Default|GetPlayer)) _asbp_pick_up_equipt_arm "None" "None")
      (Development|PrintString "end should be limb" true true "(R=0.000000,G=0.660000,B=1.000000,A=1.000000)" 1e+01)
      (Actor|DestroyActor :!label _label))
    (:CastFailed
      (Utilities|Casting|CastToBP_PickUpEquiptLeg OtherActor
        (:then
          (Development|PrintString "Hit leg" true true "(R=1.000000,G=0.024888,B=0.000000,A=1.000000)"))
        (:CastFailed
          (Class|BPIGrapple|OnGrapple(Message) OtherActor)
          (Class|CableComponent|SetAttachEndto (Variables|/Game/BP_ThirdPersonCharacter.BP_ThirdPersonCharacter_C|GetCable (Variables|Default|GetPlayer)) OtherActor "None" "None")
          (goto _label))))))

(event EventBeginPlay
  (bind _returnvalue (Actor|GetActorOfClass "/Game/BP_ThirdPersonCharacter.BP_ThirdPersonCharacter_C"))
  (Variables|Default|SetPlayer _returnvalue)
  (Utilities|FlowControl|Delay 3.0)
  (Actor|DestroyActor))

(event Collision|EventActorBeginOverlap
  (params (OtherActor :type Actor%20Object%20Reference)))

(event EventTick
  (params (DeltaSeconds :type Float%20%28single-precision%29)))

(fn ConstructionScript)