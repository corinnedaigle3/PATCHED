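; BP_Steam is a steam actor that travels along a referenced spline and detects overlaps with its box component.
; The MoveSteam event sets a timeline play rate from TimeToComplete, then each update maps the track alpha to spline distance to set world location and rotation.
; The box overlap only prints a "Hit Player" debug string, without checking which actor entered.
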(event OnComponentBeginOverlap(BoxSteam)
  (params (OverlappedComponent :type Primitive%20Component%20Object%20Reference) (OtherActor :type Actor%20Object%20Reference) (OtherComp :type Primitive%20Component%20Object%20Reference) (OtherBodyIndex :type Integer) (bFromSweep :type Boolean) (SweepResult :type Hit%20Result%20Structure%20%28by%20ref%29))
  (Development|PrintString "Hit Player"))

(event Custom|MoveSteam
  (bind _spline_to_follow (Variables|Default|GetSpline%20To%20Follow))
  (bind _spline (Variables|/Game/Blueprints_Code/BP_SplineHazards.BP_SplineHazards_C|GetSpline _spline_to_follow))
  (Components|Timeline|SetPlayRate (Variables|Default|GetT_MSteam) (/ 1.0 (Variables|Default|GetTime%20To%20Complete)))
  (bind _newtrack_1 (Timeline|T_MSteam Play)
    (:Update
      (Transformation|SetActorLocationAndRotation (Spline|GetLocationatDistanceAlongSpline _spline (Math|Float|Lerp 0.0 (Spline|GetSplineLength _spline) _newtrack_1) "World") (Spline|GetRotationatDistanceAlongSpline _spline (Math|Float|Lerp 0.0 (Spline|GetSplineLength _spline) _newtrack_1) "World")))))

(event EventBeginPlay)

(fn ConstructionScript)