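; BP_EnemySimple is an experimental simple enemy that chases the player, extending a parent enemy Blueprint.
; BeginPlay creates a looping timer for ChasePlayer but pauses it immediately, and optionally adds whoosh audio.
; ChasePlayer uses DoOnce to pause the timer and run AI MoveTo toward CharRef at chase speed, stopping inside attack range.
; Success plays audio and rearms the timer and DoOnce, while failure only clears the Chase flag.
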(event Custom|ChasePlayer
  (Utilities|FlowControl|DoOnce false :!label _label
    (:Completed
      (if (not (Variables|Default|GetHospitalChaseEnemey))
        (Audio|Components|Audio|Play (Variables|Default|GetSFX_DeafScream) 0.0))
      (Variables|Default|SetChase true)
      (Utilities|Time|PauseTimerbyHandle (Variables|Default|GetTimer))
      (AI|AIMoveTo self "0, 0, 0" (Variables|Default|GetCharRef) (- (Variables|Default|GetAttack%20Range) 2e+01) false
        (:then
          (Variables|/Script/Engine.CharacterMovementComponent|SetMaxWalkSpeed (Variables|Character|GetCharacterMovement) (Variables|Default|GetChaseSpeed)))
        (:OnSuccess
          (if (not (Variables|Default|GetHospitalChaseEnemey))
            (Audio|PlaySound2D "/Game/Audio/SFX/GameMech/SFX_Whoosh1.SFX_Whoosh1" 1.0 1.0 0.0 0 0))
          (Variables|Default|SetChase false)
          (Audio|Components|Audio|Play (Variables|Default|GetWhooshSFX) 0.0)
          (Utilities|Time|UnpauseTimerbyHandle (Variables|Default|GetTimer))
          (goto _label Reset))
        (:OnFail
          (Variables|Default|SetChase false))))))

(event EventBeginPlay
  (|CallParentFunction)
  (Variables|Default|SetSimple? true)
  (bind _returnvalue (Utilities|Time|SetTimerbyEvent (delegate Custom|ChasePlayer) 2.0 true))
  (bind _output_get (Variables|Default|SetTimer _returnvalue))
  (Utilities|Time|PauseTimerbyHandle _output_get)
  (if (Variables|Default|GetCanPlayAudio)
    (bind _returnvalue_2 (AddComponent|AddAudioComponent false))
    (Variables|Default|SetWhooshSFX _returnvalue_2)))

(event Collision|EventActorBeginOverlap
  (params (OtherActor :type Actor%20Object%20Reference)))

(fn ConstructionScript
  (|CallParentFunction))