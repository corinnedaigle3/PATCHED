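; BP_SimpleEnemyB is an experimental melee enemy that chases and attacks the player.
; Its AI_Blind or AI_Deaf controller event triggers ChasePlayer, a one-shot AI move at chase speed, followed by a range check.
; The attack sphere-traces forward, ignoring same-class enemies, and costs the player a life, or shield life when parrying.
; After a hit, ResetChase replays animations and re-enters the chase's DoOnce, which is never reset.
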(event Custom|ChasePlayer
  (Utilities|FlowControl|DoOnce false
    (:Completed
      (CallFunction|ChaseAnimation)
      (AI|AIMoveTo self "0, 0, 0" (Variables|Default|GetCharRef) (- (Variables|Default|GetAttack%20Range) 2e+01) false
        (:then
          (Variables|/Script/Engine.CharacterMovementComponent|SetMaxWalkSpeed (Variables|Character|GetCharacterMovement) (Variables|Default|GetChaseSpeed)))
        (:OnSuccess
          (bind _in_range (CallFunction|CheckifinRange))
          (if _in_range
            (if (not (Variables|Default|GetAttacked))
              (CallFunction|AttackPlayer))))
        (:OnFail
          (Development|PrintString "Hello"))))))

(event Custom|Attack%20Player
  (bind _returnvalue (Transformation|GetActorLocation))
  (bind _charref (Variables|Default|GetCharRef))
  ;[0.15 0.15 0.15 0.5] Catched the player
  (if (not (Variables|Default|GetAttacked))
    (bind _animationattack (Variables|Default|GetAnimationAttack)
      (:then
        (Components|Animation|PlayAnimation (Variables|Character|GetMesh) _animationattack false))
      (:else
        _))
    (bind (_outhit _returnvalue_2) (Collision|SphereTraceForObjects _returnvalue (+ _returnvalue (* (Math|Vector|GetForwardVector (Transformation|GetActorRotation)) (Variables|Default|GetAttack%20Range))) 5e+01 (Utilities|Array|MakeArray "ObjectTypeQuery3") false (Variables|Default|GetActors) "ForDuration" true "(R=1.000000,G=0.000000,B=0.000000,A=1.000000)" "(R=0.000000,G=1.000000,B=0.000000,A=1.000000)" 1.0))
    (if _returnvalue_2
      (bind _asbp_third_person_character (Utilities|Casting|CastToBP_ThirdPersonCharacter (.HitActor (Collision|BreakHitResult _outhit)))
        (:then
          (if (not (Variables|Default|GetAttacked))
            (Variables|Default|SetAttacked true)
            (if (Variables|/Game/BP_ThirdPersonCharacter.BP_ThirdPersonCharacter_C|GetisParrying _charref)
              (Development|PrintString "StunEnemy")
              (Default|ShieldLoseLife (Variables|/Game/BP_ThirdPersonCharacter.BP_ThirdPersonCharacter_C|GetShield _charref))
              (else
                (Default|LoseALive _asbp_third_person_character)
                (Development|PrintString "playr should lose a liveeeeeeeeeeeeeeee" true true "(R=0.598958,G=0.040344,B=0.060081,A=1.000000)" 1e+01)))
            (Utilities|FlowControl|Delay 0.5)
            (Variables|Default|SetAttacked false)
            (CallFunction|ResetChase)))
        (:CastFailed
          (Development|PrintString "Did not reach palyerrrrrrrrrrrrrrrrrrrrrrrrrrrrrr"))))
    (else
      (Development|PrintString "already attacked "))))

(event Custom|Reset%20Chase
  (Components|Animation|PlayAnimation (Variables|Character|GetMesh) (Variables|Default|GetAnimationIdl) false)
  (Utilities|FlowControl|Delay 1.0)
  (CallFunction|ChaseAnimation)
  (Utilities|FlowControl|DoOnce false
    (:Completed
      (CallFunction|ChaseAnimation)
      (AI|AIMoveTo self "0, 0, 0" (Variables|Default|GetCharRef) (- (Variables|Default|GetAttack%20Range) 2e+01) false
        (:then
          (Variables|/Script/Engine.CharacterMovementComponent|SetMaxWalkSpeed (Variables|Character|GetCharacterMovement) (Variables|Default|GetChaseSpeed)))
        (:OnSuccess
          (bind _in_range (CallFunction|CheckifinRange))
          (if _in_range
            (if (not (Variables|Default|GetAttacked))
              (CallFunction|AttackPlayer))))
        (:OnFail
          (Development|PrintString "Hello"))))))

(event Custom|Chase%20Animation
  (Components|Animation|PlayAnimation (Variables|Character|GetMesh) "/Game/Animations/Enemy_Anims/AS_Enemy_Chase.AS_Enemy_Chase" true))

(event EventBeginPlay
  (bind _outactors (Actor|GetAllActorsOfClass "BP_SimpleEnemyB_C"))
  (Variables|Default|SetActors _outactors)
  (bind _asbp_third_person_character (Utilities|Casting|CastToBP_ThirdPersonCharacter (Game|Player|GetPlayerPawn 0)))
  (Variables|Default|SetCharRef _asbp_third_person_character)
  (AddComponent|AddAudioComponent false)
  (bind _output_get (Variables|Default|SetAiController (AI|GetAIController self)))
  (bind _asai_blind (Utilities|Casting|CastToAI_Blind _output_get)
    (:then
      (EventDispatchers|BindEventtoChasingPlayer _asai_blind (delegate Custom|ChasePlayer)))
    (:CastFailed
      (bind _asai_deaf (Utilities|Casting|CastToAI_Deaf _output_get))
      (EventDispatchers|AssignSawPlayer _asai_deaf (delegate Custom|ChasePlayer)))))

(fn ConstructionScript)

(fn CheckifinRange
  (Variables|Default|GetCharRef
    (:then
      _)
    (:else
      (bind _returnvalue (Actor|GetActorOfClass "/Game/BP_ThirdPersonCharacter.BP_ThirdPersonCharacter_C"))
      (Variables|Default|SetCharRef _returnvalue)))
  (return (<= (Math|Vector|VectorLength (- (Transformation|GetActorLocation) (Transformation|GetActorLocation (Variables|Default|GetCharRef)))) (Variables|Default|GetAttack%20Range))))