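; Experimental enemy spawner meant to place blind or deaf enemies, chosen by the Blind flag, at an array of spawn locations.
; SpawnEnemy spawns one at the indexed location, then calls SpawnLoop, which recurses back while IndexP is within an inclusive length check.
; IndexP is reset to 1 each spawn, so the recursion never advances.
; The EventGraph's delayed-loop logic is disconnected, and no event here starts spawning.
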(fn ConstructionScript)

(fn SpawnEnemy
  (params (index :type Integer))
  (bind _enemysapwnlocation (Variables|Default|GetEnemySapwnLocation))
  (bind _output (Utilities|Array|Get(acopy) _enemysapwnlocation index))
  (bind _location (Math|Transform|BreakTransform _output))
  (if (Variables|Default|GetBlind?)
    (Game|SpawnActorfromClass "/Game/Blueprints_Code/Experimental/BP_NewEnemyBlind.BP_NewEnemyBlind_C" (Math|Transform|MakeTransform _location "0, 0, 0" "1.000000,1.000000,1.000000") "Undefined" "MultiplyWithRoot" 0 0)
    (else
      (Game|SpawnActorfromClass "/Game/Blueprints_Code/Experimental/BP_NewEnemyDeaf.BP_NewEnemyDeaf_C" (Math|Transform|MakeTransform _location "0, 0, 0" "1.000000,1.000000,1.000000") "Undefined" "MultiplyWithRoot" 0 0)))
  (Variables|Default|SetIndexP (+ 0 1))
  (Utilities|SpawnLoop))