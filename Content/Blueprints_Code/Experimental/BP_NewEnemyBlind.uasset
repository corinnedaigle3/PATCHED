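; Blind enemy character, driven by an AI_Blind controller, that chases and attacks the player.
; Tick switches walk speed between normal and chase values based on the Chase flag, which is set outside this Blueprint.
; AttackPlayer sphere-traces forward, ignoring blind and deaf enemies, and costs the player a life unless parrying, with a short cooldown.
; Parry stun is only a debug print, and the Box overlap attack and movement-pause logic are disconnected.
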(event OnComponentBeginOverlap(Box)
  (params (OverlappedComponent :type Primitive%20Component%20Object%20Reference) (OtherActor :type Actor%20Object%20Reference) (OtherComp :type Primitive%20Component%20Object%20Reference) (OtherBodyIndex :type Integer) (bFromSweep :type Boolean) (SweepResult :type Hit%20Result%20Structure%20%28by%20ref%29)))

(event Custom|Attack%20Player
  (bind _returnvalue (Transformation|GetActorLocation))
  ;[0.15 0.15 0.15 0.5] Catched the player
  (if (not (Variables|Default|GetAttacked))
    (Components|Activation|SetActive (Variables|Default|GetBox) false false)
    (bind (_outhit _returnvalue_2) (Collision|SphereTraceForObjects _returnvalue (+ _returnvalue (* (Math|Vector|GetForwardVector (Transformation|GetActorRotation)) (Variables|Default|GetAttack%20Range))) 5e+01 (Utilities|Array|MakeArray "ObjectTypeQuery3") false (Variables|Default|GetActors) "ForDuration" true "(R=1.000000,G=0.000000,B=0.000000,A=1.000000)" "(R=0.000000,G=1.000000,B=0.000000,A=1.000000)" 1.0))
    (if _returnvalue_2
      (bind _asbp_third_person_character (Utilities|Casting|CastToBP_ThirdPersonCharacter (.HitActor (Collision|BreakHitResult _outhit)))
        (:then
          (if (not (Variables|Default|GetAttacked))
            (Variables|Default|SetAttacked true)
            (if (Variables|/Game/BP_ThirdPersonCharacter.BP_ThirdPersonCharacter_C|GetisParrying (Variables|Default|GetCharRef))
              (Development|PrintString "StunEnemy")
              (else
                (Default|LoseALive _asbp_third_person_character)
                (Development|PrintString "playr should lose a liveeeeeeeeeeeeeeee" true true "(R=0.598958,G=0.040344,B=0.060081,A=1.000000)" 1e+01)))
            (Utilities|FlowControl|Delay 0.5)
            (Variables|Default|SetAttacked false)))
        (:CastFailed
          (Development|PrintString "Did not reach palyerrrrrrrrrrrrrrrrrrrrrrrrrrrrrr"))))
    (else
      (Development|PrintString "already attacked "))))

(event EventBeginPlay
  (bind _outactors (Actor|GetAllActorsOfClass "BP_NewEnemyBlind_C"))
  (for _array_element _outactors
    (Utilities|Array|AddUnique (Variables|Default|GetActors) _array_element))
  (bind _outactors_2 (Actor|GetAllActorsOfClass "/Game/Blueprints_Code/Experimental/BP_NewEnemyDeaf.BP_NewEnemyDeaf_C"))
  (for _array_element_2 _outactors_2
    (Utilities|Array|AddUnique (Variables|Default|GetActors) _array_element_2))
  (bind _returnvalue (Actor|GetActorOfClass "/Game/BP_ThirdPersonCharacter.BP_ThirdPersonCharacter_C"))
  (Variables|Default|SetPlayer _returnvalue)
  (bind _asai_blind (Utilities|Casting|CastToAI_Blind (AI|GetAIController self)))
  (Variables|Default|SetAi _asai_blind)
  (bind _asbp_third_person_character (Utilities|Casting|CastToBP_ThirdPersonCharacter (Game|Player|GetPlayerPawn 0)))
  (Variables|Default|SetCharRef _asbp_third_person_character))

(event Collision|EventActorBeginOverlap
  (params (OtherActor :type Actor%20Object%20Reference)))

(event EventTick
  (params (DeltaSeconds :type Float%20%28single-precision%29))
  ;[0.15 0.15 0.15 0.5] Updates varaible in AI Class
  (CallFunction|DetermineSpeed))

(fn ConstructionScript)

(fn DetermineSpeed
  (bind _chasespeed (Variables|Default|GetChaseSpeed))
  (bind _normalspeed (Variables|Default|GetNormalSpeed))
  (bind _charactermovement (Variables|Character|GetCharacterMovement))
  (if (Variables|Default|GetChase)
    (if (!= (Variables|/Script/Engine.CharacterMovementComponent|GetMaxWalkSpeed _charactermovement) _chasespeed)
      (Variables|/Script/Engine.CharacterMovementComponent|SetMaxWalkSpeed _charactermovement _chasespeed))
    (elif (!= (Variables|/Script/Engine.CharacterMovementComponent|GetMaxWalkSpeed (Variables|Character|GetCharacterMovement)) _normalspeed)
      (Variables|/Script/Engine.CharacterMovementComponent|SetMaxWalkSpeed _charactermovement _normalspeed))))