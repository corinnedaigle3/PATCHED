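; Experimental AI pawn, apparently a simple "blind" enemy, that chases a referenced character when ChasePlayer fires.
; A DoOnce with no reset lets the chase run once, starting an AI MoveTo to just inside attack range at chase speed.
; The chase flag clears a second after arrival, while failure only prints debug text.
; Tick is empty, leaving the distance-based AttackPlayer check disconnected.
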(event Custom|ChasePlayer
  (Utilities|FlowControl|DoOnce false
    (:Completed
      (Variables|Default|SetChase true)
      (Development|PrintString "i am chasing " true true "(R=1.000000,G=0.000000,B=0.190167,A=1.000000)")
      (AI|AIMoveTo self "0, 0, 0" (Variables|Default|GetCharRef) (- (Variables|Default|GetAttack%20Range) 2e+01) false
        (:then
          (Variables|/Script/Engine.CharacterMovementComponent|SetMaxWalkSpeed (Variables|Character|GetCharacterMovement) (Variables|Default|GetChaseSpeed)))
        (:OnSuccess
          (Utilities|FlowControl|Delay 1.0)
          (Variables|Default|SetChase false))
        (:OnFail
          (Development|PrintString "Hello"))))))

(event EventBeginPlay
  (|CallParentFunction))

(event Collision|EventActorBeginOverlap
  (params (OtherActor :type Actor%20Object%20Reference)))

(event EventTick
  (params (DeltaSeconds :type Float%20%28single-precision%29)))

(fn ConstructionScript
  (|CallParentFunction))