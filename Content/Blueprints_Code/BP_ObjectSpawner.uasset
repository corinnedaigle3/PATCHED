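; BP_ObjectSpawner is an actor that repeatedly spawns a configurable class of object at its own transform.
; On Tick, a Waiting flag gates the spawn, so the first one happens on the first tick.
; After each spawn, a Delay of SpawnRateSec clears the flag, making that variable the interval between spawns rather than using a timer.
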(event EventBeginPlay)

(event Collision|EventActorBeginOverlap
  (params (OtherActor :type Actor%20Object%20Reference)))

(event EventTick
  (params (DeltaSeconds :type Float%20%28single-precision%29))
  (if (not (Variables|Default|GetWaiting))
    (Variables|Default|SetWaiting true)
    (Game|SpawnActorfromClass (Variables|Default|GetObjectToSpawn) (Transformation|GetActorTransform self) "Undefined" "MultiplyWithRoot" 0 0)
    (Utilities|FlowControl|Delay (Variables|Default|GetSpawnRateSec))
    (Variables|Default|SetWaiting false)))

(fn ConstructionScript)