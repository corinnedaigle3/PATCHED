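; Stationary enemy AI that watches for the player by turning in place, and screams when it spots them.
; A looping timer cycles through preset target rotations, which Tick eases toward with RInterpTo.
; PawnSensing sightings of BP_ThirdPersonCharacter pause the rotation and play the scream, rate-limited by a DoOnce with a delayed reset.
; Retriggerable delays act as a lost-sight timeout that resumes turning, then fades out the scream.
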(event OnSeePawn(PawnSensing)
  (params (Pawn :type Pawn%20Object%20Reference))
  ;[0.15 0.15 0.15 0.5] Sensing Player
  (Utilities|FlowControl|Sequence
    (:then_0
      (if (not (Variables|Default|GetCanSeePlayer))
        (Utilities|Casting|CastToBP_ThirdPersonCharacter Pawn)
        (Variables|Default|SetCanSeePlayer true)
        (Variables|Default|SetIsRotating false)
        (CallFunction|Scream)))
    (:then_1
      (Utilities|FlowControl|RetriggerableDelay 1.0)
      (Variables|Default|SetCanSeePlayer false)
      (Variables|Default|SetIsRotating true)
      (Utilities|FlowControl|RetriggerableDelay 1.5)
      (if (not (Variables|Default|GetCanSeePlayer))
        (CallFunction|StopScream)
        (CallFunction|NextRotation)))))

(event Custom|Scream
  ;[0.15 0.15 0.15 0.5] Screaming at Player
  (CallFunction|PlayScream)
  (Variables|Default|SetCanSeePlayer false)
  (Variables|Default|SetIsRotating false)
  (CallFunction|NextRotation))

(event Custom|NextRotation
  ;[0.15 0.15 0.15 0.5] Rotates enemy every 3 seconds
  (if (Variables|Default|GetIsRotating)
    (switch int (Variables|Default|GetRotationIndex)
      (:0
        (Variables|Default|SetTargetRotation "0.000000,90.000000,0.000000")
        (Math|Integer|IncrementInt (Variables|Default|GetRotationIndex)
          (:%20%20
            _)))
      (:1
        (Variables|Default|SetTargetRotation "0.000000,180.000000,0.000000")
        (Math|Integer|IncrementInt (Variables|Default|GetRotationIndex)
          (:%20%20
            _)))
      (:2
        (Variables|Default|SetTargetRotation "0.000000,-90.000000,0.000000")
        (Math|Integer|IncrementInt (Variables|Default|GetRotationIndex)
          (:%20%20
            _)))
      (:3
        (Variables|Default|SetTargetRotation "0.000000,180.000000,0.000000")
        (Math|Integer|IncrementInt (Variables|Default|GetRotationIndex)
          (:%20%20
            _))))
    (if (> (Variables|Default|GetRotationIndex) 3)
      (Variables|Default|SetRotationIndex 0))))

(event Custom|PlayScream
  ;[0.15 0.15 0.15 0.5] Plays Enemy Audio Scream
  (Utilities|FlowControl|DoOnce false :!label _label
    (:Completed
      (Audio|Components|Audio|Play (Variables|Default|GetSFX_DeafScream) 0.0)
      (Utilities|FlowControl|Delay 5.5)
      (goto _label Reset))))

(event Custom|StopScream
  ;[0.15 0.15 0.15 0.5] Fades Enemy Audio Scream
  (Audio|Components|Audio|FadeOut (Variables|Default|GetSFX_DeafScream) 2.0 0.0 "Linear" :!class /Script/Engine.AudioComponent))

(event EventBeginPlay
  ;[0.15 0.15 0.15 0.5] Rotates enemy every 3 seconds
  (Utilities|Time|SetTimerbyEvent (delegate Custom|NextRotation) 3.0 true))

(event EventTick
  (params (DeltaSeconds :type Float%20%28single-precision%29))
  ;[0.15 0.15 0.15 0.5] Creates a smooth rotation
  (if (Variables|Default|GetIsRotating)
    (Transformation|SetActorRotation (Math|Interpolation|RInterpTo (Transformation|GetActorRotation) (Variables|Default|GetTargetRotation) (Utilities|Time|GetWorldDeltaSeconds) 2.0))))

(fn ConstructionScript
  (|CallParentFunction))