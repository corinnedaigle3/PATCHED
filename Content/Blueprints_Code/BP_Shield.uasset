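; BP_Shield is an interactable, physics-simulated shield that the player carries, attaches and uses for a single parry.
; Pickup requires an arm and a free hand, snapping it to a carry socket; AttachShield moves it to the left-side socket, with objective widgets prompting.
; Box overlaps with deaf or blind enemies enable parrying, which destroys the shield after a brief delay.
; Tick drops an attached shield if the arm is lost.
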(event OnComponentBeginOverlap(Box)
  (params (OverlappedComponent :type Primitive%20Component%20Object%20Reference) (OtherActor :type Actor%20Object%20Reference) (OtherComp :type Primitive%20Component%20Object%20Reference) (OtherBodyIndex :type Integer) (bFromSweep :type Boolean) (SweepResult :type Hit%20Result%20Structure%20%28by%20ref%29))
  ;[0.15 0.15 0.15 0.5] Check if overlaping enemy
  (Utilities|FlowControl|Sequence
    (:then_0
      (Utilities|Casting|CastToBP_NewEnemyDeaf OtherActor))
    (:then_1
      (Utilities|Casting|CastToBP_NewEnemyBlind OtherActor)))
  (Variables|Default|SetCanParry true)
  (Development|PrintString "Can Parry"))

(event OnComponentEndOverlap(Box)
  (params (OverlappedComponent :type Primitive%20Component%20Object%20Reference) (OtherActor :type Actor%20Object%20Reference) (OtherComp :type Primitive%20Component%20Object%20Reference) (OtherBodyIndex :type Integer))
  ;[0.15 0.15 0.15 0.5] Check if overlaping enemy
  (Utilities|FlowControl|Sequence
    (:then_0
      (Utilities|Casting|CastToBP_NewEnemyDeaf OtherActor))
    (:then_1
      (Utilities|Casting|CastToBP_NewEnemyBlind OtherActor)))
  (Variables|Default|SetCanParry false)
  (Development|PrintString "Can't Parry"))

(event Custom|PickupShield
  (bind _charref (Variables|Default|GetCharRef))
  (bind _charref_2 (Variables|Default|GetCharRef))
  ;[0.15 0.15 0.15 0.5] Adding and removeing shield and shield collisions
  (if (Variables|/Game/BP_ThirdPersonCharacter.BP_ThirdPersonCharacter_C|GetHasArm _charref_2)
    (if (not (Variables|/Game/BP_ThirdPersonCharacter.BP_ThirdPersonCharacter_C|GetHasItemInHand _charref_2))
      (Variables|/Game/BP_ThirdPersonCharacter.BP_ThirdPersonCharacter_C|SetPickUpShield _charref_2 self)
      (Audio|Components|Audio|Play (Variables|Default|GetPickUp) 0.0)
      (Physics|SetSimulatePhysics (Variables|Default|GetButtonShield) false)
      (Variables|/Game/BP_ThirdPersonCharacter.BP_ThirdPersonCharacter_C|SetHasItemInHand _charref true)
      (Variables|/Game/BP_ThirdPersonCharacter.BP_ThirdPersonCharacter_C|SetShieldInHand _charref true)
      (Transformation|AttachComponentToComponent (Variables|/Script/Engine.Character|GetMesh _charref) "CarryShieldR" "SnapToTarget" "SnapToTarget" "SnapToTarget" false)
      (Collision|SetCollisionResponsetoChannel (Variables|Default|GetButtonShield) "ECC_GameTraceChannel2" "ECR_Ignore")
      (bind _returnvalue (UserInterface|CreateWidget "/Game/Blueprints_UI/WBP_Ojective.WBP_Ojective_C" 0 "Hold X/E to attach"))
      (Default|ObjectiveActive _returnvalue))
    (else
      (bind _returnvalue_2 (UserInterface|CreateWidget "/Game/Blueprints_UI/WBP_Ojective.WBP_Ojective_C" 0 "Must have Left ARM"))
      (Default|ObjectiveActive _returnvalue_2))))

(event Custom|RemoveShield
  ;[0.15 0.15 0.15 0.5] Adding and removeing shield and shield collisions
  (CallFunction|DropShield)
  (Actor|DestroyActor))

(event Custom|DropShield
  (bind _charref (Variables|Default|GetCharRef))
  ;[0.15 0.15 0.15 0.5] Adding and removeing shield and shield collisions
  (Variables|Default|SetCanParry false)
  (Development|PrintString "Shield Removed")
  (Transformation|DetachFromComponent (Variables|Default|GetButtonShield) "KeepRelative" "KeepRelative" "KeepRelative" false)
  (Collision|SetCollisionResponsetoChannel (Variables|Default|GetButtonShield) "ECC_GameTraceChannel2" "ECR_Block")
  (Physics|SetSimulatePhysics (Variables|Default|GetButtonShield) true)
  (Variables|/Game/BP_ThirdPersonCharacter.BP_ThirdPersonCharacter_C|SetHasShield _charref false)
  (Variables|/Game/BP_ThirdPersonCharacter.BP_ThirdPersonCharacter_C|SetHasItemInHand _charref false)
  (Variables|/Game/BP_ThirdPersonCharacter.BP_ThirdPersonCharacter_C|SetShieldInHand _charref false))

(event Custom|Parrying
  ;[0.15 0.15 0.15 0.5] Parrying Logic
  (if (Variables|/Game/BP_ThirdPersonCharacter.BP_ThirdPersonCharacter_C|GetHasShield (Variables|Default|GetCharRef))
    (if (Variables|Default|GetCanParry)
      (Variables|Default|SetIsParrying true)
      (Audio|Components|Audio|Play (Variables|Default|Gethit) 0.0)
      (Development|PrintText "Parry Animation")
      (Utilities|FlowControl|Delay 1.0)
      (Variables|Default|SetIsParrying false)
      (CallFunction|RemoveShield))))

(event Custom|AttachShield
  (bind _charref (Variables|Default|GetCharRef))
  ;[0.15 0.15 0.15 0.5] Adding and removeing shield and shield collisions
  (Variables|/Game/BP_ThirdPersonCharacter.BP_ThirdPersonCharacter_C|SetHasItemInHand _charref false)
  (Variables|/Game/BP_ThirdPersonCharacter.BP_ThirdPersonCharacter_C|SetShieldInHand _charref false)
  (Variables|/Game/BP_ThirdPersonCharacter.BP_ThirdPersonCharacter_C|SetHasShield _charref true)
  (Transformation|AttachComponentToComponent (Variables|/Script/Engine.Character|GetMesh _charref) "ShieldL" "SnapToTarget" "SnapToTarget" "SnapToTarget" false)
  (bind _returnvalue (UserInterface|CreateWidget "/Game/Blueprints_UI/WBP_Ojective.WBP_Ojective_C" 0 "Press LB/T to Parry"))
  (Default|ObjectiveActive _returnvalue))

(event EventBeginPlay
  (bind _asbp_third_person_character (Utilities|Casting|CastToBP_ThirdPersonCharacter (Game|Player|GetPlayerPawn 0)))
  (Variables|Default|SetCharRef _asbp_third_person_character)
  (bind _returnvalue (AddComponent|AddAudioComponent false))
  (Variables|Default|SetPickUp _returnvalue)
  (bind _returnvalue_2 (AddComponent|AddAudioComponent false))
  (Variables|Default|Sethit _returnvalue_2))

(event EventTick
  (params (DeltaSeconds :type Float%20%28single-precision%29))
  (bind _charref (Variables|Default|GetCharRef))
  (if (not (Variables|/Game/BP_ThirdPersonCharacter.BP_ThirdPersonCharacter_C|GetHasArm _charref))
    (if (Variables|/Game/BP_ThirdPersonCharacter.BP_ThirdPersonCharacter_C|GetHasShield _charref)
      (CallFunction|DropShield))))

(fn ConstructionScript)

(fn Interact
  (params (Character :type BP%20Third%20Person%20Character%20Object%20Reference))
  (if (not (Variables|/Game/BP_ThirdPersonCharacter.BP_ThirdPersonCharacter_C|GetHasItemInHand (Variables|Default|GetCharRef)))
    (CallFunction|PickupShield)
    (return false)))