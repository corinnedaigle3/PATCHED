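; BP_DisableInvisibleWall is a trigger volume meant to switch off an invisible wall while the third-person character is inside it.
; Its Box overlap events filter for BP_ThirdPersonCharacter, deactivating the Box component of the referenced Collider on entry and reactivating it on exit.
; The toggle uses SetActive on that component and does not change collision settings directly.
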(event OnComponentBeginOverlap(Box)
  (params (OverlappedComponent :type Primitive%20Component%20Object%20Reference) (OtherActor :type Actor%20Object%20Reference) (OtherComp :type Primitive%20Component%20Object%20Reference) (OtherBodyIndex :type Integer) (bFromSweep :type Boolean) (SweepResult :type Hit%20Result%20Structure%20%28by%20ref%29))
  (if (Class|GameplayStatics|ObjectIsA OtherActor "/Game/BP_ThirdPersonCharacter.BP_ThirdPersonCharacter_C")
    (Components|Activation|SetActive (Variables|/Game/ThirdPerson/Blueprints/BP_InvisibleWall.BP_InvisibleWall_C|GetBox (Variables|Default|GetCollider)) false false)))

(event OnComponentEndOverlap(Box)
  (params (OverlappedComponent :type Primitive%20Component%20Object%20Reference) (OtherActor :type Actor%20Object%20Reference) (OtherComp :type Primitive%20Component%20Object%20Reference) (OtherBodyIndex :type Integer))
  (if (Class|GameplayStatics|ObjectIsA OtherActor "/Game/BP_ThirdPersonCharacter.BP_ThirdPersonCharacter_C")
    (Components|Activation|SetActive (Variables|/Game/ThirdPerson/Blueprints/BP_InvisibleWall.BP_InvisibleWall_C|GetBox (Variables|Default|GetCollider)) true false)))

(event EventBeginPlay)

(event Collision|EventActorBeginOverlap
  (params (OtherActor :type Actor%20Object%20Reference)))

(event EventTick
  (params (DeltaSeconds :type Float%20%28single-precision%29)))

(fn ConstructionScript)