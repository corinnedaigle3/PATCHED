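; BP_Cube is a box that the third-person character moves while interacting with it.
; Overlapping the Fwd component toggles CanInteractBox on the cached character reference, without checking what overlapped.
; While both interaction flags are set, Tick turns the character's input axes into SMCube movement along its own axes, using its right vector for forward/back.
; SpeedDirection interpolates relative location without sweep; Interact only returns false.
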(event OnComponentBeginOverlap(Fwd)
  (params (OverlappedComponent :type Primitive%20Component%20Object%20Reference) (OtherActor :type Actor%20Object%20Reference) (OtherComp :type Primitive%20Component%20Object%20Reference) (OtherBodyIndex :type Integer) (bFromSweep :type Boolean) (SweepResult :type Hit%20Result%20Structure%20%28by%20ref%29))
  (Development|PrintString "Can Interact" true true "(R=0.000000,G=1.000000,B=0.187769,A=1.000000)")
  (Variables|/Game/BP_ThirdPersonCharacter.BP_ThirdPersonCharacter_C|SetCanInteractBox?? (Variables|Default|GetCharREF) true))

(event OnComponentEndOverlap(Fwd)
  (params (OverlappedComponent :type Primitive%20Component%20Object%20Reference) (OtherActor :type Actor%20Object%20Reference) (OtherComp :type Primitive%20Component%20Object%20Reference) (OtherBodyIndex :type Integer))
  (Development|PrintString "Cannot Interact" true true "(R=1.000000,G=0.005107,B=0.042764,A=1.000000)")
  (Variables|/Game/BP_ThirdPersonCharacter.BP_ThirdPersonCharacter_C|SetCanInteractBox?? (Variables|Default|GetCharREF) false))

(event EventBeginPlay
  (bind _returnvalue (Actor|GetActorOfClass "/Game/BP_ThirdPersonCharacter.BP_ThirdPersonCharacter_C"))
  (Variables|Default|SetCharREF _returnvalue))

(event Collision|EventActorBeginOverlap
  (params (OtherActor :type Actor%20Object%20Reference)))

(event EventTick
  (params (DeltaSeconds :type Float%20%28single-precision%29))
  (bind _charref (Variables|Default|GetCharREF))
  (bind _charref_2 (Variables|Default|GetCharREF))
  (bind _action_value_x (Variables|/Game/BP_ThirdPersonCharacter.BP_ThirdPersonCharacter_C|GetAction%20Value%20X _charref_2))
  (bind _action_value_y (Variables|/Game/BP_ThirdPersonCharacter.BP_ThirdPersonCharacter_C|GetAction%20Value%20Y _charref_2))
  (if (Variables|/Game/BP_ThirdPersonCharacter.BP_ThirdPersonCharacter_C|GetIsInteractingBox?? _charref)
    (if (Variables|/Game/BP_ThirdPersonCharacter.BP_ThirdPersonCharacter_C|GetCanInteractBox?? _charref)
      (Utilities|FlowControl|Sequence
        (:then_0
          (if (== _action_value_y 0.0)
            (Development|PrintString "Is not moving forward or backwards" true true "(R=0.000000,G=0.367746,B=1.000000,A=1.000000)" 2.0 "67456757")
            (elif (>= _action_value_y 0.1)
              (Development|PrintString "is moving forwards" true true "(R=1.000000,G=0.532358,B=0.593024,A=1.000000)" 2.0 "364564356")
              (Utilities|Speed/Direction true -5.0)
              (else
                (Development|PrintString "is moving backwards" true true "(R=1.000000,G=0.532358,B=0.593024,A=1.000000)" 2.0 "55353535")
                (Utilities|Speed/Direction true 5.0)))))
        (:then_1
          (if (== _action_value_x 0.0)
            (Development|PrintString "Is not moving right of left" true true "(R=0.000000,G=0.367746,B=1.000000,A=1.000000)" 2.0 "67456757")
            (elif (>= _action_value_x 0.1)
              (Development|PrintString "is moving right" true true "(R=1.000000,G=0.532358,B=0.593024,A=1.000000)" 2.0 "55353535")
              (Utilities|Speed/Direction false 5.0)
              (else
                (Development|PrintString "is moving left" true true "(R=1.000000,G=0.532358,B=0.593024,A=1.000000)" 2.0 "364564356")
                (Utilities|Speed/Direction false -5.0)))))))))

(fn ConstructionScript)

(fn Interact
  (params (Character :type Character%20Object%20Reference))
  (return false))